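; Track manager actor that builds rail splines from data tables and spawns a train on the first track at BeginPlay.
; Construction rebuilds tracks 0 and 2 as linear splines from row positions, recording station-type node indices per track and marking them with debug arrows.
; The train spawns at the station list's second entry, aligned to the spline, with its rail distance initialized.
; Tick prints track 0's station nodes for debugging.
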(event `self.ReceiveBeginPlay`
  (bind _returnvalue (`self.GetStationsFromId` 0))
  (bind _returnvalue_2 (`self.GetTrackFromId` 0))
  (bind _output (`|GetArrayItem` _returnvalue 1))
  (if (`KismetArrayLibrary.Array_IsValidIndex` _returnvalue)
    (set `self.r` (`KismetMathLibrary.RandomInteger` (`KismetArrayLibrary.Array_Length` _returnvalue)))
    (bind _returnvalue_3 (`|SpawnActorFromClass` "/Game/vehicles/blueprints/Train.Train_C" (`KismetMathLibrary.MakeTransform` (`SplineComponent.GetLocationAtSplinePoint` _returnvalue_2 _output "World") (`KismetMathLibrary.Conv_VectorToRotator` (`SplineComponent.GetDirectionAtSplinePoint` _returnvalue_2 _output "World"))) "AlwaysSpawn" "OverrideRootScale" null null 0 "NewEnumerator138" "NewEnumerator3" "" null))
    (set `/Game/vehicles/blueprints/Train.CurrentRailDistance` (`SplineComponent.GetDistanceAlongSplineAtSplinePoint` _returnvalue_2 _output) _returnvalue_3)))

(event `self.ReceiveTick`
  (params (DeltaSeconds :type "Float (single-precision)"))
  (bind (_arrayindex _arrayelement) (`/Engine/EditorBlueprintResources/StandardMacros.ReverseForEachLoop` (`self.TrackStations`))
    (:`LoopBody`
      (`KismetSystemLibrary.PrintString` (`VictoryBPFunctionLibrary.AppendMultiple` "Station " (`KismetStringLibrary.Conv_IntToString` _arrayindex) " at NodeId " (`KismetStringLibrary.Conv_IntToString` _arrayelement)) true true (struct :`R` 1.0 :`G` 0.936296 :`B` 0.009047 :`A` 1.0) 0.0))))

(fn `CreatePositionArray`
  (params (Id :type Integer) (Positions :type "Array of Vector Structure (by ref)"))
  (locals (track_data :type "Array of DataTable Object Reference"))
  (bind _output (`|GetArrayItem` (`local.track_data`) Id))
  (bind _returnvalue (select `int` Id :`0` (`self.TrackStations`) :`1` (`self.Track2Stations`) :`2` (`self.Track3Stations`) :`3` (`self.Track4Stations`)))
  (`KismetArrayLibrary.Array_Clear` _returnvalue)
  (bind _outrownames (`DataTableFunctionLibrary.GetDataTableRowNames` _output))
  (for (_array_element _array_index) _outrownames
    (bind _returnvalue_2 (`|GetDataTableRow` _output _array_element)
      (:`then`
        (bind (_position _type) (break `/Game/core/paths/structures/sTracks` _returnvalue_2))
        (`KismetArrayLibrary.Array_Add` Positions _position)
        (switch `/Game/core/paths/enumeration/eTrackNodeType` _type
          (:`NewEnumerator1`
            (`KismetArrayLibrary.Array_Add` _returnvalue _array_index)
            ;[1 0 0] DEBUG Station ARROWS
            (`AddComponent|NODE_AddArrowComponent-3` :`RelativeTransform` (`KismetMathLibrary.MakeTransform` (+ _position (0.0 0.0 10000.0)) (struct :`Pitch` -90.0)))))))))

(fn `CreateTrack`
  (params (Id :type Integer))
  (locals (Nodes :type "Array of Vector Structure"))
  (bind _nodes (`local.Nodes`))
  (`self.CreatePositionArray` Id (`local.Nodes`))
  (bind _returnvalue (`AddComponent|NODE_AddSplineComponent-1`))
  (`self.DestroyTrack` Id)
  (`KismetArrayLibrary.Array_Set` (`self.tracks`) Id _returnvalue)
  (`SplineComponent.SetSplinePoints` _returnvalue _nodes "World" true)
  (for _index (range (+ (`KismetArrayLibrary.Array_LastIndex` _nodes) 1))
    (`SplineComponent.SetSplinePointType` _returnvalue _index "Linear" false))
  (`SplineComponent.UpdateSpline` _returnvalue)
  (`KismetArrayLibrary.Array_Clear` (`local.Nodes`)))

(fn `DestroyTrack`
  (params (Id :type Integer))
  (bind _output (`|GetArrayItem` (`self.tracks`) Id))
  (`/Engine/EditorBlueprintResources/StandardMacros.IsValid` _output
    (:`Is Valid`
      (`ActorComponent.K2_DestroyComponent` _output))))

(fn `GetStationsFromId`
  (params (Id :type Integer))
  (returns (ReturnValue :type "Array of Integer"))
  (return (select `int` Id :`0` (`self.TrackStations`) :`1` (`self.Track2Stations`) :`2` (`self.Track3Stations`) :`3` (`self.Track4Stations`))))

(fn `GetTrackFromId`
  (params (Id :type Integer))
  (returns (ReturnValue :type "SplineComponent Object Reference"))
  (return (`|GetArrayItem` (`self.tracks`) Id)))

(fn `UserConstructionScript`
  (`self.CreateTrack` 0)
  (`self.CreateTrack` 2))