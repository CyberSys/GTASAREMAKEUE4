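; Traffic light actor that displays car and pedestrian signal phases and switches its light components on at night, driven by the Timecycle actor.
; On BeginPlay it binds to the Timecycle's night and pedestrian events, plus the North/South or East/West event matching its type.
; Construction creates dynamic materials by slot name; phase functions select the lit lamp through a one-hot color vector parameter.
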(event `self.ReceiveBeginPlay`
  (bind _outactors (`GameplayStatics.GetAllActorsOfClass` "/Game/core/timecycle/Timecycle.Timecycle_C"))
  (if (`KismetArrayLibrary.Array_IsValidIndex` _outactors)
    (bind _output_get (set `self.Timecycle` (`|GetArrayItem` _outactors)))
    (add `/Game/core/timecycle/Timecycle.Night` _output_get (delegate `Switch`))
    (add `/Game/core/timecycle/Timecycle.TrafficlightPed` _output_get (`|CreateDelegate` :!event `PED_LIGHTS`))
    (switch `/Game/core/timecycle/enumerations/eTrafficLightType` (`self.TrafficLightType`)
      (:`NewEnumerator1`
        (add `/Game/core/timecycle/Timecycle.TrafficlightN/S` _output_get (`|CreateDelegate` :!event `LIGHTS_FOR_CARS`)))
      (:`NewEnumerator2`
        (add `/Game/core/timecycle/Timecycle.TrafficlightE/W` _output_get (`|CreateDelegate` :!event `LIGHTS_FOR_CARS`))))))

(event `Switch`
  (bind _returnvalue (`self.K2_GetComponentsByClass` "/Script/Engine.LightComponent"))
  (if (`KismetArrayLibrary.Array_IsValidIndex` _returnvalue)
    (for _array_element _returnvalue
      (`SceneComponent.SetHiddenInGame` _array_element (not (`/Game/core/timecycle/Timecycle.GetIsTimeInRange` (`self.Timecycle`) 21 7)) false))))

(fn `LIGHTS_FOR_CARS`
  (params (Phase :type "/Game/core/trafficlights/eTrafficlightForCars Enum" :default "NewEnumerator0"))
  (switch `/Game/core/trafficlights/eTrafficlightForCars` Phase
    (:`NewEnumerator0`
      (`MaterialInstanceDynamic.SetVectorParameterValue` (`self.LIGHT_FOR_CARS`) "phase" (struct :`B` 1.0 :`A` 1.0)))
    (:`NewEnumerator1`
      (`MaterialInstanceDynamic.SetVectorParameterValue` (`self.LIGHT_FOR_CARS`) "phase" (struct :`G` 1.0 :`A` 1.0)))
    (:`NewEnumerator2`
      (`MaterialInstanceDynamic.SetVectorParameterValue` (`self.LIGHT_FOR_CARS`) "phase" (struct :`R` 1.0 :`A` 1.0)))))

(fn `PED_LIGHTS`
  (params (Phase :type "/Game/core/trafficlights/eTrafficlightsPed Enum" :default "NewEnumerator0"))
  (bind _ped_light (`self.PED_LIGHT`))
  (bind _ped_light_2 (`self.PED_LIGHT`))
  (bind _ped_light_3 (`self.PED_LIGHT`))
  (switch `/Game/core/trafficlights/eTrafficlightsPed` Phase
    (:`NewEnumerator0`
      (`/Engine/EditorBlueprintResources/StandardMacros.IsValid` _ped_light_2
        (:`Is Valid`
          (`MaterialInstanceDynamic.SetVectorParameterValue` _ped_light_2 "phase" (struct :`R` 1.0 :`A` 1.0)))))
    (:`NewEnumerator1`
      (`/Engine/EditorBlueprintResources/StandardMacros.IsValid` _ped_light_3
        (:`Is Valid`
          (`MaterialInstanceDynamic.SetVectorParameterValue` _ped_light_3 "phase" (struct :`G` 1.0 :`A` 1.0)))))
    (:`NewEnumerator2`
      (`/Engine/EditorBlueprintResources/StandardMacros.IsValid` _ped_light
        (:`Is Valid`
          (`MaterialInstanceDynamic.SetVectorParameterValue` _ped_light "phase" (struct :`B` 1.0 :`A` 1.0)))))))

(fn `UserConstructionScript`
  (bind _staticmesh (`self.StaticMesh`))
  (for (_array_element _array_index) (`MeshComponent.GetMaterialSlotNames` (`self.StaticMesh`))
    (switch `name` _array_element
      (:`PED_LIGHT`
        (bind _returnvalue (`PrimitiveComponent.GetMaterial` (`self.StaticMesh`) _array_index))
        (bind _returnvalue_2 (`PrimitiveComponent.CreateDynamicMaterialInstance` _staticmesh _array_index _returnvalue "None"))
        (set `self.PED_LIGHT` _returnvalue_2))
      (:`LIGHT_FOR_CARS`
        (bind _returnvalue_3 (`PrimitiveComponent.CreateDynamicMaterialInstance` _staticmesh _array_index _returnvalue "None"))
        (set `self.LIGHT_FOR_CARS` _returnvalue_3)))))