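; Water actor that builds water surfaces from rows of the Water data table.
; Its construction script adds one unrotated instance to the Planes component per row, centred between opposite corners Point1 and Point4 and scaled by their absolute difference.
; Positions are converted by multiplying by 100 and negating Y, while the scale keeps the table's units.
; BeginPlay is empty, so there is no runtime logic.
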(event `self.ReceiveBeginPlay`)

(fn `UserConstructionScript`
  (bind _water (`self.water`))
  (bind _outrownames (`DataTableFunctionLibrary.GetDataTableRowNames` _water))
  (for _array_element _outrownames
    (bind _returnvalue (`|GetDataTableRow` _water _array_element)
      (:`then`
        (bind (_point_1 _point_1_speed _point_1_wave _point_1_waveheight _point_2 _point_2_speed _point_2_wave _point_2_waveheight _point_3 _point_3_speed _point_3_wave _point_3_waveheight _point_4) (break `/Game/core/water/struct_water` _returnvalue))
        (bind _returnvalue_2 (- _point_1 _point_4))
        (`InstancedStaticMeshComponent.AddInstanceWorldSpace` (`self.Planes`) (`KismetMathLibrary.MakeTransform` (* (+ (/ _returnvalue_2 2.0) _point_4) (100.0 -100.0 100.0)) (struct) (`KismetMathLibrary.Vector_GetAbs` _returnvalue_2)))))))