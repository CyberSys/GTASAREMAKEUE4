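; M4 weapon Blueprint for the player, handling automatic fire and reloading with a clip ammo struct.
; A Gate and retriggerable delay loop shots at a rate set by BreakoutTime.
; When a camera trace hits, it spends a round and spawns a projectile from the muzzle toward the impact, with sparks.
; Releasing fire triggers auto-reload on an empty clip; reloading plays a montage and timed flag, but never refills ammo.
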(event `self.ReceiveBeginPlay`
  (bind _asplayer (cast `/Game/Player/blueprint/player` (`GameplayStatics.GetPlayerCharacter` 0)))
  (set `self.Player_Ref` _asplayer)
  (setmembers `/Game/Player/blueprint/struct_weapondata` :`StructRef` (`self.weapondata`) :`ammoClip` (`self.ammoClip`) :`ammoCurrent` (`/Game/Player/blueprint/player.Stat_Ammo_m4` _asplayer)))

(event `StartFire`
  (bind _weapondata (`self.weapondata`))
  (bind _returnvalue (`SceneComponent.GetSocketLocation` (`self.M4`) "Muzzle"))
  (bind _bp_camera (`/Game/Player/blueprint/player.bp_camera` (`self.Player_Ref`)))
  (bind _returnvalue_2 (`SceneComponent.K2_GetComponentLocation` _bp_camera))
  (`|ExecutionSequence` :!label _label
    (:`then_0`
      (goto _label_2 :!via `Open`))
    (:`then_1`
      (`/Engine/EditorBlueprintResources/StandardMacros.Gate` true :!label _label_2
        (:`Exit`
          (`|ExecutionSequence`
            (:`then_0`
              (`GameplayStatics.PlaySoundAtLocation` "/Game/Sounds/Weapon/weapon_m4_fire.weapon_m4_fire" (`self.K2_GetActorLocation`) (struct) 1.0 1.0 0.0 null null null)
              (`KismetSystemLibrary.RetriggerableDelay` (/ 60.0 (`KismetMathLibrary.Conv_IntToDouble` (`self.breakoutTime`))))
              (goto _label_2))
            (:`then_1`
              (if (<= (`.ammoClipCurrent_10_FB9E8DFF41CA64472B2FDDBD99D2CDE9` (break `/Game/Player/blueprint/struct_weapondata` (`self.weapondata`))) 0)
                (`KismetSystemLibrary.PrintString` "OutOfAmmo" true true (struct :`R` 1.0 :`G` 0.083552 :`A` 1.0) 0.5)
                (else
                  (bind (_outhit _returnvalue_3) (`KismetSystemLibrary.LineTraceSingle` _returnvalue_2 (+ _returnvalue_2 (* (`SceneComponent.GetForwardVector` _bp_camera) 15000.0)) "TraceTypeQuery1"))
                  (if _returnvalue_3
                    (`GameplayStatics.PlaySound2D` "/Game/Sounds/Weapon/weapon_m4_fire.weapon_m4_fire" 1.0 1.0 0.0 null null)
                    (`Character.PlayAnimMontage` (`self.Player_Ref`) (`self.fire_montage`) 1.0 "None")
                    (setmembers `/Game/Player/blueprint/struct_weapondata` :`StructRef` _weapondata :`ammoClipCurrent` (- (`.ammoClipCurrent_10_FB9E8DFF41CA64472B2FDDBD99D2CDE9` (break `/Game/Player/blueprint/struct_weapondata` _weapondata)) 1))
                    (bind (_bblockinghit _binitialoverlap _time _distance _location _impactpoint _normal _impactnormal _physmat _hitactor _hitcomponent _hitbonename _hititem _faceindex _tracestart _traceend) (`GameplayStatics.BreakHitResult` _outhit))
                    (`|SpawnActorFromClass` "/Game/Weapons/M4/M4Projectile.M4Projectile_C" (`KismetMathLibrary.MakeTransform` _returnvalue (`KismetMathLibrary.FindLookAtRotation` _returnvalue (`KismetMathLibrary.SelectVector` _impactpoint _traceend _returnvalue_3))) "Undefined" "OverrideRootScale" null null)
                    (`GameplayStatics.SpawnEmitterAtLocation` "/Game/Particle/StarterContent/Particles/P_Sparks.P_Sparks" _location)))))))))))

(event `StopFire`
  (goto _label_2 :!via `Close`))

(event `FirePress`
  (goto _label))

(event `FireRelease`
  (set `self.canFire` false)
  (`self.StopFire`)
  (`self.AutoReload`))

(event `AutoReload`
  (bind (_ammoclip _ammoclipcurrent) (break `/Game/Player/blueprint/struct_weapondata` (`self.weapondata`)))
  (if (== _ammoclipcurrent 0)
    (if (== _ammoclip 0)
      (`KismetSystemLibrary.PrintString` "Hello")
      (else
        (set `self.isReloading` true)
        (`self.Reload`)
        (`KismetSystemLibrary.Delay` 2.0) ; Reload Anim Time
        (set `self.isReloading` false)))))

(event `Reload`
  (bind (_ammoclip _ammoclipcurrent) (break `/Game/Player/blueprint/struct_weapondata` (`self.weapondata`)))
  (if (== _ammoclip 0)
    (`KismetSystemLibrary.PrintString` "Find Ammo")
    (elif (== _ammoclip _ammoclipcurrent)
      (`KismetSystemLibrary.PrintString` "Full Ammo")
      (else
        (bind _output_get (set `self.isReloading` true))
        (if _output_get
          (`self.WeaponReload`)
          (`KismetSystemLibrary.Delay` 2.0)
          (set `self.isReloading` false))))))

(event `WeaponReload`
  (bind _player_ref (`self.Player_Ref`))
  (if (`self.canFire`)
    _
    (elif true
      (set `/Game/Player/blueprint/player.UpperBody` true _player_ref)
      (bind _asplayer_abp (cast `/Game/Player/blueprint/player_abp` (`SkeletalMeshComponent.GetAnimInstance` (`Character.Mesh` _player_ref))))
      (`AnimInstance.Montage_Play` _asplayer_abp "/Game/Player/animations/weapons/mon_Rifle_load.mon_Rifle_load" 1.0 "MontageLength" 0.0 true)
      (if (> (`.ammoCurrent_11_C8644090486F67AA57028DA879DF4357` (break `/Game/Player/blueprint/struct_weapondata` (`self.weapondata`))) 0)
        _))))

(fn `UserConstructionScript`)