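; Minigun weapon Blueprint that drives its barrel sound from how the barrel rotates.
; Each Tick runs the parent logic, then maps BarrelRotationValue to a clamped range and feeds it into the "rotation" float parameter of Sound016.
; It also prints the raw rotation value every frame as debug output.
; BeginPlay and overlap events are disabled stubs, and the construction script only calls its parent.
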(event `self.ReceiveTick`
  (params (DeltaSeconds :type "Float (single-precision)"))
  (bind _barrelrotationvalue (`self.BarrelRotationValue`))
  (`parent.ReceiveTick` DeltaSeconds)
  (`AudioComponent.SetFloatParameter` (`self.sound_016`) "rotation" (`KismetMathLibrary.MapRangeClamped` _barrelrotationvalue 0.0 50.0 0.0 1.0))
  (`KismetSystemLibrary.PrintString` (`KismetStringLibrary.Conv_DoubleToString` _barrelrotationvalue)))

(fn `UserConstructionScript`
  (`parent.UserConstructionScript`))