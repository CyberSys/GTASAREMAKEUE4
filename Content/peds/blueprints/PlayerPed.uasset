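; Player character for a GTA-style game, handling modular appearance, vitals, wanted level and movement speed.
; Construction binds body meshes to a master pose and applies savegame clothing, using data tables for meshes, fat/muscle morphs and torso-material tattoo textures.
; Initialize derives health, armour, stamina and air from player stats, while fat and muscle also blend walk speeds.
; Chaos thresholds set wanted tiers and police limits; Tick drives rain density from Timecycle.
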(event `self.ReceiveBeginPlay`
  (`parent.ReceiveBeginPlay`))

(event `self.ReceiveTick`
  (params (DeltaSeconds :type "Float (single-precision)"))
  (`parent.ReceiveTick` DeltaSeconds)
  (`FXSystemComponent.SetFloatParameter` (`self.rain_fx`) "density" (`/Game/core/timecycle/Timecycle.RainDensity` (`self.Timecycle`))))

(fn `CalculateWalkSpeed`
  (params (MoveState :type "/Game/peds/enumerations/eMoveState Enum" :default "NewEnumerator0"))
  (bind _returnvalue (`KismetMathLibrary.Lerp` (`KismetMathLibrary.Lerp` 155.583328 143.314285 (`self.fat`)) 155.583328 (`self.muscle`)))
  (set `CharacterMovementComponent.MaxWalkSpeed` (select `/Game/peds/enumerations/eMoveState` MoveState :`NewEnumerator0` _returnvalue :`NewEnumerator1` _returnvalue :`NewEnumerator2` _returnvalue :`NewEnumerator3` (`KismetMathLibrary.Lerp` (`KismetMathLibrary.Lerp` 570.681824 394.043488 (`self.fat`)) 540.75 (`self.muscle`)) :`NewEnumerator4` (`KismetMathLibrary.Lerp` (`KismetMathLibrary.Lerp` 956.25 778.166687 (`self.fat`)) 778.166687 (`self.muscle`))) (`self.CharacterMovement`)))

(fn `GetClothesByBodyPartName`
  (params (Clothes :type "/Game/peds/enumerations/ePlayerComponents Enum" :default "NewEnumerator0"))
  (returns (Component :type "SkeletalMeshComponent Object Reference"))
  (return (select `/Game/peds/enumerations/ePlayerComponents` Clothes :`NewEnumerator0` (`self.Mesh`) :`NewEnumerator1` (`self.head`) :`NewEnumerator2` (`self.legs`) :`NewEnumerator3` (`self.shoes`) :`NewEnumerator26` (`self.necklace`) :`NewEnumerator27` (`self.watch`) :`NewEnumerator28` (`self.glasses`) :`NewEnumerator29` (`self.hats`) :`NewEnumerator30` (`self.hands`))))

(fn `GetClothesInfoIndexFromBodyPart`
  (params (Clothes :type "/Game/peds/enumerations/ePlayerComponents Enum" :default "NewEnumerator0"))
  (returns (Id :type Integer))
  (bind (_part0_torsomodel _part1_headmodel _part2_legsmodel _part3_feetmodel _part4_ularm _part5_llarm _part6_urarm _part7_lrarm _part8_back _part9_lchest _part10_rchest _part11_stomach _part12_lowback _part13_chainsmodel _part14_watchmodel _part15_shadesmodel _part16_hatmodel _part17_specialmodel) (break `/Game/core/GAME/savegame/structures/tClothing` (`self.Clothing`)))
  (return (`|GetArrayItem` (`|MakeArray` (`KismetMathLibrary.Conv_ByteToInt` _part0_torsomodel) (`KismetMathLibrary.Conv_ByteToInt` _part1_headmodel) (`KismetMathLibrary.Conv_ByteToInt` _part2_legsmodel) (`KismetMathLibrary.Conv_ByteToInt` _part3_feetmodel) (`KismetMathLibrary.Conv_ByteToInt` _part4_ularm) (`KismetMathLibrary.Conv_ByteToInt` _part5_llarm) (`KismetMathLibrary.Conv_ByteToInt` _part6_urarm) (`KismetMathLibrary.Conv_ByteToInt` _part7_lrarm) (`KismetMathLibrary.Conv_ByteToInt` _part8_back) (`KismetMathLibrary.Conv_ByteToInt` _part9_lchest) (`KismetMathLibrary.Conv_ByteToInt` _part10_rchest) (`KismetMathLibrary.Conv_ByteToInt` _part11_stomach) (`KismetMathLibrary.Conv_ByteToInt` _part12_lowback) (`KismetMathLibrary.Conv_ByteToInt` _part13_chainsmodel) (`KismetMathLibrary.Conv_ByteToInt` _part14_watchmodel) (`KismetMathLibrary.Conv_ByteToInt` _part15_shadesmodel) (`KismetMathLibrary.Conv_ByteToInt` _part16_hatmodel) (`KismetMathLibrary.Conv_ByteToInt` _part17_specialmodel)) (`KismetMathLibrary.Conv_ByteToInt` Clothes))))

(fn `HasVisibleTattoo`
  (returns (return :type Boolean))
  (bind ((`Part4_ULArm_48_DCE9F367465AB46EEF06919ADA841276` _part4_ularm) (`Part5_LLArm_49_BDCC0C3D4585FE835C4034987A75E815` _part5_llarm) (`Part6_URArm_50_5C0C7A02425F1B779023F7A019F12489` _part6_urarm) (`Part7_LRArm_53_881450B14825297466EA39AECEDF0B31` _part7_lrarm) (`Part8_Back_52_954C03304A5DF57EF465258EDC336282` _part8_back) (`Part9_LChest_54_A273425A444BE21BF8F55C9BD7C01785` _part9_lchest) (`Part10_RChest_55_57E68F984FAD2680A5EAFAB5491F2C4F` _part10_rchest) (`Part11_Stomach_56_8F09920243309B143AF8DEB5305D291D` _part11_stomach) (`Part12_LowBack_57_269B101544F52DBE069F9F82B8E43EC8` _part12_lowback)) (break `/Game/core/GAME/savegame/structures/tClothing` (`self.Clothing`)))
  (return (or (`|EnumInequality` _part4_ularm "NewEnumerator50") (`|EnumInequality` _part5_llarm "NewEnumerator50") (`|EnumInequality` _part6_urarm "NewEnumerator50") (`|EnumInequality` _part7_lrarm "NewEnumerator50") (`|EnumInequality` _part8_back "NewEnumerator50") (`|EnumInequality` _part9_lchest "NewEnumerator50") (`|EnumInequality` _part10_rchest "NewEnumerator50") (`|EnumInequality` _part11_stomach "NewEnumerator50") (`|EnumInequality` _part12_lowback "NewEnumerator50"))))

(fn `Initialize`
  (params (PlayerInfo :type "/Game/peds/blueprints/PlayerInfo Object Reference"))
  (bind _output_get (set `self.PlayerInfo` PlayerInfo))
  (bind _stats (`/Game/peds/blueprints/PlayerInfo.Stats` _output_get))
  (bind _result (`/Game/peds/blueprints/Stats.getFatAndMuscleModifier` _stats "NewEnumerator9"))
  (bind _output_get_2 (set `self.maxHealth` _result))
  (bind _output_get_3 (set `self.health` _output_get_2))
  (`/Game/frontend/widget/hud.setHealth` (`/Game/peds/blueprints/PlayerInfo.Hud` (`local.PlayerInfo`)) _output_get_3 _output_get_3)
  (bind _output_get_4 (set `self.armour` (`/Game/peds/blueprints/Stats.getStatValue` (`/Game/peds/blueprints/PlayerInfo.Stats` (`local.PlayerInfo`)) 164)))
  (`/Game/frontend/widget/hud.setArmor` (`/Game/peds/blueprints/PlayerInfo.Hud` (`local.PlayerInfo`)) (`KismetMathLibrary.Round` _output_get_4) 150)
  (bind _result_2 (`/Game/peds/blueprints/Stats.getFatAndMuscleModifier` _stats "NewEnumerator7"))
  (bind _output_get_5 (set `self.maxStamina` _result_2))
  (set `self.stamina` _output_get_5)
  (bind _result_3 (`/Game/peds/blueprints/Stats.getFatAndMuscleModifier` _stats "NewEnumerator8"))
  (set `self.airInLung` _result_3))

(fn `RebuildPlayer`)

(fn `ReportCrimeNow`
  (params (NewParam :type "/Game/peds/enumerations/eCrimeType Enum" :default "NewEnumerator0")))

(fn `SetTextureAndModel`
  (params (Component :type "/Game/peds/enumerations/ePlayerComponents Enum" :default "NewEnumerator0") (Key :type Name))
  (bind _returnvalue (`KismetStringLibrary.Conv_StringToName` (`|GetEnumeratorNameAsString` Component)))
  (if (or (< Component 4) (> Component 12))
    (bind _returnvalue_2 (`|GetDataTableRow` "/Game/peds/data/shopping.shopping" Key)
      (:`then`
        (bind (_skeletalmesh _texture _component) (break `/Game/peds/structures/sShopping` _returnvalue_2))
        (bind _component_2 (`self.GetClothesByBodyPartName` _component))
        (`SkinnedMeshComponent.SetSkinnedAssetAndUpdate` _component_2 _skeletalmesh true)
        (bind _returnvalue_3 (`PrimitiveComponent.CreateDynamicMaterialInstance` _component_2 0 (`PrimitiveComponent.GetMaterial` _component_2 0) "None"))
        (`MaterialInstanceDynamic.SetTextureParameterValue` _returnvalue_3 "diffuse" _texture)
        (`SkeletalMeshComponent.SetMorphTarget` _component_2 "fat" (`self.fat`) true)
        (`SkeletalMeshComponent.SetMorphTarget` _component_2 "ripped" (`self.muscle`) true))
      (:`RowNotFound`
        (if (`|EnumEquality` Component "NewEnumerator30")
          (bind _component_3 (`self.GetClothesByBodyPartName` "NewEnumerator30"))
          (`SkinnedMeshComponent.SetSkinnedAssetAndUpdate` _component_3 "/Game/peds/meshes/player/hands.hands" true)
          (`PrimitiveComponent.CreateDynamicMaterialInstance` _component_3 0 (`PrimitiveComponent.GetMaterial` _component_3 0) "None"))))
    (else
      (bind _returnvalue_4 (`|GetDataTableRow` "/Game/peds/data/tattoos.tattoos" Key)
        (:`then`
          (bind _component_4 (`self.GetClothesByBodyPartName` "NewEnumerator0"))
          (bind _asmaterial_instance_dynamic (cast `MaterialInstanceDynamic` (`PrimitiveComponent.GetMaterial` _component_4 0)))
          (`MaterialInstanceDynamic.SetTextureParameterValue` _asmaterial_instance_dynamic _returnvalue (`.texture_4_0A04DB6943F36B3944090598E2840392` (break `/Game/peds/structures/sTattoos` _returnvalue_4))))
        (:`RowNotFound`
          (bind _component_5 (`self.GetClothesByBodyPartName` "NewEnumerator0"))
          (bind _asmaterial_instance_dynamic_2 (cast `MaterialInstanceDynamic` (`PrimitiveComponent.GetMaterial` _component_5 0)))
          (`MaterialInstanceDynamic.SetTextureParameterValue` _asmaterial_instance_dynamic_2 _returnvalue "/Game/peds/textures/player/tattoo/white.white"))))))

(fn `SetWantedLevel`
  (params (Level :type Integer))
  (bind _returnvalue (`KismetMathLibrary.Min` Level 6))
  (bind _structout (setmembers `/Game/peds/structures/sWanted` :`StructRef` (`self.Wanted`) :`WantedLevel` _returnvalue))
  (set `self.Wanted` _structout)
  (bind _asplayer_info (cast `/Game/peds/blueprints/PlayerInfo` (`self.GetController`)))
  (`/Game/frontend/widget/hud.setWanted` (`/Game/peds/blueprints/PlayerInfo.Hud` _asplayer_info) 0 _returnvalue)
  (set `self.Chaos` (select `int` _returnvalue :`0` 0 :`1` 60 :`2` 220 :`3` 420 :`4` 820 :`5` 1620 :`6` 3220))
  (`self.UpdateWantedLevel`))

(fn `SetWantedLevelNoDrop`
  (params (Level :type Integer))
  (if (> Level (`.WantedLevel_41_E1C7453E43500686DF10CE9153D47458` (break `/Game/peds/structures/sWanted` (`self.Wanted`))))
    (`self.SetWantedLevel` Level)))

(fn `TryClothes`
  (params (Component :type "/Game/peds/enumerations/ePlayerComponents Enum" :default "NewEnumerator0") (Key :type Name))
  (`self.SetTextureAndModel` Component Key)
  (`self.RebuildPlayer`))

(fn `UpdateWantedLevel`
  (locals (CurrWantedLevel :type Integer))
  (bind _chaos (`self.Chaos`))
  (bind _chaos_2 (`self.Chaos`))
  (bind _chaos_3 (`self.Chaos`))
  (bind _chaos_4 (`self.Chaos`))
  (bind _chaos_5 (`self.Chaos`))
  (bind _chaos_6 (`self.Chaos`))
  (set `local.CurrWantedLevel` (`.WantedLevel_41_E1C7453E43500686DF10CE9153D47458` (break `/Game/peds/structures/sWanted` (`self.Wanted`))))
  (set `self.Chaos` (`KismetMathLibrary.Min` (`self.Chaos`) (`self.maximumChaos`)))
  (`|ExecutionSequence`
    (:`then_0`
      ;[0 1 0] Level 0
      (if (and (>= _chaos_4 0) (< _chaos_4 40))
        (bind _structout (setmembers `/Game/peds/structures/sWanted` :`StructRef` (`self.Wanted`) :`MaxCops` 0 :`MaximumLawEnforcerVehicles` 0 :`RoadblockDensity` 0 :`WantedLevel` 0))
        (set `self.Wanted` _structout)
        (else
          ;[0 0 0] Level 1
          (if (and (>= _chaos_5 40) (< _chaos_5 200))
            (bind _structout_2 (setmembers `/Game/peds/structures/sWanted` :`StructRef` (`self.Wanted`) :`MaxCops` 1 :`MaximumLawEnforcerVehicles` 1 :`RoadblockDensity` 0 :`WantedLevel` 1))
            (set `self.Wanted` _structout_2)
            (else
              ;[0 0 0] Level 2
              (if (and (>= _chaos_6 200) (< _chaos_6 400))
                (bind _structout_3 (setmembers `/Game/peds/structures/sWanted` :`StructRef` (`self.Wanted`) :`MaxCops` 3 :`MaximumLawEnforcerVehicles` 2 :`RoadblockDensity` 0 :`WantedLevel` 2))
                (set `self.Wanted` _structout_3)
                (else
                  ;[0 0 0] Level 3
                  (if (and (>= _chaos 400) (< _chaos 800))
                    (bind _structout_4 (setmembers `/Game/peds/structures/sWanted` :`StructRef` (`self.Wanted`) :`MaxCops` 4 :`MaximumLawEnforcerVehicles` 2 :`RoadblockDensity` 4 :`WantedLevel` 3))
                    (set `self.Wanted` _structout_4)
                    (else
                      ;[0 0 0] Level 4
                      (if (and (>= _chaos_2 800) (< _chaos_2 1600))
                        (bind _structout_5 (setmembers `/Game/peds/structures/sWanted` :`StructRef` (`self.Wanted`) :`MaxCops` 6 :`MaximumLawEnforcerVehicles` 2 :`RoadblockDensity` 8 :`WantedLevel` 4))
                        (set `self.Wanted` _structout_5)
                        (else
                          ;[0 0 0] Level 5
                          (if (and (>= _chaos_3 1600) (< _chaos_3 3200))
                            (bind _structout_6 (setmembers `/Game/peds/structures/sWanted` :`StructRef` (`self.Wanted`) :`MaxCops` 8 :`MaximumLawEnforcerVehicles` 3 :`RoadblockDensity` 10 :`WantedLevel` 5))
                            (set `self.Wanted` _structout_6)
                            (else
                              ;[0 0 0] Level 6
                              (if (>= (`self.Chaos`) 3200)
                                (bind _structout_7 (setmembers `/Game/peds/structures/sWanted` :`StructRef` (`self.Wanted`) :`MaxCops` 10 :`MaximumLawEnforcerVehicles` 3 :`RoadblockDensity` 12 :`WantedLevel` 6))
                                (set `self.Wanted` _structout_7)))))))))))))))
    (:`then_1`
      (if (!= (`.WantedLevel_41_E1C7453E43500686DF10CE9153D47458` (break `/Game/peds/structures/sWanted` (`self.Wanted`))) (`local.CurrWantedLevel`))
        (set `self.LastWantedLevelChange` (`/Game/core/timecycle/Timecycle.TimeInMilliseconds` (`self.Timecycle`)))))))

(fn `UserConstructionScript`
  (bind _returnvalue (enumliteral `/Game/core/GAME/savegame/enumerations/eTattoo` "NewEnumerator50"))
  (bind (_part0_torsomodel _part1_headmodel _part2_legsmodel _part3_feetmodel _part4_ularm _part5_llarm _part6_urarm _part7_lrarm _part8_back _part9_lchest _part10_rchest _part11_stomach _part12_lowback _part13_chainsmodel _part14_watchmodel _part15_shadesmodel _part16_hatmodel _part17_specialmodel) (break `/Game/core/GAME/savegame/structures/tClothing` (`self.Clothing`)))
  (`parent.UserConstructionScript`)
  ;[1 1 1] make all mesh components child of master component animation
  (`SkinnedMeshComponent.SetLeaderPoseComponent` (`self.head`) (`self.Mesh`) true)
  (`SkinnedMeshComponent.SetLeaderPoseComponent` (`self.legs`) (`self.Mesh`) true)
  (`SkinnedMeshComponent.SetLeaderPoseComponent` (`self.watch`) (`self.Mesh`) true)
  (`SkinnedMeshComponent.SetLeaderPoseComponent` (`self.glasses`) (`self.Mesh`) true)
  (`SkinnedMeshComponent.SetLeaderPoseComponent` (`self.hats`) (`self.Mesh`) true)
  (`SkinnedMeshComponent.SetLeaderPoseComponent` (`self.hands`) (`self.Mesh`) true)
  (`SkinnedMeshComponent.SetLeaderPoseComponent` (`self.shoes`) (`self.Mesh`) true)
  (`SkinnedMeshComponent.SetLeaderPoseComponent` (`self.necklace`) (`self.Mesh`) true)
  ;[0 0 1] Load Playerped
  (bind _asgta_gameinstance (cast `/Game/core/GAME/gta_gameinstance` (`GameplayStatics.GetGameInstance`)))
  (bind _savegame (`/Game/core/GAME/gta_gameinstance.Savegame` _asgta_gameinstance))
  (`/Engine/EditorBlueprintResources/StandardMacros.IsValid` _savegame
    (:`Is Valid`
      (bind (_clothing _fat _muscle) (break `/Game/core/GAME/savegame/structures/tPlayer` (`.PlayerPed_6_64AC2FD84FE7347120E65E9FE7DC6300` (break `/Game/core/GAME/savegame/Blocks/tBlock02` (`/Game/core/GAME/savegame/gta_savegame.Pools` _savegame)))))
      (set `self.Clothing` _clothing)
      (set `self.fat` _fat)
      (set `self.muscle` _muscle)
      (bind _enumvalue (foreach `/Game/peds/enumerations/ePlayerComponents` false)
        (:`LoopBody`
          (`self.SetTextureAndModel` _enumvalue (`|GetArrayItem` (`|MakeArray` (`KismetStringLibrary.Conv_StringToName` (`|GetEnumeratorNameAsString` _part0_torsomodel)) (`KismetStringLibrary.Conv_StringToName` (`|GetEnumeratorNameAsString` _part1_headmodel)) (`KismetStringLibrary.Conv_StringToName` (`|GetEnumeratorNameAsString` _part2_legsmodel)) (`KismetStringLibrary.Conv_StringToName` (`|GetEnumeratorNameAsString` _part3_feetmodel)) (`KismetStringLibrary.Conv_StringToName` (`|GetEnumeratorNameAsString` _part4_ularm)) (`KismetStringLibrary.Conv_StringToName` (`|GetEnumeratorNameAsString` _part5_llarm)) (`KismetStringLibrary.Conv_StringToName` (`|GetEnumeratorNameAsString` _part6_urarm)) (`KismetStringLibrary.Conv_StringToName` (`|GetEnumeratorNameAsString` _part7_lrarm)) (`KismetStringLibrary.Conv_StringToName` (`|GetEnumeratorNameAsString` _part8_back)) (`KismetStringLibrary.Conv_StringToName` (`|GetEnumeratorNameAsString` _part9_lchest)) (`KismetStringLibrary.Conv_StringToName` (`|GetEnumeratorNameAsString` _part10_rchest)) (`KismetStringLibrary.Conv_StringToName` (`|GetEnumeratorNameAsString` _part11_stomach)) (`KismetStringLibrary.Conv_StringToName` (`|GetEnumeratorNameAsString` _part12_lowback)) (`KismetStringLibrary.Conv_StringToName` (`|GetEnumeratorNameAsString` _part13_chainsmodel)) (`KismetStringLibrary.Conv_StringToName` (`|GetEnumeratorNameAsString` _part14_watchmodel)) (`KismetStringLibrary.Conv_StringToName` (`|GetEnumeratorNameAsString` _part15_shadesmodel)) (`KismetStringLibrary.Conv_StringToName` (`|GetEnumeratorNameAsString` _part16_hatmodel)) (`KismetStringLibrary.Conv_StringToName` (`|GetEnumeratorNameAsString` _part17_specialmodel))) (`KismetMathLibrary.Conv_ByteToInt` _enumvalue))))))
    (:`Is Not Valid`
      ;;[1 0 0] DEBUG
      (bind _enumvalue_2 (foreach `/Game/peds/enumerations/ePlayerComponents` false)
        (:`LoopBody`
          (`self.SetTextureAndModel` _enumvalue_2 (`|GetArrayItem` (`|MakeArray` (`KismetStringLibrary.Conv_StringToName` (`|GetEnumeratorNameAsString` (enumliteral `/Game/core/GAME/savegame/enumerations/eTorsoModels` "NewEnumerator0"))) (`KismetStringLibrary.Conv_StringToName` (`|GetEnumeratorNameAsString` (enumliteral `/Game/core/GAME/savegame/enumerations/eHeadModels` "NewEnumerator0"))) (`KismetStringLibrary.Conv_StringToName` (`|GetEnumeratorNameAsString` (enumliteral `/Game/core/GAME/savegame/enumerations/eLegsModels` "NewEnumerator6"))) (`KismetStringLibrary.Conv_StringToName` (`|GetEnumeratorNameAsString` (enumliteral `/Game/core/GAME/savegame/enumerations/eFeetModels` "NewEnumerator6"))) (`KismetStringLibrary.Conv_StringToName` (`|GetEnumeratorNameAsString` _returnvalue)) (`KismetStringLibrary.Conv_StringToName` (`|GetEnumeratorNameAsString` _returnvalue)) (`KismetStringLibrary.Conv_StringToName` (`|GetEnumeratorNameAsString` _returnvalue)) (`KismetStringLibrary.Conv_StringToName` (`|GetEnumeratorNameAsString` _returnvalue)) (`KismetStringLibrary.Conv_StringToName` (`|GetEnumeratorNameAsString` _returnvalue)) (`KismetStringLibrary.Conv_StringToName` (`|GetEnumeratorNameAsString` _returnvalue)) (`KismetStringLibrary.Conv_StringToName` (`|GetEnumeratorNameAsString` _returnvalue)) (`KismetStringLibrary.Conv_StringToName` (`|GetEnumeratorNameAsString` _returnvalue)) (`KismetStringLibrary.Conv_StringToName` (`|GetEnumeratorNameAsString` (enumliteral `/Game/core/GAME/savegame/enumerations/eChainsModels` "NewEnumerator0"))) (`KismetStringLibrary.Conv_StringToName` (`|GetEnumeratorNameAsString` (enumliteral `/Game/core/GAME/savegame/enumerations/eWatchModels` "NewEnumerator0"))) (`KismetStringLibrary.Conv_StringToName` (`|GetEnumeratorNameAsString` (enumliteral `/Game/core/GAME/savegame/enumerations/eShadesModels` "NewEnumerator0"))) (`KismetStringLibrary.Conv_StringToName` (`|GetEnumeratorNameAsString` (enumliteral `/Game/core/GAME/savegame/enumerations/eHatModels` "NewEnumerator57"))) (`KismetStringLibrary.Conv_StringToName` (`|GetEnumeratorNameAsString` (enumliteral `/Game/peds/enumerations/ePeds_special` "NewEnumerator0"))) (`KismetStringLibrary.Conv_StringToName` (`|GetEnumeratorNameAsString` (enumliteral `/Game/core/GAME/savegame/enumerations/eHandsModels` "NewEnumerator0")))) (`KismetMathLibrary.Conv_ByteToInt` _enumvalue_2))))))))