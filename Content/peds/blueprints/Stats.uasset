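; Player stats Blueprint that turns stored stats into ability modifiers and limits such as run time, lung air and max health.
; GetFatAndMuscleModifier selects a hard-coded formula per ability, mostly linear blends of normalized stats with clamps, several still under placeholder names.
; GetStatValue reads one continuous index across the float and integer stat arrays, with integer stats following the floats.
; The event graph and construction script are empty.
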(event `self.ReceiveBeginPlay`)

(fn `getFatAndMuscleModifier`
  (params (statModAbilities :type "/Game/peds/enumerations/eStatModAbilities Enum" :default "NewEnumerator0"))
  (returns (result :type "Float (double-precision)"))
  (bind _output (`|GetArrayItem` (`self.playerStatsFloat`) (`KismetMathLibrary.Conv_ByteToInt` (enumliteral `/Game/peds/enumerations/eFStats` "NewEnumerator21"))))
  (switch `/Game/peds/enumerations/eStatModAbilities` statModAbilities
    (:`NewEnumerator0`
      (if (> _output 800.0)
        (return 2.0)
        (elif (> _output 400.0)
          (return 1.0)
          (else
            (return 0.0)))))
    (:`NewEnumerator1`
      (return (`KismetMathLibrary.FMax` (+ (* (`KismetMathLibrary.FMax` 0.0 (/ (- (`|GetArrayItem` (`self.playerStatsFloat`) (`KismetMathLibrary.Conv_ByteToInt` (enumliteral `/Game/peds/enumerations/eFStats` "NewEnumerator21"))) 200.0) (- 1000.0 200.0))) -0.400001) 1.0 (/ (* (- (`|GetArrayItem` (`self.playerStatsFloat`) (`KismetMathLibrary.Conv_ByteToInt` (enumliteral `/Game/peds/enumerations/eFStats` "NewEnumerator23"))) 50.0) 0.2) (- 1000.0 50.0))) 0.699999)))
    (:`NewEnumerator2`
      (return (`KismetMathLibrary.FMax` (+ (+ (* (`KismetMathLibrary.FMax` 0.0 (/ (- (`|GetArrayItem` (`self.playerStatsFloat`) (`KismetMathLibrary.Conv_ByteToInt` (enumliteral `/Game/peds/enumerations/eFStats` "NewEnumerator21"))) 200.0) (- 1000.0 200.0))) -0.2) 1.0) (/ (* (- (`|GetArrayItem` (`self.playerStatsFloat`) (`KismetMathLibrary.Conv_ByteToInt` (enumliteral `/Game/peds/enumerations/eFStats` "NewEnumerator23"))) 50.0) -0.1) (- 1000.0 50.0))) 0.8)))
    (:`NewEnumerator3`
      (return (`KismetMathLibrary.FMax` (+ (/ (* (- (`|GetArrayItem` (`self.playerStatsFloat`) (`KismetMathLibrary.Conv_ByteToInt` (enumliteral `/Game/peds/enumerations/eFStats` "NewEnumerator21"))) 200.0) -0.2) (- 1000.0 200.0)) (* (- (`|GetArrayItem` (`self.playerStatsFloat`) (`KismetMathLibrary.Conv_ByteToInt` (enumliteral `/Game/peds/enumerations/eFStats` "NewEnumerator23"))) 50.0) -0.1)) 0.8)))
    (:`NewEnumerator4`
      (return (`KismetMathLibrary.FClamp` (+ (/ (* (- (`|GetArrayItem` (`self.playerStatsFloat`) (`KismetMathLibrary.Conv_ByteToInt` (enumliteral `/Game/peds/enumerations/eFStats` "NewEnumerator21"))) 200.0) 0.5) (- 1000.0 200.0)) 1.0 (/ (* (- (`|GetArrayItem` (`self.playerStatsFloat`) (`KismetMathLibrary.Conv_ByteToInt` (enumliteral `/Game/peds/enumerations/eFStats` "NewEnumerator23"))) 50.0) 1.0) (- 1000.0 50.0))) 0.5 2.0)))
    (:`NewEnumerator5`
      (return (`KismetMathLibrary.FClamp` (+ (/ (* (- (`|GetArrayItem` (`self.playerStatsFloat`) (`KismetMathLibrary.Conv_ByteToInt` (enumliteral `/Game/peds/enumerations/eFStats` "NewEnumerator21"))) 200.0) -1.0) (- 1000.0 200.0)) 1.0 (/ (* (- (`|GetArrayItem` (`self.playerStatsFloat`) (`KismetMathLibrary.Conv_ByteToInt` (enumliteral `/Game/peds/enumerations/eFStats` "NewEnumerator23"))) 50.0) 0.5) (- 1000.0 50.0)) (* (`|GetArrayItem` (`self.playerStatsFloat`) (`KismetMathLibrary.Conv_ByteToInt` (enumliteral `/Game/peds/enumerations/eFStats` "NewEnumerator22"))) 0.001 0.5) (* (* (`|GetArrayItem` (`self.playerStatsInteger`) (`KismetMathLibrary.Conv_ByteToInt` (enumliteral `/Game/peds/enumerations/eIStats` "NewEnumerator108"))) 0.001) 1.0)) 0.5 2.0)))
    (:`NewEnumerator6`
      (return (`KismetMathLibrary.FClamp` (+ (/ (* (- (`|GetArrayItem` (`self.playerStatsFloat`) (`KismetMathLibrary.Conv_ByteToInt` (enumliteral `/Game/peds/enumerations/eFStats` "NewEnumerator21"))) 200.0) -0.5) (- 1000.0 200.0)) 1.0 (* (* (`|GetArrayItem` (`self.playerStatsInteger`) (`KismetMathLibrary.Conv_ByteToInt` (enumliteral `/Game/peds/enumerations/eIStats` "NewEnumerator108"))) 0.001) 1.0)) 0.5 2.0)))
    (:`NewEnumerator7`
      (return (+ (* (`|GetArrayItem` (`self.playerStatsFloat`) (`KismetMathLibrary.Conv_ByteToInt` (enumliteral `/Game/peds/enumerations/eFStats` "NewEnumerator22"))) 0.001 3000.0) 150.0)))
    (:`NewEnumerator8`
      (return (+ (* (* (+ (`|GetArrayItem` (`self.playerStatsInteger`) (`KismetMathLibrary.Conv_ByteToInt` (enumliteral `/Game/peds/enumerations/eIStats` "NewEnumerator105"))) (`KismetMathLibrary.FTrunc` (`|GetArrayItem` (`self.playerStatsFloat`) (`KismetMathLibrary.Conv_ByteToInt` (enumliteral `/Game/peds/enumerations/eFStats` "NewEnumerator22"))))) 0.0005) 3000.0) 1000.0)))
    (:`NewEnumerator9`
      (return (* (`|GetArrayItem` (`self.playerStatsFloat`) (`KismetMathLibrary.Conv_ByteToInt` (enumliteral `/Game/peds/enumerations/eFStats` "NewEnumerator24"))) 0.001 176.0)))
    (:`NewEnumerator10`
      (return 176.0))
    (:`NewEnumerator11`
      (return (+ (* (`KismetMathLibrary.FMax` 1.0 (* (`|GetArrayItem` (`self.playerStatsInteger`) (`KismetMathLibrary.Conv_ByteToInt` (enumliteral `/Game/peds/enumerations/eIStats` "NewEnumerator107"))) 0.001)) 0.5) 1.0)))
    (:`NewEnumerator12`
      (return (+ (* (`KismetMathLibrary.FMax` 1.0 (* (`|GetArrayItem` (`self.playerStatsInteger`) (`KismetMathLibrary.Conv_ByteToInt` (enumliteral `/Game/peds/enumerations/eIStats` "NewEnumerator107"))) 0.001)) 0.300001) 1.0)))
    (:`NewEnumerator13`
      (return (+ (* (`KismetMathLibrary.FMax` 1.0 (* (`|GetArrayItem` (`self.playerStatsInteger`) (`KismetMathLibrary.Conv_ByteToInt` (enumliteral `/Game/peds/enumerations/eIStats` "NewEnumerator107"))) 0.001)) 0.25) 1.0)))
    (:`NewEnumerator14`
      (return (`KismetMathLibrary.FMin` (+ (/ (* (- (`|GetArrayItem` (`self.playerStatsFloat`) (`KismetMathLibrary.Conv_ByteToInt` (enumliteral `/Game/peds/enumerations/eFStats` "NewEnumerator21"))) 200.0) -0.5) (- 1000.0 200.0)) (* (* (`|GetArrayItem` (`self.playerStatsInteger`) (`KismetMathLibrary.Conv_ByteToInt` (enumliteral `/Game/peds/enumerations/eIStats` "NewEnumerator40"))) 0.001) 0.5) 1.0) 1.0)))
    (:`NewEnumerator16`
      (return (`KismetMathLibrary.FMax` (+ (/ (* (- (`|GetArrayItem` (`self.playerStatsFloat`) (`KismetMathLibrary.Conv_ByteToInt` (enumliteral `/Game/peds/enumerations/eFStats` "NewEnumerator21"))) 200.0) -0.5) (- 1000.0 200.0)) 1.0 (/ (* (- (`|GetArrayItem` (`self.playerStatsFloat`) (`KismetMathLibrary.Conv_ByteToInt` (enumliteral `/Game/peds/enumerations/eFStats` "NewEnumerator23"))) 50.0) -0.25) (- 1000.0 50.0))) 0.5)))))

(fn `getStatValue`
  (params (StatValue :type Integer))
  (returns (value :type "Float (double-precision)"))
  (bind _returnvalue (`KismetArrayLibrary.Array_Length` (`self.playerStatsFloat`)))
  (if (>= StatValue _returnvalue)
    (return (`KismetMathLibrary.Conv_IntToDouble` (`|GetArrayItem` (`self.playerStatsInteger`) (- StatValue _returnvalue))))
    (else
      (return (`|GetArrayItem` (`self.playerStatsFloat`) StatValue)))))

(fn `UserConstructionScript`)