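; Player controller for a GTA San Andreas-style game that manages the HUD, main menu and possession of peds or vehicles.
; Possession caches the pawn and sets up the player ped's camera, while BeginPlay finds the Timecycle on gameplay maps.
; Typed keys accumulate into timer-cleared cheat codes for items, spawning, game speed, time and weather.
; An idle-mouse timer triggers a timeline that swings the camera behind the vehicle until the mouse moves.
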(event `self.ReceivePossess`
  (params (PossessedPawn :type "Pawn Object Reference"))
  (`/Engine/EditorBlueprintResources/StandardMacros.IsValid` (`self.Hud`)
    (:`Is Valid`
      (if (not (`Widget.IsVisible` (`self.Hud`)))
        (`UserWidget.AddToViewport` (stale _output_get) 0 :!label _label)))
    (:`Is Not Valid`
      (bind _returnvalue (`|CreateWidget` "/Game/frontend/widget/hud.hud_C"))
      (bind _output_get (set `self.Hud` _returnvalue))
      (goto _label)))
  (bind _asplayer_ped (cast `/Game/peds/blueprints/PlayerPed` PossessedPawn)
    (:`then`
      (bind _output_get_2 (set `self.PlayerPed` _asplayer_ped))
      (set `self.Ped` _output_get_2)
      (`self.SetViewTargetWithBlend` (`GameplayStatics.GetPlayerController` 0) (`ChildActorComponent.ChildActor` (`/Game/peds/blueprints/Ped.Camera` _output_get_2)) 0.0 "VTBlend_Linear" 0.0 false)
      (bind _asstats (cast `/Game/peds/blueprints/Stats` (`self.PlayerState`)))
      (set `self.Stats` _asstats)
      (`/Game/peds/blueprints/PlayerPed.Initialize` _output_get_2 self))
    (:`CastFailed`
      (bind _asvehicle (cast `/Game/vehicles/blueprints/Vehicle` PossessedPawn)
        (:`then`
          (set `self.Vehicle` _asvehicle))
        (:`CastFailed`
          (bind _asped (cast `/Game/peds/blueprints/Ped` PossessedPawn))
          (bind _output_get_3 (set `self.Ped` _asped)))))))

(event `self.ReceiveBeginPlay`
  (bind _returnvalue (`GameplayStatics.GetPlayerCameraManager` 0))
  (bind _returnvalue_2 (`GameplayStatics.GetCurrentLevelName` true))
  (switch `string` _returnvalue_2
    (:`test`
      (bind _outactors (`GameplayStatics.GetAllActorsOfClass` "/Game/core/timecycle/Timecycle.Timecycle_C" :!label _label_2))
      (bind _astimecycle (cast `/Game/core/timecycle/Timecycle` (`|GetArrayItem` _outactors)))
      (set `self.Timecycle` _astimecycle)
      (set `PlayerCameraManager.ViewPitchMin` -70.0 _returnvalue)
      (set `PlayerCameraManager.ViewPitchMax` 70.0 _returnvalue))
    (:`SanAndreas`
      (goto _label_2))
    (:`gta`
      (`UserWidget.AddToViewport` (`self.Menu`) 0))))

(event `Key|Escape`
  (params (Key :type "Key Structure"))
  (:`Pressed`
    (`self.AddRemoveMainMenu` false)))

(event `self.ReceiveTick`
  (params (DeltaSeconds :type "Float (single-precision)"))
  (`self.CheckMouseMove`))

(event `Key|AnyKey` :consume false
  (params (Key :type "Key Structure"))
  (:`Pressed`
    (`self.CheatInput` Key)))

(event `ResetCameraDirection`
  (bind _myvehicle (`/Game/peds/blueprints/Ped.MyVehicle` (`self.Ped`)))
  ;[1 1 1] Reset Camera Direction when no mouse move is detected
  (bind _asvehicle (cast `/Game/vehicles/blueprints/Vehicle` (`self.K2_GetPawn`)))
  (set `self.Old Rotation` (`self.GetControlRotation`))
  (set `self.NewRotation` (`self.K2_GetActorRotation` _asvehicle))
  (bind (_direction _alpha) (`Timeline|Timeline_ResetDirection` :!via `PlayFromStart`)
    (:`Update`
      (bind (_returnvalue_roll _returnvalue_pitch _returnvalue_yaw) (`KismetMathLibrary.BreakRotator` (`KismetMathLibrary.RLerp` (`self.Old Rotation`) (`self.NewRotation`) _alpha true)))
      (`self.SetControlRotation` (`KismetMathLibrary.MakeRotator` 0.0 _returnvalue_pitch _returnvalue_yaw)))
    (:`Finished`
      (`KismetSystemLibrary.K2_ClearAndInvalidateTimerHandle` (`self.timer_ResetCameraDirection`))
      (`/Engine/EditorBlueprintResources/StandardMacros.IsValid` _myvehicle
        (:`Is Valid`
          (`/Game/vehicles/blueprints/Vehicle.CameraResetDirection` _myvehicle true)
          (set `self.CameraFollowsVehicle` true))))))

(fn `AddRemoveMainMenu`
  (params (Remove :type Boolean))
  (bind _hud (`self.Hud`))
  (bind _hud_2 (`self.Hud`))
  (if Remove
    ;[1 1 1] remove
    (`Widget.RemoveFromParent` (`self.Menu`))
    (`/Engine/EditorBlueprintResources/StandardMacros.IsValid` _hud_2
      (:`Is Valid`
        (`UserWidget.AddToViewport` _hud_2 0))
      (:`Is Not Valid`
        _))
    (set `self.bShowMouseCursor` false)
    (`self.GivePlayerControlBackToPawn`)
    (else
      ;[1 1 1] create
      (`/Engine/EditorBlueprintResources/StandardMacros.IsValid` (`self.Menu`)
        (:`Is Valid`
          _)
        (:`Is Not Valid`
          (bind _returnvalue (`|CreateWidget` "/Game/frontend/widget/menu/menu.menu_C"))
          (set `self.Menu` _returnvalue)))
      ;[1 1 1] add
      (`/Engine/EditorBlueprintResources/StandardMacros.IsValid` _hud
        (:`Is Valid`
          (`Widget.RemoveFromParent` _hud))
        (:`Is Not Valid`
          _))
      (if (not (`Widget.IsVisible` (`self.Menu`)))
        (`UserWidget.AddToViewport` (`self.Menu`) 0)
        (`WidgetBlueprintLibrary.SetInputMode_UIOnlyEx` (`GameplayStatics.GetPlayerController` 0) (`self.Menu`) "LockInFullscreen")
        (set `self.bShowMouseCursor` true)))))

(fn `CheatInput`
  (params (Key :type "Key Structure (by ref)"))
  (bind _returnvalue (`GameplayStatics.GetGlobalTimeDilation`))
  (bind _returnvalue_2 (`self.K2_GetPawn`))
  (bind _returnvalue_3 (`self.K2_GetPawn`))
  (bind (_returnvalue_roll _returnvalue_pitch _returnvalue_yaw) (`KismetMathLibrary.BreakRotator` (`self.GetControlRotation`)))
  (bind _timecycle (`self.Timecycle`))
  (bind _timecycle_2 (`self.Timecycle`))
  (bind _timecycle_3 (`self.Timecycle`))
  (bind _timecycle_4 (`self.Timecycle`))
  (bind _returnvalue_4 (* _returnvalue 2.0))
  (bind _returnvalue_5 (* _returnvalue 0.5))
  (bind _output_get (set `self.Cheatcode` (`KismetStringLibrary.Concat_StrStr` (`self.Cheatcode`) (`KismetTextLibrary.Conv_TextToString` (`KismetInputLibrary.Key_GetDisplayName` Key)))))
  (switch `string` _output_get
    (:`Default`
      (`KismetSystemLibrary.K2_SetTimer` null "ResetCheatInput" (* (`GameplayStatics.GetGlobalTimeDilation`) 1.0)))
    (:`skydive`
      (bind _asped (cast `/Game/peds/blueprints/Ped` _returnvalue_3)
        (:`then`
          (`/Game/peds/blueprints/Ped.GiveParachute` _asped)
          ;[1 1 1] item
          (`/Game/frontend/widget/hud.setHint_Text` (`self.Hud`) (`|FormatText` "Cheat activated: \nyou now have a parachute!"))
          (`self.ResetCheatInput` :!label _label))
        (:`CastFailed`
          (cast `/Game/vehicles/blueprints/Vehicle` _returnvalue_3))))
    (:`rocketman`
      (bind _asped_2 (cast `/Game/peds/blueprints/Ped` _returnvalue_2)
        (:`then`
          (`/Game/peds/blueprints/Ped.GiveJetpack` _asped_2)
          (`/Game/frontend/widget/hud.setHint_Text` (`self.Hud`) (`|FormatText` "Cheat activated: \nyou now have a jetpack!"))
          (goto _label))
        (:`CastFailed`
          (cast `/Game/vehicles/blueprints/Vehicle` _returnvalue_2))))
    (:`aiwprton`
      ;[1 1 1] vehicle
      (`|SpawnActorFromClass` "/Game/vehicles/blueprints/Automobile.Automobile_C" (`KismetMathLibrary.MakeTransform` (+ (`self.K2_GetActorLocation`) (* (`KismetMathLibrary.GetForwardVector` (`KismetMathLibrary.MakeRotator` 0.0 0.0 _returnvalue_yaw)) 700.0)) (`KismetMathLibrary.Conv_VectorToRotator` (`KismetMathLibrary.GetRightVector` (`KismetMathLibrary.MakeRotator` 0.0 0.0 _returnvalue_yaw)))) "Undefined" "OverrideRootScale" null "NewEnumerator32" "NewEnumerator0" "" null)
      (`/Game/frontend/widget/hud.setHint_Text` (`self.Hud`) (`|FormatText` "Cheat activated: \nspawned Rhino!"))
      (`self.ResetCheatInput`))
    (:`speeditup`
      ;[1 1 1] speed
      (if (<= _returnvalue_4 8.0)
        (`GameplayStatics.SetGlobalTimeDilation` _returnvalue_4)
        (`self.ResetCheatInput` :!label _label_2)
        (`/Game/core/timecycle/Timecycle.RecaptureSkyTimerReInititalize` (`self.Timecycle`))
        (`/Game/frontend/widget/hud.setHint_Text` (`self.Hud`) (`|FormatText` "Cheat activated: \nset play speed to {time dilation}x" (`GameplayStatics.GetGlobalTimeDilation`)))))
    (:`slowitdown`
      (if (>= _returnvalue_5 0.125)
        (`GameplayStatics.SetGlobalTimeDilation` _returnvalue_5)
        (goto _label_2)))
    (:`nightprowler`
      ;[1 1 1] time
      (set `/Game/core/timecycle/Timecycle.GameClockHours` 0 _timecycle_2)
      (set `/Game/core/timecycle/Timecycle.GameClockMinutes` 0 _timecycle_2)
      (`/Game/frontend/widget/hud.setHint_Text` (`self.Hud`) (`|FormatText` "Cheat activated: \nnow its midnight!"))
      (`/Game/core/timecycle/Timecycle.UpdateSunAndMoonDirection` _timecycle :!label _label_3)
      (`/Game/core/timecycle/Timecycle.UpdateTimeControlled` _timecycle_4)
      (`/Game/core/timecycle/Timecycle.Night` _timecycle)
      (`SkyLightComponent.RecaptureSky` (`/Game/core/timecycle/Timecycle.SkyLight` _timecycle_4))
      (`self.ResetCheatInput`))
    (:`daywalker`
      (set `/Game/core/timecycle/Timecycle.GameClockHours` 12 _timecycle_3)
      (set `/Game/core/timecycle/Timecycle.GameClockMinutes` 0 _timecycle_3)
      (`/Game/frontend/widget/hud.setHint_Text` (`self.Hud`) (`|FormatText` "Cheat activated: \nnow its midday!"))
      (goto _label_3))
    (:`pleasentlywarm`
      ;[1 1 1] weather
      (`/Game/core/timecycle/Timecycle.ForceWeatherNow` (`self.Timecycle`) "NewEnumerator0")
      (`/Game/frontend/widget/hud.setHint_Text` (`self.Hud`) (`|FormatText` "Cheat activated: \nsunny weather!"))
      (`self.ResetCheatInput` :!label _label_4))
    (:`toodamnhot`
      (`/Game/core/timecycle/Timecycle.ForceWeatherNow` (`self.Timecycle`) "NewEnumerator4")
      (`/Game/frontend/widget/hud.setHint_Text` (`self.Hud`) (`|FormatText` "Cheat activated: \nextrasunny weather!"))
      (goto _label_4))
    (:`noview`
      (`/Game/core/timecycle/Timecycle.ForceWeatherNow` (`self.Timecycle`) "NewEnumerator6")
      (`/Game/frontend/widget/hud.setHint_Text` (`self.Hud`) (`|FormatText` "Cheat activated: \nfoggy weather!"))
      (goto _label_4))
    (:`kill`
      (`/Game/peds/blueprints/Ped.AddHealth` (`self.PlayerPed`) -1000.0)
      (`self.ResetCheatInput`))))

(fn `CheckMouseMove`
  (bind _timeline_resetdirection (`self.Timeline_ResetDirection`))
  (bind _myvehicle (`/Game/peds/blueprints/Ped.MyVehicle` (`self.Ped`)))
  (if (`self.AutoResetDirection`)
    (if (and (<= (`self.GetInputAxisKeyValue`) 0.05) (<= (`self.GetInputAxisKeyValue`) 0.05))
      ;[1 0.5 0] 'OnMouseStopMove' start timer when inside a vehicle
      (if (not (`self.CameraFollowsVehicle`))
        (if (not (`KismetSystemLibrary.K2_IsTimerActiveHandle` (`self.timer_ResetCameraDirection`)))
          (bind _returnvalue (`KismetSystemLibrary.K2_SetTimerDelegate` (`|CreateDelegate` :!event `ResetCameraDirection`) 2.0))
          (set `self.timer_ResetCameraDirection` _returnvalue)))
      (else
        ;[1 1 1] 'OnMouseStartMove' reset timer/animation and give player back mouse control
        (if (`self.CameraFollowsVehicle`)
          (cast `/Game/vehicles/blueprints/Vehicle` (`self.K2_GetPawn`))
          (`self.SetControlRotation` (`PlayerCameraManager.GetCameraRotation` (`GameplayStatics.GetPlayerCameraManager` 0))))
        (set `self.CameraFollowsVehicle` false)
        (`|ExecutionSequence`
          (:`then_0`
            (if (`KismetSystemLibrary.K2_IsTimerActiveHandle` (`self.timer_ResetCameraDirection`))
              (`KismetSystemLibrary.K2_ClearAndInvalidateTimerHandle` (`self.timer_ResetCameraDirection`))))
          (:`then_1`
            (if (`TimelineComponent.IsPlaying` _timeline_resetdirection)
              (`TimelineComponent.Stop` _timeline_resetdirection)))
          (:`then_2`
            (`/Engine/EditorBlueprintResources/StandardMacros.IsValid` _myvehicle
              (:`Is Valid`
                (`/Game/vehicles/blueprints/Vehicle.CameraResetDirection` _myvehicle false)))))))))

(fn `GivePlayerControlBackToPawn`
  (bind _returnvalue (`self.K2_GetPawn`))
  (bind _asped (cast `/Game/peds/blueprints/Ped` _returnvalue)
    (:`then`
      (`/Game/peds/blueprints/Ped.GivePlayerControlOverThisPawn` _asped))
    (:`CastFailed`
      (bind _asvehicle (cast `/Game/vehicles/blueprints/Vehicle` _returnvalue))
      (`/Game/vehicles/blueprints/Vehicle.GivePlayerControlOverThisPawn` _asvehicle))))

(fn `ResetCheatInput`
  (set `self.Cheatcode` ""))

(fn `UserConstructionScript`)