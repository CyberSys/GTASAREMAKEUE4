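; Actor Blueprint in the models folder that plays an explosion effect when its Hit event fires, then removes itself.
; Hit loops over the particle count, spawning P_Explosion at each Location entry, with Y negated on odd indices and passed through the actor's inverse transform.
; The loop body starts a three-second delay before destroying the actor.
; Loop completion sets the static mesh's hidden-in-game flag to false.
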(event `self.ReceiveBeginPlay`)

(event `self.ReceiveHit`
  (params (MyComp :type "PrimitiveComponent Object Reference") (Other :type "Actor Object Reference") (OtherComp :type "PrimitiveComponent Object Reference") (bSelfMoved :type Boolean) (HitLocation :type "Vector Structure") (HitNormal :type "Vector Structure") (NormalImpulse :type "Vector Structure") (Hit :type "HitResult Structure (by ref)"))
  (for _index (range (+ (`self.Particles`) 1))
    (bind (_output_x _output_y _output_z) (`KismetMathLibrary.BreakVector` (`|GetArrayItem` (`self.Location`) _index)))
    (`GameplayStatics.SpawnEmitterAtLocation` "/Game/Particle/StarterContent/Particles/P_Explosion.P_Explosion" (`KismetMathLibrary.InverseTransformLocation` (`self.GetTransform`) (`KismetMathLibrary.MakeVector` _output_x (* _output_y (select `bool` (== (mod _index 2) 0) :`false` -1.0 :`true` 1.0 :!type "Float (single-precision)")) _output_z)))
    (`KismetSystemLibrary.Delay` 3.0)
    (`self.K2_DestroyActor`))
  (`SceneComponent.SetHiddenInGame` (`self.StaticMesh`) false false))

(fn `UserConstructionScript`)