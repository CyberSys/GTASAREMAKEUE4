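; Sign Blueprint that builds configurable text labels on itself at construction time.
; The Construction Script loops over a Textnumbers count, adding a Text Render component each pass.
; The loop index selects each label's transform and text from two preset slots, Location1/Text1 and Location2/Text2.
; The Event Graph holds only disabled default events, so it runs no gameplay logic.
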(fn `UserConstructionScript`
  (for _index (range (`self.textnumbers`))
    (bind _returnvalue (`AddComponent|NODE_AddTextRenderComponent-0` :`RelativeTransform` (select `int` _index :`0` (`self.Location1`) :`1` (`self.Location2`))))
    (`TextRenderComponent.K2_SetText` _returnvalue (select `int` _index :`0` (`self.Text1`) :`1` (`self.Text2`)))))