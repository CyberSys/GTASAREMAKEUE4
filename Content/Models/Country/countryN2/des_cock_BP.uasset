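; Country-level decorative Blueprint that animates the roll of its Cockhead component on a repeating timeline.
; BeginPlay caches the head's world rotation, and the RotateTime timeline lerps it toward a 45-degree roll offset from that start.
; Tick calls Play every frame, and on finish the timeline restarts in its current direction.
; An unconnected relative-rotation branch is left in the graph and never runs.
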(event `self.ReceiveTick`
  (params (DeltaSeconds :type "Float (single-precision)"))
  (bind (_direction _newtrack_0) (`Timeline|RotateTime` :!label _label)
    (:`Update`
      (bind _output_get (set `self.GoToRotation` (`KismetMathLibrary.RLerp` (stale `self.ReceiveBeginPlay` _output_get) (`KismetMathLibrary.MakeRotator` (+ (.roll (stale `self.ReceiveBeginPlay` _output_get)) 45.0) (.pitch (stale `self.ReceiveBeginPlay` _output_get)) (.yaw (stale `self.ReceiveBeginPlay` _output_get))) _newtrack_0)))
      (`SceneComponent.K2_SetWorldRotation` (`self.cockhead`) _output_get false false))
    (:`Finished`
      (switch `ETimelineDirection` _direction
        (:`Forward`
          (goto _label :!via `PlayFromStart`))
        (:`Backward`
          (goto _label :!via `ReverseFromEnd`))))))

(event `self.ReceiveBeginPlay`
  (bind _output_get (set `self.InitRotation` (`SceneComponent.K2_GetComponentRotation` (`self.cockhead`)))))

(fn `UserConstructionScript`)