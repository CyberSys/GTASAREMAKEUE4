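; Animated nodding donkey (oil pumpjack) base Blueprint that runs continuously from BeginPlay.
; A slowed Rotate timeline drives the relative pitch of Object01 from a vector curve and Object04 from a 360 track.
; Each update also resets Object02 and Object03 to zero world rotation, so they keep a fixed orientation while the other parts move.
; The timeline restarts itself on finishing to loop the motion.
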(event `self.ReceiveBeginPlay`
  (`TimelineComponent.SetPlayRate` (`self.rotate`) 0.3)
  (bind (_direction _360 _newcurvebase) (`Timeline|rotate` :!via `PlayFromStart` :!label _label)
    (:`Update`
      (`SceneComponent.K2_SetRelativeRotation` (`self.Object01`) (`KismetMathLibrary.MakeRotator` 0.0 (.x _newcurvebase)) false false)
      (`SceneComponent.K2_SetWorldRotation` (`self.Object02`) (`KismetMathLibrary.MakeRotator` 0.0) false false)
      (`SceneComponent.K2_SetWorldRotation` :`self` (`self.Object03`))
      (`SceneComponent.K2_SetRelativeRotation` (`self.Object04`) (`KismetMathLibrary.MakeRotator` 0.0 _360) false false))
    (:`Finished`
      (goto _label :!via `PlayFromStart`))))

(fn `UserConstructionScript`)