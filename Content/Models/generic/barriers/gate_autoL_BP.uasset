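; Automatic left gate barrier that slides open when a car enters its trigger box and closes when the car leaves.
; Box overlap events accept only bp_car actors and use MoveComponentTo to shift the GateAutoL component to the Distance offset, or back to its default zero target.
; Audio plays at the start and end of each timed movement.
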(event `self.Box.OnComponentBeginOverlap`
  (params (OverlappedComponent :type "PrimitiveComponent Object Reference") (OtherActor :type "Actor Object Reference") (OtherComp :type "PrimitiveComponent Object Reference") (OtherBodyIndex :type Integer) (bFromSweep :type Boolean) (SweepResult :type "HitResult Structure (by ref)"))
  (bind _audio (`self.Audio`))
  (cast `/Game/Vehicle/generic/blueprint/bp_car` OtherActor)
  (if true
    (`AudioComponent.Play` _audio 0.0)
    (`KismetSystemLibrary.MoveComponentTo` (`self.gate_autoL`) (`self.Distance`) (struct) false false 1.5)
    (`AudioComponent.Play` _audio 0.0)))

(event `self.Box.OnComponentEndOverlap`
  (params (OverlappedComponent :type "PrimitiveComponent Object Reference") (OtherActor :type "Actor Object Reference") (OtherComp :type "PrimitiveComponent Object Reference") (OtherBodyIndex :type Integer))
  (bind _audio (`self.Audio`))
  (cast `/Game/Vehicle/generic/blueprint/bp_car` OtherActor)
  (`AudioComponent.Play` _audio 0.0)
  (`KismetSystemLibrary.MoveComponentTo` (`self.gate_autoL`) (0.0 0.0 0.0) (struct) false false 1.5)
  (`AudioComponent.Play` _audio 0.0))

(fn `UserConstructionScript`)