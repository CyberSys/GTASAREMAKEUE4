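; Streetlamp actor that switches its light and lamppost material on or off, apparently following the level's Timecycle actors.
; The construction script finds all Timecycle actors and binds an event to their time switch.
; The Lights event takes a boolean that sets PointLight visibility and swaps the lamppost mesh between on and off materials.
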(event `self.ReceiveBeginPlay`)

(event `Lights`
  (params (NewParam :type Boolean))
  (bind _materialindex (`self.MaterialIndex`))
  (bind _lamppost3 (`self.lamppost3`))
  (`SceneComponent.SetVisibility` (`self.PointLight`) NewParam false)
  (if NewParam
    (`PrimitiveComponent.SetMaterial` _lamppost3 _materialindex (`self.MaterialOn`))
    (else
      (`PrimitiveComponent.SetMaterial` _lamppost3 _materialindex (`self.MaterialOff`)))))

(fn `UserConstructionScript`
  (bind _outactors (`GameplayStatics.GetAllActorsOfClass` "/Game/data/timecycle/timecycle.timecycle_C"))
  (add `/Game/data/timecycle/timecycle.timeswitch` _outactors (`|CreateDelegate` :!event `Lights`)))