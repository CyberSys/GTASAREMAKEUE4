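; Lamppost Blueprint that switches its light on at night and off by day.
; On BeginPlay it binds to the WeatherManager's timeswitch, which toggles SpotLight visibility and swaps the post's material between on and off versions.
; SpotLight shadow casting is enabled when a car or player enters the sphere and disabled when one ends overlap with the actor, limiting shadows by proximity.
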(event `self.ReceiveBeginPlay`
  (bind _outactors (`GameplayStatics.GetAllActorsOfClass` "/Game/data/timecycle/weatherManager.weatherManager_C"))
  (add `/Game/data/timecycle/weatherManager.timeswitch` _outactors (delegate `Lights`)))

(event `Lights`
  (params (night :type Boolean))
  (bind _lamppost3 (`self.lamppost3`))
  (bind _materialindex (`self.MaterialIndex`))
  (`SceneComponent.SetVisibility` (`self.SpotLight`) night false)
  (if night
    (`PrimitiveComponent.SetMaterial` _lamppost3 _materialindex (`self.MaterialOn`))
    (else
      (`PrimitiveComponent.SetMaterial` _lamppost3 _materialindex (`self.MaterialOff`)))))

(event `self.Sphere.OnComponentBeginOverlap`
  (params (OverlappedComponent :type "PrimitiveComponent Object Reference") (OtherActor :type "Actor Object Reference") (OtherComp :type "PrimitiveComponent Object Reference") (OtherBodyIndex :type Integer) (bFromSweep :type Boolean) (SweepResult :type "HitResult Structure (by ref)"))
  (cast `/Game/Vehicle/generic/blueprint/bp_car` OtherActor
    (:`then`
      _)
    (:`CastFailed`
      (cast `/Game/Player/blueprint/player` OtherActor)))
  (`LightComponentBase.SetCastShadows` (`self.SpotLight`) true))

(event `self.ReceiveActorEndOverlap`
  (params (OtherActor :type "Actor Object Reference"))
  (cast `/Game/Vehicle/generic/blueprint/bp_car` OtherActor
    (:`then`
      _)
    (:`CastFailed`
      (cast `/Game/Player/blueprint/player` OtherActor)))
  (`LightComponentBase.SetCastShadows` (`self.SpotLight`) false))

(fn `UserConstructionScript`)