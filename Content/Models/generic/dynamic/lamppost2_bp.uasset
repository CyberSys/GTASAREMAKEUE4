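; Lamppost actor blueprint that switches its lights on at night and off during the day.
; On BeginPlay it finds the WeatherManager actors and binds its Lights event to their Timeswitch dispatcher.
; The event uses the Night flag to set visibility on two spot lights and swap the lamppost mesh material between on and off variants.
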(event `self.ReceiveBeginPlay`
  (bind _outactors (`GameplayStatics.GetAllActorsOfClass` "/Game/data/timecycle/weatherManager.weatherManager_C"))
  (add `/Game/data/timecycle/weatherManager.timeswitch` _outactors (delegate `Lights`)))

(event `Lights`
  (params (night :type Boolean))
  (bind _materialindex (`self.MaterialIndex`))
  (bind _lamppost3 (`self.lamppost3`))
  (`SceneComponent.SetVisibility` (`self.SpotLight`) night false)
  (`SceneComponent.SetVisibility` (`self.SpotLight1`) night false)
  (if night
    (`PrimitiveComponent.SetMaterial` _lamppost3 _materialindex (`self.MaterialOn`))
    (else
      (`PrimitiveComponent.SetMaterial` _lamppost3 _materialindex (`self.MaterialOff`)))))

(fn `UserConstructionScript`)