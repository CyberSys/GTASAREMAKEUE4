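; Destructible mesh prop that applies fixed damage to its destructible MeshDam when a bp_car hits Mesh, pushed along the car's velocity.
; The actor destroys itself after a delay.
; The construction script sets Mesh and MeshDam visibility from Damaged, resets the flag and disables Mesh collision.
; Mesh-swap, impact-speed check and timed-destroy logic are left disconnected and never run.
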(event `self.ReceiveAnyDamage`
  (params (Damage :type "Float (single-precision)") (DamageType :type "DamageType Object Reference") (InstigatedBy :type "Controller Object Reference") (DamageCauser :type "Actor Object Reference")))

(event `destroy`
  (`self.K2_DestroyActor`))

(event `self.mesh.OnComponentHit`
  (params (HitComponent :type "PrimitiveComponent Object Reference") (OtherActor :type "Actor Object Reference") (OtherComp :type "PrimitiveComponent Object Reference") (NormalImpulse :type "Vector Structure") (Hit :type "HitResult Structure (by ref)"))
  (bind _asbp_car (cast `/Game/Vehicle/generic/blueprint/bp_car` OtherActor))
  (`DestructibleComponent.ApplyDamage` (`self.mesh_dam`) 100.0 (`.Location` (`GameplayStatics.BreakHitResult` Hit)) (`self.GetVelocity` _asbp_car) 100.0)
  (`KismetSystemLibrary.Delay` 10.0)
  (`self.K2_DestroyActor`))

(fn `UserConstructionScript`
  (bind _damaged (`self.damaged`))
  (bind _mesh (`self.mesh`))
  (`SceneComponent.SetHiddenInGame` _mesh _damaged false)
  (`SceneComponent.SetHiddenInGame` (`self.mesh_dam`) (not _damaged) false)
  (set `self.damaged` false)
  (`PrimitiveComponent.SetCollisionEnabled` _mesh "NoCollision"))