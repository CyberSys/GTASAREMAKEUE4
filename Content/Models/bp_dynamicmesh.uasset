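; Dynamic mesh prop actor that plays an impact sound when a bp_car hits it.
; On a static mesh hit, it subtracts the mesh's speed from the car's and plays the audio if the scaled, clamped difference passes a small threshold.
; A DoOnce that resets after a short delay keeps repeated hits from retriggering the sound.
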(event `self.StaticMesh.OnComponentHit`
  (params (HitComponent :type "PrimitiveComponent Object Reference") (OtherActor :type "Actor Object Reference") (OtherComp :type "PrimitiveComponent Object Reference") (NormalImpulse :type "Vector Structure") (Hit :type "HitResult Structure (by ref)"))
  (bind _asbp_car (cast `/Game/Vehicle/generic/blueprint/bp_car` OtherActor))
  (if (> (`KismetMathLibrary.FClamp` (/ (- (`KismetMathLibrary.VSize` (`self.GetVelocity` _asbp_car)) (`KismetMathLibrary.VSize` (`SceneComponent.GetComponentVelocity` (`self.StaticMesh`)))) 100.0) 0.0 100.0) 0.5)
    (`/Engine/EditorBlueprintResources/StandardMacros.DoOnce` false :!label _label
      (:`Completed`
        (`AudioComponent.Play` (`self.Audio`) 0.0)
        (`KismetSystemLibrary.Delay` 0.5)
        (goto _label :!via `Reset`)))))

(fn `UserConstructionScript`)