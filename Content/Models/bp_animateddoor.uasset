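; Animated garage door Blueprint that opens when an actor controlled by player_pc enters its trigger box and closes when it leaves.
; Overlap events open a Gate on Tick that advances or reverses a clamped time, sampling a vector curve for door height and pitch.
; At either limit the Gate closes and the looping sound switches to an end sound.
; The construction script scales travel from mesh bounds and offsets two debug planes.
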(event `self.ReceiveTick`
  (params (DeltaSeconds :type "Float (single-precision)"))
  (bind _time (`self.time`))
  (bind _audio (`self.Audio`))
  (bind _time_2 (`self.time`))
  (bind (_returnvalue_x _returnvalue_y _returnvalue_z) (`KismetMathLibrary.BreakVector` (`CurveVector.GetVectorValue` (`self.curve`) (`self.time`))))
  (bind _returnvalue (* (`GameplayStatics.GetWorldDeltaSeconds`) 0.45))
  ;[1 1 1] check wether player is overlapping and then start 'tick'
  (`/Engine/EditorBlueprintResources/StandardMacros.Gate` true :!label _label
    (:`Exit`
      ;[1 1 1] calculate position and rotation
      (if (!= (`KismetMathLibrary.Conv_BoolToDouble` (`self.Enter`)) 0.0)
        (set `self.time` (`KismetMathLibrary.FClamp` (+ _returnvalue _time)))
        (else
          (set `self.time` (`KismetMathLibrary.FClamp` (- _time _returnvalue)))))
      ;[1 1 1] dooranimation
      (`SceneComponent.K2_SetRelativeLocationAndRotation` (`self.modlas2`) (`KismetMathLibrary.MakeVector` 0.0 0.0 (* _returnvalue_z (`self.size`))) (`KismetMathLibrary.MakeRotator` 0.0 _returnvalue_y) false false)
      ;[1 1 1] check wether door is completely open/closed and end 'tick'
      (if (or (== _time_2 0.0) (== _time_2 1.0))
        (`self.End`)
        ;[0.3512 1 0.9402] play closing sound
        (`AudioComponent.Stop` _audio)
        (`AudioComponent.SetSound` _audio "/Game/Sounds/Doors/garage_door_end.garage_door_end")
        (`AudioComponent.Play` _audio 0.0)))))

(event `Start`
  ;[1 1 1] check wether player is overlapping and then start 'tick'
  (goto _label :!via `Open`))

(event `End`
  ;[1 1 1] check wether player is overlapping and then start 'tick'
  (goto _label :!via `Close`))

(event `self.Box.OnComponentBeginOverlap`
  (params (OverlappedComponent :type "PrimitiveComponent Object Reference") (OtherActor :type "Actor Object Reference") (OtherComp :type "PrimitiveComponent Object Reference") (OtherBodyIndex :type Integer) (bFromSweep :type Boolean) (SweepResult :type "HitResult Structure (by ref)"))
  (bind _audio (`self.Audio`))
  ;[1 0.2876 0.2378] Check wether this actor has to tick
  (cast `/Game/Player/blueprint/player_pc` (`self.GetInstigatorController` OtherActor))
  (set `self.Enter` true)
  (`self.Start`)
  ;[1 1 1] start sound loop
  (`AudioComponent.SetSound` _audio "/Game/Sounds/Doors/garage_door_loop.garage_door_loop")
  (if (not (`AudioComponent.IsPlaying` _audio))
    (`AudioComponent.Play` _audio 0.0)))

(event `self.Box.OnComponentEndOverlap`
  (params (OverlappedComponent :type "PrimitiveComponent Object Reference") (OtherActor :type "Actor Object Reference") (OtherComp :type "PrimitiveComponent Object Reference") (OtherBodyIndex :type Integer))
  (bind _audio (`self.Audio`))
  ;[1 0.2876 0.2378] Check wether this actor has to tick
  (cast `/Game/Player/blueprint/player_pc` (`self.GetInstigatorController` OtherActor))
  (set `self.Enter` false)
  (`self.Start`)
  ;[1 1 1] start sound loop
  (`AudioComponent.SetSound` _audio "/Game/Sounds/Doors/garage_door_loop.garage_door_loop")
  (if (not (`AudioComponent.IsPlaying` _audio))
    (`AudioComponent.Play` _audio 0.0)))

(fn `UserConstructionScript`
  (bind _plane (`self.Plane`))
  (bind _plane1 (`self.Plane1`))
  (bind (_origin _boxextent) (`KismetSystemLibrary.GetComponentBounds` (`self.modlas2`)))
  (bind (_relativelocation_x _relativelocation_y _relativelocation_z) (`KismetMathLibrary.BreakVector` (`SceneComponent.RelativeLocation` _plane1)))
  (bind (_relativelocation_x_2 _relativelocation_y_2 _relativelocation_z_2) (`KismetMathLibrary.BreakVector` (`SceneComponent.RelativeLocation` _plane)))
  (bind _returnvalue (+ (/ (.z _boxextent) 2.0) 10.0))
  ;[1 0.821 0.115] get size of door to set scale of animation
  (set `self.size` (/ (.z _boxextent) 100.0))
  ;[1 0 0.01785] DEBUG ARROW
  (`SceneComponent.K2_SetRelativeLocation` _plane (`KismetMathLibrary.MakeVector` _relativelocation_x_2 _relativelocation_y_2 (- _relativelocation_z_2 _returnvalue)) false false)
  (`SceneComponent.K2_SetRelativeLocation` _plane1 (`KismetMathLibrary.MakeVector` _relativelocation_x _relativelocation_y (- _relativelocation_z _returnvalue)) false false))