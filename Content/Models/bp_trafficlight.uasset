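; Traffic light prop that cycles lamps and pedestrian signal, and can be knocked over by cars.
; Construction script sets initial lamps by direction and sidedness, creating the "handman" dynamic material only when two-sided.
; Phase events from the first Trafficlight actor's north/south and east/west dispatchers switch lamps and time material changes.
; A bp_car hit enables physics, plays sound, hides lamps, clears all bindings on those shared dispatchers, then destroys it after a delay.
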(event `self.StaticMesh.OnComponentBeginOverlap`
  (params (OverlappedComponent :type "PrimitiveComponent Object Reference") (OtherActor :type "Actor Object Reference") (OtherComp :type "PrimitiveComponent Object Reference") (OtherBodyIndex :type Integer) (bFromSweep :type Boolean) (SweepResult :type "HitResult Structure (by ref)")))

(event `self.ReceiveHit`
  (params (MyComp :type "PrimitiveComponent Object Reference") (Other :type "Actor Object Reference") (OtherComp :type "PrimitiveComponent Object Reference") (bSelfMoved :type Boolean) (HitLocation :type "Vector Structure") (HitNormal :type "Vector Structure") (NormalImpulse :type "Vector Structure") (Hit :type "HitResult Structure (by ref)"))
  (bind _staticmesh (`self.StaticMesh`))
  (cast `/Game/Vehicle/generic/blueprint/bp_car` Other)
  (`PrimitiveComponent.SetSimulatePhysics` _staticmesh true)
  (`/Engine/EditorBlueprintResources/StandardMacros.DoOnce` false
    (:`Completed`
      (`GameplayStatics.PlaySoundAtLocation` "/Game/Sounds/bank_033/sound_033.sound_033" (`self.K2_GetActorLocation`) (struct) 1.0 1.0 0.0 "/Game/Sounds/bank_033/sound_hit.sound_hit" null null)
      (`PrimitiveComponent.SetCollisionResponseToChannel` _staticmesh "ECC_GameTraceChannel1" "ECR_Block")
      (`KismetSystemLibrary.PrintString` (`KismetStringLibrary.Conv_DoubleToString` (* (`KismetMathLibrary.VSize` (`self.GetVelocity` Other)) (`PrimitiveComponent.GetMass` OtherComp))) true false)
      (`SceneComponent.SetHiddenInGame` (`self.f_red`) true false)
      (`SceneComponent.SetHiddenInGame` (`self.f_yellow`) true false)
      (`SceneComponent.SetHiddenInGame` (`self.f_green`) true false)
      (`SceneComponent.SetHiddenInGame` (`self.r_red`) true false)
      (`SceneComponent.SetHiddenInGame` (`self.r_yellow`) true false)
      (`SceneComponent.SetHiddenInGame` (`self.r_green`) true false)
      (bind _output (`|GetArrayItem` (stale `self.ReceiveBeginPlay` _outactors)))
      (clear `/Game/data/Paths/trafficlight.north/south` _output)
      (clear `/Game/data/Paths/trafficlight.east/west` _output)
      (`|ExecutionSequence`
        (:`then_0`
          (`KismetSystemLibrary.Delay` 0.5)
          (`PrimitiveComponent.SetCollisionResponseToChannel` (`self.StaticMesh`) "ECC_Pawn" "ECR_Ignore"))
        (:`then_1`
          (`KismetSystemLibrary.K2_SetTimerDelegate` (delegate `DestroySelf`) 10.0))))))

(event `DestroySelf`
  (`self.K2_DestroyActor`))

(event `self.ReceiveBeginPlay`
  (bind _outactors (`GameplayStatics.GetAllActorsOfClass` "/Game/data/Paths/trafficlight.trafficlight_C"))
  (bind _output (`|GetArrayItem` _outactors))
  (add `/Game/data/Paths/trafficlight.north/south` _output (delegate `north/south`))
  (add `/Game/data/Paths/trafficlight.east/west` _output (delegate `est/west`)))

(event `est/west`
  (params (phase :type Integer))
  (bind _handman (`self.handman`))
  (bind _handman_2 (`self.handman`))
  (bind _handman_3 (`self.handman`))
  (bind _handman_4 (`self.handman`))
  (bind _handman_5 (`self.handman`))
  (bind _handman_6 (`self.handman`))
  (if (`|EnumEquality` (`self.trafficlight_direction`) "NewEnumerator1")
    (if (not (`self.2sided`))
      (switch `int` phase
        (:`0`
          ;[0.966 1 0.2499] 1sid
          ;;[1 1 1] red
          (`SceneComponent.SetVisibility` (`self.f_yellow`) false false :!label _label)
          (`SceneComponent.SetVisibility` (`self.f_green`) false false)
          (`SceneComponent.SetVisibility` (`self.f_red`) true false)
          ;[1 1 1] green
          (`MaterialInstanceDynamic.SetScalarParameterValue` _handman_4 "blink" 0.0)
          (`MaterialInstanceDynamic.SetScalarParameterValue` _handman_4 "phase" 0.0)
          (`KismetSystemLibrary.Delay` 4.0)
          ;[1 1 1] amber
          (`MaterialInstanceDynamic.SetScalarParameterValue` _handman_3 "blink" 1.0)
          (`MaterialInstanceDynamic.SetScalarParameterValue` _handman_3 "phase" 0.0))
        (:`1`
          ;;[1 1 1] yellow
          (`SceneComponent.SetVisibility` (`self.f_red`) false false :!label _label_2)
          (`SceneComponent.SetVisibility` (`self.f_green`) false false)
          (`SceneComponent.SetVisibility` (`self.f_yellow`) true false))
        (:`2`
          ;;[1 1 1] green
          (`SceneComponent.SetVisibility` (`self.f_red`) false false :!label _label_3)
          (`SceneComponent.SetVisibility` (`self.f_yellow`) false false)
          (`SceneComponent.SetVisibility` (`self.f_green`) true false)
          ;[1 1 1] red
          (`MaterialInstanceDynamic.SetScalarParameterValue` _handman_2 "blink" 0.0)
          (`MaterialInstanceDynamic.SetScalarParameterValue` _handman_2 "phase" 1.0)))
      (else
        (switch `int` phase
          (:`0`
            ;[1 0.3075 0.3872] 2sid
            ;;[1 1 1] red
            (`SceneComponent.SetVisibility` (`self.f_yellow`) false false :!label _label_4)
            (`SceneComponent.SetVisibility` (`self.f_green`) false false)
            (`SceneComponent.SetVisibility` (`self.r_green`) false false)
            (`SceneComponent.SetVisibility` (`self.r_yellow`) false false)
            (`SceneComponent.SetVisibility` (`self.r_red`) true false)
            (`SceneComponent.SetVisibility` (`self.f_red`) true false)
            (`KismetSystemLibrary.Delay` 1.0)
            ;[1 1 1] green
            (`MaterialInstanceDynamic.SetScalarParameterValue` _handman_5 "blink" 0.0)
            (`MaterialInstanceDynamic.SetScalarParameterValue` _handman_5 "phase" 0.0)
            (`KismetSystemLibrary.Delay` 5.0)
            ;[1 1 1] amber
            (`MaterialInstanceDynamic.SetScalarParameterValue` _handman "blink" 1.0)
            (`MaterialInstanceDynamic.SetScalarParameterValue` _handman "phase" 0.0)
            (`KismetSystemLibrary.Delay` 5.0)
            ;[1 1 1] red
            (`MaterialInstanceDynamic.SetScalarParameterValue` _handman_6 "blink" 0.0)
            (`MaterialInstanceDynamic.SetScalarParameterValue` _handman_6 "phase" 1.0))
          (:`1`
            ;;[1 1 1] yellow
            (`SceneComponent.SetVisibility` (`self.f_red`) false false :!label _label_5)
            (`SceneComponent.SetVisibility` (`self.f_green`) false false)
            (`SceneComponent.SetVisibility` (`self.r_red`) false false)
            (`SceneComponent.SetVisibility` (`self.f_green`) false false)
            (`SceneComponent.SetVisibility` (`self.r_yellow`) true false)
            (`SceneComponent.SetVisibility` (`self.f_yellow`) true false))
          (:`2`
            ;;[1 1 1] green
            (`SceneComponent.SetVisibility` (`self.f_red`) false false :!label _label_6)
            (`SceneComponent.SetVisibility` (`self.f_yellow`) false false)
            (`SceneComponent.SetVisibility` (`self.r_red`) false false)
            (`SceneComponent.SetVisibility` (`self.r_yellow`) false false)
            (`SceneComponent.SetVisibility` (`self.r_green`) true false)
            (`SceneComponent.SetVisibility` (`self.f_green`) true false)))))))

(event `north/south`
  (params (phase :type Integer))
  (if (`|EnumEquality` (`self.trafficlight_direction`) "NewEnumerator0")
    (if (not (`self.2sided`))
      (switch `int` phase
        (:`0`
          (goto _label))
        (:`1`
          (goto _label_2))
        (:`2`
          (goto _label_3)))
      (else
        (switch `int` phase
          (:`0`
            (goto _label_4))
          (:`1`
            (goto _label_5))
          (:`2`
            (goto _label_6)))))))

(fn `UserConstructionScript`
  (bind _staticmesh (`self.StaticMesh`))
  (if (not (`self.2sided`))
    ;[1 1 1] 1sided
    (switch `/Game/data/Paths/trafficlight_direction` (`self.trafficlight_direction`) :!label _label
      (:`NewEnumerator2`
        (`SceneComponent.SetVisibility` (`self.f_yellow`) false false)
        (`SceneComponent.SetVisibility` (`self.f_green`) false false)
        (`SceneComponent.SetVisibility` (`self.f_red`) false false)
        (`SceneComponent.SetVisibility` (`self.r_green`) false false)
        (`SceneComponent.SetVisibility` (`self.r_yellow`) false false)
        (`SceneComponent.SetVisibility` (`self.r_red`) false false))
      (:`NewEnumerator0`
        (`SceneComponent.SetVisibility` (`self.f_red`) false false)
        (`SceneComponent.SetVisibility` (`self.f_yellow`) false false)
        (`SceneComponent.SetVisibility` (`self.r_green`) false false)
        (`SceneComponent.SetVisibility` (`self.r_yellow`) false false)
        (`SceneComponent.SetVisibility` (`self.r_red`) false false)
        (`SceneComponent.SetVisibility` (`self.f_green`) true false))
      (:`NewEnumerator1`
        (`SceneComponent.SetVisibility` (`self.f_green`) false false)
        (`SceneComponent.SetVisibility` (`self.f_yellow`) false false)
        (`SceneComponent.SetVisibility` (`self.r_red`) false false)
        (`SceneComponent.SetVisibility` (`self.r_yellow`) false false)
        (`SceneComponent.SetVisibility` (`self.r_green`) false false)
        (`SceneComponent.SetVisibility` (`self.f_red`) true false)))
    (else
      (`|ExecutionSequence`
        (:`then_0`
          (goto _label))
        (:`then_1`
          ;[1 1 1] 2sided
          (switch `/Game/data/Paths/trafficlight_direction` (`self.trafficlight_direction`)
            (:`NewEnumerator2`
              (`SceneComponent.SetVisibility` (`self.f_yellow`) false false)
              (`SceneComponent.SetVisibility` (`self.f_green`) false false)
              (`SceneComponent.SetVisibility` (`self.f_red`) false false)
              (`SceneComponent.SetVisibility` (`self.r_red`) false false)
              (`SceneComponent.SetVisibility` (`self.r_yellow`) false false)
              (`SceneComponent.SetVisibility` (`self.r_green`) false false))
            (:`NewEnumerator0`
              (`SceneComponent.SetVisibility` (`self.f_red`) false false)
              (`SceneComponent.SetVisibility` (`self.f_yellow`) false false)
              (`SceneComponent.SetVisibility` (`self.r_red`) false false)
              (`SceneComponent.SetVisibility` (`self.r_yellow`) false false)
              (`SceneComponent.SetVisibility` (`self.f_green`) true false)
              (`SceneComponent.SetVisibility` (`self.r_green`) true false))
            (:`NewEnumerator1`
              (`SceneComponent.SetVisibility` (`self.f_green`) false false)
              (`SceneComponent.SetVisibility` (`self.f_yellow`) false false)
              (`SceneComponent.SetVisibility` (`self.r_yellow`) false false)
              (`SceneComponent.SetVisibility` (`self.r_green`) false false)
              (`SceneComponent.SetVisibility` (`self.f_red`) true false)
              (`SceneComponent.SetVisibility` (`self.r_red`) true false))))
        (:`then_2`
          ;[1 1 1] material 'handman'
          (for (_array_element _array_index) (`MeshComponent.GetMaterialSlotNames` _staticmesh)
            (if (`KismetStringLibrary.Contains` (`KismetStringLibrary.Conv_NameToString` _array_element) "handman")
              (bind _returnvalue (`PrimitiveComponent.CreateDynamicMaterialInstance` (`self.StaticMesh`) _array_index (`PrimitiveComponent.GetMaterial` _staticmesh _array_index) "None"))
              (set `self.handman` _returnvalue))))))))