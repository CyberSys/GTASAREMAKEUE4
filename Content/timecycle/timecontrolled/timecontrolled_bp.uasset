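; Actor that places data-table-driven static meshes and shows each only during its time window in the TimeCycle.
; The construction script adds a mesh component per table row at the row's location, converted to actor-local space, and maps it by row name.
; A handler bound to the first TimeCycle's Night event, also run at BeginPlay, hides meshes whose time range excludes the current time.
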(event `self.ReceiveBeginPlay`
  (bind _outactors (`GameplayStatics.GetAllActorsOfClass` "/Game/timecycle/TimeCycle.TimeCycle_C"))
  (bind _output_get (set `self.timecycle` (`|GetArrayItem` _outactors)))
  (add `/Game/timecycle/TimeCycle.night` _output_get (`|CreateDelegate` :!event `night`))
  (`self.night`))

(event `night`
  ;[1 1 1] Switch On Time
  (bind _outrownames (`DataTableFunctionLibrary.GetDataTableRowNames` (`self.tobj`)))
  (for _array_element _outrownames
    (bind _returnvalue (`|GetDataTableRow` (`self.tobj`) _array_element)
      (:`then`
        (bind (_time_x _time_y) (break `IntPoint` (break `/Game/timecycle/timecontrolled/data/tobj` _returnvalue)))
        (`SceneComponent.SetHiddenInGame` (`BlueprintMapLibrary.Map_Find` (`self.inserted`) _array_element) (not (`/Game/timecycle/TimeCycle.GetIsTimeInRange` (`self.timecycle`) _time_x _time_y)) false)))))

(fn `AddObjects`
  (bind _outrownames (`DataTableFunctionLibrary.GetDataTableRowNames` (`self.tobj`)))
  (for _array_element _outrownames
    (bind _returnvalue (`|GetDataTableRow` (`self.tobj`) _array_element)
      (:`then`
        (bind (_model _location) (break `/Game/timecycle/timecontrolled/data/tobj` _returnvalue))
        (bind _returnvalue_2 (`AddComponent|NODE_AddStaticMeshComponent-1` :`RelativeTransform` (`KismetMathLibrary.MakeTransform` (`KismetMathLibrary.InverseTransformLocation` (`self.GetTransform`) _location))))
        (`StaticMeshComponent.SetStaticMesh` _returnvalue_2 _model)
        (`BlueprintMapLibrary.Map_Add` (`self.inserted`) _array_element _returnvalue_2)))))

(fn `UserConstructionScript`
  ;[1 1 1] bind event 'night'
  (bind _outactors (`GameplayStatics.GetAllActorsOfClass` "/Game/timecycle/TimeCycle.TimeCycle_C"))
  (if (`KismetArrayLibrary.Array_IsValidIndex` _outactors)
    (add `/Game/timecycle/TimeCycle.night` (`|GetArrayItem` _outactors) (`|CreateDelegate` :!event `night`)))
  (`self.AddObjects`))