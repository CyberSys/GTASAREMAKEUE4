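; Mirror actor that pairs a plane mesh (WaterPlane) with a Planar Reflection component to render reflections.
; The construction script scales both components from a shared Size, with a fixed factor for the reflection, and converts a reflection distance in meters into the max view distance override.
; EnablePlanarReflection toggles capture every frame, capture on movement and in-game visibility together; the event graph has no active logic.
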(fn `EnablePlanarReflection`
  (params (bCaptureEveryFrame :type Boolean))
  (set `SceneCaptureComponent.bCaptureEveryFrame` bCaptureEveryFrame (`self.PlanarReflection`))
  (set `SceneCaptureComponent.bCaptureOnMovement` bCaptureEveryFrame (`self.PlanarReflection`))
  (`SceneComponent.SetHiddenInGame` (`self.PlanarReflection`) (not bCaptureEveryFrame) false))

(fn `setReflectionProperties`
  (set `SceneCaptureComponent.MaxViewDistanceOverride` (* (`self.ReflectionsDistance(m)`) 100.0) (`self.PlanarReflection`)))

(fn `setScale`
  (bind _size (`self.size`))
  (`SceneComponent.SetRelativeScale3D` (`self.water_plane`) (`KismetMathLibrary.Conv_Vector2DToVector` _size 1.0))
  (`SceneComponent.SetRelativeScale3D` (`self.PlanarReflection`) (`KismetMathLibrary.Conv_Vector2DToVector` (* _size 0.025) 1.0)))

(fn `UserConstructionScript`
  (`self.setScale`)
  (`self.setReflectionProperties`))