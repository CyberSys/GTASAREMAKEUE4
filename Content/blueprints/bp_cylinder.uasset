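; Shop marker placed per EnumShop type (clothing, barber, tattoo, food, Ammun, wardrobe), with a tinted cylinder and a matching camera.
; Food and Ammun shops spawn a clerk ped at BeginPlay.
; Capsule overlap blends to its camera, snaps the player into place and, for most types, opens a shopping HUD.
; HUD items come from cross-matching master DataTables against per-shop tables, or from the player's two wardrobe arrays for Wardrobe.
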(event `self.ReceiveBeginPlay`
  (bind _returnvalue (`self.GetTransform`))
  (switch `/Game/data/shoppingOLD/enum_shops` (`self.enum_shop`)
    (:`NewEnumerator0`
      (`ActorComponent.SetActive` (`self.Camera_Body`) true false :!label _label))
    (:`NewEnumerator1`
      (goto _label))
    (:`NewEnumerator2`
      (goto _label))
    (:`NewEnumerator3`
      (goto _label))
    (:`NewEnumerator4`
      (goto _label))
    (:`NewEnumerator5`
      (goto _label))
    (:`NewEnumerator6`
      (goto _label))
    (:`NewEnumerator7`
      (set `self.Ped` "wfyburg")
      (`ActorComponent.SetActive` (`self.Camera_Counter`) true false :!label _label_2)
      (bind _returnvalue_2 (`|SpawnActorFromClass` "/Game/Peds/blueprints/bp_ped_OLD.bp_ped_OLD_C" (`KismetMathLibrary.MakeTransform` (`KismetMathLibrary.TransformLocation` (`KismetMathLibrary.MakeTransform` (.location _returnvalue) (`KismetMathLibrary.MakeRotator` (.roll (.rotation _returnvalue)) (.pitch (.rotation _returnvalue)) (.yaw (.rotation _returnvalue)))) (220.0 0.0 100.0)) (`KismetMathLibrary.MakeRotator` (.roll (.rotation _returnvalue)) (.pitch (.rotation _returnvalue)) (+ (.yaw (.rotation _returnvalue)) 180.0))) "Undefined" "OverrideRootScale" null (`self.Ped`) null))
      (bind _output_get (set `self.Child_Ped` _returnvalue_2))
      (bind _asbp_ped_old (cast `/Game/Peds/blueprints/bp_ped_OLD` _output_get))
      (set `/Game/Peds/blueprints/bp_ped_OLD.enum_shop` (`self.enum_shop`) _asbp_ped_old))
    (:`NewEnumerator8`
      (set `self.Ped` "wmybell")
      (goto _label_2))
    (:`NewEnumerator9`
      (set `self.Ped` "wmypizz")
      (goto _label_2))
    (:`NewEnumerator18`
      (set `self.Ped` "wmyammo" :!label _label_3)
      (goto _label_2))
    (:`NewEnumerator20`
      (goto _label_3))
    (:`NewEnumerator21`
      (goto _label_3))
    (:`NewEnumerator22`
      (goto _label_3))
    (:`NewEnumerator23`
      (goto _label_3))
    (:`NewEnumerator19`
      (goto _label))
    (:`NewEnumerator15`
      (goto _label))
    (:`NewEnumerator16`
      (goto _label))))

(event `self.Capsule.OnComponentBeginOverlap`
  (params (OverlappedComponent :type "PrimitiveComponent Object Reference") (OtherActor :type "Actor Object Reference") (OtherComp :type "PrimitiveComponent Object Reference") (OtherBodyIndex :type Integer) (bFromSweep :type Boolean) (SweepResult :type "HitResult Structure (by ref)"))
  (bind _dat_shopping (`self.dat_shopping`))
  (bind _ref_player (`self.Ref_Player`))
  (bind _dat_weapons (`self.dat_weapons`))
  (bind _cylinder (`self.cylinder`))
  (bind _dat_food (`self.dat_food`))
  (bind (_returnvalue_x _returnvalue_y) (`KismetMathLibrary.BreakVector` (`SceneComponent.K2_GetComponentLocation` _cylinder)))
  (bind (_returnvalue_roll _returnvalue_pitch _returnvalue_yaw) (`KismetMathLibrary.BreakRotator` (`SceneComponent.K2_GetComponentRotation` _cylinder)))
  (bind _returnvalue (select `/Game/data/shoppingOLD/enum_shops` (`self.enum_shop`) :`NewEnumerator18` "/Game/data/shoppingOLD/dat_ammun1.dat_ammun1" :`NewEnumerator20` "/Game/data/shoppingOLD/dat_ammun2.dat_ammun2" :`NewEnumerator21` "/Game/data/shoppingOLD/dat_ammun3.dat_ammun3" :`NewEnumerator22` "/Game/data/shoppingOLD/dat_ammun4.dat_ammun4" :`NewEnumerator23` "/Game/data/shoppingOLD/dat_ammun5.dat_ammun5" :!type "DataTable Object Reference"))
  (bind _returnvalue_2 (select `/Game/data/shoppingOLD/enum_shops` (`self.enum_shop`) :`NewEnumerator0` "/Game/data/shoppingOLD/dat_Cschp.dat_Cschp" :`NewEnumerator1` "/Game/data/shoppingOLD/dat_Csexl.dat_Csexl" :`NewEnumerator2` "/Game/data/shoppingOLD/dat_Csprt.dat_Csprt" :`NewEnumerator3` "/Game/data/shoppingOLD/dat_CLACS1.dat_CLACS1" :`NewEnumerator4` "/Game/data/shoppingOLD/dat_shops_Uniform.dat_shops_Uniform" :`NewEnumerator5` "/Game/data/shoppingOLD/dat_Cdesgn.dat_Cdesgn" :`NewEnumerator6` "/Game/data/shoppingOLD/dat_Cgp.dat_Cgp" :`NewEnumerator15` "/Game/data/shoppingOLD/dat_shops_barbershop1.dat_shops_barbershop1" :!type "DataTable Object Reference"))
  (bind _returnvalue_3 (select `/Game/data/shoppingOLD/enum_shops` (`self.enum_shop`) :`NewEnumerator7` "/Game/data/shoppingOLD/dat_FDburg.dat_FDburg" :`NewEnumerator8` "/Game/data/shoppingOLD/dat_FDchick.dat_FDchick" :`NewEnumerator9` "/Game/data/shoppingOLD/dat_FDpizza.dat_FDpizza" :!type "DataTable Object Reference"))
  (bind _asplayer (cast `/Game/Player/blueprint/player` OtherActor))
  (bind _output_get (set `self.Ref_Player` _asplayer))
  (`/Engine/EditorBlueprintResources/StandardMacros.IsValid` _output_get
    (:`Is Valid`
      (`|ExecutionSequence`
        (:`then_0`
          ;[1 1 1] Switch Camera when entering
          (`PlayerController.SetViewTargetWithBlend` (`GameplayStatics.GetPlayerController` 0) self 0.5 "VTBlend_Linear" 0.0 false)
          ;[1 1 1] play shopping animation
          (bind _asplayer_abp (cast `/Game/Player/blueprint/player_abp` (`SkeletalMeshComponent.GetAnimInstance` (`Character.Mesh` _output_get))))
          (`AnimInstance.Montage_Play` _asplayer_abp "/Game/Player/animations/Clothes/Clothes.Clothes" 1.0 "MontageLength" 0.0 true)
          (switch `/Game/data/shoppingOLD/enum_shops` (`self.enum_shop`)
            (:`NewEnumerator0`
              (`/Game/Player/blueprint/player.hud_shopping_clothes` _output_get :!label _label_4)
              ;[0.2891 0.3963 1] Shop Clothing/Hair/Tattoo
              ;;[1 1 1] all items
              (bind _outrownames (`DataTableFunctionLibrary.GetDataTableRowNames` _dat_shopping))
              (for (_array_element _array_index) _outrownames
                (bind _returnvalue_4 (`|GetDataTableRow` _dat_shopping _array_element)
                  (:`then`
                    ;;[1 1 1] collection of items
                    (bind _outrownames_2 (`DataTableFunctionLibrary.GetDataTableRowNames` _returnvalue_2))
                    (for _array_element_2 _outrownames_2
                      (bind _returnvalue_5 (`|GetDataTableRow` _returnvalue_2 _array_element_2)
                        (:`then`
                          (bind (_name _nametag _type _fat _health _calories _stamina _respect _sexy _price _texturename _mesh _material _texture _displayname) (break `/Game/data/shoppingOLD/struct_shoppingOLD` _returnvalue_4))
                          (if (`KismetStringLibrary.EqualEqual_StrStr` _texturename (`KismetStringLibrary.Conv_NameToString` (`.item_3_E73416504F8254883EFC12BC3BF7DDC2` (break `/Game/data/shoppingOLD/struct_shopsOLD` _returnvalue_5))))
                            (`/Game/UserInterface/menus/shop/hud_shopping_clothes.Add Item` (`/Game/Player/blueprint/player.REF_Hud_shopping_clothing` (`self.Ref_Player`)) (`KismetTextLibrary.Conv_NameToText` _displayname) _type _array_index (!= (`KismetArrayLibrary.Array_Find` (`/Game/Player/blueprint/player.wardrobe` (`self.Ref_Player`)) _array_index) -1) false _price)))))))))
            (:`NewEnumerator1`
              (goto _label_4))
            (:`NewEnumerator2`
              (goto _label_4))
            (:`NewEnumerator3`
              (goto _label_4))
            (:`NewEnumerator5`
              (goto _label_4))
            (:`NewEnumerator6`
              (goto _label_4))
            (:`NewEnumerator7`
              ;[1 1 1] Start Anim Montage On Ped
              (bind _asbp_ped_old (cast `/Game/Peds/blueprints/bp_ped_OLD` (`self.Child_Ped`) :!label _label_5))
              (bind _returnvalue_6 (`SkeletalMeshComponent.GetAnimInstance` (`Character.Mesh` _asbp_ped_old)))
              (`AnimInstance.Montage_Play` _returnvalue_6 "/Game/Peds/animations/food/SHP_Food.SHP_Food" 1.0 "MontageLength" 0.0 true)
              (`AnimInstance.Montage_JumpToSection` _returnvalue_6 "Lift_In" (`AnimInstance.GetCurrentActiveMontage` _returnvalue_6))
              (`/Game/Player/blueprint/player.hud_shopping_food` _output_get)
              ;[1 0.5386 0.7562] Shop Food
              ;;[1 1 1] all items
              (bind _outrownames_3 (`DataTableFunctionLibrary.GetDataTableRowNames` _dat_food))
              (for (_array_element_3 _array_index_2) _outrownames_3
                (bind _returnvalue_7 (`|GetDataTableRow` _dat_food _array_element_3)
                  (:`then`
                    ;;[1 1 1] collection of items
                    (bind _outrownames_4 (`DataTableFunctionLibrary.GetDataTableRowNames` _returnvalue_3))
                    (for _array_element_4 _outrownames_4
                      (bind _returnvalue_8 (`|GetDataTableRow` _returnvalue_3 _array_element_4)
                        (:`then`
                          (bind (_name_2 _nametag_2 _health_2 _calories_2 _price_2 _mesh_2 _displayname_2) (break `/Game/data/shoppingOLD/struct_foodOLD` _returnvalue_7))
                          (if (`KismetStringLibrary.EqualEqual_StrStr` (`KismetStringLibrary.Conv_NameToString` _name_2) (`KismetStringLibrary.Conv_NameToString` (`.item_3_E73416504F8254883EFC12BC3BF7DDC2` (break `/Game/data/shoppingOLD/struct_shopsOLD` _returnvalue_8))))
                            (`/Game/UserInterface/menus/food/hud_shopping_food.Add Item` (`/Game/Player/blueprint/player.REF_Hud_shopping_food` (`self.Ref_Player`)) (`KismetTextLibrary.Conv_NameToText` _displayname_2) _array_index_2 _health_2 _calories_2 _price_2)))))))))
            (:`NewEnumerator8`
              (goto _label_5))
            (:`NewEnumerator9`
              (goto _label_5))
            (:`NewEnumerator18`
              ;[1 1 1] Start Anim Montage On Ped
              (bind _asbp_ped_old_2 (cast `/Game/Peds/blueprints/bp_ped_OLD` (`self.Child_Ped`) :!label _label_6))
              (bind _returnvalue_9 (`SkeletalMeshComponent.GetAnimInstance` (`Character.Mesh` _asbp_ped_old_2)))
              (`AnimInstance.Montage_Play` _returnvalue_9 "/Game/Peds/animations/weapons/SHP_Weapons.SHP_Weapons" 1.0 "MontageLength" 0.0 true)
              (`AnimInstance.Montage_JumpToSection` _returnvalue_9 "Tray_In" (`AnimInstance.GetCurrentActiveMontage` _returnvalue_9))
              (`/Game/Player/blueprint/player.hud_shopping_weapons` _output_get)
              ;[0.3521 0.474 0.202] Shop Weapons
              ;;[1 1 1] all items
              (bind _outrownames_5 (`DataTableFunctionLibrary.GetDataTableRowNames` _dat_weapons))
              (for (_array_element_5 _array_index_3) _outrownames_5
                (bind _returnvalue_10 (`|GetDataTableRow` _dat_weapons _array_element_5)
                  (:`then`
                    ;;[1 1 1] collection of items
                    (bind _outrownames_6 (`DataTableFunctionLibrary.GetDataTableRowNames` _returnvalue))
                    (for _array_element_6 _outrownames_6
                      (bind _returnvalue_11 (`|GetDataTableRow` _returnvalue _array_element_6)
                        (:`then`
                          (bind (_name_3 _nametag_3 _ammo _price_3 _mesh_3 _displayname_3) (break `/Game/data/shoppingOLD/struct_weaponsOLD` _returnvalue_10))
                          (if (`KismetStringLibrary.EqualEqual_StrStr` (`KismetStringLibrary.Conv_NameToString` _name_3) (`KismetStringLibrary.Conv_NameToString` (`.item_3_E73416504F8254883EFC12BC3BF7DDC2` (break `/Game/data/shoppingOLD/struct_shopsOLD` _returnvalue_11))))
                            (`/Game/UserInterface/menus/weapon/hud_shopping_weapons.Add Item` (`/Game/Player/blueprint/player.REF_Hud_shopping_weapons` (`self.Ref_Player`)) (`KismetTextLibrary.Conv_NameToText` _displayname_3) _array_index_3 _ammo _price_3 "None")))))))))
            (:`NewEnumerator20`
              (goto _label_6))
            (:`NewEnumerator21`
              (goto _label_6))
            (:`NewEnumerator22`
              (goto _label_6))
            (:`NewEnumerator23`
              (goto _label_6))
            (:`NewEnumerator19`
              (`/Game/Player/blueprint/player.hud_shopping_clothes` _output_get)
              ;[1 0.6955 0.3496] Wardrobe
              (for _array_element_7 (select `int` (`self.uniforms`) :`0` (`/Game/Player/blueprint/player.wardrobe` _ref_player) :`1` (`/Game/Player/blueprint/player.wardrobe_uniforms` _ref_player)) :!label _label_7
                (bind _returnvalue_12 (`|GetDataTableRow` (`self.dat_shopping`) (`KismetStringLibrary.Conv_StringToName` (`KismetStringLibrary.Conv_IntToString` _array_element_7)))
                  (:`then`
                    (bind (_name_4 _nametag_4 _type_2 _fat_2 _health_3 _calories_3 _stamina_2 _respect_2 _sexy_2 _price_4 _texturename_2 _mesh_4 _material_2 _texture_2 _displayname_4) (break `/Game/data/shoppingOLD/struct_shoppingOLD` _returnvalue_12))
                    (`/Game/UserInterface/menus/shop/hud_shopping_clothes.Add Item` (`/Game/Player/blueprint/player.REF_Hud_shopping_clothing` (`self.Ref_Player`)) (`KismetTextLibrary.Conv_NameToText` _displayname_4) _type_2 _array_element_7 false true _price_4))))
              (if (== (`self.uniforms`) 0)
                (set `self.uniforms` 1)
                (goto _label_7)
                (else
                  (set `self.uniforms` 0))))
            (:`NewEnumerator15`
              (goto _label_4))))
        (:`then_1`
          (`SceneComponent.SetHiddenInGame` (`self.cylinder`) true false)
          (bind (_returnvalue_x_2 _returnvalue_y_2 _returnvalue_z) (`KismetMathLibrary.BreakVector` (`self.K2_GetActorLocation` _output_get)))
          ;[1 0 0] Set Player Location and Rotation TEMP
          (`self.K2_SetActorLocationAndRotation` _output_get (`KismetMathLibrary.MakeVector` _returnvalue_x _returnvalue_y _returnvalue_z) (`KismetMathLibrary.MakeRotator` 0.0 0.0 (+ _returnvalue_yaw (select `/Game/data/shoppingOLD/enum_shops` (`self.enum_shop`) :`NewEnumerator7` 180.0 :`NewEnumerator8` 180.0 :`NewEnumerator9` 180.0 :`NewEnumerator18` 180.0 :`NewEnumerator20` 180.0 :`NewEnumerator21` 180.0 :`NewEnumerator22` 180.0 :`NewEnumerator23` 180.0 :!type "Float (single-precision)"))) false false))))))

(event `self.Capsule.OnComponentEndOverlap`
  (params (OverlappedComponent :type "PrimitiveComponent Object Reference") (OtherActor :type "Actor Object Reference") (OtherComp :type "PrimitiveComponent Object Reference") (OtherBodyIndex :type Integer))
  (`SceneComponent.SetHiddenInGame` (`self.cylinder`) false false))

(fn `UserConstructionScript`
  (bind _returnvalue (`PrimitiveComponent.CreateDynamicMaterialInstance` (`self.cylinder`) 0 "/Game/Material/ingame/diamond_Inst.diamond_Inst" "None"))
  (bind _output_get (set `self.Material` _returnvalue))
  (switch `/Game/data/shoppingOLD/enum_shops` (`self.enum_shop`)
    (:`NewEnumerator0`
      (`MaterialInstanceDynamic.SetVectorParameterValue` _output_get "Color" (struct :`R` 1.0 :`A` 1.0) :!label _label))
    (:`NewEnumerator1`
      (goto _label))
    (:`NewEnumerator2`
      (goto _label))
    (:`NewEnumerator3`
      (goto _label))
    (:`NewEnumerator4`
      (goto _label))
    (:`NewEnumerator5`
      (goto _label))
    (:`NewEnumerator6`
      (goto _label))
    (:`NewEnumerator7`
      (`MaterialInstanceDynamic.SetVectorParameterValue` _output_get "Color" (struct :`R` 1.0 :`G` 0.093989 :`B` 0.766463 :`A` 1.0) :!label _label_2))
    (:`NewEnumerator8`
      (goto _label_2))
    (:`NewEnumerator9`
      (goto _label_2))
    (:`NewEnumerator18`
      (goto _label))
    (:`NewEnumerator19`
      (`MaterialInstanceDynamic.SetVectorParameterValue` _output_get "Color" (struct :`B` 1.0 :`A` 1.0)))
    (:`NewEnumerator15`
      (`MaterialInstanceDynamic.SetVectorParameterValue` _output_get "Color" (struct :`R` 1.0 :`G` 1.0 :`A` 1.0) :!label _label_3))
    (:`NewEnumerator16`
      (goto _label_3))))