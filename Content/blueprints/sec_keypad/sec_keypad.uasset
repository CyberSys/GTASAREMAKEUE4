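; Security keypad actor that lets the player swipe a keycard to open a linked door once.
; A box overlap shows and hides an interaction prompt for the local player while the door is closed.
; On interact, it snaps the player beside the keypad and plays a swipe montage, whose notifies attach and remove a mesh on the hand.
; When the montage completes, a timeline swings the door forward or backward.
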(event `/Game/Player/interfaces/interact_interface.OnInteractStart`
  (params (Player :type "/Game/Player/blueprint/player Object Reference"))
  (bind _returnvalue (`self.GetTransform`))
  (bind (_returnvalue_roll _returnvalue_pitch _returnvalue_yaw) (`KismetMathLibrary.BreakRotator` (`self.K2_GetActorRotation`)))
  (bind (_returnvalue_x _returnvalue_y _returnvalue_z) (`KismetMathLibrary.BreakVector` (`self.K2_GetActorLocation` Player)))
  (bind _mesh (`Character.Mesh` Player))
  (bind _doorinitrotation (`self.DoorInitRotation`))
  (bind (_returnvalue_roll_2 _returnvalue_pitch_2 _returnvalue_yaw_2) (`KismetMathLibrary.BreakRotator` (`self.K2_GetActorRotation` (`self.Door`))))
  (if (not (`self.open`))
    (message `/Game/Player/interfaces/interact_interface.OnMessageStop` (`self.GetInstigatorController` Player))
    (`/Game/Player/blueprint/player.StopAndDisableMovement` Player)
    (`self.K2_SetActorLocationAndRotation` Player (`KismetMathLibrary.TransformLocation` (`KismetMathLibrary.MakeTransform` (`KismetMathLibrary.MakeVector` (.x (.location _returnvalue)) (.y (.location _returnvalue)) _returnvalue_z) (.rotation _returnvalue) (.scale _returnvalue)) (10.0 75.0 0.0)) (`KismetMathLibrary.MakeRotator` _returnvalue_roll _returnvalue_pitch (+ _returnvalue_yaw -90.0)) false true)
    (`|PlayMontage` _mesh "/Game/Player/animations/heist9/mon_use_swipecard.mon_use_swipecard"
      (:`OnCompleted`
        (`/Game/Player/blueprint/player.StartAndEnableMovement` Player)
        (message `/Game/Player/interfaces/interact_interface.OnInteractStop` (`self.GetInstigatorController` Player))
        (set `self.open` true)
        (set `self.DoorInitRotation` _returnvalue_yaw_2)
        ;[1 1 1] Door animation
        (bind (_direction _rotation) (`Timeline|OpenDoor` :!via `PlayFromStart`)
          (:`Update`
            (`self.K2_SetActorRotation` (`self.Door`) (`KismetMathLibrary.MakeRotator` 0.0 0.0 (`KismetMathLibrary.SelectFloat` (+ _doorinitrotation _rotation) (- _doorinitrotation _rotation) (`self.doorOpensForward?`))) false))))
      (:`OnNotifyBegin`
        (bind _returnvalue_2 (`AddComponent|NODE_AddStaticMeshComponent-0` :`RelativeTransform` (`KismetMathLibrary.MakeTransform` (0.0 0.0 0.0) (struct) (0.2 0.2 0.2))))
        (`SceneComponent.K2_AttachToComponent` _returnvalue_2 _mesh "R-Finger0NubSocket" "SnapToTarget" "SnapToTarget" "KeepWorld" true))
      (:`OnNotifyEnd`
        (`ActorComponent.K2_DestroyComponent` _returnvalue_2)))))

(event `self.Box.OnComponentBeginOverlap`
  (params (OverlappedComponent :type "PrimitiveComponent Object Reference") (OtherActor :type "Actor Object Reference") (OtherComp :type "PrimitiveComponent Object Reference") (OtherBodyIndex :type Integer) (bFromSweep :type Boolean) (SweepResult :type "HitResult Structure (by ref)"))
  (bind _returnvalue (`self.GetInstigatorController` OtherActor))
  (if (and (== _returnvalue (`GameplayStatics.GetPlayerController` 0)) (not (`self.open`)))
    (bind _message (`/Game/blueprints/GlobalFunctions.DisplayText` true "swipe keycard and enter the door."))
    (message `/Game/Player/interfaces/interact_interface.OnMessageStart` _returnvalue _message)))

(event `self.Box.OnComponentEndOverlap`
  (params (OverlappedComponent :type "PrimitiveComponent Object Reference") (OtherActor :type "Actor Object Reference") (OtherComp :type "PrimitiveComponent Object Reference") (OtherBodyIndex :type Integer))
  (bind _returnvalue (`self.GetInstigatorController` OtherActor))
  (if (and (== _returnvalue (`GameplayStatics.GetPlayerController` 0)) (not (`self.open`)))
    (message `/Game/Player/interfaces/interact_interface.OnMessageStop` _returnvalue)))

(fn `UserConstructionScript`)