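; Vending machine actor that lets the player buy and drink a soda through the interact interface.
; Its box overlap shows or hides a prompt on controllers implementing that interface.
; On interaction, it teleports the player to an offset spot facing the machine, plays a sound, and locks movement during the use montage.
; It then restores walking for an upper-body drink montage with head look disabled, and finally notifies the controller that interaction has stopped.
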(event `/Game/Player/interfaces/interact_interface.OnInteractStart`
  (params (Player :type "/Game/Player/blueprint/player Object Reference"))
  (bind _returnvalue (`self.K2_GetActorRotation`))
  (bind (_returnvalue_x _returnvalue_y _returnvalue_z) (`KismetMathLibrary.BreakVector` (`self.K2_GetActorLocation` Player)))
  (bind (_returnvalue_x_2 _returnvalue_y_2) (`KismetMathLibrary.BreakVector` (`self.K2_GetActorLocation`)))
  (bind _ref_player_abp (`/Game/Player/blueprint/player.Ref_player_abp` Player))
  (bind _charactermovement (`Character.CharacterMovement` Player))
  (bind _returnvalue_2 (+ (`KismetMathLibrary.MakeVector` _returnvalue_x_2 _returnvalue_y_2 _returnvalue_z) (* (`KismetMathLibrary.GetRightVector` _returnvalue) 100.0) (* (`KismetMathLibrary.GetForwardVector` _returnvalue) 25.0)))
  (bind (_returnvalue_roll _returnvalue_pitch _returnvalue_yaw) (`KismetMathLibrary.BreakRotator` (`KismetMathLibrary.FindLookAtRotation` _returnvalue_2 (`KismetMathLibrary.TransformLocation` (`self.GetTransform`) (25.0 0.0 0.0)))))
  ;[0.4688 1 1] InterfaceCall from Player
  (message `/Game/Player/interfaces/interact_interface.OnMessageStop` (`self.GetInstigatorController` Player))
  (`self.K2_SetActorLocationAndRotation` Player _returnvalue_2 (`KismetMathLibrary.MakeRotator` 0.0 0.0 _returnvalue_yaw) false true)
  (`CharacterMovementComponent.DisableMovement` _charactermovement)
  (`GameplayStatics.SpawnSoundAtLocation` "/Game/Sounds/script/bank_204/sound_001.sound_001" _returnvalue_2 (struct) 1.0 1.0 0.0 "/Game/Sounds/ATTENUATIONSETTINGS/Generic.Generic" null)
  (`CharacterMovementComponent.SetMovementMode` _charactermovement "MOVE_None" 0)
  (bind _returnvalue_3 (`AnimInstance.Montage_Play` _ref_player_abp "/Game/Player/animations/vend/mon_vend_use.mon_vend_use" 1.0 "Duration" 0.0 true))
  (`KismetSystemLibrary.Delay` _returnvalue_3)
  (`CharacterMovementComponent.SetMovementMode` _charactermovement "MOVE_Walking" 0)
  (set `/Game/Player/blueprint/player.UpperBody` true Player)
  (set `/Game/Player/blueprint/player_abp.HeadLook` false _ref_player_abp)
  (bind _returnvalue_4 (`AnimInstance.Montage_Play` _ref_player_abp "/Game/Player/animations/vend/mon_vend_drink_p.mon_vend_drink_p" 1.0 "Duration" 0.0 true))
  (`KismetSystemLibrary.Delay` _returnvalue_4)
  (set `/Game/Player/blueprint/player.UpperBody` false Player)
  (set `/Game/Player/blueprint/player_abp.HeadLook` true _ref_player_abp)
  (message `/Game/Player/interfaces/interact_interface.OnInteractStop` (`Pawn.GetController` Player)))

(event `self.Box.OnComponentBeginOverlap`
  (params (OverlappedComponent :type "PrimitiveComponent Object Reference") (OtherActor :type "Actor Object Reference") (OtherComp :type "PrimitiveComponent Object Reference") (OtherBodyIndex :type Integer) (bFromSweep :type Boolean) (SweepResult :type "HitResult Structure (by ref)"))
  (bind _returnvalue (`self.GetInstigatorController` OtherActor))
  ;[1 1 1] Overlap
  (if (`KismetSystemLibrary.DoesImplementInterface` _returnvalue "/Game/Player/interfaces/interact_interface.interact_interface_C")
    (bind _message (`/Game/blueprints/GlobalFunctions.DisplayText` true "buy a soda."))
    (message `/Game/Player/interfaces/interact_interface.OnMessageStart` _returnvalue _message) ; press f (Input 'Interact')....
  ))

(event `self.Box.OnComponentEndOverlap`
  (params (OverlappedComponent :type "PrimitiveComponent Object Reference") (OtherActor :type "Actor Object Reference") (OtherComp :type "PrimitiveComponent Object Reference") (OtherBodyIndex :type Integer))
  (bind _returnvalue (`self.GetInstigatorController` OtherActor))
  ;[1 1 1] Overlap
  (if (`KismetSystemLibrary.DoesImplementInterface` _returnvalue "/Game/Player/interfaces/interact_interface.interact_interface_C")
    (message `/Game/Player/interfaces/interact_interface.OnMessageStop` _returnvalue)))

(fn `UserConstructionScript`)