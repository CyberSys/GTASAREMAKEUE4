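; Interactable street food cart with chilidog, ice and noodle variants, where the Cart setting selects the mesh, vendor ped and prompt text.
; Construction applies the mesh and a red marker material, and BeginPlay spawns the vendor at an offset from the cart.
; Capsule overlap shows or hides the prompt through the controller's interact interface.
; Interacting freezes the player for an upper-body eating montage, then restores movement.
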(event `/Game/Player/interfaces/interact_interface.OnInteractStart`
  (params (Player :type "/Game/Player/blueprint/player Object Reference"))
  (bind _ref_player_abp (`/Game/Player/blueprint/player.Ref_player_abp` Player))
  (message `/Game/Player/interfaces/interact_interface.OnMessageStop` (`self.GetInstigatorController` Player))
  (`/Game/Player/blueprint/player.StopAndDisableMovement` Player)
  (set `/Game/Player/blueprint/player_abp.UpperBody` true _ref_player_abp)
  (bind _returnvalue (`AnimInstance.Montage_Play` _ref_player_abp "/Game/Player/animations/food/mon_eat_burger.mon_eat_burger" 1.0 "Duration" 0.0 true))
  (`KismetSystemLibrary.Delay` _returnvalue)
  (set `/Game/Player/blueprint/player_abp.UpperBody` false _ref_player_abp)
  (`/Game/Player/blueprint/player.StartAndEnableMovement` Player)
  (message `/Game/Player/interfaces/interact_interface.OnInteractStop` (`self.GetInstigatorController` Player)))

(event `self.ReceiveBeginPlay`
  ;[0.5841 0.2159 0.956] Spawn Ped
  (`|SpawnActorFromClass` "/Game/Peds/blueprints/bp_ped.bp_ped_C" (`KismetMathLibrary.MakeTransform` (`KismetMathLibrary.TransformLocation` (`self.GetTransform`) (-100.0 0.0 0.0)) (`self.K2_GetActorRotation`)) "Undefined" "OverrideRootScale" null (select `/Game/blueprints/cart/cart` (`self.cart`) :`NewEnumerator0` "bmochil" :`NewEnumerator1` "bmochil" :`NewEnumerator2` "omonood" :!type "Name") null))

(event `self.Capsule.OnComponentBeginOverlap`
  (params (OverlappedComponent :type "PrimitiveComponent Object Reference") (OtherActor :type "Actor Object Reference") (OtherComp :type "PrimitiveComponent Object Reference") (OtherBodyIndex :type Integer) (bFromSweep :type Boolean) (SweepResult :type "HitResult Structure (by ref)"))
  (bind _returnvalue (`self.GetInstigatorController` OtherActor))
  ;[0.7913 0.1981 0.3968] Message
  (if (`KismetSystemLibrary.DoesImplementInterface` _returnvalue "/Game/Player/interfaces/interact_interface.interact_interface_C")
    (bind _message (`/Game/blueprints/GlobalFunctions.DisplayText` true (select `/Game/blueprints/cart/cart` (`self.cart`) :`NewEnumerator0` "buy childog." :`NewEnumerator1` "buy ice." :`NewEnumerator2` "buy noodles." :!type "Text")))
    (message `/Game/Player/interfaces/interact_interface.OnMessageStart` _returnvalue _message) ; press f (Input 'Interact')....
  ))

(event `self.Capsule.OnComponentEndOverlap`
  (params (OverlappedComponent :type "PrimitiveComponent Object Reference") (OtherActor :type "Actor Object Reference") (OtherComp :type "PrimitiveComponent Object Reference") (OtherBodyIndex :type Integer))
  (bind _returnvalue (`self.GetInstigatorController` OtherActor))
  ;[0.7913 0.1981 0.3968] Message
  (if (`KismetSystemLibrary.DoesImplementInterface` _returnvalue "/Game/Player/interfaces/interact_interface.interact_interface_C")
    (message `/Game/Player/interfaces/interact_interface.OnMessageStop` _returnvalue)))

(fn `UserConstructionScript`
  (`StaticMeshComponent.SetStaticMesh` (`self.cart_mesh`) (select `/Game/blueprints/cart/cart` (`self.cart`) :`NewEnumerator0` "/Game/Models/generic/dynamic2/chillidogcart.chillidogcart" :`NewEnumerator1` "/Game/Models/generic/dynamic2/icescart_prop.icescart_prop" :`NewEnumerator2` "/Game/Models/generic/dynamic2/noodlecart_prop.noodlecart_prop" :!type "StaticMesh Object Reference"))
  (bind _returnvalue (`PrimitiveComponent.CreateDynamicMaterialInstance` (`self.cylinder`) 0 "/Game/Material/ingame/diamond.diamond" "None"))
  (`MaterialInstanceDynamic.SetVectorParameterValue` _returnvalue "color" (struct :`R` 1.0 :`A` 1.0)))