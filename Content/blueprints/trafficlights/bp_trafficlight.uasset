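; Traffic light actor that switches signal and pedestrian displays from TimeCycle events for its north/south or east/west direction.
; Construction script creates dynamic materials, adds colored lights at mesh sockets and derives direction from actor rotation, adding a color-coded marker mesh.
; Phase events set material parameters and show the matching tagged lights.
; Lights tagged "light" follow a night time range and cast shadows only while the player overlaps the lamp's sphere.
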(event `self.ReceiveBeginPlay`
  (bind _outactors (`GameplayStatics.GetAllActorsOfClass` "/Game/timecycle/TimeCycle.TimeCycle_C"))
  (if (`KismetArrayLibrary.Array_IsValidIndex` _outactors)
    (bind _astime_cycle (cast `/Game/timecycle/TimeCycle` (`|GetArrayItem` _outactors)))
    (switch `/Game/data/Paths/trafficlight_direction` (`self.trafficlight_direction`)
      (:`NewEnumerator0`
        (add `/Game/timecycle/TimeCycle.north/south` _astime_cycle (`|CreateDelegate` :!event `phase`)))
      (:`NewEnumerator1`
        (add `/Game/timecycle/TimeCycle.east/west` _astime_cycle (`|CreateDelegate` :!event `phase`))))
    (if (`KismetSystemLibrary.IsValid` (`self.mat_handman`))
      (add `/Game/timecycle/TimeCycle.handman` _astime_cycle (`|CreateDelegate` :!event `ped_light`))
      (add `/Game/timecycle/TimeCycle.night` _astime_cycle (`|CreateDelegate` :!event `night`)))))

(event `phase`
  (params (phase :type Integer))
  (`MaterialInstanceDynamic.SetVectorParameterValue` (`self.mat_light`) "phase" (select `int` phase :`0` (struct :`B` 1.0 :`A` 1.0) :`1` (struct :`G` 1.0 :`A` 1.0) :`2` (struct :`R` 1.0 :`A` 1.0) :!type "LinearColor Structure"))
  (for _array_element (`self.K2_GetComponentsByClass` "/Script/Engine.LightComponent")
    (switch `name` (`|GetArrayItem` (`ActorComponent.ComponentTags` _array_element))
      (:`red`
        ;[1 1 1] switch on/off depending on phase
        (`SceneComponent.SetHiddenInGame` _array_element (!= 2 phase) false))
      (:`yellow`
        (`SceneComponent.SetHiddenInGame` _array_element (!= 1 phase) false))
      (:`green`
        (`SceneComponent.SetHiddenInGame` _array_element (!= 0 phase) false)))))

(event `ped_light`
  (params (phase :type Integer))
  (`MaterialInstanceDynamic.SetVectorParameterValue` (`self.mat_handman`) "phase" (select `int` phase :`0` (struct :`B` 1.0 :`A` 1.0) :`1` (struct :`G` 1.0 :`A` 1.0) :`2` (struct :`R` 1.0 :`A` 1.0) :!type "LinearColor Structure")))

(event `BeginOverlap`
  (params (OverlappedComponent :type "PrimitiveComponent Object Reference") (OtherActor :type "Actor Object Reference") (OtherComp :type "PrimitiveComponent Object Reference") (OtherBodyIndex :type Integer) (bFromSweep :type Boolean) (SweepResult :type "HitResult Structure (by ref)"))
  (if (== (`self.GetInstigatorController` OtherActor) (`GameplayStatics.GetPlayerController` 0))
    (for _array_element (`self.GetComponentsByTag` "/Script/Engine.LightComponent" "light")
      (`LightComponentBase.SetCastShadows` _array_element true))))

(event `EndOverlap`
  (params (OverlappedComponent :type "PrimitiveComponent Object Reference") (OtherActor :type "Actor Object Reference") (OtherComp :type "PrimitiveComponent Object Reference") (OtherBodyIndex :type Integer))
  (if (== (`self.GetInstigatorController` OtherActor) (`GameplayStatics.GetPlayerController` 0))
    (for _array_element (`self.GetComponentsByTag` "/Script/Engine.LightComponent" "light")
      (`LightComponentBase.SetCastShadows` _array_element false))))

(event `night`
  (bind _returnvalue (`self.GetComponentsByTag` "/Script/Engine.LightComponent" "light"))
  (if (`KismetArrayLibrary.Array_IsValidIndex` _returnvalue)
    (for _array_element _returnvalue
      (`SceneComponent.SetHiddenInGame` _array_element (not (`/Game/timecycle/TimeCycle.GetIsTimeInRange` (`self.timecycle`) 21 7)) false))))

(fn `FindOrientationForTrafficLightType`
  (params (orientation :type "Float (double-precision)"))
  (returns (phase :type "/Game/data/Paths/trafficlight_direction Enum"))
  (`KismetSystemLibrary.PrintString` (`KismetStringLibrary.Conv_DoubleToString` orientation))
  (if (and (or (<= orientation 60.0) (>= orientation 150.0)) (or (<= orientation 240.0) (>= orientation 310.0)))
    (return "NewEnumerator0")
    (else
      (return "NewEnumerator1"))))

(fn `FindTrafficLightTypeFromOrientation`
  (bind (_returnvalue_roll _returnvalue_pitch) (`KismetMathLibrary.BreakRotator` (`self.K2_GetActorRotation`)))
  (bind _returnvalue (`KismetMathLibrary.MakeTransform` (+ (`self.GetActorBounds` false) (0.0 0.0 500.0))))
  (bind _phase (`self.FindOrientationForTrafficLightType` (`self.GetATanOfXY` (`KismetMathLibrary.MakeVector2D` _returnvalue_roll (* _returnvalue_pitch 57.295776)))))
  (bind _output_get (set `self.trafficlight_direction` _phase))
  (switch `/Game/data/Paths/trafficlight_direction` _output_get
    (:`NewEnumerator0`
      (bind _returnvalue_2 (`AddComponent|NODE_AddStaticMeshComponent-1` :`RelativeTransform` _returnvalue))
      (bind _returnvalue_3 (`PrimitiveComponent.CreateDynamicMaterialInstance` _returnvalue_2 0 "/Game/Material/aacolors/Color_Mat.Color_Mat" "None"))
      (`MaterialInstanceDynamic.SetVectorParameterValue` _returnvalue_3 "color" (struct :`R` 1.0 :`A` 1.0)))
    (:`NewEnumerator1`
      (bind _returnvalue_4 (`AddComponent|NODE_AddStaticMeshComponent-2` :`RelativeTransform` _returnvalue))
      (bind _returnvalue_5 (`PrimitiveComponent.CreateDynamicMaterialInstance` _returnvalue_4 0 "/Game/Material/aacolors/Color_Mat.Color_Mat" "None"))
      (`MaterialInstanceDynamic.SetVectorParameterValue` _returnvalue_5 "color" (struct :`R` 1.0 :`G` 1.0 :`A` 1.0)))))

(fn `GetATanOfXY`
  (params (Orientation :type "Vector2D Structure"))
  (returns (result :type "Float (double-precision)"))
  (locals (Vec :type "Vector2D Structure"))
  (bind (_vec_x _vec_y) (`KismetMathLibrary.BreakVector2D` (`local.Vec`)))
  (bind (_vec_x_2 _vec_y_2) (`KismetMathLibrary.BreakVector2D` (`local.Vec`)))
  (bind (_vec_x_3 _vec_y_3) (`KismetMathLibrary.BreakVector2D` (`local.Vec`)))
  (bind (_vec_x_4 _vec_y_4) (`KismetMathLibrary.BreakVector2D` (`local.Vec`)))
  (bind _vec_x_5 (`KismetMathLibrary.BreakVector2D` (`local.Vec`)))
  (bind (_vec_x_6 _vec_y_5) (`KismetMathLibrary.BreakVector2D` (`local.Vec`)))
  (bind (_vec_x_7 _vec_y_6) (`KismetMathLibrary.BreakVector2D` (`local.Vec`)))
  (bind (_vec_x_8 _vec_y_7) (`KismetMathLibrary.BreakVector2D` (`local.Vec`)))
  (bind (_vec_x_9 _vec_y_8) (`KismetMathLibrary.BreakVector2D` (`local.Vec`)))
  (bind _returnvalue (or (< _vec_x_5 0.0) (== _vec_x_5 0.0)))
  (bind _output_get (set `local.Vec` Orientation))
  (if (or (!= (`KismetMathLibrary.BreakVector2D` _output_get) 0.0) (!= (`.Y` (`KismetMathLibrary.BreakVector2D` _output_get)) 0.0))
    (if true
      (if (`KismetMathLibrary.Conv_IntToBool` (`KismetMathLibrary.And_IntInt` 0 65))
        (if _returnvalue
          (return (+ (`KismetMathLibrary.DegAtan2` 1.0 (/ _vec_y_3 _vec_x_3)) (`KismetMathLibrary.GetPI`)))
          (else
            (return (- (* (`KismetMathLibrary.GetPI`) 2.0) (`KismetMathLibrary.DegAtan2` 1.0 (/ -1.0 (* _vec_x _vec_y)))))))
        (elif _returnvalue
          (return (- (`KismetMathLibrary.GetPI`) (`KismetMathLibrary.DegAtan2` 1.0 (/ -1.0 (* _vec_x_9 _vec_y_8)))))
          (else
            (return (`KismetMathLibrary.DegAtan2` 1.0 (/ _vec_y_4 _vec_x_4))))))
      (elif (`KismetMathLibrary.Conv_IntToBool` (`KismetMathLibrary.And_IntInt` 0 65))
        (if _returnvalue
          (return (- (* (`KismetMathLibrary.GetPI`) 1.5) (`KismetMathLibrary.DegAtan2` 1.0 (/ -1.0 (* _vec_x_8 _vec_y_7)))))
          (else
            (return (+ (`KismetMathLibrary.DegAtan2` 1.0 (/ -1.0 (* _vec_x_7 _vec_y_6))) (* (`KismetMathLibrary.GetPI`) 1.5)))))
        (elif _returnvalue
          (return (+ (`KismetMathLibrary.DegAtan2` 1.0 (/ -1.0 (* _vec_x_6 _vec_y_5))) (/ (`KismetMathLibrary.GetPI`) 2.0)))
          (else
            (return (- (/ (`KismetMathLibrary.GetPI`) 2.0) (`KismetMathLibrary.DegAtan2` 1.0 (/ _vec_x_2 _vec_y_2))))))))
    (else
      (return 0.0))))

(fn `UserConstructionScript`
  (locals (index :type Name))
  (bind _staticmesh (`self.StaticMesh`))
  (bind _returnvalue (`SceneComponent.GetAllSocketNames` (`self.StaticMesh`)))
  (`|ExecutionSequence`
    (:`then_0`
      ;[1 1 1] create dynamic material
      (for _array_element (`MeshComponent.GetMaterialSlotNames` (`self.StaticMesh`))
        (switch `name` _array_element
          (:`light`
            (bind _returnvalue_2 (`MeshComponent.GetMaterialIndex` (`self.StaticMesh`) _array_element))
            (bind _returnvalue_3 (`PrimitiveComponent.GetMaterial` (`self.StaticMesh`) _returnvalue_2))
            (bind _returnvalue_4 (`PrimitiveComponent.CreateDynamicMaterialInstance` _staticmesh _returnvalue_2 _returnvalue_3 "None"))
            (set `self.mat_light` _returnvalue_4))
          (:`handman`
            (bind _returnvalue_5 (`PrimitiveComponent.CreateDynamicMaterialInstance` _staticmesh _returnvalue_2 _returnvalue_3 "None"))
            (set `self.mat_handman` _returnvalue_5)))))
    (:`then_1`
      ;[1 1 1] add lights
      (if (`KismetArrayLibrary.Array_IsValidIndex` _returnvalue)
        (for _array_element_2 _returnvalue
          (bind _returnvalue_6 (`SceneComponent.GetSocketTransform` (`self.StaticMesh`) _array_element_2 "RTS_Actor"))
          (bind _returnvalue_7 (`AddComponent|NODE_AddPointLightComponent-1` :`RelativeTransform` _returnvalue_6))
          (bind _returnvalue_8 (`KismetStringLibrary.Conv_NameToString` _array_element_2))
          (switch `string` (`KismetStringLibrary.Right` _returnvalue_8 1)
            (:`Default`
              (if (`KismetStringLibrary.EqualEqual_StrStr` _returnvalue_8 "lamp")
                (bind _returnvalue_9 (`AddComponent|NODE_AddSpotLightComponent-0` :`RelativeTransform` _returnvalue_6))
                (`LightComponent.SetLightColor` _returnvalue_9 (`self.light color`) true)
                (set `ActorComponent.ComponentTags` (`|MakeArray` "green" :!type "Name") _returnvalue_9)
                (bind _returnvalue_10 (`AddComponent|NODE_AddSphereComponent-0`))
                (`SphereComponent.SetSphereRadius` _returnvalue_10 (`LocalLightComponent.AttenuationRadius` _returnvalue_9) true)
                (add `PrimitiveComponent.OnComponentBeginOverlap` _returnvalue_10 (`|CreateDelegate` :!event `BeginOverlap`))
                (add `PrimitiveComponent.OnComponentEndOverlap` _returnvalue_10 (`|CreateDelegate` :!event `EndOverlap`))))
            (:`2`
              (`LightComponent.SetLightColor` _returnvalue_7 (struct :`R` 1.0 :`A` 1.0) true)
              (set `ActorComponent.ComponentTags` (`|MakeArray` "red" :!type "Name") _returnvalue_7))
            (:`1`
              (`LightComponent.SetLightColor` _returnvalue_7 (struct :`R` 1.0 :`G` 0.5 :`A` 1.0) true)
              (set `ActorComponent.ComponentTags` (`|MakeArray` "yellow" :!type "Name") _returnvalue_7))
            (:`0`
              (`LightComponent.SetLightColor` _returnvalue_7 (struct :`G` 1.0 :`A` 1.0) true)
              (set `ActorComponent.ComponentTags` (`|MakeArray` "green" :!type "Name") _returnvalue_7))))))
    (:`then_2`
      (`self.FindTrafficLightTypeFromOrientation`))))