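; Race checkpoint actor that links to a NextCheckPoint, forming a chain the first player passes in order.
; Construction builds a tinted cylinder material, plus an arrow aimed at the next checkpoint or a finish-flag billboard at the chain's end.
; BeginPlay deactivates the successor and hides the one after, so two show.
; An overlap while active plays a sound, reveals and activates the successor, reveals the following one and destroys itself.
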(event `self.ReceiveBeginPlay`
  (bind _nextcheckpoint (`self.NextCheckPoint`))
  (bind _nextcheckpoint_2 (`/Game/blueprints/checkpoint/race_checkpoints.NextCheckPoint` _nextcheckpoint))
  ;[1 1 1] Show only the next two checkpoints on begin play make make only these available
  (if (`KismetSystemLibrary.IsValid` _nextcheckpoint)
    (`self.UpdateArrowRotation`)
    (if (`KismetSystemLibrary.IsValid` _nextcheckpoint_2)
      (`self.SetActorHiddenInGame` _nextcheckpoint_2 true))
    (`MaterialInstanceDynamic.SetVectorParameterValue` (`/Game/blueprints/checkpoint/race_checkpoints.Cylinder_Mat` _nextcheckpoint) "color" (struct :`R` 1.0 :`G` 0.5 :`B` 0.5 :`A` 1.0)) ; color of next but one checkpoint
    (set `/Game/blueprints/checkpoint/race_checkpoints.active?` false _nextcheckpoint)))

(event `self.Capsule.OnComponentBeginOverlap`
  (params (OverlappedComponent :type "PrimitiveComponent Object Reference") (OtherActor :type "Actor Object Reference") (OtherComp :type "PrimitiveComponent Object Reference") (OtherBodyIndex :type Integer) (bFromSweep :type Boolean) (SweepResult :type "HitResult Structure (by ref)"))
  (bind _nextcheckpoint (`self.NextCheckPoint`))
  ;[1 1 1] when overlapping, update next checkpoints
  (if (and (`self.active?`) (== (`self.GetInstigatorController` OtherActor) (`GameplayStatics.GetPlayerController` 0)))
    (`self.SetActorHiddenInGame` _nextcheckpoint false)
    (`MaterialInstanceDynamic.SetVectorParameterValue` (`/Game/blueprints/checkpoint/race_checkpoints.Cylinder_Mat` _nextcheckpoint) "color" (struct :`R` 1.0 :`A` 1.0)) ; reset color of next checkpoint
    (`self.SetActorHiddenInGame` (`/Game/blueprints/checkpoint/race_checkpoints.NextCheckPoint` _nextcheckpoint) false)
    (`GameplayStatics.PlaySound2D` "/Game/Sounds/bank_53/sound_019.sound_019" 1.0 1.0 0.0 null null)
    (set `/Game/blueprints/checkpoint/race_checkpoints.active?` true _nextcheckpoint)
    (`self.K2_DestroyActor`)))

(fn `MakeCheckPoint`
  (bind _returnvalue (`PrimitiveComponent.CreateDynamicMaterialInstance` (`self.cylinder`) 0 "/Game/Material/ingame/diamond.diamond" "None"))
  (bind _output_get (set `self.Cylinder_Mat` _returnvalue))
  (`MaterialInstanceDynamic.SetVectorParameterValue` _output_get "color" (struct :`R` 0.5 :`A` 1.0))
  (`MaterialInstanceDynamic.SetScalarParameterValue` (`self.Cylinder_Mat`) "opacity" 0.75)
  (`MaterialInstanceDynamic.SetScalarParameterValue` (`self.Cylinder_Mat`) "opacityContrast" 0.25)
  (if (`KismetSystemLibrary.IsValid` (`self.NextCheckPoint`))
    ;[1 1 1] checkpointarrow
    (bind _returnvalue_2 (`AddComponent|NODE_AddStaticMeshComponent-0` :`RelativeTransform` (`KismetMathLibrary.MakeTransform` (0.0 0.0 1000.0) (`KismetMathLibrary.MakeRotator` (.roll (`KismetMathLibrary.FindLookAtRotation` (+ (`self.K2_GetActorLocation`) (0.0 0.0 200.0)) (+ (`self.K2_GetActorLocation` (`self.NextCheckPoint`)) (0.0 0.0 200.0)))) (+ (.pitch (`KismetMathLibrary.FindLookAtRotation` (+ (`self.K2_GetActorLocation`) (0.0 0.0 200.0)) (+ (`self.K2_GetActorLocation` (`self.NextCheckPoint`)) (0.0 0.0 200.0)))) 90.0) (.yaw (`KismetMathLibrary.FindLookAtRotation` (+ (`self.K2_GetActorLocation`) (0.0 0.0 200.0)) (+ (`self.K2_GetActorLocation` (`self.NextCheckPoint`)) (0.0 0.0 200.0))))) (5.0 5.0 5.0))))
    (bind _output_get_2 (set `self.arrow` _returnvalue_2))
    (bind _returnvalue_3 (`PrimitiveComponent.CreateDynamicMaterialInstance` _output_get_2 0 "/Game/Material/ingame/diamond2.diamond2" "None"))
    (`MaterialInstanceDynamic.SetVectorParameterValue` _returnvalue_3 "color2" (struct :`G` 1.0 :`A` 1.0)) ; tip color
    (`MaterialInstanceDynamic.SetVectorParameterValue` _returnvalue_3 "color" (struct :`B` 1.0 :`A` 1.0)) ; root color
    (`MaterialInstanceDynamic.SetVectorParameterValue` _returnvalue_3 "color3" (struct :`A` 1.0)) ; rim color
    (`SceneComponent.K2_AddLocalOffset` (`self.arrow`) (0.0 0.0 100.0) false false) ; fix wrong pivot of diamond (arrow)
    (else
      ;[1 1 1] finishline
      (bind _returnvalue_4 (`AddComponent|NODE_AddMaterialBillboardComponent-0` :`RelativeTransform` (`KismetMathLibrary.MakeTransform` (0.0 0.0 1000.0))))
      (bind _returnvalue_5 (`KismetMaterialLibrary.CreateDynamicMaterialInstance` "/Game/Material/ingame/finish.finish"))
      (`MaterialInstanceDynamic.SetTextureParameterValue` _returnvalue_5 "diffuse" "/Game/Particle/finishFlag.finishFlag")
      (`MaterialInstanceDynamic.SetScalarParameterValue` _returnvalue_5 "intensity" 10.0)
      (`MaterialInstanceDynamic.SetScalarParameterValue` _returnvalue_5 "X" 1.5)
      (`MaterialBillboardComponent.SetElements` _returnvalue_4 (`|MakeArray` (make `MaterialSpriteElement` _returnvalue_5 null false 200.0 400.0) :!type "MaterialSpriteElement Structure")))))

(fn `UpdateArrowRotation`
  (`SceneComponent.K2_SetRelativeRotation` (`self.arrow`) (`KismetMathLibrary.MakeRotator` (.roll (`KismetMathLibrary.FindLookAtRotation` (+ (`self.K2_GetActorLocation`) (0.0 0.0 200.0)) (+ (`self.K2_GetActorLocation` (`self.NextCheckPoint`)) (0.0 0.0 200.0)))) (+ (.pitch (`KismetMathLibrary.FindLookAtRotation` (+ (`self.K2_GetActorLocation`) (0.0 0.0 200.0)) (+ (`self.K2_GetActorLocation` (`self.NextCheckPoint`)) (0.0 0.0 200.0)))) 90.0) (.yaw (`KismetMathLibrary.FindLookAtRotation` (+ (`self.K2_GetActorLocation`) (0.0 0.0 200.0)) (+ (`self.K2_GetActorLocation` (`self.NextCheckPoint`)) (0.0 0.0 200.0))))) false false))

(fn `UserConstructionScript`
  (`self.MakeCheckPoint`))