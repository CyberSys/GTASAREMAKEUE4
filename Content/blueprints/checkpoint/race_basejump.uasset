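; Basejump landing target in the checkpoint race set that scores how close player 0 lands to its center.
; The first overlap on the target passes a DoOnce, then checks that the instigator controller is the first player's.
; The distance from the actor's location to the sweep impact point selects tiered points, with closer hits earning more.
; The score prints on screen, then the actor destroys itself after a short delay.
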(event `self.basejump_target.OnComponentBeginOverlap`
  (params (OverlappedComponent :type "PrimitiveComponent Object Reference") (OtherActor :type "Actor Object Reference") (OtherComp :type "PrimitiveComponent Object Reference") (OtherBodyIndex :type Integer) (bFromSweep :type Boolean) (SweepResult :type "HitResult Structure (by ref)"))
  (bind _returnvalue (`KismetMathLibrary.VSize` (- (`self.K2_GetActorLocation`) (`.ImpactPoint` (`GameplayStatics.BreakHitResult` SweepResult)))))
  (`/Engine/EditorBlueprintResources/StandardMacros.DoOnce` false
    (:`Completed`
      (if (== (`self.GetInstigatorController` OtherActor) (`GameplayStatics.GetPlayerController` 0))
        (`|ExecutionSequence`
          (:`then_0`
            (if (and (>= _returnvalue 0.0) (<= _returnvalue 100.0))
              (set `self.points` 35)
              (elif (and (> _returnvalue 100.0) (<= _returnvalue 200.0))
                (set `self.points` 20)
                (elif (and (> _returnvalue 200.0) (<= _returnvalue 400.0))
                  (set `self.points` 10)
                  (elif (and (> _returnvalue 400.0) (<= _returnvalue 600.0))
                    (set `self.points` 5))))))
          (:`then_1`
            (`KismetSystemLibrary.PrintString` (`KismetStringLibrary.Concat_StrStr` "You achieved " (`KismetStringLibrary.Conv_ByteToString` (`self.points`)) " points!"))
            (`KismetSystemLibrary.Delay` 2.0)
            (`self.K2_DestroyActor`)))))))

(fn `UserConstructionScript`)