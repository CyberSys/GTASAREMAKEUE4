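; Air race checkpoint hoop, linked to the following one through a Next reference to form an ordered course.
; At BeginPlay each hoop deactivates its Next and hides the one after, leaving the current and upcoming hoops visible.
; When the local player's pawn passes an active hoop, it activates Next, reveals the following hoop, plays a sound and destroys itself.
; A dynamic material distinguishes current, upcoming and final hoops by color.
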(event `self.ReceiveBeginPlay`
  (bind _next (`self.next`))
  (bind _next_2 (`/Game/blueprints/checkpoint/race_checkpoint_air.next` _next))
  (if (`KismetSystemLibrary.IsValid` (`self.next`))
    (set `/Game/blueprints/checkpoint/race_checkpoint_air.active?` false _next)
    (if (`KismetSystemLibrary.IsValid` _next_2)
      (`self.SetActorHiddenInGame` _next_2 true)
      (`MaterialInstanceDynamic.SetVectorParameterValue` (`/Game/blueprints/checkpoint/race_checkpoint_air.hoop_mat` _next) "color" (struct :`R` 1.0 :`G` 1.0 :`B` 0.5 :`A` 1.0)))
    (else
      (`MaterialInstanceDynamic.SetVectorParameterValue` (`self.hoop_mat`) "color" (struct :`R` 1.0 :`A` 1.0)) ; Last Checkpoint
    )))

(event `self.hoop.OnComponentBeginOverlap`
  (params (OverlappedComponent :type "PrimitiveComponent Object Reference") (OtherActor :type "Actor Object Reference") (OtherComp :type "PrimitiveComponent Object Reference") (OtherBodyIndex :type Integer) (bFromSweep :type Boolean) (SweepResult :type "HitResult Structure (by ref)"))
  (bind _next (`self.next`))
  (bind _next_2 (`/Game/blueprints/checkpoint/race_checkpoint_air.next` _next))
  (if (and (== (`self.GetInstigatorController` OtherActor) (`GameplayStatics.GetPlayerController` 0)) (`self.active?`))
    (set `/Game/blueprints/checkpoint/race_checkpoint_air.active?` true _next)
    (if (`KismetSystemLibrary.IsValid` _next_2)
      (`MaterialInstanceDynamic.SetVectorParameterValue` (`/Game/blueprints/checkpoint/race_checkpoint_air.hoop_mat` _next) "color" (struct :`R` 1.0 :`G` 1.0 :`A` 1.0))
      (`self.SetActorHiddenInGame` _next_2 false))
    (`GameplayStatics.PlaySound2D` "/Game/Sounds/bank_53/sound_019.sound_019" 1.0 1.0 0.0 null null)
    (`self.K2_DestroyActor`)))

(fn `UserConstructionScript`
  (bind _returnvalue (`PrimitiveComponent.CreateDynamicMaterialInstance` (`self.hoop`) 0 "/Game/Material/ingame/hoop.hoop" "None"))
  (bind _output_get (set `self.hoop_mat` _returnvalue))
  (`MaterialInstanceDynamic.SetVectorParameterValue` _output_get "color" (select `bool` (`KismetSystemLibrary.IsValid` (`self.next`)) :`false` (struct :`R` 1.0 :`A` 1.0) :`true` (struct :`R` 1.0 :`G` 1.0 :`A` 1.0) :!type "LinearColor Structure"))
  (`MaterialInstanceDynamic.SetScalarParameterValue` _output_get "opacity" 1.0))