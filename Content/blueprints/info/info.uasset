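; Info pickup actor that shows a text message to the player who walks into it.
; Its Info component spins constantly on Tick.
; On box overlap, if the instigator controller implements Interact_interface, a DoOnce hides the actor, plays a sound and sends InfoText to that controller as a message.
; After InfoTextDuration it stops the message, reappears and resets the DoOnce, so it can trigger again.
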(event `self.ReceiveTick`
  (params (DeltaSeconds :type "Float (single-precision)"))
  (`SceneComponent.K2_AddLocalRotation` (`self.info`) (`KismetMathLibrary.MakeRotator` 0.0 0.0 (* DeltaSeconds 120.0)) false false))

(event `self.Box.OnComponentBeginOverlap`
  (params (OverlappedComponent :type "PrimitiveComponent Object Reference") (OtherActor :type "Actor Object Reference") (OtherComp :type "PrimitiveComponent Object Reference") (OtherBodyIndex :type Integer) (bFromSweep :type Boolean) (SweepResult :type "HitResult Structure (by ref)"))
  (bind _returnvalue (`self.GetInstigatorController` OtherActor))
  (if (`KismetSystemLibrary.DoesImplementInterface` _returnvalue "/Game/Player/interfaces/interact_interface.interact_interface_C")
    (`/Engine/EditorBlueprintResources/StandardMacros.DoOnce` false :!label _label
      (:`Completed`
        (`self.SetActorHiddenInGame` true)
        (`GameplayStatics.PlaySound2D` "/Game/Sounds/bank_53/sound_015.sound_015" 1.0 1.0 0.0 null null)
        (bind _message (`/Game/blueprints/GlobalFunctions.DisplayText` false (`self.InfoText`)))
        (message `/Game/Player/interfaces/interact_interface.OnMessageStart` _returnvalue _message)
        (`KismetSystemLibrary.Delay` (`self.InfoTextDuration`))
        (message `/Game/Player/interfaces/interact_interface.OnMessageStop` _returnvalue)
        (`self.SetActorHiddenInGame` false)
        (goto _label :!via `Reset`)))))

(fn `UserConstructionScript`)