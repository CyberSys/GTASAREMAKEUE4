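; Export-list blackboard with three rounds of cars, crossed off as they are marked exported.
; Capsule overlap shows a prompt; interacting marks the current round's first unexported car, despite the prompt saying "random".
; AddToList updates that round's map, and UpdateList drives per-vehicle scalar parameters on a dynamic list material.
; UpdateRound handles completion, swapping the list texture and clearing entries for the next round, or playing a sound after the last.
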(event `/Game/Player/interfaces/interact_interface.OnInteractStart`
  (params (Player :type "/Game/Player/blueprint/player Object Reference"))
  (bind _list3 (`self.List3`))
  (bind _list1 (`self.List1`))
  (bind _list2 (`self.List2`))
  (message `/Game/Player/interfaces/interact_interface.OnMessageStop` Player)
  (switch `int` (`KismetMathLibrary.Conv_ByteToInt` (`self.Round`))
    (:`0`
      (bind _keys (`BlueprintMapLibrary.Map_Keys` _list1))
      (for _array_element _keys
        (if (not (`.exported?_6_2109B8F34A14D5994EC5BEBE8FEDBFF6` (break `/Game/blueprints/blackboard/exported` (`BlueprintMapLibrary.Map_Find` _list1 _array_element))))
          (`self.AddToList` _array_element)
          (break))))
    (:`1`
      (bind _keys_2 (`BlueprintMapLibrary.Map_Keys` _list2))
      (for _array_element_2 _keys_2
        (if (not (`.exported?_6_2109B8F34A14D5994EC5BEBE8FEDBFF6` (break `/Game/blueprints/blackboard/exported` (`BlueprintMapLibrary.Map_Find` _list2 _array_element_2))))
          (`self.AddToList` _array_element_2)
          (break))))
    (:`2`
      (bind _keys_3 (`BlueprintMapLibrary.Map_Keys` _list3))
      (for _array_element_3 _keys_3
        (if (not (`.exported?_6_2109B8F34A14D5994EC5BEBE8FEDBFF6` (break `/Game/blueprints/blackboard/exported` (`BlueprintMapLibrary.Map_Find` _list3 _array_element_3))))
          (`self.AddToList` _array_element_3)
          (break)))))
  (`KismetSystemLibrary.Delay` 0.5)
  (message `/Game/Player/interfaces/interact_interface.OnInteractStop` (`Pawn.GetController` Player)))

(event `self.Capsule.OnComponentBeginOverlap`
  (params (OverlappedComponent :type "PrimitiveComponent Object Reference") (OtherActor :type "Actor Object Reference") (OtherComp :type "PrimitiveComponent Object Reference") (OtherBodyIndex :type Integer) (bFromSweep :type Boolean) (SweepResult :type "HitResult Structure (by ref)"))
  (bind _returnvalue (`self.GetInstigatorController` OtherActor))
  (if (== _returnvalue (`GameplayStatics.GetPlayerController` 0))
    (bind _message (`/Game/blueprints/GlobalFunctions.DisplayText` true "add one random car to the list (aka exported so it can be crossed from the list)"))
    (message `/Game/Player/interfaces/interact_interface.OnMessageStart` _returnvalue _message)))

(event `self.Capsule.OnComponentEndOverlap`
  (params (OverlappedComponent :type "PrimitiveComponent Object Reference") (OtherActor :type "Actor Object Reference") (OtherComp :type "PrimitiveComponent Object Reference") (OtherBodyIndex :type Integer))
  (bind _returnvalue (`self.GetInstigatorController` OtherActor))
  (if (== _returnvalue (`GameplayStatics.GetPlayerController` 0))
    (message `/Game/Player/interfaces/interact_interface.OnMessageStop` _returnvalue)))

(fn `AddToList`
  (params (vehiclename :type Name))
  (bind _list1 (`self.List1`))
  (bind _list2 (`self.List2`))
  (bind _list3 (`self.List3`))
  (bind (_value _returnvalue) (`BlueprintMapLibrary.Map_Find` _list3 vehiclename))
  (bind (_value_2 _returnvalue_2) (`BlueprintMapLibrary.Map_Find` _list1 vehiclename))
  (bind (_value_3 _returnvalue_3) (`BlueprintMapLibrary.Map_Find` _list2 vehiclename))
  (switch `int` (`KismetMathLibrary.Conv_ByteToInt` (`self.Round`))
    (:`0`
      (if _returnvalue_2
        (`BlueprintMapLibrary.Map_Add` _list1 vehiclename (make `/Game/blueprints/blackboard/exported` (break `/Game/blueprints/blackboard/exported` _value_2) true))
        (`self.UpdateList` _list1)))
    (:`1`
      (if _returnvalue_3
        (`BlueprintMapLibrary.Map_Add` _list2 vehiclename (make `/Game/blueprints/blackboard/exported` (break `/Game/blueprints/blackboard/exported` _value_3) true))
        (`self.UpdateList` _list2)))
    (:`2`
      (if _returnvalue
        (`BlueprintMapLibrary.Map_Add` _list3 vehiclename (make `/Game/blueprints/blackboard/exported` (break `/Game/blueprints/blackboard/exported` _value) true))
        (`self.UpdateList` _list3)))))

(fn `ClearList`
  (bind _list3 (`self.List3`))
  (bind _list1 (`self.List1`))
  (bind _list2 (`self.List2`))
  (switch `int` (`KismetMathLibrary.Conv_ByteToInt` (`self.Round`))
    (:`0`
      (bind _keys (`BlueprintMapLibrary.Map_Keys` _list1))
      (for _array_element _keys
        (bind _value (`BlueprintMapLibrary.Map_Find` _list1 _array_element))
        (`BlueprintMapLibrary.Map_Add` _list1 _array_element (make `/Game/blueprints/blackboard/exported` (break `/Game/blueprints/blackboard/exported` _value)))
        (`MaterialInstanceDynamic.SetScalarParameterValue` (`self.List_mat`) (`KismetStringLibrary.Conv_StringToName` (`KismetStringLibrary.Concat_StrStr` "vehicle" (`KismetStringLibrary.Conv_ByteToString` (break `/Game/blueprints/blackboard/exported` _value)))) 0.0)))
    (:`1`
      (bind _keys_2 (`BlueprintMapLibrary.Map_Keys` _list2))
      (for _array_element_2 _keys_2
        (bind _value_2 (`BlueprintMapLibrary.Map_Find` _list2 _array_element_2))
        (`BlueprintMapLibrary.Map_Add` _list2 _array_element_2 (make `/Game/blueprints/blackboard/exported` (break `/Game/blueprints/blackboard/exported` _value_2)))
        (`MaterialInstanceDynamic.SetScalarParameterValue` (`self.List_mat`) (`KismetStringLibrary.Conv_StringToName` (`KismetStringLibrary.Concat_StrStr` "vehicle" (`KismetStringLibrary.Conv_ByteToString` (break `/Game/blueprints/blackboard/exported` _value_2)))) 0.0)))
    (:`2`
      (bind _keys_3 (`BlueprintMapLibrary.Map_Keys` _list3))
      (for _array_element_3 _keys_3
        (bind _value_3 (`BlueprintMapLibrary.Map_Find` _list3 _array_element_3))
        (`BlueprintMapLibrary.Map_Add` _list3 _array_element_3 (make `/Game/blueprints/blackboard/exported` (break `/Game/blueprints/blackboard/exported` _value_3)))
        (`MaterialInstanceDynamic.SetScalarParameterValue` (`self.List_mat`) (`KismetStringLibrary.Conv_StringToName` (`KismetStringLibrary.Concat_StrStr` "vehicle" (`KismetStringLibrary.Conv_ByteToString` (break `/Game/blueprints/blackboard/exported` _value_3)))) 0.0)))))

(fn `UpdateList`
  (params (CurrentList :type "Map of Name to /Game/blueprints/blackboard/exported Structure (by ref)"))
  (bind _keys (`BlueprintMapLibrary.Map_Keys` CurrentList))
  (for _array_element _keys
    (bind _value (`BlueprintMapLibrary.Map_Find` CurrentList _array_element))
    (`MaterialInstanceDynamic.SetScalarParameterValue` (`self.List_mat`) (`KismetStringLibrary.Conv_StringToName` (`KismetStringLibrary.Concat_StrStr` "vehicle" (`KismetStringLibrary.Conv_ByteToString` (break `/Game/blueprints/blackboard/exported` _value)))) (`KismetMathLibrary.Conv_BoolToDouble` (`.exported?_6_2109B8F34A14D5994EC5BEBE8FEDBFF6` (break `/Game/blueprints/blackboard/exported` _value)))))
  (`self.UpdateRound`))

(fn `UpdateRound`
  (locals (complete :type Boolean :default true))
  (switch `int` (`KismetMathLibrary.Conv_ByteToInt` (`self.Round`))
    (:`0`
      (bind _values (`BlueprintMapLibrary.Map_Values` (`self.List1`)))
      (for _array_element _values
        (if (not (`.exported?_6_2109B8F34A14D5994EC5BEBE8FEDBFF6` (break `/Game/blueprints/blackboard/exported` _array_element)))
          (set `local.complete` false)
          (break)))
      (if (`local.complete`)
        (set `self.Round` (+ (`self.Round`) 1) :!label _label)
        (`MaterialInstanceDynamic.SetTextureParameterValue` (`self.List_mat`) "List" (select `byte` (`self.Round`) :`0` "/Game/Textures/WCList1.WCList1" :`1` "/Game/Textures/WCList2.WCList2" :`2` "/Game/Textures/WCList3.WCList3" :!type "Texture Object Reference"))
        (`self.ClearList`)))
    (:`1`
      (bind _values_2 (`BlueprintMapLibrary.Map_Values` (`self.List2`)))
      (for _array_element_2 _values_2
        (if (not (`.exported?_6_2109B8F34A14D5994EC5BEBE8FEDBFF6` (break `/Game/blueprints/blackboard/exported` _array_element_2)))
          (set `local.complete` false)
          (break)))
      (if (`local.complete`)
        (goto _label)))
    (:`2`
      (bind _values_3 (`BlueprintMapLibrary.Map_Values` (`self.List3`)))
      (for _array_element_3 _values_3
        (if (not (`.exported?_6_2109B8F34A14D5994EC5BEBE8FEDBFF6` (break `/Game/blueprints/blackboard/exported` _array_element_3)))
          (set `local.complete` false)
          (break)))
      (if (`local.complete`)
        (`GameplayStatics.PlaySound2D` "/Game/Sounds/bank_53/sound_019.sound_019" 1.0 1.0 0.0 null null)))))

(fn `UserConstructionScript`
  (bind _list_mesh (`self.List_mesh`))
  ;[1 1 1] has player already unlocked export?
  (if (`self.active?`)
    (if (not (`KismetSystemLibrary.IsValid` (`self.List_mesh`)))
      (bind _returnvalue (`AddComponent|NODE_AddStaticMeshComponent-1`))
      (bind _output_get (set `self.List_mesh` _returnvalue)))
    (`StaticMeshComponent.SetStaticMesh` _output_get (select `byte` (`self.Round`) :`0` "/Game/Models/generic/levelxre/nf_list_1.nf_list_1" :`1` "/Game/Models/generic/levelxre/nf_list_2.nf_list_2" :`2` "/Game/Models/generic/levelxre/nf_list_3.nf_list_3" :!type "StaticMesh Object Reference"))
    (bind _returnvalue_2 (`PrimitiveComponent.CreateDynamicMaterialInstance` _list_mesh (`KismetArrayLibrary.Array_Find` (`MeshComponent.GetMaterialSlotNames` _list_mesh) "list") "/Game/blueprints/blackboard/WC_List.WC_List" "None"))
    (bind _output_get_2 (set `self.List_mat` _returnvalue_2))
    (`MaterialInstanceDynamic.SetTextureParameterValue` _output_get_2 "List" (select `byte` (`self.Round`) :`0` "/Game/Textures/WCList1.WCList1" :`1` "/Game/Textures/WCList2.WCList2" :`2` "/Game/Textures/WCList3.WCList3" :!type "Texture Object Reference"))
    ;[1 1 1] cylinder
    (bind _returnvalue_3 (`PrimitiveComponent.CreateDynamicMaterialInstance` (`self.cylinder`) 0 "/Game/Material/ingame/diamond.diamond" "None"))
    (`MaterialInstanceDynamic.SetVectorParameterValue` _returnvalue_3 "color" (struct :`R` 1.0 :`A` 1.0))
    (`self.ClearList`)))