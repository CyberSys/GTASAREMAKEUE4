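; Park bench interactable that lets the player sit down and stand up.
; A box overlap shows or hides a "have a seat" prompt through the controller's Interact_interface.
; Interacting toggles seating: it snaps the player to the bench with collision, movement and input off, then plays turn and sit montages.
; Standing slides the capsule out during its montage before restoring control, with montage durations timing each step and an interact-stop message closing both.
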(event `/Game/Player/interfaces/interact_interface.OnInteractStart`
  (params (Player :type "/Game/Player/blueprint/player Object Reference"))
  (bind _returnvalue (`self.K2_GetActorRotation`))
  (bind (_returnvalue_x _returnvalue_y _returnvalue_z) (`KismetMathLibrary.BreakVector` (`self.K2_GetActorLocation` Player)))
  (bind (_returnvalue_x_2 _returnvalue_y_2) (`KismetMathLibrary.BreakVector` (`self.K2_GetActorLocation`)))
  (bind (_returnvalue_roll _returnvalue_pitch _returnvalue_yaw) (`KismetMathLibrary.BreakRotator` (`self.K2_GetActorRotation` Player)))
  (bind _ref_player_abp (`/Game/Player/blueprint/player.Ref_player_abp` Player))
  (bind _charactermovement (`Character.CharacterMovement` Player))
  (bind _returnvalue_2 (+ (`KismetMathLibrary.MakeVector` _returnvalue_x_2 _returnvalue_y_2 _returnvalue_z) (* (`KismetMathLibrary.GetRightVector` _returnvalue) 0.0) (* (`KismetMathLibrary.GetForwardVector` _returnvalue) -50.0)))
  (bind (_returnvalue_roll_2 _returnvalue_pitch_2 _returnvalue_yaw_2) (`KismetMathLibrary.BreakRotator` (`KismetMathLibrary.FindLookAtRotation` _returnvalue_2 (`KismetMathLibrary.TransformLocation` (`self.GetTransform`) (100.0 0.0 0.0)))))
  (bind _output_get (set `self.pendingPossess?` (not (`self.pendingPossess?`))))
  (if _output_get
    (message `/Game/Player/interfaces/interact_interface.OnMessageStop` (`self.GetInstigatorController` Player))
    (`PrimitiveComponent.SetCollisionEnabled` (`Character.CapsuleComponent` Player) "NoCollision")
    (`self.K2_SetActorLocationAndRotation` Player _returnvalue_2 (`KismetMathLibrary.MakeRotator` 0.0 0.0 _returnvalue_yaw_2) false true)
    (`MovementComponent.StopMovementImmediately` _charactermovement)
    (`CharacterMovementComponent.SetMovementMode` _charactermovement "MOVE_None" 0)
    (`self.DisableInput` Player (`GameplayStatics.GetPlayerController` 0))
    (bind _returnvalue_3 (`AnimInstance.Montage_Play` _ref_player_abp "/Game/Player/animations/ped/mon_turn_180.mon_turn_180" 1.0 "Duration" 0.0 true))
    (`KismetSystemLibrary.Delay` _returnvalue_3)
    (`|ExecutionSequence`
      (:`then_0`
        (`self.K2_SetActorRotation` Player (`KismetMathLibrary.MakeRotator` _returnvalue_roll _returnvalue_pitch (* _returnvalue_yaw -1.0)) true))
      (:`then_1`
        (bind _returnvalue_4 (`AnimInstance.Montage_Play` _ref_player_abp "/Game/Player/animations/ped/mon_seat_down.mon_seat_down" 1.0 "Duration" 0.0 true))
        (set `/Game/Player/blueprint/player_abp.state` "NewEnumerator7" _ref_player_abp)
        (`KismetSystemLibrary.Delay` _returnvalue_4)
        (message `/Game/Player/interfaces/interact_interface.OnInteractStop` (`Pawn.GetController` Player) :!label _label)))
    (else
      (`CharacterMovementComponent.SetMovementMode` _charactermovement "MOVE_Walking" 0)
      (bind _returnvalue_5 (`AnimInstance.Montage_Play` _ref_player_abp "/Game/Player/animations/ped/mon_seat_up.mon_seat_up" 1.0 "Duration" 0.0 true))
      (set `/Game/Player/blueprint/player_abp.state` "NewEnumerator1" _ref_player_abp)
      (`KismetSystemLibrary.MoveComponentTo` (`Character.CapsuleComponent` Player) (+ _returnvalue_2 (0.0 -50.0 0.0)) (`self.K2_GetActorRotation` Player) false false _returnvalue_5)
      (`KismetSystemLibrary.Delay` _returnvalue_5)
      (`PrimitiveComponent.SetCollisionEnabled` (`Character.CapsuleComponent` Player) "QueryAndPhysics")
      (`self.EnableInput` Player (`GameplayStatics.GetPlayerController` 0))
      (goto _label))))

(event `self.Box.OnComponentBeginOverlap`
  (params (OverlappedComponent :type "PrimitiveComponent Object Reference") (OtherActor :type "Actor Object Reference") (OtherComp :type "PrimitiveComponent Object Reference") (OtherBodyIndex :type Integer) (bFromSweep :type Boolean) (SweepResult :type "HitResult Structure (by ref)"))
  (bind _returnvalue (`self.GetInstigatorController` OtherActor))
  (if (`KismetSystemLibrary.DoesImplementInterface` _returnvalue "/Game/Player/interfaces/interact_interface.interact_interface_C")
    (bind _message (`/Game/blueprints/GlobalFunctions.DisplayText` true "have a seat."))
    (message `/Game/Player/interfaces/interact_interface.OnMessageStart` _returnvalue _message) ; press f (Input 'Interact')....
  ))

(event `self.Box.OnComponentEndOverlap`
  (params (OverlappedComponent :type "PrimitiveComponent Object Reference") (OtherActor :type "Actor Object Reference") (OtherComp :type "PrimitiveComponent Object Reference") (OtherBodyIndex :type Integer))
  (bind _returnvalue (`self.GetInstigatorController` OtherActor))
  (if (`KismetSystemLibrary.DoesImplementInterface` _returnvalue "/Game/Player/interfaces/interact_interface.interact_interface_C")
    (message `/Game/Player/interfaces/interact_interface.OnMessageStop` _returnvalue)))

(fn `UserConstructionScript`)