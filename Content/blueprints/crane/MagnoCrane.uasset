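; MagnoCrane is a drivable crane the player enters through an interaction prompt, which possesses it, hides the player and blends to a child-actor camera.
; While possessed, Tick maps PlayerPC input axes to slewing, clamped linear travel and rope length, the last driving both constraint limit and cable length.
; The camera tracks a crane part, and input toggles engine-load audio.
; The construction script tints the marker cylinder and snaps it to the ground.
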(event `self.ReceiveTick`
  (params (DeltaSeconds :type "Float (single-precision)"))
  (if (`self.possessed`)
    ;[1 1 1] movement
    (`self.AngularMovement`)
    (`self.LinearMovement`)
    (`self.RopeLength`)
    (`self.CameraRotation`)
    (bind _returnvalue (`self.Audio`))
    ;[1 1 1] Unload Audio
    (if (== _returnvalue true)
      (goto _label :!via `Reset`)
      (elif (== _returnvalue false)
        (`/Engine/EditorBlueprintResources/StandardMacros.DoOnce` true :!label _label
          (:`Completed`
            (`GameplayStatics.SpawnSoundAtLocation` "/Game/Sounds/gen/bank_38/sound_003.sound_003" (`SceneComponent.K2_GetComponentLocation` (`self.EngineSound`)) (struct) 0.5 1.0 0.0 "/Game/Sounds/ATTENUATIONSETTINGS/Generic.Generic" null)))))))

(event `/Game/Player/interfaces/interact_interface.OnInteractStart`
  (params (Player :type "/Game/Player/blueprint/player Object Reference"))
  (bind _returnvalue (`GameplayStatics.GetPlayerController` 0))
  ;[1 1 1] Possess
  (`self.SetActorHiddenInGame` Player true)
  (message `/Game/Player/interfaces/interact_interface.OnMessageStop` (`self.GetInstigatorController` Player))
  (`Controller.Possess` _returnvalue self)
  (`PlayerController.SetViewTargetWithBlend` _returnvalue (`ChildActorComponent.ChildActor` (`self.bp_camera`)) 0.0 "VTBlend_Linear" 0.0 false)
  (`self.K2_AttachToComponent` Player (`self.MagnoCrane_01`) "None" "KeepWorld" "KeepWorld" "KeepRelative" true)
  (bind _asplayer_pc (cast `/Game/Player/blueprint/player_pc` (`GameplayStatics.GetPlayerController` 0)))
  (set `self.PlayerPC` _asplayer_pc)
  (set `self.possessed` true)
  (`ActorComponent.Activate` (`self.EngineSound`) true)
  (`SceneComponent.SetHiddenInGame` (`self.cylinder`) true true))

(event `/Game/Player/interfaces/interact_interface.OnInteractStop`
  ;[1 1 1] Possess
  (`self.SetActorHiddenInGame` (stale `/Game/Player/interfaces/interact_interface.OnInteractStart` Player) false)
  (`Controller.Possess` (`GameplayStatics.GetPlayerController` 0) (stale `/Game/Player/interfaces/interact_interface.OnInteractStart` Player))
  (`self.K2_DetachFromActor` (stale `/Game/Player/interfaces/interact_interface.OnInteractStart` Player) "KeepWorld" "KeepWorld" "KeepRelative")
  (set `self.possessed` false)
  (message `/Game/Player/interfaces/interact_interface.OnInteractStop` (`self.GetInstigatorController` (stale `/Game/Player/interfaces/interact_interface.OnInteractStart` Player)))
  (`ActorComponent.Deactivate` (`self.EngineSound`))
  (`SceneComponent.SetHiddenInGame` (`self.cylinder`) false true))

(event `self.Capsule.OnComponentBeginOverlap`
  (params (OverlappedComponent :type "PrimitiveComponent Object Reference") (OtherActor :type "Actor Object Reference") (OtherComp :type "PrimitiveComponent Object Reference") (OtherBodyIndex :type Integer) (bFromSweep :type Boolean) (SweepResult :type "HitResult Structure (by ref)"))
  ;[1 1 1] Message
  (bind _message (`/Game/blueprints/GlobalFunctions.DisplayText` true "enter crane"))
  (message `/Game/Player/interfaces/interact_interface.OnMessageStart` (`self.GetInstigatorController` OtherActor) _message))

(event `self.Capsule.OnComponentEndOverlap`
  (params (OverlappedComponent :type "PrimitiveComponent Object Reference") (OtherActor :type "Actor Object Reference") (OtherComp :type "PrimitiveComponent Object Reference") (OtherBodyIndex :type Integer))
  ;[1 1 1] Message
  (message `/Game/Player/interfaces/interact_interface.OnMessageStop` (`self.GetInstigatorController` OtherActor)))

(fn `AngularMovement`
  (bind _moveforward (`/Game/Player/blueprint/player_pc.MoveForward` (`self.PlayerPC`)))
  (bind _returnvalue (+ (* _moveforward (* (`GameplayStatics.GetWorldDeltaSeconds`) 15.0)) (`self.CurrentRotation`)))
  (if (!= _moveforward 0.0)
    (bind _output_get (set `self.CurrentRotation` (select `bool` (or (>= _returnvalue 360.0) (<= _returnvalue -360.0)) :`false` _returnvalue)))
    (`SceneComponent.K2_SetRelativeRotation` (`self.MagnoCrane_02`) (`KismetMathLibrary.MakeRotator` 0.0 0.0 _output_get) false false)))

(fn `Audio`
  (returns (ReturnValue :type Boolean))
  (bind _playerpc (`self.PlayerPC`))
  (bind _moveforward (`/Game/Player/blueprint/player_pc.MoveForward` _playerpc))
  (bind _moveright (`/Game/Player/blueprint/player_pc.MoveRight` _playerpc))
  (bind _returnvalue (`KismetMathLibrary.Conv_IntToBool` (`KismetMathLibrary.FTrunc` (`KismetMathLibrary.FMin` 1.0 (+ (* _moveforward (`KismetMathLibrary.SignOfFloat` _moveforward)) (* _moveright (`KismetMathLibrary.SignOfFloat` _moveright)))))))
  (`AudioComponent.SetBoolParameter` (`self.EngineSound`) "load" _returnvalue)
  (return _returnvalue))

(fn `CameraRotation`
  (bind _bp_camera (`self.bp_camera`))
  (`SceneComponent.K2_SetWorldRotation` _bp_camera (`KismetMathLibrary.FindLookAtRotation` (`SceneComponent.K2_GetComponentLocation` _bp_camera) (`SceneComponent.K2_GetComponentLocation` (`self.MagnoCrane_04`))) false false))

(fn `LinearMovement`
  (bind _moveright (`/Game/Player/blueprint/player_pc.MoveRight` (`self.PlayerPC`)))
  (if (!= _moveright 0.0)
    (bind _output_get (set `self.CurrentLocation` (`KismetMathLibrary.FClamp` (+ (* _moveright (* (`GameplayStatics.GetWorldDeltaSeconds`) 350.0)) (`self.CurrentLocation`)) -2000.0 2000.0)))
    (`SceneComponent.K2_SetRelativeLocation` (`self.MagnoCrane_01`) (`KismetMathLibrary.MakeVector` _output_get) false false)))

(fn `RopeLength`
  (bind _updown (`/Game/Player/blueprint/player_pc.Updown` (`self.PlayerPC`)))
  (if (!= _updown 0.0)
    (bind _output_get (set `self.CurrentLength` (`KismetMathLibrary.FClamp` (+ (* _updown (* (`GameplayStatics.GetWorldDeltaSeconds`) 350.0)) (`self.CurrentLength`)) 100.0 3700.0)))
    (`PhysicsConstraintComponent.SetLinearZLimit` (`self.constraint`) "LCM_Limited" _output_get)
    (set `CableComponent.CableLength` _output_get (`self.Cable`))))

(fn `UserConstructionScript`
  (bind _cylinder (`self.cylinder`))
  (bind (_returnvalue_x _returnvalue_y) (`KismetMathLibrary.BreakVector` (`SceneComponent.K2_GetComponentLocation` _cylinder)))
  (bind _returnvalue (`SceneComponent.K2_GetComponentLocation` (`self.cylinder`)))
  (bind _returnvalue_2 (`PrimitiveComponent.CreateDynamicMaterialInstance` (`self.cylinder`) 0 "/Game/Material/ingame/diamond.diamond" "None"))
  (`MaterialInstanceDynamic.SetVectorParameterValue` _returnvalue_2 "color" (struct :`R` 1.0 :`A` 1.0))
  (bind (_outhit _returnvalue_3) (`KismetSystemLibrary.LineTraceSingle` _returnvalue (- _returnvalue (0.0 0.0 100.0)) "TraceTypeQuery1" true))
  (if _returnvalue_3
    (`SceneComponent.K2_SetWorldLocation` _cylinder (`KismetMathLibrary.MakeVector` _returnvalue_x _returnvalue_y (.z (`.Location` (`GameplayStatics.BreakHitResult` _outhit)))) false true)))