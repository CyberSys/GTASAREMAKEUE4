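; An interactable, destructible ATM that lets the player check savings and spills money when wrecked.
; Box overlap shows a prompt through the controller's Interact_interface; interacting snaps the player beside the machine and locks movement and input during a montage.
; Damage lowers Life and swaps meshes: the first stage removes the interaction box, while near-zero Life starts a one-time delayed loop launching Money pickups with randomized impulses until MoneyCount reaches zero.
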(event `/Game/Player/interfaces/interact_interface.OnInteractStart`
  (params (Player :type "/Game/Player/blueprint/player Object Reference"))
  (bind _returnvalue (`self.K2_GetActorRotation`))
  (bind (_returnvalue_x _returnvalue_y _returnvalue_z) (`KismetMathLibrary.BreakVector` (`self.K2_GetActorLocation` Player)))
  (bind (_returnvalue_x_2 _returnvalue_y_2) (`KismetMathLibrary.BreakVector` (`self.K2_GetActorLocation`)))
  (bind _charactermovement (`Character.CharacterMovement` Player))
  (bind _returnvalue_2 (+ (`KismetMathLibrary.MakeVector` _returnvalue_x_2 _returnvalue_y_2 _returnvalue_z) (* (`KismetMathLibrary.GetRightVector` _returnvalue) 100.0) (* (`KismetMathLibrary.GetForwardVector` _returnvalue) 25.0)))
  (bind (_returnvalue_roll _returnvalue_pitch _returnvalue_yaw) (`KismetMathLibrary.BreakRotator` (`KismetMathLibrary.FindLookAtRotation` _returnvalue_2 (`KismetMathLibrary.TransformLocation` (`self.GetTransform`) (25.0 0.0 0.0)))))
  (message `/Game/Player/interfaces/interact_interface.OnMessageStop` (`self.GetInstigatorController` Player))
  (`self.K2_SetActorLocationAndRotation` Player _returnvalue_2 (`KismetMathLibrary.MakeRotator` 0.0 0.0 _returnvalue_yaw) false true)
  (`MovementComponent.StopMovementImmediately` _charactermovement)
  (`CharacterMovementComponent.SetMovementMode` _charactermovement "MOVE_None" 0)
  (`self.DisableInput` Player (`GameplayStatics.GetPlayerController` 0))
  (bind _returnvalue_3 (`AnimInstance.Montage_Play` (`/Game/Player/blueprint/player.Ref_player_abp` Player) "/Game/Player/animations/ped/mon_atm.mon_atm" 1.0 "Duration" 0.0 true))
  (`KismetSystemLibrary.Delay` _returnvalue_3)
  (`CharacterMovementComponent.SetMovementMode` _charactermovement "MOVE_Walking" 0)
  (`self.EnableInput` Player (`GameplayStatics.GetPlayerController` 0))
  (message `/Game/Player/interfaces/interact_interface.OnInteractStop` (`Pawn.GetController` Player)))

(event `self.ReceiveAnyDamage`
  (params (Damage :type "Float (single-precision)") (DamageType :type "DamageType Object Reference") (InstigatedBy :type "Controller Object Reference") (DamageCauser :type "Actor Object Reference"))
  (bind _returnvalue (`self.K2_GetActorRotation`))
  (bind _output_get (set `self.life` (- (`self.life`) Damage)))
  (if (and (< _output_get 75.0) (>= _output_get 50.0))
    (`StaticMeshComponent.SetStaticMesh` (`self.kmb_atm1`) "/Game/Models/generic/levelxre/kmb_atm2.kmb_atm2")
    (`ActorComponent.K2_DestroyComponent` (`self.Box`))
    (elif (< _output_get 5.0)
      (`StaticMeshComponent.SetStaticMesh` (`self.kmb_atm1`) "/Game/Models/generic/levelxre/kmb_atm3.kmb_atm3")
      (`/Engine/EditorBlueprintResources/StandardMacros.DoOnce` false
        (:`Completed`
          (`/Engine/EditorBlueprintResources/StandardMacros.DecrementInt` (`self.MoneyCount`) :!label _label
            (:`  `
              (`KismetSystemLibrary.Delay` 0.1)
              (bind _returnvalue_2 (`|SpawnActorFromClass` "/Game/blueprints/atm/money.money_C" (`self.GetTransform`) "AlwaysSpawn" "OverrideRootScale" null 1000 false null))
              (`PrimitiveComponent.AddImpulse` (`/Game/blueprints/atm/money.Box` _returnvalue_2) (+ (* (`KismetMathLibrary.GetForwardVector` _returnvalue) (`KismetMathLibrary.RandomFloatInRange` -10.0 10.0)) (* (`KismetMathLibrary.GetRightVector` _returnvalue) (+ 25.0 (`KismetMathLibrary.RandomFloatInRange` -10.0 10.0))) (* (`KismetMathLibrary.GetUpVector` _returnvalue) (+ 25.0 (`KismetMathLibrary.RandomFloatInRange` -10.0 10.0)))) "None" false)
              (if (!= (`self.MoneyCount`) 0)
                (goto _label)))))))))

(event `self.Box.OnComponentBeginOverlap`
  (params (OverlappedComponent :type "PrimitiveComponent Object Reference") (OtherActor :type "Actor Object Reference") (OtherComp :type "PrimitiveComponent Object Reference") (OtherBodyIndex :type Integer) (bFromSweep :type Boolean) (SweepResult :type "HitResult Structure (by ref)"))
  (bind _returnvalue (`self.GetInstigatorController` OtherActor))
  (if (`KismetSystemLibrary.DoesImplementInterface` _returnvalue "/Game/Player/interfaces/interact_interface.interact_interface_C")
    (bind _message (`/Game/blueprints/GlobalFunctions.DisplayText` true "check your savings."))
    (message `/Game/Player/interfaces/interact_interface.OnMessageStart` _returnvalue _message) ; press f (Input 'Interact')....
  ))

(event `self.Box.OnComponentEndOverlap`
  (params (OverlappedComponent :type "PrimitiveComponent Object Reference") (OtherActor :type "Actor Object Reference") (OtherComp :type "PrimitiveComponent Object Reference") (OtherBodyIndex :type Integer))
  (bind _returnvalue (`self.GetInstigatorController` OtherActor))
  (if (`KismetSystemLibrary.DoesImplementInterface` _returnvalue "/Game/Player/interfaces/interact_interface.interact_interface_C")
    (message `/Game/Player/interfaces/interact_interface.OnMessageStop` _returnvalue)))

(fn `UserConstructionScript`)