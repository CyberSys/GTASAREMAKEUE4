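; Money pickup actor that spins continuously around its yaw axis and disappears when the player touches it.
; Overlap on the Money component checks that the other actor's instigator is player controller 0 and casts it to player_pc before destroying the pickup.
; The construction script rolls a bounded random Value when Random is set, otherwise keeping the set one.
; The overlap logic does not pass Value to the player.
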(event `self.ReceiveTick`
  (params (DeltaSeconds :type "Float (single-precision)"))
  ;[0.1221 0.1559 0.3231] constant rotation
  (`SceneComponent.K2_AddLocalRotation` (`self.money`) (`KismetMathLibrary.MakeRotator` 0.0 0.0 (* DeltaSeconds 120.0)) false false))

(event `self.money.OnComponentBeginOverlap`
  (params (OverlappedComponent :type "PrimitiveComponent Object Reference") (OtherActor :type "Actor Object Reference") (OtherComp :type "PrimitiveComponent Object Reference") (OtherBodyIndex :type Integer) (bFromSweep :type Boolean) (SweepResult :type "HitResult Structure (by ref)"))
  (bind _returnvalue (`GameplayStatics.GetPlayerController` 0))
  ;[1 1 1] Overlap
  (if (== (`self.GetInstigatorController` OtherActor) _returnvalue)
    (cast `/Game/Player/blueprint/player_pc` _returnvalue)
    (`self.K2_DestroyActor`)))

(fn `UserConstructionScript`
  (bind _output_get (set `self.random?` (`self.random?`)))
  (if _output_get
    (set `self.value` (`KismetMathLibrary.RandomIntegerInRange` 0 200))
    (else
      (set `self.value` (`self.value`)))))