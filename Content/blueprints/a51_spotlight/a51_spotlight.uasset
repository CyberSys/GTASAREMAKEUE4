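; Area 51 searchlight actor that sweeps along a looping path and can be shot out.
; The construction script builds the target spline from a configurable start location, point count and relative point array, and records its length.
; Tick advances a distance by Speed, turning the housing toward that spline point with a yaw offset.
; An INSTANT_HITE hit on the bulb removes the light, swaps the bulb material and stops the sweep.
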(event `self.ReceiveTick`
  (params (DeltaSeconds :type "Float (single-precision)"))
  (bind (_returnvalue_roll _returnvalue_pitch _returnvalue_yaw) (`KismetMathLibrary.BreakRotator` (`KismetMathLibrary.FindLookAtRotation` (`SceneComponent.K2_GetComponentLocation` (`self.a51_spothousing`)) (`SplineComponent.GetLocationAtDistanceAlongSpline` (`self.Spline`) (`self.CurrentDistance`) "World"))))
  (if (not (`self.destroyed`))
    (`/Engine/EditorBlueprintResources/StandardMacros.CompareFloat` (`self.CurrentDistance`) (`self.TotalDistance`)
      (:`>`
        (set `self.CurrentDistance` 0.0 :!label _label))
      (:`==`
        (goto _label))
      (:`<`
        (`SceneComponent.K2_SetRelativeRotation` (`self.a51_spothousing`) (`KismetMathLibrary.MakeRotator` _returnvalue_roll _returnvalue_pitch (+ _returnvalue_yaw -90.0)) false false)
        (set `self.CurrentDistance` (+ (`self.CurrentDistance`) (* DeltaSeconds (`self.Speed`))))))))

(event `self.ReceiveHit`
  (params (MyComp :type "PrimitiveComponent Object Reference") (Other :type "Actor Object Reference") (OtherComp :type "PrimitiveComponent Object Reference") (bSelfMoved :type Boolean) (HitLocation :type "Vector Structure") (HitNormal :type "Vector Structure") (NormalImpulse :type "Vector Structure") (Hit :type "HitResult Structure (by ref)"))
  (if (and (== MyComp (`self.a51_spotbulb`)) (== (`GameplayStatics.GetObjectClass` Other) "/Game/Weapons/INSTANT_HITE.INSTANT_HITE_C"))
    (`ActorComponent.K2_DestroyComponent` (`self.SpotLight`))
    (`PrimitiveComponent.CreateDynamicMaterialInstance` (`self.a51_spotbulb`) 0 "/Game/Material/Misc/dts_spotlight.dts_spotlight" "None")
    (set `self.destroyed` true)))

(fn `UserConstructionScript`
  (bind _returnvalue (`KismetMathLibrary.Max` (`self.splinepoints`) 3))
  (`SceneComponent.K2_SetRelativeLocation` (`self.Spline`) (`self.StartLocation`) false true)
  (`KismetArrayLibrary.Array_Resize` (`self.SplinePointRelativeLocation`) (- _returnvalue 1))
  (for _index (range 2 _returnvalue)
    (`SplineComponent.AddSplinePointAtIndex` (`self.Spline`) (0.0 0.0 0.0) _index "Local" true))
  (for (_array_element _array_index) (`self.SplinePointRelativeLocation`)
    (`SplineComponent.SetLocationAtSplinePoint` (`self.Spline`) (+ _array_index 1) _array_element "Local" true)
    (set `self.TotalDistance` (`SplineComponent.GetSplineLength` (`self.Spline`)))))