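; Dam turbine objective where the player plants an explosive charge.
; A sphere overlap prompts the first player while unarmed, and interacting locks movement during a planting montage.
; The montage notify snaps the player's yaw around the turbine to one of eight segments, where SpawnLocation adds a rotated bomb mesh tagged "bomb".
; Montage completion restores movement, sets Armed and briefly confirms placement on screen.
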(event `/Game/Player/interfaces/interact_interface.OnInteractStart`
  (params (Player :type "/Game/Player/blueprint/player Object Reference"))
  (bind _returnvalue (`self.GetInstigatorController` Player))
  (bind (_returnvalue_roll _returnvalue_pitch _returnvalue_yaw) (`KismetMathLibrary.BreakRotator` (`KismetMathLibrary.FindLookAtRotation` (`self.K2_GetActorLocation`) (`self.K2_GetActorLocation` Player))))
  (bind _returnvalue_2 (* (/ 360.0 8.0) 5.0))
  (bind _returnvalue_3 (* (/ 360.0 8.0) 6.0))
  (bind _returnvalue_4 (* (/ 360.0 8.0) 7.0))
  (bind _returnvalue_5 (* (/ 360.0 8.0) 0.0))
  (bind _returnvalue_6 (* (/ 360.0 8.0) 1.0))
  (bind _returnvalue_7 (* (/ 360.0 8.0) 2.0))
  (bind _returnvalue_8 (* (/ 360.0 8.0) 3.0))
  (bind _returnvalue_9 (* (/ 360.0 8.0) 4.0))
  (bind _returnvalue_10 (+ _returnvalue_yaw 180.0))
  (if (not (`self.armed`))
    (message `/Game/Player/interfaces/interact_interface.OnMessageStop` (`self.GetInstigatorController` Player))
    (`/Game/Player/blueprint/player.StopAndDisableMovement` Player)
    (`|PlayMontage` (`Character.Mesh` Player) "/Game/Player/animations/bomber/mon_bom_plant.mon_bom_plant"
      (:`OnCompleted`
        (`/Game/Player/blueprint/player.StartAndEnableMovement` Player)
        (message `/Game/Player/interfaces/interact_interface.OnInteractStop` _returnvalue)
        (set `self.armed` true)
        (bind _message (`/Game/blueprints/GlobalFunctions.DisplayText` false "Charge placed."))
        (message `/Game/Player/interfaces/interact_interface.OnMessageStart` _returnvalue _message)
        (`KismetSystemLibrary.Delay` 2.0)
        (message `/Game/Player/interfaces/interact_interface.OnMessageStop` _returnvalue))
      (:`OnNotifyBegin`
        ;[1 1 1] Get segment from player position relative to the turbine
        (if (and (>= _returnvalue_10 _returnvalue_5) (< _returnvalue_10 _returnvalue_6))
          (`self.SpawnLocation` _returnvalue_5)
          (elif (and (>= _returnvalue_10 _returnvalue_6) (< _returnvalue_10 _returnvalue_7))
            (`self.SpawnLocation` _returnvalue_6)
            (elif (and (>= _returnvalue_10 _returnvalue_7) (< _returnvalue_10 _returnvalue_8))
              (`self.SpawnLocation` _returnvalue_7)
              (elif (and (>= _returnvalue_10 _returnvalue_8) (< _returnvalue_10 _returnvalue_9))
                (`self.SpawnLocation` _returnvalue_8)
                (elif (and (>= _returnvalue_10 _returnvalue_9) (< _returnvalue_10 _returnvalue_2))
                  (`self.SpawnLocation` _returnvalue_9)
                  (elif (and (>= _returnvalue_10 _returnvalue_2) (< _returnvalue_10 _returnvalue_3))
                    (`self.SpawnLocation` _returnvalue_2)
                    (elif (and (>= _returnvalue_10 _returnvalue_3) (< _returnvalue_10 _returnvalue_4))
                      (`self.SpawnLocation` _returnvalue_3)
                      (elif (and (>= _returnvalue_10 _returnvalue_4) (< _returnvalue_10 (* (/ 360.0 8.0) 8.0)))
                        (`self.SpawnLocation` _returnvalue_4)))))))))))))

(event `self.Sphere.OnComponentBeginOverlap`
  (params (OverlappedComponent :type "PrimitiveComponent Object Reference") (OtherActor :type "Actor Object Reference") (OtherComp :type "PrimitiveComponent Object Reference") (OtherBodyIndex :type Integer) (bFromSweep :type Boolean) (SweepResult :type "HitResult Structure (by ref)"))
  (bind _returnvalue (`self.GetInstigatorController` OtherActor))
  (if (and (== _returnvalue (`GameplayStatics.GetPlayerController` 0)) (not (`self.armed`)))
    (bind _message (`/Game/blueprints/GlobalFunctions.DisplayText` true "plant charge."))
    (message `/Game/Player/interfaces/interact_interface.OnMessageStart` _returnvalue _message)
    (`GameplayStatics.PlaySound2D` "/Game/Sounds/bank_53/sound_015.sound_015" 1.0 1.0 0.0 null null)))

(event `self.Sphere.OnComponentEndOverlap`
  (params (OverlappedComponent :type "PrimitiveComponent Object Reference") (OtherActor :type "Actor Object Reference") (OtherComp :type "PrimitiveComponent Object Reference") (OtherBodyIndex :type Integer))
  (bind _returnvalue (`self.GetInstigatorController` OtherActor))
  (if (and (== _returnvalue (`GameplayStatics.GetPlayerController` 0)) (not (`self.armed`)))
    (message `/Game/Player/interfaces/interact_interface.OnMessageStop` _returnvalue)))

(fn `UserConstructionScript`)