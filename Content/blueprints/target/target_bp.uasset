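; Shooting target Blueprint that rotates on a timeline with audio as actors enter or leave its capsule.
; Projectile hits arrive through PassInstigator, award points by the body part's numeric component tag via Target_interface, then play a sound and destroy that part.
; Losing all parts or ending overlap reverses the rotation, after which the target respawns itself as a fresh actor.
; The construction script tints the mesh red through a dynamic material.
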(event `self.ReceiveBeginPlay`
  ;[1 1 1] Set beginning rotation
  (`SceneComponent.K2_SetRelativeRotation` (`self.target_frame`) (struct :`Roll` 90.0) false false))

(event `/Game/blueprints/target/target_interface.PassInstigator`
  (params (Instigator :type "Pawn Object Reference") (Component :type "PrimitiveComponent Object Reference"))
  ;[1 1 1] When COmponent gets hit do something...
  (if (`KismetSystemLibrary.DoesImplementInterface` Instigator "/Game/blueprints/target/target_interface.target_interface_C")
    (message `/Game/blueprints/target/target_interface.AddPoints` Instigator (select `int` (`KismetStringLibrary.Conv_StringToInt` (`KismetStringLibrary.Conv_NameToString` (`|GetArrayItem` (`ActorComponent.ComponentTags` Component)))) :`0` 10 :`1` 10 :`2` 15 :`3` 10 :`4` 10 :`5` 15 :`6` 30))
    (if (!= Component (`self.target_frame`))
      (`GameplayStatics.SpawnSoundAtLocation` "/Game/Sounds/script/bank_164/sound_003_Cue.sound_003_Cue" (`SceneComponent.K2_GetComponentLocation` Component) (struct) 1.0 1.0 0.0 "/Game/Sounds/bank_033/sound_hit.sound_hit" null)
      (`ActorComponent.K2_DestroyComponent` Component)
      (if (== (`SceneComponent.GetNumChildrenComponents` (`self.target_frame`)) 0)
        (`TimelineComponent.ReverseFromEnd` (`self.Rotate`))))))

(event `self.Capsule.OnComponentBeginOverlap`
  (params (OverlappedComponent :type "PrimitiveComponent Object Reference") (OtherActor :type "Actor Object Reference") (OtherComp :type "PrimitiveComponent Object Reference") (OtherBodyIndex :type Integer) (bFromSweep :type Boolean) (SweepResult :type "HitResult Structure (by ref)"))
  ;[1 1 1] enter exit player
  (`TimelineComponent.PlayFromStart` (`self.Rotate`)))

(event `self.Capsule.OnComponentEndOverlap`
  (params (OverlappedComponent :type "PrimitiveComponent Object Reference") (OtherActor :type "Actor Object Reference") (OtherComp :type "PrimitiveComponent Object Reference") (OtherBodyIndex :type Integer))
  ;[1 1 1] enter exit player
  (`TimelineComponent.ReverseFromEnd` (`self.Rotate`)))

(fn `Respawn`
  (`|SpawnActorFromClass` "target_bp_C" (`self.GetTransform`) "Undefined" "OverrideRootScale" null null)
  (`self.K2_DestroyActor`))

(fn `UserConstructionScript`
  (bind _returnvalue (`PrimitiveComponent.CreateDynamicMaterialInstance` (`self.StaticMesh`) 0 "/Game/Material/ingame/diamond.diamond" "None"))
  (`MaterialInstanceDynamic.SetVectorParameterValue` _returnvalue "color" (struct :`R` 1.0 :`A` 1.0)))