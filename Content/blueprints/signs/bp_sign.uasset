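; Sign actor that builds its text at construction and toggles its lights with the time of day.
; The construction script spawns a text render component per Sign entry, applying position, yaw, scale and a Color data table lookup.
; CreateString joins multi-line entries with "<br>".
; If lights exist, BeginPlay binds to the TimeCycle actor's night event, which shows them only during night hours.
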(event `self.ReceiveBeginPlay`
  ;[1 1 1] 1. check wether sign has light / 2. bind to timecycle and hide light depending on time
  (if (`KismetArrayLibrary.Array_IsValidIndex` (`self.K2_GetComponentsByClass` "/Script/Engine.LightComponent"))
    (bind _outactors (`GameplayStatics.GetAllActorsOfClass` "/Game/timecycle/TimeCycle.TimeCycle_C"))
    (if (`KismetArrayLibrary.Array_IsValidIndex` _outactors)
      (bind _astime_cycle (cast `/Game/timecycle/TimeCycle` (`|GetArrayItem` _outactors)))
      (add `/Game/timecycle/TimeCycle.night` _astime_cycle (delegate `night`)))))

(event `night`
  ;[1 1 1] 1. check wether sign has light / 2. bind to timecycle and hide light depending on time
  (for _array_element (`self.K2_GetComponentsByClass` "/Script/Engine.LightComponent")
    (`SceneComponent.SetHiddenInGame` _array_element (not (`/Game/timecycle/TimeCycle.GetIsTimeInRange` (stale `self.ReceiveBeginPlay` _astime_cycle) 21 7)) false)))

(fn `CreateString`
  (params (ID :type Integer))
  (returns (Text :type Text))
  (locals (String :type String))
  (bind ((`text_23_F507320E4B92D43DD649E791E26A7723` _text)) (break `/Game/blueprints/signs/bp_sign_struct` (`|GetArrayItem` (`self.sign`) ID)))
  (if (`KismetArrayLibrary.Array_IsValidIndex` _text 1)
    (set `local.String` (`KismetStringLibrary.Conv_NameToString` (`|GetArrayItem` _text)))
    (for _index (range 1 (+ (`KismetArrayLibrary.Array_LastIndex` _text) 1))
      (set `local.String` (`KismetStringLibrary.Concat_StrStr` (`local.String`) "<br>" (`KismetStringLibrary.Conv_NameToString` (`|GetArrayItem` _text _index)))))
    (return (`KismetTextLibrary.Conv_StringToText` (`local.String`)))))

(fn `UserConstructionScript`
  (if (`KismetArrayLibrary.Array_IsValidIndex` (`self.sign`))
    ;[0.1302 0.03963 1] assign text properties
    (for (_array_element _array_index) (`self.sign`)
      (bind _returnvalue (`AddComponent|NODE_AddTextRenderComponent-1` :`RelativeTransform` (`KismetMathLibrary.MakeTransform` (break `/Game/blueprints/signs/bp_sign_struct` _array_element) (`KismetMathLibrary.MakeRotator` 0.0 0.0 (`.rotation_21_DE7954374A93373521D4EC9E790727D0` (break `/Game/blueprints/signs/bp_sign_struct` _array_element))) (1.0 1.0 1.0))))
      (`TextRenderComponent.SetYScale` _returnvalue (`.Y` (`KismetMathLibrary.BreakVector2D` (`.size_11_3094C250443A8C687721B58B23461963` (break `/Game/blueprints/signs/bp_sign_struct` _array_element)))))
      (`TextRenderComponent.SetXScale` _returnvalue (`KismetMathLibrary.BreakVector2D` (`.size_11_3094C250443A8C687721B58B23461963` (break `/Game/blueprints/signs/bp_sign_struct` _array_element))))
      (`TextRenderComponent.K2_SetText` _returnvalue (`self.CreateString` _array_index))
      (bind _returnvalue_2 (`|GetDataTableRow` (`self.color`) (select `/Game/blueprints/signs/bp_sign_color` (`.color_17_82413040403793D92BCE71B0A18C3FE7` (break `/Game/blueprints/signs/bp_sign_struct` _array_element)) :`NewEnumerator4` "light_grey" :`NewEnumerator5` "mid_grey" :`NewEnumerator6` "dark_grey" :`NewEnumerator7` "light_red" :!type "Name"))
        (:`then`
          (`TextRenderComponent.SetTextRenderColor` _returnvalue (`.color_2_54BF787D47A6C82A1D40D288AA7675D3` (break `/Game/NEW/ui/colors/colors` _returnvalue_2))))))))