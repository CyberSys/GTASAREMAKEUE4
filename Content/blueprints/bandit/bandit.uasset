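; Slot machine (one-armed bandit) Blueprint with three reels, each given a random target among 20 positions at BeginPlay.
; StartGamble opens a gate in the Gamble graph, whose spin logic rotates active reels and stops them sequentially at staggered turn counts plus target offsets, with sounds.
; Tick separately interpolates reel roll toward the targets, sharing one Rotated variable with the spin logic.
; Gamble's Enter input has no caller here.
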(event `self.ReceiveBeginPlay`
  (for _index (range 3)
    (`KismetArrayLibrary.Array_Set` (`self.targetslot`) _index (`KismetMathLibrary.RandomIntegerInRange` 1 20))))

(event `StartGamble`
  (`self.Gamble` 0.0 :!via `Open`))

(event `self.ReceiveTick`
  (params (DeltaSeconds :type "Float (single-precision)"))
  (for _index (range 3)
    (bind _output_get (set `self.rotated` (`KismetMathLibrary.FInterpTo` (`self.rotated`) (* (`|GetArrayItem` (`self.targetslot`) _index) 18.0) DeltaSeconds 1.0)))
    (`SceneComponent.K2_SetRelativeRotation` (select `int` _index :`0` (`self.reel01`) :`1` (`self.reel02`) :`2` (`self.reel03`) :!type "SceneComponent Object Reference") (`KismetMathLibrary.MakeRotator` _output_get) false false)))

(fn `UserConstructionScript`)