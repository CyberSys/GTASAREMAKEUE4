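; Collectible pickup actor whose type (tag, oyster, horseshoe, camera or two killfrenzy variants) selects its mesh and collision in the construction script.
; Oysters, horseshoes and cameras spin; overlap by a collectible-interface actor sends it type and ID, plays a sound and destroys the pickup.
; Tags use their own trace channel and a dynamic material that AddTag intensifies stepwise until TagGrove is set.
; The already-collected self-destroy check is unwired.
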(event `self.ReceiveBeginPlay`
  (bind _tag_life (`self.Tag_Life`))
  (switch `/Game/blueprints/collectible/cj_collectible_enum` (`self.Collectible`)
    (:`NewEnumerator0`
      ;[1 1 1] Set Tag State
      (`MaterialInstanceDynamic.SetScalarParameterValue` (`self.Tag_mat`) "intensity" (* _tag_life 10.0))
      (set `self.Tag_Grove?` (>= _tag_life 1.0)))))

(event `self.ReceiveTick`
  (params (DeltaSeconds :type "Float (single-precision)"))
  ;[1 1 1] constant rotation
  (switch `/Game/blueprints/collectible/cj_collectible_enum` (`self.Collectible`)
    (:`NewEnumerator1`
      _)
    (:`NewEnumerator2`
      _)
    (:`NewEnumerator3`
      _))
  (`SceneComponent.K2_AddLocalRotation` (`self.StaticMesh`) (`KismetMathLibrary.MakeRotator` 0.0 0.0 (* DeltaSeconds 120.0)) false false))

(event `self.StaticMesh.OnComponentBeginOverlap`
  (params (OverlappedComponent :type "PrimitiveComponent Object Reference") (OtherActor :type "Actor Object Reference") (OtherComp :type "PrimitiveComponent Object Reference") (OtherBodyIndex :type Integer) (bFromSweep :type Boolean) (SweepResult :type "HitResult Structure (by ref)"))
  ;[1 1 1] When player collects item
  (if (`KismetSystemLibrary.DoesImplementInterface` OtherActor "/Game/blueprints/collectible/cj_collectible_interface.cj_collectible_interface_C")
    (message `/Game/blueprints/collectible/cj_collectible_interface.OnCollect` OtherActor (`self.Collectible`) (`self.ID`))
    (`GameplayStatics.PlaySound2D` "/Game/Sounds/bank_53/sound_019.sound_019" 1.0 1.0 0.0 null null)
    (`self.K2_DestroyActor`)))

(event `/Game/blueprints/collectible/cj_collectible_interface.AddTag`
  (bind _returnvalue (+ (`self.Tag_Life`) 0.05))
  (if (not (`self.Tag_Grove?`))
    (bind _output_get (set `self.Tag_Life` _returnvalue))
    (`MaterialInstanceDynamic.SetScalarParameterValue` (`self.Tag_mat`) "intensity" (* _output_get 2.0))
    (if (>= _returnvalue 1.0)
      (set `self.Tag_Grove?` true)
      (`GameplayStatics.PlaySound2D` "/Game/Sounds/bank_53/sound_019.sound_019" 1.0 1.0 0.0 null null)
      (else
        (set `self.Tag_Grove?` false)))))

(fn `UserConstructionScript`
  (bind _staticmesh (`self.StaticMesh`))
  (`StaticMeshComponent.SetStaticMesh` (`self.StaticMesh`) (select `/Game/blueprints/collectible/cj_collectible_enum` (`self.Collectible`) :`NewEnumerator0` "/Game/Models/generic/dynamic2/tag_01.tag_01" :`NewEnumerator1` "/Game/Models/interior/propext/CJ_OYSTER.CJ_OYSTER" :`NewEnumerator2` "/Game/Models/interior/propext/cj_horse_Shoe.cj_horse_Shoe" :`NewEnumerator3` "/Game/Models/generic/dynamic/camerapickup.camerapickup" :`NewEnumerator4` "/Game/Models/generic/dynamic/killfrenzy.killfrenzy" :`NewEnumerator5` "/Game/Models/generic/dynamic/killfrenzy2plyr.killfrenzy2plyr" :!type "StaticMesh Object Reference"))
  (switch `/Game/blueprints/collectible/cj_collectible_enum` (`self.Collectible`)
    (:`NewEnumerator0`
      (`PrimitiveComponent.SetCollisionObjectType` _staticmesh "ECC_GameTraceChannel10")
      (bind _returnvalue (`PrimitiveComponent.CreateDynamicMaterialInstance` (`self.StaticMesh`) 1 "/Game/Material/ingame/tag_mat.tag_mat" "None"))
      (set `self.Tag_mat` _returnvalue))
    (:`NewEnumerator1`
      (`PrimitiveComponent.SetCollisionObjectType` _staticmesh "ECC_WorldStatic" :!label _label))
    (:`NewEnumerator2`
      (goto _label))
    (:`NewEnumerator3`
      (goto _label))
    (:`NewEnumerator4`
      (goto _label))
    (:`NewEnumerator5`
      (goto _label))))