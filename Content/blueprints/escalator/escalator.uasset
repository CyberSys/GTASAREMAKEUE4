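; Escalator Blueprint that builds one or more flights of steps and animates them moving along spline paths.
; The construction script creates an HISM and a linear four-point spline per flight, with alternating X offsets and a lowered return run, then spaces step instances along it.
; Tick repositions every instance by a shared wrapping distance, which advances per instance, so speed scales with step count; path length comes from the last spline built.
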(event `self.ReceiveTick`
  (params (DeltaSeconds :type "Float (single-precision)"))
  (bind _hism_components (`self.HISM-Components`))
  (`/Engine/EditorBlueprintResources/StandardMacros.CompareFloat` (`self.CurrentDistance`) (`self.TotalDistance`)
    (:`>`
      (set `self.CurrentDistance` 0.0 :!label _label))
    (:`==`
      (goto _label))
    (:`<`
      (for (_ _array_index) _hism_components
        (bind _output (`|GetArrayItem` _hism_components _array_index))
        (for _index (range (`InstancedStaticMeshComponent.GetInstanceCount` _output))
          (`InstancedStaticMeshComponent.UpdateInstanceTransform` _output _index (`KismetMathLibrary.MakeTransform` (`SplineComponent.GetLocationAtDistanceAlongSpline` (`|GetArrayItem` (`self.Splines`) _array_index) (mod (+ (* _index (`self.SingleDistance`)) (`self.CurrentDistance`)) (`self.TotalDistance`)) "World")) true false false)
          (set `self.CurrentDistance` (+ (`self.CurrentDistance`) (* DeltaSeconds 1.0))))))))

(fn `esc`
  (params (ID :type Integer))
  (bind _steps (`self.steps`))
  (bind _offset (`self.Offset`))
  (bind (_output_x _output_y _output_z) (`KismetMathLibrary.BreakVector` (`|GetArrayItem` (`self.StartLocation`) ID)))
  (bind _returnvalue (`AddComponent|NODE_AddHierarchicalInstancedStaticMeshComponent-0`))
  (`KismetArrayLibrary.Array_Set` (`self.HISM-Components`) ID _returnvalue)
  (bind _returnvalue_2 (`AddComponent|NODE_AddSplineComponent-0` :`RelativeTransform` (`KismetMathLibrary.MakeTransform` (`KismetMathLibrary.MakeVector` (+ _output_x (select `int` (mod ID 2) :`0` _offset :`1` (* _offset -1.0))) _output_y _output_z) (struct :`Yaw` 90.0)))) ; Start location
  (`KismetArrayLibrary.Array_Set` (`self.Splines`) ID _returnvalue_2)
  (`SplineComponent.SetLocationAtSplinePoint` _returnvalue_2 1 (`|GetArrayItem` (`self.EndLocation`) ID) "Local" true) ; End location
  (bind (_returnvalue_x _returnvalue_y _returnvalue_z) (`KismetMathLibrary.BreakVector` (`SplineComponent.GetLocationAtSplinePoint` _returnvalue_2 1 "World")))
  (`SplineComponent.AddSplinePointAtIndex` _returnvalue_2 (`KismetMathLibrary.MakeVector` _returnvalue_x _returnvalue_y (- _returnvalue_z 50.0)) 2 "World" true)
  (bind (_returnvalue_x_2 _returnvalue_y_2 _returnvalue_z_2) (`KismetMathLibrary.BreakVector` (`SplineComponent.GetLocationAtSplinePoint` _returnvalue_2 0 "World")))
  (`SplineComponent.AddSplinePointAtIndex` _returnvalue_2 (`KismetMathLibrary.MakeVector` _returnvalue_x_2 _returnvalue_y_2 (- _returnvalue_z_2 50.0)) 3 "World" true)
  (for _index (range (`SplineComponent.GetNumberOfSplinePoints` _returnvalue_2))
    (`SplineComponent.SetSplinePointType` _returnvalue_2 _index "Linear" true))
  (bind _returnvalue_3 (`SplineComponent.GetSplineLength` _returnvalue_2))
  (set `self.TotalDistance` _returnvalue_3)
  (bind _returnvalue_4 (/ _returnvalue_3 (`KismetMathLibrary.Conv_IntToDouble` _steps)))
  (set `self.SingleDistance` _returnvalue_4)
  (for _index_2 (range _steps)
    (`InstancedStaticMeshComponent.AddInstanceWorldSpace` _returnvalue (`KismetMathLibrary.MakeTransform` (`SplineComponent.GetLocationAtDistanceAlongSpline` _returnvalue_2 (* _index_2 _returnvalue_4) "World") (struct) (1.0 1.0 1.0)))))

(fn `UserConstructionScript`
  (bind _returnvalue (`KismetMathLibrary.Max` (`self.stairs`) 1))
  (`KismetArrayLibrary.Array_Resize` (`self.HISM-Components`) _returnvalue)
  (`KismetArrayLibrary.Array_Resize` (`self.Splines`) _returnvalue)
  (`KismetArrayLibrary.Array_Resize` (`self.StartLocation`) _returnvalue)
  (`KismetArrayLibrary.Array_Resize` (`self.EndLocation`) _returnvalue)
  (for _index (range _returnvalue)
    (`self.esc` _index)))