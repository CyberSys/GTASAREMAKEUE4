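; Sky sphere Blueprint that drives a panning-cloud sky material from the scene's sun and moon lights.
; The construction script creates the dynamic material instance on the sphere mesh.
; UpdateSunDirection pushes both light directions, sky colors, gradient blends and HDR values into it.
; Sun pitch is remapped to a height that varies horizon falloff and blends in stars when negative; Tick and BeginPlay are empty.
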(event `self.ReceiveTick`
  (params (DeltaSeconds :type "Float (single-precision)")))

(event `self.ReceiveBeginPlay`)

(fn `UpdateSunDirection`
  (bind _sky_material (`self.Sky material`))
  (bind _sky_material_2 (`self.Sky material`))
  (bind _sun_height (`self.Sun height`))
  ;[1 1 1] sun/moon position
  (`MaterialInstanceDynamic.SetVectorParameterValue` (`self.Sky material`) "MoonDirection" (`KismetMathLibrary.Conv_VectorToLinearColor` (`KismetMathLibrary.Conv_RotatorToVector` (`self.K2_GetActorRotation` (`self.MoonLight`)))))
  (`MaterialInstanceDynamic.SetVectorParameterValue` (`self.Sky material`) "Light direction" (`KismetMathLibrary.Conv_VectorToLinearColor` (`KismetMathLibrary.Conv_RotatorToVector` (`self.K2_GetActorRotation` (`self.sun`)))))
  ;[1 1 1] sun height
  (set `self.Sun height` (`KismetMathLibrary.MapRangeUnclamped` (.pitch (`self.K2_GetActorRotation` (`self.sun`))) 0.0 -18.0 0.0 1.0))
  ;[1 1 1] colors
  (`MaterialInstanceDynamic.SetVectorParameterValue` _sky_material "sky_sun_disc_col" (`self.sky_sun_disc_col`))
  (`MaterialInstanceDynamic.SetVectorParameterValue` _sky_material "sky_zenith_transition_col" (`self.sky_zenith_transition_col`))
  (`MaterialInstanceDynamic.SetVectorParameterValue` _sky_material "sky_zenith_col" (`self.sky_zenith_col`))
  (`MaterialInstanceDynamic.SetVectorParameterValue` _sky_material "sky_cloud_base_col" (`self.sky_cloud_base_col`))
  (`MaterialInstanceDynamic.SetVectorParameterValue` _sky_material "sky_azimuth_east_col" (`self.sky_azimuth_east_col`))
  (`MaterialInstanceDynamic.SetVectorParameterValue` _sky_material "sky_azimuth_west_col" (`self.sky_azimuth_west_col`))
  (`MaterialInstanceDynamic.SetVectorParameterValue` _sky_material "sky_azimuth_transition_col" (`self.sky_azimuth_transition_col`))
  (`MaterialInstanceDynamic.SetScalarParameterValue` _sky_material_2 "sky_zenith_transition_west_blend" (`self.sky_zenith_transition_west_blend`))
  (`MaterialInstanceDynamic.SetScalarParameterValue` _sky_material_2 "sky_zenith_transition_east_blend" (`self.sky_zenith_transition_east_blend`))
  (`MaterialInstanceDynamic.SetScalarParameterValue` _sky_material_2 "sky_azimuth_transition_position" (`self.sky_azimuth_transition_position`))
  (`MaterialInstanceDynamic.SetScalarParameterValue` _sky_material_2 "sky_zenith_transition_position" (`self.sky_zenith_transition_position`))
  (`MaterialInstanceDynamic.SetScalarParameterValue` _sky_material_2 "sky_hdr" (`self.sky_hdr`))
  (`MaterialInstanceDynamic.SetScalarParameterValue` _sky_material_2 "sky_sun_hdr" (`self.sky_sun_hdr`))
  ;[1 1 1] floats
  (`MaterialInstanceDynamic.SetScalarParameterValue` _sky_material "Horizon falloff" (`KismetMathLibrary.Lerp` 3.0 8.0 (`KismetMathLibrary.Abs` (`self.Sun height`))))
  (`MaterialInstanceDynamic.SetScalarParameterValue` _sky_material "Sun height" (`KismetMathLibrary.SelectFloat` (`KismetMathLibrary.Abs` _sun_height) 0.0 (< _sun_height 0.0))))

(fn `UserConstructionScript`
  (bind _returnvalue (`PrimitiveComponent.CreateDynamicMaterialInstance` (`self.Sky Sphere mesh`) 0 "/Game/Weather/Sky/M_Sky_Panning_Clouds2_Inst.M_Sky_Panning_Clouds2_Inst" "None"))
  (set `self.Sky material` _returnvalue))