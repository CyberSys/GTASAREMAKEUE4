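; Weather manager Blueprint that runs a day/night cycle on a configurable day length, though it holds no weather logic yet.
; Seeds elapsed time from a start time, then advances it each Tick and derives the current day, hour and minute.
; A vector curve sampled by elapsed game hours sets sun pitch and refreshes the sky.
; Sun intensity ramps over one game hour, rising or falling according to the sunrise and sunset hours.
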(event `self.ReceiveBeginPlay`
  (`|ExecutionSequence`
    (:`then_0`
      (`self.SetElapsedTimeBasedOnStart`))))

(event `self.ReceiveTick`
  (params (DeltaSeconds :type "Float (single-precision)"))
  (`|ExecutionSequence`
    (:`then_0`
      (`self.UpdateElapsedTime`))
    (:`then_1`
      (`self.UpdateSunPosition`))
    (:`then_2`
      (`self.UpdateCurrentTime`))
    (:`then_3`
      (`self.FadeSun`))))

(fn `DetermineCurrentTime`
  (returns (time :type "/Game/Weather/WeatherManager/struct_time Structure"))
  (bind _returnvalue (`self.GetFractionOfDay`))
  (return (make `/Game/Weather/WeatherManager/struct_time` (`KismetMathLibrary.FTrunc` _returnvalue) (`KismetMathLibrary.FTrunc` (* (mod _returnvalue 1.0) 24.0)) (`KismetMathLibrary.FTrunc` (mod (* _returnvalue 1440.0) 60.0)))))

(fn `DetermineifNight`
  (returns (ReturnValue :type Boolean))
  (bind (_currenttime_days _currenttime_hours) (break `/Game/Weather/WeatherManager/struct_time` (`self.CurrentTime`)))
  (return (or (< _currenttime_hours (`self.SunUpTime`)) (>= _currenttime_hours (`self.SunDownTime`)))))

(fn `FadeSun`
  (bind _lightcomponent (`Light.LightComponent` (`self.Sun`)))
  (`LightComponent.SetIntensity` _lightcomponent (`KismetMathLibrary.FClamp` (+ (`LightComponentBase.Intensity` _lightcomponent) (* (`GameplayStatics.GetWorldDeltaSeconds`) (/ 24.0 (`self.SecondsPerDay`)) (`self.SunIntensity`) (select `bool` (`self.DetermineifNight`) :`false` 1.0 :`true` -1.0 :!type "Float (single-precision)"))) 0.0 (`self.SunIntensity`))))

(fn `GetFractionOfDay`
  (returns (ReturnValue :type "Float (double-precision)"))
  (return (/ (`self.ElapsedTime`) (`self.SecondsPerDay`))))

(fn `GetTimeAsSeconds`
  (params (struct_time :type "/Game/Weather/WeatherManager/struct_time Structure (by ref)"))
  (returns (ReturnValue :type Integer))
  (bind (_days _hours _minutes) (break `/Game/Weather/WeatherManager/struct_time` struct_time))
  (return (+ (* _days 86400) (* _hours 3600) (* _minutes 60))))

(fn `SetElapsedTimeBasedOnStart`
  (set `self.ElapsedTime` (* (`self.GetTimeAsSeconds` (`self.StartTime`)) (/ (`self.SecondsPerDay`) 86400.0))))

(fn `UpdateCurrentTime`
  (set `self.CurrentTime` (`self.DetermineCurrentTime`)))

(fn `UpdateElapsedTime`
  (set `self.ElapsedTime` (+ (`self.ElapsedTime`) (`GameplayStatics.GetWorldDeltaSeconds`))))

(fn `UpdateSunPosition`
  (bind (_returnvalue_x _returnvalue_y) (`KismetMathLibrary.BreakVector` (`CurveVector.GetVectorValue` (`self.SunPosition`) (* (`self.GetFractionOfDay`) 24.0))))
  (`SceneComponent.K2_SetRelativeRotation` (`Light.LightComponent` (`self.Sun`)) (`KismetMathLibrary.MakeRotator` 0.0 _returnvalue_y) false false)
  (`/Engine/EngineSky/BP_Sky_Sphere.UpdateSunDirection` (`self.Sky`)))

(fn `UserConstructionScript`
  (set `self.SecondsPerDay` (* (`self.MinutesPerDay`) 60.0)))