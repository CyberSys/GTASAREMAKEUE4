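; Player camera Blueprint that toggles underwater visuals when its Box component begins overlapping a bp_water actor.
; Each begin overlap flips an Underwater flag, passes it to the water actor's SwitchLighting, and enables or disables that actor's PostProcess to match.
; The state alternates on successive begin overlaps, with no end-overlap handling.
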(event `self.ReceiveBeginPlay`)

(event `self.Box.OnComponentBeginOverlap`
  (params (OverlappedComponent :type "PrimitiveComponent Object Reference") (OtherActor :type "Actor Object Reference") (OtherComp :type "PrimitiveComponent Object Reference") (OtherBodyIndex :type Integer) (bFromSweep :type Boolean) (SweepResult :type "HitResult Structure (by ref)"))
  (bind _asbp_water (cast `/Game/data/water/bp_water` OtherActor))
  (if (not (`self.underwater`))
    (bind _output_get (set `self.underwater` true))
    (`/Game/data/water/bp_water.SwitchLighting` _asbp_water _output_get)
    (bind _postprocess (`/Game/data/water/bp_water.PostProcess` _asbp_water))
    (set `PostProcessComponent.bEnabled` true _postprocess)
    (else
      (bind _output_get_2 (set `self.underwater` false))
      (`/Game/data/water/bp_water.SwitchLighting` _asbp_water _output_get_2)
      (set `PostProcessComponent.bEnabled` false _postprocess))))

(fn `UserConstructionScript`)