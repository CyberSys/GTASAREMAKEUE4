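; Spectator pawn that gives the player a free-flying camera.
; On begin play it blends the view to its child-actor bp_camera and enables pawn control rotation on that camera.
; Each tick it moves along the actor's pitch-and-yaw axes from move variables, turns the actor from look variables with clamped pitch, and raises the floating movement's max speed while Boost is set.
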(event `self.ReceiveBeginPlay`
  ;[1 1 1] begin play
  (`PlayerController.SetViewTargetWithBlend` (`GameplayStatics.GetPlayerController` 0) (`ChildActorComponent.ChildActor` (`self.bp_camera`)) 0.0 "VTBlend_Linear" 0.0 false)
  (bind _asbp_camera (cast `/Game/Player/blueprint/bp_camera` (`ChildActorComponent.ChildActor` (`self.bp_camera`))))
  (set `CameraComponent.bUsePawnControlRotation` true (`/Game/Player/blueprint/bp_camera.Camera` _asbp_camera)))

(event `self.ReceiveTick`
  (params (DeltaSeconds :type "Float (single-precision)"))
  (bind (_returnvalue_roll _returnvalue_pitch _returnvalue_yaw) (`KismetMathLibrary.BreakRotator` (`self.K2_GetActorRotation`)))
  (bind (_returnvalue_roll_2 _returnvalue_pitch_2 _returnvalue_yaw_2) (`KismetMathLibrary.BreakRotator` (`self.K2_GetActorRotation`)))
  (bind _returnvalue (`KismetMathLibrary.MakeRotator` 0.0 _returnvalue_pitch_2 _returnvalue_yaw_2))
  ;[1 1 1] movement
  (`self.AddMovementInput` (`KismetMathLibrary.GetForwardVector` _returnvalue) (`self.MoveForward`))
  (`self.AddMovementInput` (`KismetMathLibrary.GetRightVector` _returnvalue) (`self.MoveRight`))
  (`self.K2_SetActorRelativeRotation` (`KismetMathLibrary.MakeRotator` 0.0 (`KismetMathLibrary.FClamp` (+ (`self.LookUp`) _returnvalue_pitch) -85.0 85.0) _returnvalue_yaw))
  (`self.K2_AddActorWorldRotation` (`KismetMathLibrary.MakeRotator` 0.0 0.0 (`self.LookRight`)))
  (set `FloatingPawnMovement.MaxSpeed` (* 3142.0 (select `bool` (`self.Boost`) :`false` 1.0 :`true` 6.0 :!type "Float (single-precision)")) (`self.FloatingPawnMovement`)))

(fn `UserConstructionScript`)