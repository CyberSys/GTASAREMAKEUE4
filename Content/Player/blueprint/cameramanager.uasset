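; Player camera manager that drives auto-focus depth of field on the bp_camera view target.
; BlueprintUpdateCamera caches that target's camera component and returns false for it, leaving the view to default handling.
; A looping timer line-traces along the camera's forward vector and uses the hit distance, or a far fallback, as focal distance.
; Each tick of that timer rebuilds the camera's post-process settings with Gaussian DOF.
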(event `self.ReceiveBeginPlay`
  ;[1 1 1] Auto Focus Depth Of Field
  (`KismetSystemLibrary.K2_SetTimer` null "UpdateDOF" 0.1 true))

(event `UpdateDOF`
  (bind _focuslocation (`self.FocusLocation`))
  (bind _cam (`self.cam`))
  (bind _returnvalue (`SceneComponent.K2_GetComponentLocation` _cam))
  ;[1 1 1] Auto Focus Depth Of Field
  (bind (_outhit _returnvalue_2) (`KismetSystemLibrary.LineTraceSingle` :`Start` _returnvalue :`End` (+ (* (`SceneComponent.GetForwardVector` _cam) 10000.0) _returnvalue) :`TraceChannel` "TraceTypeQuery1" :`bTraceComplex` true :`DrawTime` 1.0))
  (if _returnvalue_2
    (set `self.FocusLocation` (`KismetMathLibrary.VSize` (- (`.Location` (`GameplayStatics.BreakHitResult` _outhit)) _returnvalue)))
    (else
      (set `self.FocusLocation` 100000.0)))
  (set `CameraComponent.PostProcessSettings` (make `PostProcessSettings` :`AutoExposureMethod` "AEM_Basic" :`DepthOfFieldMethod` "DOFM_Gaussian" :`AutoExposureMinBrightness` -3.0 :`AutoExposureMaxBrightness` 5.0 :`DepthOfFieldFocalDistance` _focuslocation :`DepthOfFieldFocalRegion` 70000.0 :`DepthOfFieldNearTransitionRegion` _focuslocation :`DepthOfFieldFarTransitionRegion` 10000.0 :`DepthOfFieldNearBlurSize` 0.005 :`DepthOfFieldFarBlurSize` 0.1 :`DepthOfFieldOcclusion` 0.18 :`DepthOfFieldSkyFocusDistance` 200000.0) (`self.cam`)))

(fn `BlueprintUpdateCamera`
  (params (CameraTarget :type "Actor Object Reference"))
  (returns (NewCameraLocation :type "Vector Structure") (NewCameraRotation :type "Rotator Structure") (NewCameraFOV :type "Float (double-precision)") (ReturnValue :type Boolean))
  (bind _asbp_camera (cast `/Game/Player/blueprint/bp_camera` CameraTarget)
    (:`then`
      (set `self.cam` (`/Game/Player/blueprint/bp_camera.Camera` _asbp_camera))
      (return (0.0 0.0 0.0) (struct) 0.0 false))
    (:`CastFailed`
      (`KismetSystemLibrary.PrintString` "Cameramanager - No Camera bp_camera Found" true true (struct :`R` 1.0 :`A` 1.0) 0.0))))

(fn `UserConstructionScript`)