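; Player controller function library meant to load, save and delete player stats in a save slot, though all three function entries are unwired, so none of the logic runs.
; The disconnected load and save graphs copy the Savegame struct between controller and save_player_stats object.
; When no save exists, the save graph creates one, seeding the clothes map from Shopping table row names.
; Save and delete graphs print their results.
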(fn `DeletGame`
  (locals (SlotName :type String :default "Default")))

(fn `LoadGame`
  (params (PlayerController :type "/Game/Player/blueprint/player_pc Object Reference"))
  (returns (Exists :type Boolean))
  (locals (SlotName :type String :default "Default")))

(fn `SaveGame`
  (params (PlayerController :type "/Game/Player/blueprint/player_pc Object Reference"))
  (locals (SlotName :type String :default "Default") (shopping :type "DataTable Object Reference") (struct_PlayerStats :type "/Game/data/stat/Savegame Structure")))