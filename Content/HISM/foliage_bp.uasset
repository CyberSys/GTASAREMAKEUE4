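; Foliage placement Blueprint that builds hierarchical instanced static mesh components from data tables at construction time.
; The construction script destroys existing HISM components, then loops over the DataTables array, creating one component per entry with a valid table and mesh.
; Each component gets its cull range from the entry's distance in meters, with a small fade margin, and one unit-scale instance per table row's location and rotation.
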(event `self.ReceiveBeginPlay`)

(fn `AddInstance`
  (params (Component :type "/Game/HISM/hismc_struct Structure"))
  (bind (_data _mesh _distancem) (break `/Game/HISM/hismc_struct` Component))
  (bind _returnvalue (* _distancem 100))
  (if (and (`KismetSystemLibrary.IsValid` _data) (`KismetSystemLibrary.IsValid` _mesh))
    (bind _returnvalue_2 (`AddComponent|NODE_AddHierarchicalInstancedStaticMeshComponent-1` :`RelativeTransform` (`KismetMathLibrary.MakeTransform` (0.0 0.0 0.0))))
    (`StaticMeshComponent.SetStaticMesh` _returnvalue_2 _mesh)
    (`InstancedStaticMeshComponent.SetCullDistances` _returnvalue_2 _returnvalue (+ _returnvalue (`KismetMathLibrary.FTrunc` (* _returnvalue 0.02))))
    (bind _outrownames (`DataTableFunctionLibrary.GetDataTableRowNames` _data))
    (for _array_element _outrownames
      (bind _returnvalue_3 (`|GetDataTableRow` _data _array_element)
        (:`then`
          (bind (_location _rotation) (break `/Game/HISM/foliage_struct` _returnvalue_3))
          (`InstancedStaticMeshComponent.AddInstance` _returnvalue_2 (`KismetMathLibrary.MakeTransform` _location _rotation)))))))

(fn `ClearComponents`
  (bind (_arrayindex _arrayelement) (`/Engine/EditorBlueprintResources/StandardMacros.ReverseForEachLoop` (`self.K2_GetComponentsByClass` "/Script/Engine.HierarchicalInstancedStaticMeshComponent"))
    (:`LoopBody`
      (`ActorComponent.K2_DestroyComponent` _arrayelement))))

(fn `UserConstructionScript`
  (`self.ClearComponents`)
  (for _array_element (`self.data_tables`)
    (`self.AddInstance` _array_element)))