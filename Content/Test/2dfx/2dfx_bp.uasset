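; Test actor that renders 2dfx corona glows as camera-facing instanced meshes placed from data tables.
; The construction script rebuilds one hierarchical instanced mesh component per offset-table row, with a colored dynamic material.
; Each placement row, except the last, transforms its type's offsets into instance locations.
; Tick turns every instance toward player 0's camera, marking render state dirty only on each component's last update.
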(event `self.ReceiveTick`
  (params (DeltaSeconds :type "Float (single-precision)"))
  (bind _components (`self.components`))
  (bind _keys (`BlueprintMapLibrary.Map_Keys` _components))
  (for _array_element _keys
    (bind _value (`BlueprintMapLibrary.Map_Find` _components _array_element))
    (bind _returnvalue (`InstancedStaticMeshComponent.GetInstanceCount` _value))
    (for _index (range (+ (- _returnvalue 2) 1))
      (`self.RotateCoronas` _value _index))
    (`self.RotateCoronas` _value (- _returnvalue 1) true)))

(fn `AddInstances`
  (bind _outrownames (`DataTableFunctionLibrary.GetDataTableRowNames` "/Game/Test/2dfx/2dfx_data.2dfx_data"))
  (for _index (range (+ (- (`KismetArrayLibrary.Array_Length` _outrownames) 2) 1))
    (bind _returnvalue (`|GetDataTableRow` "/Game/Test/2dfx/2dfx_data.2dfx_data" (`|GetArrayItem` _outrownames _index))
      (:`then`
        (bind (_component _location _rotation) (break `/Game/Test/2dfx/2dfx_data_struct` _returnvalue))
        (bind _returnvalue_2 (`|GetDataTableRow` "/Game/Test/2dfx/2dfx_offset.2dfx_offset" _component)
          (:`then`
            (for _array_element (`.position_3_F00A9BAE4D836E16A21C4DA6D08CC8BD` (break `/Game/Test/2dfx/2dfx_offset_struct` _returnvalue_2))
              (`InstancedStaticMeshComponent.AddInstance` (`BlueprintMapLibrary.Map_Find` (`self.components`) _component) (`KismetMathLibrary.MakeTransform` (`KismetMathLibrary.TransformLocation` (`KismetMathLibrary.MakeTransform` _location _rotation) _array_element) (struct) (3.0 3.0 3.0))))))))))

(fn `ClearComponents`
  (bind (_arrayindex _arrayelement) (`/Engine/EditorBlueprintResources/StandardMacros.ReverseForEachLoop` (`self.K2_GetComponentsByClass` "/Script/Engine.HierarchicalInstancedStaticMeshComponent"))
    (:`LoopBody`
      (`ActorComponent.K2_DestroyComponent` _arrayelement))))

(fn `RotateCoronas`
  (params (Component :type "HierarchicalInstancedStaticMeshComponent Object Reference") (Index :type Integer) (MarkAsDirty :type Boolean))
  (bind _location (.location (`InstancedStaticMeshComponent.GetInstanceTransform` Component Index true)))
  (`InstancedStaticMeshComponent.UpdateInstanceTransform` Component Index (`KismetMathLibrary.MakeTransform` _location (`KismetMathLibrary.FindLookAtRotation` _location (`PlayerCameraManager.GetCameraLocation` (`PlayerController.PlayerCameraManager` (`GameplayStatics.GetPlayerController` 0)))) (.scale (`InstancedStaticMeshComponent.GetInstanceTransform` Component Index true))) true MarkAsDirty false))

(fn `SetupComponents`
  (bind _outrownames (`DataTableFunctionLibrary.GetDataTableRowNames` "/Game/Test/2dfx/2dfx_offset.2dfx_offset"))
  (for _array_element _outrownames
    (bind _returnvalue (`|GetDataTableRow` "/Game/Test/2dfx/2dfx_offset.2dfx_offset" _array_element)
      (:`then`
        (bind _returnvalue_2 (`AddComponent|NODE_AddHierarchicalInstancedStaticMeshComponent-0`))
        (bind _returnvalue_3 (`PrimitiveComponent.CreateDynamicMaterialInstance` _returnvalue_2 0 "/Game/Test/2dfx/coronastar_Mat1.coronastar_Mat1" "None"))
        (`MaterialInstanceDynamic.SetVectorParameterValue` _returnvalue_3 "color" (select `int` (`.color_6_A815DE2D4F95ABB61BD7CC9F9F1E12FB` (break `/Game/Test/2dfx/2dfx_offset_struct` _returnvalue)) :`0` (struct :`R` 1.0 :`G` 1.0 :`B` 1.0 :`A` 1.0) :`1` (struct :`R` 1.0 :`G` 0.47 :`B` 0.03 :`A` 1.0) :`2` (struct :`R` 0.130382 :`G` 0.68622 :`B` 0.770833 :`A` 1.0) :`3` (struct :`R` 0.8125 :`B` 0.02502 :`A` 1.0) :!type "LinearColor Structure"))
        (`BlueprintMapLibrary.Map_Add` (`self.components`) _array_element _returnvalue_2)))))

(fn `UserConstructionScript`
  (`self.ClearComponents`)
  (`self.SetupComponents`)
  (`self.AddInstances`))