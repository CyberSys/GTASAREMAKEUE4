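; Towable trailer that hitches to an Automobile and can be detached.
; An overlap sphere on the "hookup" socket starts a looping timer that sphere-traces for vehicles whose "misc_a" socket is close enough.
; Linking snaps the trailer into alignment, raises its first Misc component, creates a physics constraint at runtime and shows a detach key hint.
; Breaking the link destroys the constraint and lowers that component again.
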(event `self.ReceiveBeginPlay`
  (`parent.ReceiveBeginPlay`)
  (bind _returnvalue (`AddComponent|NODE_AddSphereComponent-0`))
  (`SceneComponent.K2_AttachToComponent` _returnvalue null "hookup" "SnapToTarget" "SnapToTarget" "KeepRelative" true)
  (add `PrimitiveComponent.OnComponentBeginOverlap` _returnvalue (delegate `BeginOverlap`))
  (add `PrimitiveComponent.OnComponentEndOverlap` _returnvalue (delegate `EndOverlap`))
  (if (not (`self.attached`))
    (`SceneComponent.K2_SetRelativeLocation` (`|GetArrayItem` (`self.misc`)) (0.0 0.0 -50.0) false false)))

(event `BeginOverlap`
  (params (OverlappedComponent :type "PrimitiveComponent Object Reference") (OtherActor :type "Actor Object Reference") (OtherComp :type "PrimitiveComponent Object Reference") (OtherBodyIndex :type Integer) (bFromSweep :type Boolean) (SweepResult :type "HitResult Structure (by ref)"))
  (cast `/Game/vehicles/blueprints/Automobile` OtherActor)
  (bind _returnvalue (`KismetSystemLibrary.K2_SetTimer` null "ScanForTowLink" 0.25 true))
  (set `self.Timer_Scan` _returnvalue))

(event `EndOverlap`
  (params (OverlappedComponent :type "PrimitiveComponent Object Reference") (OtherActor :type "Actor Object Reference") (OtherComp :type "PrimitiveComponent Object Reference") (OtherBodyIndex :type Integer))
  (cast `/Game/vehicles/blueprints/Automobile` OtherActor)
  (if (`KismetSystemLibrary.K2_IsTimerActiveHandle` (`self.Timer_Scan`))
    (`KismetSystemLibrary.K2_ClearAndInvalidateTimerHandle` (`self.Timer_Scan`))))

(event `self.ReceiveActorBeginOverlap`
  (params (OtherActor :type "Actor Object Reference"))
  (`parent.ReceiveActorBeginOverlap` OtherActor))

(event `OnTowLinkBroken`
  (params (ConstraintIndex :type Integer))
  (`self.BreakTowLink`))

(fn `BreakTowLink`
  (set `self.TowAutomobile` null)
  (bind _returnvalue (`PhysicsConstraintComponent.IsBroken` (`self.Constraint`)))
  (if (not _returnvalue)
    (`PhysicsConstraintComponent.BreakConstraint` (`self.Constraint`)))
  (`ActorComponent.K2_DestroyComponent` (`self.Constraint`))
  (set `self.attached` false)
  (`SceneComponent.K2_SetRelativeLocation` (`|GetArrayItem` (`self.misc`)) (0.0 0.0 -50.0) false false))

(fn `ScanForTowLink`
  (bind _returnvalue (`SceneComponent.GetSocketLocation` (`self.chassis`) "hookup"))
  (`KismetSystemLibrary.PrintString` "Trailer:: Check for overlapping vehicle")
  (bind (_outhits _returnvalue_2) (`KismetSystemLibrary.SphereTraceMultiForObjects` _returnvalue (- _returnvalue (0.0 0.0 1.0)) 100.0 (`|MakeArray` "ObjectTypeQuery5" :!type "EObjectTypeQuery Enum")))
  (if _returnvalue_2
    (for _array_element _outhits
      (bind _asautomobile (cast `/Game/vehicles/blueprints/Automobile` (`.HitActor` (`GameplayStatics.BreakHitResult` _array_element))))
      (if (< (`KismetMathLibrary.Vector_Distance` (`SceneComponent.GetSocketLocation` (`/Game/vehicles/blueprints/Vehicle.chassis` _asautomobile) "misc_a") (`SceneComponent.GetSocketLocation` (`self.chassis`) "hookup")) 40.0)
        (set `self.attached` true)
        (`self.SetTowLink` _asautomobile)
        (`KismetSystemLibrary.K2_ClearAndInvalidateTimerHandle` (`self.Timer_Scan`))))))

(fn `SetTowLink`
  (params (Automobile :type "/Game/vehicles/blueprints/Automobile Object Reference"))
  (bind (_returnvalue_x _returnvalue_y _returnvalue_z) (`KismetMathLibrary.BreakVector` (`self.K2_GetActorLocation`)))
  (bind _towautomobile (`self.TowAutomobile`))
  (bind _returnvalue_location (`KismetMathLibrary.BreakTransform` (`SceneComponent.GetSocketTransform` (`self.chassis`) "hookup" "RTS_Actor")))
  (bind _returnvalue_location_2 (`KismetMathLibrary.BreakTransform` (`SceneComponent.GetSocketTransform` (`self.chassis`) "hookup" "RTS_Actor")))
  (bind (_returnvalue_x_2 _returnvalue_y_2 _returnvalue_z_2) (`KismetMathLibrary.BreakVector` (`self.K2_GetActorLocation` (`self.TowAutomobile`))))
  (bind (_returnvalue_x_3 _returnvalue_y_3) (`KismetMathLibrary.BreakVector` (`SceneComponent.GetSocketLocation` (`/Game/vehicles/blueprints/Vehicle.chassis` _towautomobile) "misc_a")))
  (bind _returnvalue_location_3 (`KismetMathLibrary.BreakTransform` (`SceneComponent.GetSocketTransform` (`/Game/vehicles/blueprints/Vehicle.chassis` (`self.TowAutomobile`)) "misc_a" "RTS_Actor")))
  (bind (_returnvalue_x_4 _returnvalue_y_4) (`KismetMathLibrary.BreakVector` (* (`self.GetActorForwardVector` _towautomobile) _returnvalue_location)))
  (set `self.TowAutomobile` Automobile)
  (`self.ShowHintText`)
  (`self.K2_SetActorLocationAndRotation` (`KismetMathLibrary.MakeVector` (- _returnvalue_x_3 _returnvalue_x_4) (- _returnvalue_y_3 _returnvalue_y_4) (+ _returnvalue_z (- (+ _returnvalue_z_2 (.z _returnvalue_location_3)) (+ _returnvalue_z (.z _returnvalue_location_2))))) (`self.K2_GetActorRotation` (`self.TowAutomobile`)))
  (`SceneComponent.K2_SetRelativeLocation` (`|GetArrayItem` (`self.misc`)) (0.0 0.0 0.0) false false)
  (bind _returnvalue (`AddComponent|NODE_AddPhysicsConstraintComponent-0`))
  (bind _output_get (set `self.Constraint` _returnvalue))
  (add `PhysicsConstraintComponent.OnConstraintBroken` _output_get (`|CreateDelegate` :!event `OnTowLinkBroken`))
  (`SceneComponent.K2_AttachToComponent` _output_get (`self.chassis`) "hookup" "SnapToTarget" "SnapToTarget" "KeepRelative" true)
  (`PhysicsConstraintComponent.SetConstrainedComponents` (`self.Constraint`) (`/Game/vehicles/blueprints/Vehicle.chassis` (`self.TowAutomobile`)) "misc_a" (`self.chassis`) "hookup"))

(fn `ShowHintText`
  (bind _asplayer_info (cast `/Game/peds/blueprints/PlayerInfo` (`GameplayStatics.GetPlayerController` 0)))
  (`/Game/frontend/widget/hud.setHint_Text` (`/Game/peds/blueprints/PlayerInfo.Hud` _asplayer_info) (`|FormatText` "Press <darkblue>{w} </>to detach trailer" (`KismetInputLibrary.Key_GetDisplayName` (`.Key` (break `InputActionKeyMapping` (`|GetArrayItem` (`InputSettings.GetActionMappingByName` (`InputSettings.GetInputSettings`) "TOGGLE_SUBMISSIONS"))))))))

(fn `UserConstructionScript`
  (`parent.UserConstructionScript`))