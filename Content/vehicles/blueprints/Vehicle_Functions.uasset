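; Vehicle function library that generates random number plate strings for vehicles.
; CreateRandomNumplateString takes a string by reference and fills it only when it is empty, so existing plates are left untouched.
; It appends random picks from a Letters string and random single digits in a fixed seven-character letter and digit pattern.
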(fn `CreateRandomNumplateString`
  (params (StringToChange :type "String (by ref)"))
  (locals (Letters :type String :default "ABCDEFGHIJKLMNOPQRSTUVWXYZ"))
  (bind _letters (`local.Letters`))
  (bind _returnvalue (`KismetStringLibrary.Len` _letters))
  (bind _returnvalue_2 (`KismetStringLibrary.GetCharacterArrayFromString` _letters))
  (if (== (`KismetStringLibrary.Len` StringToChange) 0)
    (`|VariableSetRef` StringToChange (`KismetStringLibrary.Concat_StrStr` (`|GetArrayItem` _returnvalue_2 (`KismetMathLibrary.RandomInteger` _returnvalue)) (`KismetStringLibrary.Conv_IntToString` (`KismetMathLibrary.RandomIntegerInRange` 0 9)) (`KismetStringLibrary.Conv_IntToString` (`KismetMathLibrary.RandomIntegerInRange` 0 9)) (`|GetArrayItem` _returnvalue_2 (`KismetMathLibrary.RandomInteger` _returnvalue)) " " (`KismetStringLibrary.Conv_IntToString` (`KismetMathLibrary.RandomIntegerInRange` 0 9)) (`|GetArrayItem` _returnvalue_2 (`KismetMathLibrary.RandomInteger` _returnvalue)) (`|GetArrayItem` _returnvalue_2 (`KismetMathLibrary.RandomInteger` _returnvalue))))
    (return)))