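; Vehicle damage manager that tracks engine, wheel, door, panel and light damage states.
; ApplyDamage maps the hit component to a group by enum-range offsets, then steps its state when weighted damage passes a threshold, firing visual-update dispatchers.
; Engine damage climbs randomly to a cap, driving status and smoke, and also rises from hard bonnet or certain bumper hits.
; Helpers force heavy damage or restore most states from class defaults.
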(fn `ApplyDamage`
  (params (component :type "/Game/vehicles/enumerations/damage/eVehicleComponent Enum" :default "NewEnumerator0") (damage :type "Float (double-precision)"))
  (locals (ComponentDamage :type "Array of Float (double-precision)"))
  (bind _returnvalue (> damage 220.0))
  (bind (_componentgroup _subcomponent _return) (`self.GetComponentGroup` component))
  (if _return
    (if (> (* (`|GetArrayItem` (`local.ComponentDamage`) _subcomponent) damage) 150.0)
      (switch `/Game/vehicles/enumerations/damage/eVehicleComponentGroup` _componentgroup
        (:`NewEnumerator1`
          (bind _return_2 (`self.ProgressWheelDamage` _subcomponent))
          (if _return_2
            (`self.UpdateDoorVisual` component _componentgroup :!label _label)))
        (:`NewEnumerator2`
          (bind _return_3 (`self.ProgressDoorDamage` _subcomponent :!label _label_2))
          (if _return_3
            (goto _label)))
        (:`NewEnumerator3`
          (if _returnvalue
            (`self.ProgressEngineDamage`)
            (`self.UpdateEngineSmoke` (`self.EngineStatus`))
            (goto _label_2)
            (else
              (goto _label_2))))
        (:`NewEnumerator4`
          (goto _label_2))
        (:`NewEnumerator8`
          (bind _return_4 (`self.ProgressLightStatus` _subcomponent))
          (if _return_4
            (`self.UpdatePanelVisual` "NewEnumerator0" "NewEnumerator8")
            (bind _return_5 (`self.ProgressPanelDamage` _subcomponent :!label _label_3))
            (if _return_5
              (`self.UpdatePanelVisual` component _componentgroup))))
        (:`NewEnumerator5`
          (goto _label_3))
        (:`NewEnumerator0`
          (if (and _returnvalue (or (`|EnumEquality` component "NewEnumerator13") (`|EnumEquality` component "NewEnumerator14") (`|EnumEquality` component "NewEnumerator17")))
            (`self.ProgressEngineDamage`)
            (`self.UpdateEngineSmoke` (`self.EngineStatus`))
            (goto _label_3)
            (else
              (goto _label_3))))
        (:`NewEnumerator6`
          (`self.ProgressEngineDamage`)
          (`self.UpdateEngineSmoke` (`self.EngineStatus`)))))
    (else
      (`KismetSystemLibrary.PrintString` "No damageable Vehiclecomponent found" true true (struct :`R` 1.0 :`A` 1.0) 4.0))))

(fn `FuckCarCompletely`
  (set `self.EngineDamage` 250)
  (for (_ _array_index) (`self.WheelStatus`)
    (`KismetArrayLibrary.Array_Set` (`self.WheelStatus`) _array_index "NewEnumerator2"))
  (for (_ _array_index_2) (`self.DoorStatus`)
    (`KismetArrayLibrary.Array_Set` (`self.DoorStatus`) _array_index_2 "NewEnumerator3"))
  (for _index (range 3)
    (`self.ProgressPanelDamage` _index)))

(fn `GetComponentGroup`
  (params (component :type "/Game/vehicles/enumerations/damage/eVehicleComponent Enum" :default "NewEnumerator0"))
  (returns (componentGroup :type "/Game/vehicles/enumerations/damage/eVehicleComponentGroup Enum") (subComponent :type Integer) (return :type Boolean))
  (bind _returnvalue (enumliteral `/Game/vehicles/enumerations/damage/eVehicleComponent` "NewEnumerator7"))
  (bind _returnvalue_2 (`KismetMathLibrary.Conv_ByteToInt` (- component (enumliteral `/Game/vehicles/enumerations/damage/eVehicleComponent` "NewEnumerator7"))))
  (if (>= component (enumliteral `/Game/vehicles/enumerations/damage/eVehicleComponent` "NewEnumerator21"))
    ;[0.06939 0 1] bumper
    (if (>= component (enumliteral `/Game/vehicles/enumerations/damage/eVehicleComponent` "NewEnumerator18"))
      (return "NewEnumerator0" (`KismetMathLibrary.Conv_ByteToInt` (- component (enumliteral `/Game/vehicles/enumerations/damage/eVehicleComponent` "NewEnumerator18"))) true)
      (elif (>= component (enumliteral `/Game/vehicles/enumerations/damage/eVehicleComponent` "NewEnumerator21"))
        ;[1 1 1] lights
        (return "NewEnumerator8" (`KismetMathLibrary.Conv_ByteToInt` (- component (enumliteral `/Game/vehicles/enumerations/damage/eVehicleComponent` "NewEnumerator13"))) true)
        (else
          ;[1 1 1] panels
          (return "NewEnumerator5" (`KismetMathLibrary.Conv_ByteToInt` (- component (enumliteral `/Game/vehicles/enumerations/damage/eVehicleComponent` "NewEnumerator21"))) true))))
    (elif (>= component _returnvalue)
      ;[1 1 1] bonnet
      (if (`|EnumEquality` component _returnvalue)
        (return "NewEnumerator3" _returnvalue_2 true)
        (else
          ;[1 1 1] boot | door
          (if (`|EnumEquality` component (enumliteral `/Game/vehicles/enumerations/damage/eVehicleComponent` "NewEnumerator8"))
            (return "NewEnumerator4" _returnvalue_2 true)
            (else
              (return "NewEnumerator2" _returnvalue_2 true)))))
      (elif (>= component (enumliteral `/Game/vehicles/enumerations/damage/eVehicleComponent` "NewEnumerator1"))
        ;[1 1 1] wheel
        (return "NewEnumerator1" (`KismetMathLibrary.Conv_ByteToInt` (- component (enumliteral `/Game/vehicles/enumerations/damage/eVehicleComponent` "NewEnumerator1"))) true)
        (elif (>= component (enumliteral `/Game/vehicles/enumerations/damage/eVehicleComponent` "NewEnumerator0"))
          ;[1 1 1] default | none
          (return "NewEnumerator6" (`KismetMathLibrary.Conv_ByteToInt` (enumliteral `/Game/vehicles/enumerations/damage/eVehicleComponent` "NewEnumerator0")) true)
          (else
            (return "NewEnumerator6" 0 false)))))))

(fn `ProgressDoorDamage`
  (params (Index :type Integer))
  (returns (return :type Boolean))
  (bind _output (`|GetArrayItem` (`self.DoorStatus`) Index))
  (if (`|EnumEquality` _output "NewEnumerator3")
    (return false)
    (else
      (`KismetArrayLibrary.Array_Set` (`self.DoorStatus`) Index (cast `/Game/vehicles/enumerations/damage/eVehicleDoorStatus` (+ _output 1)))
      (return true))))

(fn `ProgressEngineDamage`
  (locals (EngineStatusValues :type "Array of Integer"))
  (bind _enginestatusvalues (`local.EngineStatusValues`))
  (bind _enginedamage (`self.EngineDamage`))
  (bind _returnvalue (+ (`self.EngineDamage`) 32 (`KismetMathLibrary.RandomInteger` 32)))
  (set `self.EngineDamage` (`KismetMathLibrary.SelectInt` 250 _returnvalue (>= _returnvalue 250)))
  (if (< _enginedamage (`|GetArrayItem` _enginestatusvalues))
    (set `self.EngineStatus` "NewEnumerator4")
    (elif (< _enginedamage (`|GetArrayItem` _enginestatusvalues 1))
      (set `self.EngineStatus` "NewEnumerator0")
      (elif (< _enginedamage (`|GetArrayItem` _enginestatusvalues 2))
        (set `self.EngineStatus` "NewEnumerator1")
        (elif (< _enginedamage (`|GetArrayItem` _enginestatusvalues 3))
          (set `self.EngineStatus` "NewEnumerator1")
          (else
            (set `self.EngineStatus` "NewEnumerator3")))))))

(fn `ProgressLightStatus`
  (params (Index :type Integer))
  (returns (Return :type Boolean))
  (if (`|EnumEquality` (`|GetArrayItem` (`self.LightStatus`) Index) "NewEnumerator1")
    (return false)
    (else
      (`KismetArrayLibrary.Array_Set` (`self.LightStatus`) Index "NewEnumerator1")
      (return true))))

(fn `ProgressPanelDamage`
  (params (Index :type Integer))
  (returns (return :type Boolean))
  (bind _returnvalue (enumliteral `/Game/vehicles/enumerations/damage/eVehicleLightStatus` "NewEnumerator1"))
  (bind _output (`|GetArrayItem` (`self.PanelStatus`) Index))
  (bind _output_2 (`|GetArrayItem` (`self.PanelStatus`) Index))
  (bind _returnvalue_2 (+ Index (`KismetMathLibrary.Conv_ByteToInt` (enumliteral `/Game/vehicles/enumerations/damage/eVehicleComponent` "NewEnumerator21"))))
  (if (>= _returnvalue_2 (`KismetMathLibrary.Conv_ByteToInt` (enumliteral `/Game/vehicles/enumerations/damage/eVehicleComponent` "NewEnumerator17")))
    (if (== _output_2 (enumliteral `/Game/vehicles/enumerations/damage/eVehiclePanelStatus` "NewEnumerator2"))
      (return false)
      (else
        (`KismetArrayLibrary.Array_Set` (`self.PanelStatus`) Index (+ _output_2 1))
        (return true)))
    (elif (>= _returnvalue_2 (`KismetMathLibrary.Conv_ByteToInt` (enumliteral `/Game/vehicles/enumerations/damage/eVehicleComponent` "NewEnumerator13")))
      (if (== (`|GetArrayItem` (`self.PanelStatus`) Index) _returnvalue)
        (return false)
        (else
          (`KismetArrayLibrary.Array_Set` (`self.PanelStatus`) Index _returnvalue)
          (return true)))
      (elif (== _output (enumliteral `/Game/vehicles/enumerations/damage/eVehiclePanelStatus` "NewEnumerator2"))
        (return false)
        (else
          (`KismetArrayLibrary.Array_Set` (`self.PanelStatus`) Index (+ _output 1))
          (return true))))))

(fn `ProgressWheelDamage`
  (params (Index :type Integer))
  (returns (return :type Boolean))
  (bind _output (`|GetArrayItem` (`self.WheelStatus`) Index))
  (if (`|EnumEquality` _output "NewEnumerator2")
    (return false)
    (else
      (`KismetArrayLibrary.Array_Set` (`self.WheelStatus`) Index (cast `/Game/vehicles/enumerations/damage/eVehicleWheelStatus` (+ _output 1)))
      (return true))))

(fn `ResetDamageStatus`
  (bind (_enginestatus _enginedamage _wheelstatus _doorstatus _panelstatus) (defaults `/Game/vehicles/blueprints/damagemanager` (`GameplayStatics.GetObjectClass` self)))
  (set `self.EngineStatus` _enginestatus)
  (set `self.EngineDamage` _enginedamage)
  (set `self.WheelStatus` _wheelstatus)
  (set `self.DoorStatus` _doorstatus)
  (set `self.PanelStatus` _panelstatus))

(fn `SetDoorStatus`
  (params (Door :type "/Game/vehicles/enumerations/damage/eVehicleComponent Enum" :default "NewEnumerator0") (DoorStatus :type "/Game/vehicles/enumerations/damage/eVehicleDoorStatus Enum" :default "NewEnumerator0"))
  (`KismetArrayLibrary.Array_Set` (`self.DoorStatus`) (`KismetMathLibrary.Conv_ByteToInt` (- Door (enumliteral `/Game/vehicles/enumerations/damage/eVehicleComponent` "NewEnumerator9"))) DoorStatus))