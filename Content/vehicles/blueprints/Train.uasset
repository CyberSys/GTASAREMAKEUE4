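; Train vehicle that runs along a Tracks spline and, without a driver, stops at stations before leaving on a timer.
; The first wagon spawns a trailing carriage, calculates speed and rail distance each tick, and broadcasts that distance to followers.
; Carriages place themselves on the spline by offset and direction, yawing bogies to the rail and spinning wheels.
; SetupComponents builds bogies, wheels and doors from data-table meshes on chassis sockets.
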(event `self.ReceiveBeginPlay`
  (bind _output (`|GetArrayItem` (`self.Bogie`)))
  (bind _returnvalue_location (`KismetMathLibrary.BreakTransform` (`SceneComponent.GetSocketTransform` _output "wheel_lf1" "RTS_Actor")))
  (bind (_returnvalue_x _returnvalue_y _returnvalue_z) (`KismetMathLibrary.BreakVector` (+ (`SceneComponent.RelativeLocation` _output) _returnvalue_location (`KismetMathLibrary.MakeVector` 0.0 0.0 (* (`.WheelScale_Front_36_6FE6E82E4E38D4343AF69996E209F524` (break `/Game/vehicles/structures/sVehicles` (`self.Vehicle`))) -50.0)))))
  (`parent.ReceiveBeginPlay`)
  (bind _outactors (`GameplayStatics.GetAllActorsOfClass` "/Game/core/paths/blueprints/tracks.tracks_C"))
  (set `self.Tracks` (`|GetArrayItem` _outactors))
  (set `self.MaxSpeed` (/ 12000.0 3.6))
  (`self.Position`)
  (`|ExecutionSequence`
    (:`then_0`
      (set `self.Z-Offset` (- 0.0 _returnvalue_z))
      (`self.FindNextStationPositionInDirection`)
      (if (== (`self.WagonId`) 0)
        (set `self.IsFirstWagon` true)
        (bind _returnvalue (`|SpawnActorFromClass` "Train_C" (`self.GetTransform`) "AlwaysSpawn" "OverrideRootScale" null self (+ (`self.WagonId`) 1) "NewEnumerator169" "NewEnumerator3" "" null))
        ;[1 1 1] Carriage offsset
        (set `self.NextCarriage` _returnvalue)
        (bind _returnvalue_2 (+ (`.SphereRadius` (`KismetSystemLibrary.GetComponentBounds` (`/Game/vehicles/blueprints/Vehicle.chassis` _returnvalue))) (`.SphereRadius` (`KismetSystemLibrary.GetComponentBounds` (`self.chassis`))) -50.0))
        (bind _output_get (set `self.CarriageOffset` (`KismetMathLibrary.SelectFloat` (- 0.0 _returnvalue_2) _returnvalue_2 (`self.IsClockWise`))))
        (set `/Game/vehicles/blueprints/Train.CurrentRailDistance` (+ (`self.CurrentRailDistance`) _output_get) _returnvalue)
        (else
          (bind _firstcarriage (`self.GetFirstCarriage`))
          (add `self.UpdateDistanceAlongSplineOnCarriage` _firstcarriage (delegate `UpdateSpeed`)))))
    (:`then_1`
      ;[1 0 0] DEBUG POSSES
      (if (`self.IsFirstWagon`)
        _))))

(event `UpdateSpeed` :!signature `self.UpdateDistanceAlongSplineOnCarriage`
  (params (CurrentDistanceAlongSpline :type "Float (double-precision)"))
  (set `self.CurrentRailDistance` CurrentDistanceAlongSpline)
  (`self.Position`)
  (`self.WheelRotation`)
  (`self.BoogieRotation`))

(event `self.ReceiveTick`
  (params (DeltaSeconds :type "Float (single-precision)"))
  (if (`self.IsFirstWagon`)
    (`self.PRINT` true)
    (`self.FindMaximumSpeedToStopAtStations`)
    (`self.SetTrainCruiseSpeed`)
    (`self.Position`)
    (`self.WheelRotation`)
    (`self.BoogieRotation`)
    (`self.UpdateDistanceAlongSplineOnCarriage` (`self.CurrentRailDistance`))))

(fn `BoogieRotation`
  (bind _returnvalue (`/Game/core/paths/blueprints/tracks.GetTrackFromId` (`self.Tracks`) (`self.TrackId`)))
  (bind _returnvalue_2 (+ (`self.CurrentRailDistance`) (`self.CarriageOffset`)))
  (bind _returnvalue_3 (`SplineComponent.GetDirectionAtDistanceAlongSpline` _returnvalue (+ _returnvalue_2 (.x (.location (`SceneComponent.GetSocketTransform` (`self.chassis`) "bogie_rear" "RTS_Actor")))) "World"))
  (bind _returnvalue_4 (`SplineComponent.GetDirectionAtDistanceAlongSpline` _returnvalue (+ _returnvalue_2 (.x (.location (`SceneComponent.GetSocketTransform` (`self.chassis`) "bogie_front" "RTS_Actor")))) "World"))
  (bind (_returnvalue_roll _returnvalue_pitch _returnvalue_yaw) (`KismetMathLibrary.BreakRotator` (`KismetMathLibrary.Conv_VectorToRotator` (`KismetMathLibrary.InverseTransformDirection` (`self.GetTransform`) (`KismetMathLibrary.SelectVector` (- (0.0 0.0 0.0) _returnvalue_3) _returnvalue_3 (`self.IsClockWise`))))))
  (bind (_returnvalue_roll_2 _returnvalue_pitch_2 _returnvalue_yaw_2) (`KismetMathLibrary.BreakRotator` (`KismetMathLibrary.Conv_VectorToRotator` (`KismetMathLibrary.InverseTransformDirection` (`self.GetTransform`) (`KismetMathLibrary.SelectVector` (- (0.0 0.0 0.0) _returnvalue_4) _returnvalue_4 (`self.IsClockWise`))))))
  ;[1 1 1] front
  (`SceneComponent.K2_SetRelativeRotation` (`|GetArrayItem` (`self.Bogie`)) (`KismetMathLibrary.MakeRotator` 0.0 0.0 _returnvalue_yaw_2) false false)
  ;[1 1 1] rear
  (`SceneComponent.K2_SetRelativeRotation` (`|GetArrayItem` (`self.Bogie`) 1) (`KismetMathLibrary.MakeRotator` 0.0 0.0 _returnvalue_yaw) false false))

(fn `FindMaximumSpeedToStopAtStations`
  (locals (Distance :type "Float (double-precision)" :default 0.0))
  (bind _stationdistance (`self.StationDistance`))
  (bind _currentraildistance (`self.CurrentRailDistance`))
  (bind _speed (`self.Speed`))
  (`/Engine/EditorBlueprintResources/StandardMacros.IsValid` (`self.Driver`)
    (:`Is Not Valid`
      (if (>= _stationdistance _currentraildistance)
        (set `local.Distance` (- _stationdistance _currentraildistance))
        (else
          (set `local.Distance` (- (+ (`SplineComponent.GetSplineLength` (`/Game/core/paths/blueprints/tracks.GetTrackFromId` (`self.Tracks`) (`self.TrackId`))) (`self.StationDistance`)) (`self.CurrentRailDistance`)))))
      (if (<= (`local.Distance`) 12000.0)
        (set `self.TrainStatus` "NewEnumerator2")
        (bind _output_get (set `self.Speed` (- _speed (- _speed (`local.Distance`)))))
        (if (<= _output_get 10.0)
          (set `self.Speed` 0.0)
          (`KismetSystemLibrary.K2_SetTimer` null "LeaveStation" 5.0)
          (`self.FindNextStationPositionInDirection`))))))

(fn `FindNextStationPositionInDirection`
  (bind _returnvalue (- (`self.NextStationId`) 1))
  (bind _returnvalue_2 (`/Game/core/paths/blueprints/tracks.GetStationsFromId` (`self.Tracks`) (`self.TrackId`)))
  (`|ExecutionSequence`
    (:`then_0`
      ;[1 1 1] Next station
      (if (not (`self.IsClockWise`))
        (set `self.NextStationId` (mod (+ (`self.NextStationId`) 1) (`KismetArrayLibrary.Array_Length` _returnvalue_2)))
        (else
          (set `self.NextStationId` (`KismetMathLibrary.SelectInt` (`KismetArrayLibrary.Array_LastIndex` _returnvalue_2) _returnvalue (< _returnvalue 0))))))
    (:`then_1`
      ;[1 1 1] distance along spline
      (set `self.StationDistance` (`SplineComponent.GetDistanceAlongSplineAtSplinePoint` (`/Game/core/paths/blueprints/tracks.GetTrackFromId` (`self.Tracks`) (`self.TrackId`)) (`|GetArrayItem` (`/Game/core/paths/blueprints/tracks.GetStationsFromId` (`self.Tracks`) (`self.TrackId`)) (`self.NextStationId`)))))))

(fn `GetFirstCarriage`
  (returns (FirstCarriage :type "/Game/vehicles/blueprints/Train Object Reference"))
  (locals (Prev :type "/Game/vehicles/blueprints/Train Object Reference"))
  (bind _prevcarriage (`self.PrevCarriage`))
  (bind _prevcarriage_2 (`/Game/vehicles/blueprints/Train.PrevCarriage` _prevcarriage))
  (`/Engine/EditorBlueprintResources/StandardMacros.IsValid` _prevcarriage
    (:`Is Valid`
      (set `local.Prev` _prevcarriage)
      (while (`KismetSystemLibrary.IsValid` _prevcarriage_2)
        (set `local.Prev` _prevcarriage_2))
      (return (`local.Prev`)))
    (:`Is Not Valid`
      (return self))))

(fn `GetLastCarriage`
  (returns (Train :type "/Game/vehicles/blueprints/Train Object Reference"))
  (locals (next :type "/Game/vehicles/blueprints/Train Object Reference"))
  (bind _nextcarriage (`self.NextCarriage`))
  (bind _nextcarriage_2 (`/Game/vehicles/blueprints/Train.NextCarriage` _nextcarriage))
  (`/Engine/EditorBlueprintResources/StandardMacros.IsValid` _nextcarriage
    (:`Is Valid`
      (set `local.next` _nextcarriage_2)
      (while (`KismetSystemLibrary.IsValid` _nextcarriage_2)
        (set `local.next` _nextcarriage_2))
      (return (`local.next`)))
    (:`Is Not Valid`
      (return self))))

(fn `LeaveStation`
  (set `self.TrainStatus` "NewEnumerator1"))

(fn `Position`
  (bind _returnvalue (`/Game/core/paths/blueprints/tracks.GetTrackFromId` (`self.Tracks`) (`self.TrackId`)))
  (bind _returnvalue_2 (+ (`self.CurrentRailDistance`) (`self.CarriageOffset`)))
  (bind _returnvalue_3 (* (`GameplayStatics.GetWorldDeltaSeconds`) (`self.Speed`)))
  (bind _returnvalue_4 (`SplineComponent.GetLocationAtDistanceAlongSpline` _returnvalue _returnvalue_2 "World"))
  (bind _returnvalue_5 (`SplineComponent.GetDirectionAtDistanceAlongSpline` _returnvalue _returnvalue_2 "World"))
  (bind _returnvalue_6 (- (`self.CurrentRailDistance`) _returnvalue_3))
  (bind _returnvalue_7 (`SplineComponent.GetSplineLength` (`/Game/core/paths/blueprints/tracks.GetTrackFromId` (`self.Tracks`) (`self.TrackId`))))
  (bind _returnvalue_8 (`KismetMathLibrary.Conv_VectorToRotator` (`KismetMathLibrary.SelectVector` (* _returnvalue_5 -1.0) _returnvalue_5 (`self.IsClockWise`))))
  (`|ExecutionSequence`
    (:`then_0`
      (if (`self.IsFirstWagon`)
        (set `self.CurrentRailDistance` (`KismetMathLibrary.SelectFloat` (`KismetMathLibrary.SelectFloat` (- _returnvalue_7 _returnvalue_6) _returnvalue_6 (< _returnvalue_6 0.0)) (mod (+ (`self.CurrentRailDistance`) _returnvalue_3) _returnvalue_7) (`self.IsClockWise`)))))
    (:`then_1`
      (`self.K2_SetActorTransform` (`KismetMathLibrary.MakeTransform` (+ (`KismetMathLibrary.SelectVector` (+ _returnvalue_4 (* (`KismetMathLibrary.GetRightVector` _returnvalue_8) 400.0)) _returnvalue_4 (`self.IsClockWise`)) (`KismetMathLibrary.MakeVector` 0.0 0.0 (`self.Z-Offset`))) _returnvalue_8)))))

(fn `PRINT`
  (params (Print :type Boolean))
  (bind _nextstationid (`self.NextStationId`))
  (if Print
    (`KismetSystemLibrary.PrintString` (`KismetStringLibrary.Concat_StrStr` "Train speed= " (`KismetStringLibrary.Conv_DoubleToString` (* (`self.Speed`) 0.036)) " km/h") true true (struct :`R` 1.0 :`G` 0.825386 :`B` 0.329681 :`A` 1.0) 0.0)
    (`KismetSystemLibrary.PrintString` (`KismetStringLibrary.Concat_StrStr` "Next station is " (`KismetStringLibrary.Conv_IntToString` _nextstationid) " at NodeId " (`KismetStringLibrary.Conv_IntToString` (`|GetArrayItem` (`/Game/core/paths/blueprints/tracks.GetStationsFromId` (`self.Tracks`) (`self.TrackId`)) _nextstationid))) true true (struct :`R` 1.0 :`G` 0.823821 :`B` 0.070054 :`A` 1.0) 0.0)))

(fn `SetTrainCruiseSpeed`
  (switch `/Game/vehicles/enumerations/eTrainStatus` (`self.TrainStatus`)
    (:`NewEnumerator1`
      (set `self.Speed` (`KismetMathLibrary.FMin` (+ (`self.Speed`) (* (`self.MaxSpeed`) (`GameplayStatics.GetWorldDeltaSeconds`) 0.02)) (`self.MaxSpeed`))))
    (:`NewEnumerator2`
      (`/Engine/EditorBlueprintResources/StandardMacros.IsValid` (`self.Driver`) :!label _label
        (:`Is Valid`
          (set `self.Speed` (`KismetMathLibrary.FMin` (- (`self.Speed`) (* (`self.MaxSpeed`) (`GameplayStatics.GetWorldDeltaSeconds`) 0.02)) (`self.MaxSpeed`))))))
    (:`NewEnumerator0`
      (goto _label))))

(fn `SetupComponents`
  (locals (Socketname :type Name))
  (bind _enumvalue (foreach `/Game/vehicles/enumerations/eTrainNodes` false)
    (:`LoopBody`
      (set `local.Socketname` (`KismetStringLibrary.Conv_StringToName` (`|GetEnumeratorNameAsString` _enumvalue)))
      (switch `/Game/vehicles/enumerations/eTrainNodes` _enumvalue
        (:`NewEnumerator0`
          ;[1 1 1] Bogie
          (bind _returnvalue (`|GetDataTableRow` (`.meshes_50_B28A7ECD4AEA7C8B391F3A8A6A3B256C` (break `/Game/vehicles/structures/sVehicles` (`self.Vehicle`))) "bogie" :!label _label)
            (:`then`
              (bind _returnvalue_2 (`AddComponent|NODE_AddStaticMeshComponent-1`))
              (`StaticMeshComponent.SetStaticMesh` _returnvalue_2 (`.ok_13_292C36804962BA96F41531A78EA23B92` (break `/Game/vehicles/structures/sVehicleMeshes` _returnvalue)))
              (`SceneComponent.K2_AttachToComponent` _returnvalue_2 (`self.chassis`) (`local.Socketname`) "SnapToTarget" "SnapToTarget" "KeepRelative" true)
              (`KismetArrayLibrary.Array_Add` (`self.Bogie`) _returnvalue_2)
              ;[1 1 1] Wheels
              (bind _returnvalue_3 (`|GetDataTableRow` (`.meshes_50_B28A7ECD4AEA7C8B391F3A8A6A3B256C` (break `/Game/vehicles/structures/sVehicles` (`self.Vehicle`))) "wheel")
                (:`then`
                  (for _array_element (`SceneComponent.GetAllSocketNames` _returnvalue_2)
                    (bind _returnvalue_4 (`AddComponent|NODE_AddStaticMeshComponent-2`))
                    (`StaticMeshComponent.SetStaticMesh` _returnvalue_4 (`.ok_13_292C36804962BA96F41531A78EA23B92` (break `/Game/vehicles/structures/sVehicleMeshes` _returnvalue_3)))
                    (`SceneComponent.K2_AttachToComponent` _returnvalue_4 _returnvalue_2 _array_element "SnapToTarget" "SnapToTarget" "KeepRelative" true)
                    (`KismetArrayLibrary.Array_Add` (`self.Wheels`) _returnvalue_4)))))))
        (:`NewEnumerator1`
          (goto _label))
        (:`NewEnumerator6`
          ;[1 1 1] Doors
          (bind _returnvalue_5 (`AddComponent|NODE_Adddoor-1` :`MaxAngle(degree)` (`KismetMathLibrary.RadiansToDegrees` (* (`KismetMathLibrary.GetPI`) (select `/Game/vehicles/enumerations/eTrainNodes` _enumvalue :`NewEnumerator6` -0.8 :`NewEnumerator7` 0.8 :!type "Float (single-precision)"))) :!label _label_2))
          (`SceneComponent.K2_AttachToComponent` _returnvalue_5 (`self.chassis`) (`KismetStringLibrary.Conv_StringToName` (`|GetEnumeratorNameAsString` (enumliteral `/Game/vehicles/enumerations/eTrainNodes` _enumvalue))) "SnapToTarget" "SnapToTarget" "SnapToTarget" true)
          (`KismetArrayLibrary.Array_Add` (`self.Doors`) _returnvalue_5)
          (bind _returnvalue_6 (`|GetDataTableRow` (`.meshes_50_B28A7ECD4AEA7C8B391F3A8A6A3B256C` (break `/Game/vehicles/structures/sVehicles` (`self.Vehicle`))) (`local.Socketname`))
            (:`then`
              (bind _returnvalue_7 (`AddComponent|NODE_AddStaticMeshComponent-4`))
              (`/Game/vehicles/blueprints/door.SetMesh` _returnvalue_5 _returnvalue_7)
              (`StaticMeshComponent.SetStaticMesh` _returnvalue_7 (`.ok_13_292C36804962BA96F41531A78EA23B92` (break `/Game/vehicles/structures/sVehicleMeshes` _returnvalue_6)))
              (`SceneComponent.K2_AttachToComponent` _returnvalue_7 (`self.chassis`) (`local.Socketname`) "SnapToTarget" "SnapToTarget" "KeepRelative" true))))
        (:`NewEnumerator7`
          (goto _label_2))))))

(fn `UserConstructionScript`)

(fn `WheelRotation`
  (for _index (range 8)
    (`SceneComponent.K2_AddLocalRotation` (`|GetArrayItem` (`self.Wheels`) _index) (`KismetMathLibrary.MakeRotator` 0.0 (- 0.0 (/ (* (`GameplayStatics.GetWorldDeltaSeconds`) (`self.Speed`)) (* (`.WheelScale_Front_36_6FE6E82E4E38D4343AF69996E209F524` (break `/Game/vehicles/structures/sVehicles` (`self.Vehicle`))) 0.5)))) false false)))