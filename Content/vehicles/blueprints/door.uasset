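; Vehicle door Blueprint that wraps a mesh and a physics constraint to drive and query a hinged door.
; SetConstraint limits Swing1 or Swing2 to half the maximum angle and offsets the constraint by that half for one-sided travel.
; Open picks a mesh yaw from ratio thresholds, updating the door state in some branches.
; Closed, fully-open and open-ratio queries read the constraint's current swing on the selected axis.
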(event `self.ReceiveBeginPlay`)

(fn `GetAngleOpenRation`
  (returns (ReturnValue :type "Float (double-precision)"))
  (bind _constraint (`self.Constraint`))
  (return (/ (`KismetMathLibrary.DegreesToRadians` (`KismetMathLibrary.SelectFloat` (`PhysicsConstraintComponent.GetCurrentSwing2` _constraint) (`PhysicsConstraintComponent.GetCurrentSwing1` _constraint) (`self.Swing2`))) (`self.MaxAngle(degree)`))))

(fn `GetConstraint`
  (returns (Constraint :type "PhysicsConstraintComponent Object Reference"))
  (return (`self.Constraint`)))

(fn `GetMesh`
  (returns (Mesh :type "StaticMeshComponent Object Reference"))
  (return (`self.Mesh`)))

(fn `IsClosed`
  (returns (ReturnValue :type Boolean))
  (bind _constraint (`self.Constraint`))
  (return (== (`KismetMathLibrary.SelectFloat` (`PhysicsConstraintComponent.GetCurrentSwing2` _constraint) (`PhysicsConstraintComponent.GetCurrentSwing1` _constraint) (`self.Swing2`)) 0.0)))

(fn `IsFullyOpen`
  (returns (ReturnValue :type Boolean))
  (bind _constraint (`self.Constraint`))
  (return (not (< (`KismetMathLibrary.DegreesToRadians` (`KismetMathLibrary.SelectFloat` (`PhysicsConstraintComponent.GetCurrentSwing2` _constraint) (`PhysicsConstraintComponent.GetCurrentSwing1` _constraint) (`self.Swing2`))) (- (`KismetMathLibrary.Abs` (`KismetMathLibrary.DegreesToRadians` (`self.MaxAngle(degree)`))) 0.5)))))

(fn `Open`
  (params (Ratio :type "Float (double-precision)"))
  (if (< Ratio 1.0)
    (if (> Ratio 0.0)
      (set `self.CurrentAngle(degree)` 0.0)
      (set `self.Doorstate` "NewEnumerator2")
      (else
        (set `self.CurrentAngle(degree)` (* (`self.MaxAngle(degree)`) Ratio))))
    (else
      (set `self.CurrentAngle(degree)` 1.0)
      (set `self.Doorstate` "NewEnumerator1")))
  (`self.K2_SetRelativeRotation` (`self.Mesh`) (`KismetMathLibrary.MakeRotator` 0.0 0.0 (`self.CurrentAngle(degree)`)) false false))

(fn `SetConstraint`
  (params (PhysicsConstraint :type "PhysicsConstraintComponent Object Reference"))
  (bind _constraint (`self.Constraint`))
  (bind _constraint_2 (`self.Constraint`))
  (bind _returnvalue (* (`self.MaxAngle(degree)`) 0.5))
  (bind _returnvalue_2 (* (`self.MaxAngle(degree)`) 0.5))
  (bind _returnvalue_3 (* (`self.MaxAngle(degree)`) 0.5))
  (bind _output_get (set `self.Constraint` PhysicsConstraint))
  (if (`self.Swing2`)
    (`PhysicsConstraintComponent.SetAngularSwing2Limit` _output_get "ACM_Limited" _returnvalue)
    (`PhysicsConstraintComponent.SetAngularOrientationTarget` _constraint (`KismetMathLibrary.MakeRotator` 0.0 _returnvalue_2))
    (`self.K2_SetRelativeRotation` _constraint_2 (`KismetMathLibrary.MakeRotator` 0.0 _returnvalue_3) false false)
    (else
      (`PhysicsConstraintComponent.SetAngularSwing1Limit` _output_get "ACM_Limited" _returnvalue)
      (`PhysicsConstraintComponent.SetAngularOrientationTarget` _constraint (`KismetMathLibrary.MakeRotator` 0.0 0.0 _returnvalue_2))
      (`self.K2_SetRelativeRotation` _constraint_2 (`KismetMathLibrary.MakeRotator` 0.0 0.0 _returnvalue_3) false false))))

(fn `SetMesh`
  (params (StaticMeshComponent :type "StaticMeshComponent Object Reference"))
  (set `self.Mesh` StaticMeshComponent))