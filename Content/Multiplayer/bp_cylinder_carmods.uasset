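; Car mod shop entrance marker: a cylinder trigger, colored by shop type (lowrider, street racer, normal), that takes the player's car into a garage.
; Overlap checks mod data and handling-flag bits, then either stops the car or shows a "can't mod" warning.
; Entering streams a level instance, teleports the car to a tagged Bp_carupgrade with suspension offset, swaps lighting and camera, and fills the HUD with mods and wheels.
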(event `self.ReceiveBeginPlay`
  (`ActorComponent.SetActive` (`self.Camera_Body`) true false))

(event `Enter Garage`
  (bind _newlevelinstance_name (`self.NewLevelInstance-Name`))
  (bind _dat_carmods (`self.dat_CarMods`))
  (bind _returnvalue (`GameplayStatics.GetStreamingLevel` _newlevelinstance_name))
  (bind _returnvalue_2 (`GameplayStatics.GetStreamingLevel` (`self.NewLevelInstance-Name`)))
  (bind _weathermanager (`/Game/Vehicle/generic/blueprint/bp_car.weathermanager` (`self.REF_car`)))
  ;[1 1 1] Check for car
  (if (`self.toInterior`)
    (set `/Game/data/timecycle/weatherManager.interior` true _weathermanager)
    (if (not (`LevelStreaming.IsLevelLoaded` _returnvalue))
      (`/Engine/EditorBlueprintResources/StandardMacros.IsValid` _returnvalue
        (:`Is Valid`
          _)
        (:`Is Not Valid`
          (`LevelStreaming.CreateInstance` (`GameplayStatics.GetStreamingLevel` (`self.LevelToLoad-Name`)) (`KismetStringLibrary.Conv_NameToString` _newlevelinstance_name))))
      (set `LevelStreaming.LevelTransform` (`KismetMathLibrary.MakeTransform` (* (`self.InstanceLocation(meter)`) 100.0)) _returnvalue_2)
      (set `LevelStreaming.bShouldBeLoaded` true _returnvalue_2)
      (set `LevelStreaming.bShouldBeVisible` true _returnvalue_2)
      (if (and (`LevelStreaming.IsLevelVisible` _returnvalue_2) (`LevelStreaming.IsLevelLoaded` _returnvalue_2)) :!label _label
        _
        (else
          (`KismetSystemLibrary.Delay` 0.2)
          (goto _label))))
    (bind _outactors (`GameplayStatics.GetAllActorsOfClass` "/Game/Multiplayer/bp_carupgrade.bp_carupgrade_C"))
    (for _array_element _outactors
      (if (`self.ActorHasTag` _array_element (`self.bp_carupgrade_Target-ActorTag`))
        (set `self.REFERENCE_carpupgrade` _array_element)
        (bind (_rotation _location) (`self.SpawnLocation` _array_element))
        (bind (_sweephitresult _returnvalue_3) (`self.K2_SetActorLocationAndRotation` (`Controller.K2_GetPawn` (`GameplayStatics.GetPlayerController` 0)) _location _rotation false true))
        (if _returnvalue_3
          (`self.EnableInput` (`GameplayStatics.GetPlayerController` 0))
          (`self.SwitchLightEnvironment`)
          (`PlayerController.SetViewTargetWithBlend` (`GameplayStatics.GetPlayerController` 0) (`ChildActorComponent.ChildActor` (`/Game/Multiplayer/bp_carupgrade.camera_colors` (`self.REFERENCE_carpupgrade`))) 0.0 "VTBlend_Linear" 0.0 false)
          (remove `/Game/Vehicle/generic/blueprint/bp_car.StopVehicle` (`self.REF_car`) (delegate `Enter Garage`))
          (set `self.inUse` true)
          ;[1 1 1] Create Hud
          (`/Game/Player/blueprint/player_pc.carmods` (`self.PlayerController`) self (`self.REFERENCE_carpupgrade`))
          ;[1 1 1] Add Items depending on car and shop
          (for _array_element_2 (stale `self.Capsule.OnComponentBeginOverlap` _mods)
            (bind _returnvalue_4 (`|GetDataTableRow` (`self.dat_CarMods`) _array_element_2)
              (:`then`
                (bind (_ok _dam _gamename _price) (break `/Game/data/vehicles/struct_CarMods` _returnvalue_4))
                (`/Game/UserInterface/menus/carmod/hud_shopping_carmods.Add Item` (`/Game/Player/blueprint/player_pc.Hud_Carmods` (`self.PlayerController`)) _array_element_2 _gamename _price))))
          ;;[0 0 0] add wheels
          (for _index (range 151 168)
            (bind _outrownames (`DataTableFunctionLibrary.GetDataTableRowNames` _dat_carmods))
            (bind _output (`|GetArrayItem` _outrownames _index))
            (bind _returnvalue_5 (`|GetDataTableRow` _dat_carmods _output)
              (:`then`
                (bind (_ok_2 _dam_2 _gamename_2 _price_2) (break `/Game/data/vehicles/struct_CarMods` _returnvalue_5))
                (`/Game/UserInterface/menus/carmod/hud_shopping_carmods.Add Item` (`/Game/Player/blueprint/player_pc.Hud_Carmods` (`self.PlayerController`)) _output _gamename_2 _price_2))))
          (`/Game/UserInterface/menus/carmod/hud_shopping_carmods.UpdateButtons` (`/Game/Player/blueprint/player_pc.Hud_Carmods` (`self.PlayerController`))))
        (else
          (`KismetSystemLibrary.PrintString` "No matching Tag!" true true (struct :`G` 0.66 :`B` 1.0 :`A` 1.0) 5.0))))
    (else
      (set `/Game/data/timecycle/weatherManager.interior` true _weathermanager))))

(event `self.Capsule.OnComponentBeginOverlap`
  (params (OverlappedComponent :type "PrimitiveComponent Object Reference") (OtherActor :type "Actor Object Reference") (OtherComp :type "PrimitiveComponent Object Reference") (OtherBodyIndex :type Integer) (bFromSweep :type Boolean) (SweepResult :type "HitResult Structure (by ref)"))
  (bind _ref_car (`self.REF_car`))
  (if (not (`self.inUse`))
    (bind _asplayer_pc (cast `/Game/Player/blueprint/player_pc` (`self.GetInstigatorController` OtherActor)))
    (bind _returnvalue (`Controller.K2_GetPawn` _asplayer_pc))
    (if (== OtherActor _returnvalue)
      (bind _asbp_car (cast `/Game/Vehicle/generic/blueprint/bp_car` _returnvalue))
      (set `self.PlayerController` _asplayer_pc)
      (set `self.REF_car` _asbp_car)
      ;[1 1 1] Check for car
      (bind _mods (`self.GetGarage` (`/Game/Vehicle/generic/blueprint/bp_car.vehiclename` _asbp_car))
        (:`LOW_RIDER`
          (add `/Game/Vehicle/generic/blueprint/bp_car.StopVehicle` _ref_car (delegate `Enter Garage`) :!label _label_2)
          (`/Game/Vehicle/generic/blueprint/bp_car.Stop Vehicle` _ref_car))
        (:`STREET_RACER`
          (goto _label_2))
        (:`NORMAL`
          (goto _label_2))
        (:`false`
          (`Widget.SetVisibility` (`/Game/UserInterface/gameplay/hud_car.cp-cant_mod_this_veh` (`/Game/Player/blueprint/player_pc.Hud_car` (`self.PlayerController`))) "Visible"))))))

(event `self.Capsule.OnComponentEndOverlap`
  (params (OverlappedComponent :type "PrimitiveComponent Object Reference") (OtherActor :type "Actor Object Reference") (OtherComp :type "PrimitiveComponent Object Reference") (OtherBodyIndex :type Integer))
  (if (not (`self.inUse`))
    (`/Engine/EditorBlueprintResources/StandardMacros.IsValid` (`self.REF_car`)
      (:`Is Valid`
        (`SceneComponent.SetHiddenInGame` (`self.cylinder`) false false)
        (`Widget.SetVisibility` (`/Game/UserInterface/gameplay/hud_car.cp-cant_mod_this_veh` (`/Game/Player/blueprint/player_pc.Hud_car` (`self.PlayerController`))) "Collapsed")))))

(fn `SpawnLocation`
  (params (TargetLocationActor :type "Actor Object Reference"))
  (returns (Rotation :type "Rotator Structure") (Location :type "Vector Structure"))
  (bind (_returnvalue_location _returnvalue_rotation) (`KismetMathLibrary.BreakTransform` (`self.GetTransform` TargetLocationActor)))
  (bind _ref_car (`self.REF_car`))
  (bind _ref_car_2 (`self.REF_car`))
  (bind _suspension_default_rest_length (break `/Game/Vehicle/generic/blueprint/suspensionStruct` (`/Game/Vehicle/generic/blueprint/bp_car.Suspension_Default` _ref_car)))
  (bind _output_radius (break `/Game/Vehicle/generic/blueprint/wheelStruct` (`|GetArrayItem` (`/Game/Vehicle/generic/blueprint/bp_car.Wheel` _ref_car))))
  (bind (_relativelocation_x _relativelocation_y _relativelocation_z) (`KismetMathLibrary.BreakVector` (`SceneComponent.RelativeLocation` (`/Game/Vehicle/generic/blueprint/bp_car.Toplink_RF` _ref_car))))
  (bind _returnvalue_x (`KismetMathLibrary.BreakVector` (`KismetMathLibrary.InverseTransformLocation` (`self.GetTransform` _ref_car_2) (`KismetSystemLibrary.GetComponentBounds` (`/Game/Vehicle/generic/blueprint/bp_car.chassis` _ref_car_2)))))
  (bind (_outhit _returnvalue) (`KismetSystemLibrary.LineTraceSingle` (+ _returnvalue_location (0.0 0.0 100.0)) (- _returnvalue_location (0.0 0.0 100.0)) "TraceTypeQuery1" true))
  (if _returnvalue
    (return _returnvalue_rotation (`KismetMathLibrary.MakeVector` (+ (.x (`.Location` (`GameplayStatics.BreakHitResult` _outhit))) _returnvalue_x) (.y (`.Location` (`GameplayStatics.BreakHitResult` _outhit))) (+ (.z (`.Location` (`GameplayStatics.BreakHitResult` _outhit))) (`KismetMathLibrary.Abs` (- (- _relativelocation_z _suspension_default_rest_length) _output_radius)))))))

(fn `SwitchLightEnvironment`
  (bind _rootcomponent (`Actor.RootComponent` (`|ConvertAsset` (`self.Sun`))))
  (bind _rootcomponent_2 (`Actor.RootComponent` (`|ConvertAsset` (`self.Fog_Interior`))))
  ;[0.03035 0.3644 1] Switch Interor/Extirior Lighting
  (if (`self.toInterior`)
    ;;[1 1 1 -34.73] Interior
    (`SceneComponent.SetVisibility` _rootcomponent false false)
    (`SceneComponent.SetVisibility` (`Actor.RootComponent` (`|ConvertAsset` (`self.Moon`))) false false)
    (`SceneComponent.SetVisibility` (`Actor.RootComponent` (`|ConvertAsset` (`self.Skylight_Exterior`))) false false)
    (`SceneComponent.SetVisibility` (`Actor.RootComponent` (`|ConvertAsset` (`self.Fog_exterior`))) false false)
    (`SceneComponent.SetHiddenInGame` _rootcomponent true false)
    (`SceneComponent.SetHiddenInGame` (`Actor.RootComponent` (`|ConvertAsset` (`self.Moon`))) true false)
    (`SceneComponent.SetHiddenInGame` (`Actor.RootComponent` (`|ConvertAsset` (`self.Skylight_Exterior`))) true false)
    (`SceneComponent.SetHiddenInGame` (`Actor.RootComponent` (`|ConvertAsset` (`self.Fog_exterior`))) true false)
    (`SceneComponent.SetVisibility` _rootcomponent_2 true false)
    (`SceneComponent.SetVisibility` (`Actor.RootComponent` (`|ConvertAsset` (`self.Skylight_Interior`))) true false)
    (`SceneComponent.SetHiddenInGame` _rootcomponent_2 false false)
    (`SceneComponent.SetHiddenInGame` (`Actor.RootComponent` (`|ConvertAsset` (`self.Skylight_Interior`))) false false)
    (else
      ;;[1 1 1 -4.222] Exterior
      (`SceneComponent.SetVisibility` _rootcomponent true false)
      (`SceneComponent.SetVisibility` (`Actor.RootComponent` (`|ConvertAsset` (`self.Moon`))) true false)
      (`SceneComponent.SetVisibility` (`Actor.RootComponent` (`|ConvertAsset` (`self.Skylight_Exterior`))) true false)
      (`SceneComponent.SetVisibility` (`Actor.RootComponent` (`|ConvertAsset` (`self.Fog_exterior`))) true false)
      (`SceneComponent.SetHiddenInGame` (`Actor.RootComponent` (`|ConvertAsset` (`self.Fog_exterior`))) false false)
      (`SceneComponent.SetHiddenInGame` (`Actor.RootComponent` (`|ConvertAsset` (`self.Skylight_Exterior`))) false false)
      (`SceneComponent.SetHiddenInGame` (`Actor.RootComponent` (`|ConvertAsset` (`self.Moon`))) false false)
      (`SceneComponent.SetHiddenInGame` _rootcomponent false false)
      (`SceneComponent.SetVisibility` _rootcomponent_2 false false)
      (`SceneComponent.SetVisibility` (`Actor.RootComponent` (`|ConvertAsset` (`self.Skylight_Interior`))) false false)
      (`SceneComponent.SetHiddenInGame` (`Actor.RootComponent` (`|ConvertAsset` (`self.Skylight_Interior`))) true false)
      (`SceneComponent.SetHiddenInGame` _rootcomponent_2 true false))))

(fn `SwitchLightEnvironmentTOExterior`
  ;[0.03035 0.3644 1] Switch Interor/Extirior Lighting
  ;;[1 1 1 -4.222] Exterior
  (`SceneComponent.SetVisibility` (`Actor.RootComponent` (`|ConvertAsset` (`self.Sun`))) true false)
  (`SceneComponent.SetVisibility` (`Actor.RootComponent` (`|ConvertAsset` (`self.Moon`))) true false)
  (`SceneComponent.SetVisibility` (`Actor.RootComponent` (`|ConvertAsset` (`self.Skylight_Exterior`))) true false)
  (`SceneComponent.SetVisibility` (`Actor.RootComponent` (`|ConvertAsset` (`self.Fog_exterior`))) true false)
  (`SceneComponent.SetHiddenInGame` (`Actor.RootComponent` (`|ConvertAsset` (`self.Fog_exterior`))) false false)
  (`SceneComponent.SetHiddenInGame` (`Actor.RootComponent` (`|ConvertAsset` (`self.Skylight_Exterior`))) false false)
  (`SceneComponent.SetHiddenInGame` (`Actor.RootComponent` (`|ConvertAsset` (`self.Moon`))) false false)
  (`SceneComponent.SetHiddenInGame` (`Actor.RootComponent` (`|ConvertAsset` (`self.Sun`))) false false)
  (`SceneComponent.SetVisibility` (`Actor.RootComponent` (`|ConvertAsset` (`self.Fog_Interior`))) false false)
  (`SceneComponent.SetVisibility` (`Actor.RootComponent` (`|ConvertAsset` (`self.Skylight_Interior`))) false false)
  (`SceneComponent.SetHiddenInGame` (`Actor.RootComponent` (`|ConvertAsset` (`self.Skylight_Interior`))) true false)
  (`SceneComponent.SetHiddenInGame` (`Actor.RootComponent` (`|ConvertAsset` (`self.Fog_Interior`))) true false))

(fn `UserConstructionScript`
  (bind _returnvalue (`PrimitiveComponent.CreateDynamicMaterialInstance` (`self.cylinder`) 0 "/Game/Material/Misc/diamond_Inst.diamond_Inst" "None"))
  (bind _output_get (set `self.Material` _returnvalue))
  (switch `/Game/data/carmods/enum_shops_carmods` (`self.enum_shop`)
    (:`NewEnumerator0`
      (`MaterialInstanceDynamic.SetVectorParameterValue` _output_get "Color" (struct :`R` 1.0 :`A` 1.0)))
    (:`NewEnumerator1`
      (`MaterialInstanceDynamic.SetVectorParameterValue` _output_get "Color" (struct :`G` 1.0 :`A` 1.0)))
    (:`NewEnumerator2`
      (`MaterialInstanceDynamic.SetVectorParameterValue` _output_get "Color" (struct :`R` 1.0 :`G` 0.319111 :`B` 0.067083 :`A` 1.0)))))