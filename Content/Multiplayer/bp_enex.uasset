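; Entrance/exit marker with an animated yellow diamond that teleports an overlapping player within the level or between the persistent level and a streamed interior.
; Entering creates or loads a level instance at a set offset, polls until ready, then finds the tagged target marker; exiting unloads it.
; SpawnLocation line-traces for ground, retrying until hit, then moves player 0 there.
; Transitions pause input, set the weather manager's interior flag and swap interior/exterior lighting.
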(event `self.ReceiveTick`
  (params (DeltaSeconds :type "Float (single-precision)"))
  ;[1 1 1] Movement
  (bind (_direction _newtrack_0) (`Timeline|Movement` :!label _label)
    (:`Update`
      (bind _output_get (set `self.GoToRotation` (`KismetMathLibrary.VLerp` (stale `self.ReceiveBeginPlay` _output_get) (`KismetMathLibrary.MakeVector` (.x (stale `self.ReceiveBeginPlay` _output_get)) (.y (stale `self.ReceiveBeginPlay` _output_get)) (+ (.z (stale `self.ReceiveBeginPlay` _output_get)) 45.0)) _newtrack_0)))
      (`SceneComponent.K2_SetRelativeLocation` (`self.diamond_3`) _output_get false false))
    (:`Finished`
      (switch `ETimelineDirection` _direction
        (:`Forward`
          (goto _label :!via `PlayFromStart`))
        (:`Backward`
          (goto _label :!via `ReverseFromEnd`))))))

(event `self.ReceiveBeginPlay`
  ;[1 1 1] Movement
  (bind _output_get (set `self.InitRotation` (`SceneComponent.RelativeLocation` (`self.diamond_3`)))))

(event `self.Box.OnComponentBeginOverlap`
  (params (OverlappedComponent :type "PrimitiveComponent Object Reference") (OtherActor :type "Actor Object Reference") (OtherComp :type "PrimitiveComponent Object Reference") (OtherBodyIndex :type Integer) (bFromSweep :type Boolean) (SweepResult :type "HitResult Structure (by ref)"))
  (bind _newlevelinstance_name (`self.NewLevelInstance-Name`))
  (bind _returnvalue (`GameplayStatics.GetStreamingLevel` _newlevelinstance_name))
  (bind _returnvalue_2 (`GameplayStatics.GetStreamingLevel` (`self.NewLevelInstance-Name`)))
  (bind _rootcomponent (`Actor.RootComponent` (`|ConvertAsset` (`self.Sun`))))
  (bind _billboard (`/Game/Multiplayer/bp_enex.Billboard` (`|ConvertAsset` (`self.PersistentLvlTargetEnex`))))
  (bind _rootcomponent_2 (`Actor.RootComponent` (`|ConvertAsset` (`self.Fog_Interior`))))
  ;[1 1 1] Load / unload level and teleport
  (bind _asplayer (cast `/Game/Player/blueprint/player` OtherActor))
  (`MovementComponent.StopMovementImmediately` (`Character.CharacterMovement` _asplayer))
  (`self.DisableInput` _asplayer (`GameplayStatics.GetPlayerController` 0))
  (if (`self.todifferentlevel`)
    (if (`self.toInterior`)
      (bind _weathermanager (`/Game/Player/blueprint/player.weathermanager` _asplayer))
      (set `/Game/data/timecycle/weatherManager.interior` true _weathermanager)
      (if (not (`LevelStreaming.IsLevelLoaded` _returnvalue))
        (`/Engine/EditorBlueprintResources/StandardMacros.IsValid` _returnvalue
          (:`Is Valid`
            _)
          (:`Is Not Valid`
            (`LevelStreaming.CreateInstance` (`GameplayStatics.GetStreamingLevel` (`self.LevelToLoad-Name`)) (`KismetStringLibrary.Conv_NameToString` _newlevelinstance_name))))
        (set `LevelStreaming.LevelTransform` (`KismetMathLibrary.MakeTransform` (* (`self.InstanceLocation(meter)`) 100.0)) _returnvalue_2)
        (set `LevelStreaming.bShouldBeLoaded` true _returnvalue_2)
        (set `LevelStreaming.bShouldBeVisible` true _returnvalue_2)
        (if (and (`LevelStreaming.IsLevelVisible` _returnvalue_2) (`LevelStreaming.IsLevelLoaded` _returnvalue_2)) :!label _label_2
          _
          (else
            (`KismetSystemLibrary.Delay` 0.2)
            (goto _label_2))))
      (bind _outactors (`GameplayStatics.GetAllActorsOfClass` "bp_enex_C"))
      (for _array_element _outactors
        (if (`self.ActorHasTag` _array_element (`self.EnexTarget-Name`))
          (`self.SpawnLocation` (`/Game/Multiplayer/bp_enex.Billboard` _array_element) _asplayer)
          (`self.EnableInput` _asplayer (`GameplayStatics.GetPlayerController` 0) :!label _label_3)
          ;;[0.03035 0.3644 1] Switch Interor/Exterior Lighting
          (if (`self.toInterior`)
            ;;;[1 1 1 -34.73] Interior
            (`SceneComponent.SetVisibility` _rootcomponent false false)
            (`SceneComponent.SetVisibility` (`Actor.RootComponent` (`|ConvertAsset` (`self.Moon`))) false false)
            (`SceneComponent.SetVisibility` (`Actor.RootComponent` (`|ConvertAsset` (`self.Skylight_Exterior`))) false false)
            (`SceneComponent.SetVisibility` (`Actor.RootComponent` (`|ConvertAsset` (`self.Fog_exterior`))) false false)
            (`SceneComponent.SetHiddenInGame` _rootcomponent true false)
            (`SceneComponent.SetHiddenInGame` (`Actor.RootComponent` (`|ConvertAsset` (`self.Moon`))) true false)
            (`SceneComponent.SetHiddenInGame` (`Actor.RootComponent` (`|ConvertAsset` (`self.Skylight_Exterior`))) true false)
            (`SceneComponent.SetHiddenInGame` (`Actor.RootComponent` (`|ConvertAsset` (`self.Fog_exterior`))) true false)
            (`SceneComponent.SetVisibility` _rootcomponent_2 true false)
            (`SceneComponent.SetVisibility` (`Actor.RootComponent` (`|ConvertAsset` (`self.Skylight_Interior`))) true false)
            (`SceneComponent.SetHiddenInGame` _rootcomponent_2 false false)
            (`SceneComponent.SetHiddenInGame` (`Actor.RootComponent` (`|ConvertAsset` (`self.Skylight_Interior`))) false false)
            (else
              ;;;[1 1 1 -4.222] Exterior
              (`SceneComponent.SetVisibility` _rootcomponent true false)
              (`SceneComponent.SetVisibility` (`Actor.RootComponent` (`|ConvertAsset` (`self.Moon`))) true false)
              (`SceneComponent.SetVisibility` (`Actor.RootComponent` (`|ConvertAsset` (`self.Skylight_Exterior`))) true false)
              (`SceneComponent.SetVisibility` (`Actor.RootComponent` (`|ConvertAsset` (`self.Fog_exterior`))) true false)
              (`SceneComponent.SetHiddenInGame` (`Actor.RootComponent` (`|ConvertAsset` (`self.Fog_exterior`))) false false)
              (`SceneComponent.SetHiddenInGame` (`Actor.RootComponent` (`|ConvertAsset` (`self.Skylight_Exterior`))) false false)
              (`SceneComponent.SetHiddenInGame` (`Actor.RootComponent` (`|ConvertAsset` (`self.Moon`))) false false)
              (`SceneComponent.SetHiddenInGame` _rootcomponent false false)
              (`SceneComponent.SetVisibility` _rootcomponent_2 false false)
              (`SceneComponent.SetVisibility` (`Actor.RootComponent` (`|ConvertAsset` (`self.Skylight_Interior`))) false false)
              (`SceneComponent.SetHiddenInGame` (`Actor.RootComponent` (`|ConvertAsset` (`self.Skylight_Interior`))) true false)
              (`SceneComponent.SetHiddenInGame` _rootcomponent_2 true false)))))
      (else
        (set `/Game/data/timecycle/weatherManager.interior` false _weathermanager)
        ;;[1 0 0.09414] Unload Level
        (`self.SpawnLocation` _billboard _asplayer)
        (set `LevelStreaming.bShouldBeLoaded` false (`GameplayStatics.GetStreamingLevel` (`self.NewLevelInstance-Name`)))
        (goto _label_3)))
    (else
      (`self.SpawnLocation` _billboard _asplayer)
      (goto _label_3))))

(fn `UserConstructionScript`
  (bind _returnvalue (`PrimitiveComponent.CreateDynamicMaterialInstance` (`self.diamond_3`) 0 "/Game/Material/Misc/diamond_Inst.diamond_Inst" "None"))
  (bind _output_get (set `self.Material` _returnvalue))
  (`MaterialInstanceDynamic.SetVectorParameterValue` _output_get "Color" (struct :`R` 1.0 :`G` 1.0 :`A` 1.0)))