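; Gym free-time marker: a cylinder that starts a workout sequence when the player enters its capsule.
; Overlap flags the player as in the gym, disables input, switches the view to this actor, hides and snaps the player to the cylinder, then plays a pickup montage before calling gym HUD and logic.
; End overlap reshows the cylinder; the construction script tints its dynamic material by shop-type enum.
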(event `self.ReceiveBeginPlay`)

(event `self.Capsule.OnComponentBeginOverlap`
  (params (OverlappedComponent :type "PrimitiveComponent Object Reference") (OtherActor :type "Actor Object Reference") (OtherComp :type "PrimitiveComponent Object Reference") (OtherBodyIndex :type Integer) (bFromSweep :type Boolean) (SweepResult :type "HitResult Structure (by ref)"))
  (bind _cylinder (`self.cylinder`))
  (bind (_returnvalue_x _returnvalue_y) (`KismetMathLibrary.BreakVector` (`SceneComponent.K2_GetComponentLocation` _cylinder)))
  (bind (_returnvalue_roll _returnvalue_pitch _returnvalue_yaw) (`KismetMathLibrary.BreakRotator` (`SceneComponent.K2_GetComponentRotation` _cylinder)))
  (`ActorComponent.SetActive` (`self.Camera_Body`) true false)
  (bind _asplayer (cast `/Game/Player/blueprint/player` OtherActor))
  (bind _output_get (set `self.Ref_Player` _asplayer))
  (set `/Game/Player/blueprint/player.inGym` true _output_get)
  (`self.DisableInput` _output_get (`GameplayStatics.GetPlayerController` 0))
  (`|ExecutionSequence`
    (:`then_0`
      (`MovementComponent.StopMovementImmediately` (`Character.CharacterMovement` _output_get))
      (`PlayerController.SetViewTargetWithBlend` (`GameplayStatics.GetPlayerController` 0) self 0.0 "VTBlend_Linear" 0.0 false)
      (bind _returnvalue (`Character.PlayAnimMontage` _output_get "/Game/Player/animations/freeweights/gym_free_pickup_Montage.gym_free_pickup_Montage" 1.0 "None"))
      (`KismetSystemLibrary.Delay` _returnvalue)
      (`/Game/Player/blueprint/player.hud_gym` _output_get)
      (`/Game/Player/blueprint/player.Gym` _output_get))
    (:`then_1`
      (`SceneComponent.SetHiddenInGame` (`self.cylinder`) true false)
      (bind (_returnvalue_x_2 _returnvalue_y_2 _returnvalue_z) (`KismetMathLibrary.BreakVector` (`self.K2_GetActorLocation` _output_get)))
      ;[1 0 0] Set Player Location and Rotation TEMP
      (`self.K2_SetActorLocationAndRotation` _output_get (`KismetMathLibrary.MakeVector` _returnvalue_x _returnvalue_y _returnvalue_z) (`KismetMathLibrary.MakeRotator` 0.0 0.0 _returnvalue_yaw) false false))))

(event `self.Capsule.OnComponentEndOverlap`
  (params (OverlappedComponent :type "PrimitiveComponent Object Reference") (OtherActor :type "Actor Object Reference") (OtherComp :type "PrimitiveComponent Object Reference") (OtherBodyIndex :type Integer))
  (`SceneComponent.SetHiddenInGame` (`self.cylinder`) false false))

(fn `UserConstructionScript`
  (bind _returnvalue (`PrimitiveComponent.CreateDynamicMaterialInstance` (`self.cylinder`) 0 "/Game/Material/ingame/diamond_Inst.diamond_Inst" "None"))
  (bind _output_get (set `self.Material` _returnvalue))
  (switch `/Game/data/shoppingOLD/enum_shops` (`self.enum_shop`)
    (:`NewEnumerator0`
      (`MaterialInstanceDynamic.SetVectorParameterValue` _output_get "Color" (struct :`R` 0.090642 :`G` 0.850048 :`B` 1.0 :`A` 1.0) :!label _label))
    (:`NewEnumerator1`
      (goto _label))
    (:`NewEnumerator2`
      (goto _label))
    (:`NewEnumerator3`
      (goto _label))
    (:`NewEnumerator4`
      (goto _label))
    (:`NewEnumerator5`
      (goto _label))
    (:`NewEnumerator6`
      (goto _label))
    (:`NewEnumerator7`
      (`MaterialInstanceDynamic.SetVectorParameterValue` _output_get "Color" (struct :`R` 1.0 :`G` 0.093989 :`B` 0.766463 :`A` 1.0) :!label _label_2))
    (:`NewEnumerator8`
      (goto _label_2))
    (:`NewEnumerator9`
      (goto _label_2))
    (:`NewEnumerator18`
      (goto _label))
    (:`NewEnumerator19`
      (`MaterialInstanceDynamic.SetVectorParameterValue` _output_get "Color" (struct :`B` 1.0 :`A` 1.0)))
    (:`NewEnumerator15`
      (`MaterialInstanceDynamic.SetVectorParameterValue` _output_get "Color" (struct :`R` 1.0 :`G` 1.0 :`A` 1.0) :!label _label_3))
    (:`NewEnumerator16`
      (goto _label_3))))