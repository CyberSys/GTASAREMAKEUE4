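; Car upgrade Blueprint that provides the camera views for browsing vehicle mod categories such as bumpers, wheels, nitro and colors.
; On BeginPlay it activates the front camera component and deactivates the rear one.
; ViewTarget maps the EnumModcam value to a camera child actor and blends player 0's view to it over a short time.
; Several categories share the front or rear camera instead of having their own.
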(event `self.ReceiveBeginPlay`
  (`ActorComponent.SetActive` (`self.camera_front`) true false)
  (`ActorComponent.SetActive` (`self.camera_rear`) false false))

(fn `UserConstructionScript`)

(fn `ViewTarget`
  (bind _childactor (`ChildActorComponent.ChildActor` (`self.camera_front`)))
  (bind _childactor_2 (`ChildActorComponent.ChildActor` (`self.camera_rear`)))
  (`PlayerController.SetViewTargetWithBlend` (`GameplayStatics.GetPlayerController` 0) (select `/Game/data/carmods/enum_modcam` (`self.enum_modcam`) :`NewEnumerator0` _childactor_2 :`NewEnumerator1` (`ChildActorComponent.ChildActor` (`self.camera_hood`)) :`NewEnumerator2` (`ChildActorComponent.ChildActor` (`self.camera_exhaust`)) :`NewEnumerator3` _childactor :`NewEnumerator4` _childactor :`NewEnumerator5` _childactor :`NewEnumerator6` _childactor :`NewEnumerator7` (`ChildActorComponent.ChildActor` (`self.camera_nitro`)) :`NewEnumerator8` _childactor_2 :`NewEnumerator9` (`ChildActorComponent.ChildActor` (`self.camera_roof`)) :`NewEnumerator10` _childactor_2 :`NewEnumerator11` _childactor :`NewEnumerator12` (`ChildActorComponent.ChildActor` (`self.camera_sideskirts`)) :`NewEnumerator13` (`ChildActorComponent.ChildActor` (`self.camera_wheels`)) :`NewEnumerator14` _childactor :`NewEnumerator15` (`ChildActorComponent.ChildActor` (`self.camera_colors`)) :`NewEnumerator16` (`ChildActorComponent.ChildActor` (`self.camera_numplate`))) 0.25 "VTBlend_Linear" 0.0 false))