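; Car bomb pickup marker, a red cylinder with a trigger capsule that fits a bomb to a player's car.
; When a player's controlled car enters, it binds EnterGarage to the car's stop event and stops it.
; EnterGarage flags the possessing player as carrying a bomb in that car, then re-enables input for player controller 0 after a three-second timer.
; Ending overlap unhides the cylinder, and debug prints remain in the overlap logic.
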(event `self.ReceiveBeginPlay`)

(event `Enter Garage`
  (remove `/Game/Vehicle/generic/blueprint/bp_car.StopVehicle` (stale `self.Capsule.OnComponentBeginOverlap` _asbp_car) (delegate `Enter Garage`))
  (bind _ref_player_possessing (`/Game/Vehicle/generic/blueprint/bp_car.Ref_Player_possessing` (stale `self.Capsule.OnComponentBeginOverlap` _asbp_car)))
  (set `/Game/Player/blueprint/player.HasBomb` true _ref_player_possessing)
  (set `/Game/Player/blueprint/player.carWithBomb` (stale `self.Capsule.OnComponentBeginOverlap` _asbp_car) _ref_player_possessing)
  (bind _returnvalue (`KismetSystemLibrary.K2_SetTimerDelegate` (delegate `ReleaseFromShop`) 3.0)))

(event `self.Capsule.OnComponentBeginOverlap`
  (params (OverlappedComponent :type "PrimitiveComponent Object Reference") (OtherActor :type "Actor Object Reference") (OtherComp :type "PrimitiveComponent Object Reference") (OtherBodyIndex :type Integer) (bFromSweep :type Boolean) (SweepResult :type "HitResult Structure (by ref)"))
  (`KismetSystemLibrary.PrintString` "Hello")
  (bind _asplayer_pc (cast `/Game/Player/blueprint/player_pc` (`self.GetInstigatorController` OtherActor)))
  (bind _returnvalue (`Controller.K2_GetPawn` _asplayer_pc))
  (bind _returnvalue_2 (== OtherActor _returnvalue))
  (`KismetSystemLibrary.PrintString` (`KismetStringLibrary.Conv_BoolToString` _returnvalue_2))
  (if _returnvalue_2
    (bind _asbp_car (cast `/Game/Vehicle/generic/blueprint/bp_car` _returnvalue))
    (add `/Game/Vehicle/generic/blueprint/bp_car.StopVehicle` _asbp_car (delegate `Enter Garage`))
    (`/Game/Vehicle/generic/blueprint/bp_car.Stop Vehicle` _asbp_car)))

(event `ReleaseFromShop`
  (`KismetSystemLibrary.K2_ClearAndInvalidateTimerHandle` (stale `Enter Garage` _returnvalue))
  (`self.EnableInput` (stale `self.Capsule.OnComponentBeginOverlap` _asbp_car) (`GameplayStatics.GetPlayerController` 0)))

(event `self.Capsule.OnComponentEndOverlap`
  (params (OverlappedComponent :type "PrimitiveComponent Object Reference") (OtherActor :type "Actor Object Reference") (OtherComp :type "PrimitiveComponent Object Reference") (OtherBodyIndex :type Integer))
  (`SceneComponent.SetHiddenInGame` (`self.cylinder`) false false))

(fn `UserConstructionScript`
  (bind _returnvalue (`PrimitiveComponent.CreateDynamicMaterialInstance` (`self.cylinder`) 0 "/Game/Material/Misc/diamond_Inst.diamond_Inst" "None"))
  (`MaterialInstanceDynamic.SetVectorParameterValue` _returnvalue "Color" (struct :`R` 1.0 :`A` 1.0)))