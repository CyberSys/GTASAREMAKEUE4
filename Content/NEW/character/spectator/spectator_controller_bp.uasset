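; Spectator player controller that adds debug-style controls for time and weather while observing the world.
; It creates a menu widget on BeginPlay and adds it to the viewport on F or Escape.
; Numpad plus and minus double or halve global time dilation within limits, while multiply steps the first TimeCycle actor's weather type with wraparound.
; Tick prints the controlled pawn's position in whole meters.
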(event `Key|F`
  (params (Key :type "Key Structure"))
  (:`Pressed`
    (`UserWidget.AddToViewport` (`self.menu`) 0 :!label _label)))

(event `Key|Escape`
  (params (Key :type "Key Structure"))
  (:`Pressed`
    (goto _label)))

(event `self.ReceiveTick`
  (params (DeltaSeconds :type "Float (single-precision)"))
  (`KismetSystemLibrary.PrintString` (`KismetStringLibrary.Conv_IntVectorToString` (`KismetMathLibrary.FTruncVector` (/ (`self.K2_GetActorLocation` (`self.K2_GetPawn`)) 100.0))) true true (struct :`R` 0.991007 :`G` 0.920669 :`B` 1.0 :`A` 1.0) 0.0))

(event `self.ReceiveBeginPlay`
  (bind _returnvalue (`|CreateWidget` "/Game/NEW/ui/widget/menu/menu.menu_C"))
  (set `self.menu` _returnvalue))

(event `Key|Add`
  (params (Key :type "Key Structure"))
  (:`Pressed`
    (`GameplayStatics.SetGlobalTimeDilation` (`KismetMathLibrary.FMin` (* (`GameplayStatics.GetGlobalTimeDilation`) 2.0) 16.0))))

(event `Key|Subtract`
  (params (Key :type "Key Structure"))
  (:`Pressed`
    (`GameplayStatics.SetGlobalTimeDilation` (`KismetMathLibrary.FMax` (/ (`GameplayStatics.GetGlobalTimeDilation`) 2.0) 0.03125))))

(event `Key|Multiply`
  (params (Key :type "Key Structure"))
  (:`Pressed`
    (bind _outactors (`GameplayStatics.GetAllActorsOfClass` "/Game/timecycle/TimeCycle.TimeCycle_C"))
    (bind _output (`|GetArrayItem` _outactors))
    (bind _returnvalue (+ (`/Game/timecycle/TimeCycle.NewWeatherType` _output) 1))
    (set `/Game/timecycle/TimeCycle.NewWeatherType` (cast `/Game/timecycle/data/WeatherType` (select `bool` (> _returnvalue 20) :`false` _returnvalue)) _output)))

(fn `UserConstructionScript`)