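; Spectator player character that provides a free-flying camera controlled by mouse and movement axes.
; Mouse input drives controller yaw and inverted pitch, while MoveForward and MoveRight add movement along control-rotation vectors, so forward travel follows the view pitch.
; GearUp and GearDown temporarily raise or lower MaxFlySpeed, restoring the default on release.
; Left Ctrl blocks the boost and Left Shift blocks the slowdown when held at press time.
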(event `self.ReceiveTick`
  (params (DeltaSeconds :type "Float (single-precision)")))

(event `InputAxisKey|MouseY`
  (params (AxisValue :type "Float (single-precision)"))
  (`self.AddControllerPitchInput` (* AxisValue -1.0)))

(event `InputAxis|MoveForward`
  (params (AxisValue :type "Float (single-precision)"))
  (bind (_returnvalue_roll _returnvalue_pitch _returnvalue_yaw) (`KismetMathLibrary.BreakRotator` (`self.GetControlRotation`)))
  (`self.AddMovementInput` (`KismetMathLibrary.GetForwardVector` (`KismetMathLibrary.MakeRotator` 0.0 _returnvalue_pitch _returnvalue_yaw)) AxisValue))

(event `InputAxisKey|MouseX`
  (params (AxisValue :type "Float (single-precision)"))
  (`self.AddControllerYawInput` AxisValue))

(event `InputAxis|MoveRight`
  (params (AxisValue :type "Float (single-precision)"))
  (bind (_returnvalue_roll _returnvalue_pitch _returnvalue_yaw) (`KismetMathLibrary.BreakRotator` (`self.GetControlRotation`)))
  (`self.AddMovementInput` (`KismetMathLibrary.GetRightVector` (`KismetMathLibrary.MakeRotator` 0.0 _returnvalue_pitch _returnvalue_yaw)) AxisValue))

(event `InputAction|GearUp`
  (params (Key :type "Key Structure"))
  (bind _charactermovement (`self.CharacterMovement`))
  (:`Pressed`
    (if (not (`PlayerController.IsInputKeyDown` (`GameplayStatics.GetPlayerController` 0) "LeftControl"))
      (set `CharacterMovementComponent.MaxFlySpeed` 80000.0 _charactermovement)))
  (:`Released`
    (set `CharacterMovementComponent.MaxFlySpeed` 10000.0 _charactermovement)))

(event `InputAction|GearDown`
  (params (Key :type "Key Structure"))
  (bind _charactermovement (`self.CharacterMovement`))
  (:`Pressed`
    (if (not (`PlayerController.IsInputKeyDown` (`GameplayStatics.GetPlayerController` 0) "LeftShift"))
      (set `CharacterMovementComponent.MaxFlySpeed` 1500.0 _charactermovement)))
  (:`Released`
    (set `CharacterMovementComponent.MaxFlySpeed` 10000.0 _charactermovement)))

(fn `UserConstructionScript`)