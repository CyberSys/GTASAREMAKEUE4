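; Player controller that creates the HUD on BeginPlay, exposes on-screen text messages through it and opens a menu widget on F.
; Axis inputs for movement and look (with optional Y inversion), plus sprint and walk states, are stored in its variables.
; Jump, crouch, fire, aim and action presses and releases go as Player_input interface messages to the controlled pawn, after an interface check, decoupling input from pawn logic.
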(event `InputAction|Jump`
  (params (Key :type "Key Structure"))
  (:`Pressed`
    (bind _controlledpawn (`self.ImplementsInputInterface?`)
      (:`True`
        (message `/Game/NEW/character/blueprint/player_input.JumpStart` _controlledpawn))))
  (:`Released`
    (bind _controlledpawn_2 (`self.ImplementsInputInterface?`)
      (:`True`
        (message `/Game/NEW/character/blueprint/player_input.JumpStop` _controlledpawn_2)))))

(event `InputAction|Crouch`
  (params (Key :type "Key Structure"))
  (:`Pressed`
    (bind _controlledpawn (`self.ImplementsInputInterface?`)
      (:`True`
        (message `/Game/NEW/character/blueprint/player_input.CrouchStart` _controlledpawn))))
  (:`Released`
    (bind _controlledpawn_2 (`self.ImplementsInputInterface?`)
      (:`True`
        (message `/Game/NEW/character/blueprint/player_input.CrouchStop` _controlledpawn_2)))))

(event `InputAction|Inventory`
  (params (Key :type "Key Structure")))

(event `InputAction|Sprint`
  (params (Key :type "Key Structure"))
  (:`Pressed`
    (set `self.Sprint` true))
  (:`Released`
    (set `self.Sprint` false)))

(event `InputAction|fire`
  (params (Key :type "Key Structure"))
  (:`Pressed`
    (bind _controlledpawn (`self.ImplementsInputInterface?`)
      (:`True`
        (message `/Game/NEW/character/blueprint/player_input.FireStart` _controlledpawn))))
  (:`Released`
    (bind _controlledpawn_2 (`self.ImplementsInputInterface?`)
      (:`True`
        (message `/Game/NEW/character/blueprint/player_input.FireStop` _controlledpawn_2)))))

(event `InputAction|action`
  (params (Key :type "Key Structure"))
  (:`Pressed`
    (bind _controlledpawn (`self.ImplementsInputInterface?`)
      (:`True`
        (message `/Game/NEW/character/blueprint/player_input.ActionStart` _controlledpawn))))
  (:`Released`
    (bind _controlledpawn_2 (`self.ImplementsInputInterface?`)
      (:`True`
        (message `/Game/NEW/character/blueprint/player_input.ActionStop` _controlledpawn_2)))))

(event `InputAction|walk`
  (params (Key :type "Key Structure"))
  (:`Pressed`
    (set `self.Walk` true))
  (:`Released`
    (set `self.Walk` false)))

(event `InputAction|walk`
  (params (Key :type "Key Structure")))

(event `InputAction|aim`
  (params (Key :type "Key Structure"))
  (:`Pressed`
    (bind _controlledpawn (`self.ImplementsInputInterface?`)
      (:`True`
        (message `/Game/NEW/character/blueprint/player_input.AimWeaponStart` _controlledpawn))))
  (:`Released`
    (bind _controlledpawn_2 (`self.ImplementsInputInterface?`)
      (:`True`
        (message `/Game/NEW/character/blueprint/player_input.AimWeaponStop` _controlledpawn_2)))))

(event `InputAxis|right`
  (params (AxisValue :type "Float (single-precision)"))
  (set `self.left/right` AxisValue))

(event `InputAxis|forward`
  (params (AxisValue :type "Float (single-precision)"))
  (set `self.forward/backward` AxisValue))

(event `InputAxis|X`
  (params (AxisValue :type "Float (single-precision)"))
  (set `self.look_left/right` AxisValue))

(event `InputAxis|Y`
  (params (AxisValue :type "Float (single-precision)"))
  (set `self.look_up/down` (* AxisValue (`KismetMathLibrary.SelectFloat` -1.0 1.0 (not (`self.InvertY`))))))

(event `Key|F`
  (params (Key :type "Key Structure"))
  (:`Pressed`
    (bind _returnvalue (`|CreateWidget` "/Game/NEW/ui/widget/menu/menu.menu_C"))
    (bind _output_get (set `self.Menu` _returnvalue))
    (`UserWidget.AddToViewport` _output_get 0)))

(event `self.ReceiveBeginPlay`
  (`self.PlayerINI`))

(event `self.ReceiveTick`
  (params (DeltaSeconds :type "Float (single-precision)")))

(event `/Game/NEW/character/blueprint/player_interact.ShowText`
  (params (text :type Text) (time :type "Float (single-precision)"))
  (message `/Game/NEW/character/blueprint/player_interact.ShowText` (`self.HUD`) text time))

(fn `PlayerINI`
  (bind _returnvalue (`|CreateWidget` "/Game/NEW/userinterface/widget/hud.hud_C"))
  (bind _output_get (set `self.HUD` _returnvalue))
  (`UserWidget.AddToViewport` _output_get 0))

(fn `UserConstructionScript`)