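; Tram stop Blueprint that halts a tram for a timed pause when it enters the stop's box.
; On overlap it saves the tram_bp's Input, zeroes it, and starts a one-shot timer.
; When the timer fires, GoOn restores the saved Input.
; If SwitchDestination is set, GoOn also copies four district variables into the tram's BExtra fields and calls its Destination function.
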(event `self.Box.OnComponentBeginOverlap`
  (params (OverlappedComponent :type "PrimitiveComponent Object Reference") (OtherActor :type "Actor Object Reference") (OtherComp :type "PrimitiveComponent Object Reference") (OtherBodyIndex :type Integer) (bFromSweep :type Boolean) (SweepResult :type "HitResult Structure (by ref)"))
  (bind _astram_bp (cast `/Game/Vehicle/train/tram_bp` OtherActor))
  (bind _output_get (set `self.Accelerate` (`/Game/Vehicle/train/train_bp.Input` _astram_bp)))
  (set `/Game/Vehicle/train/train_bp.Input` 0.0 _astram_bp)
  (`KismetSystemLibrary.K2_SetTimerDelegate` (delegate `GoOn`) 10.0))

(event `GoOn`
  (set `/Game/Vehicle/train/train_bp.Input` (stale `self.Box.OnComponentBeginOverlap` _output_get) (stale `self.Box.OnComponentBeginOverlap` _astram_bp))
  (if (`self.SwitchDestination?`)
    (set `/Game/Vehicle/train/tram_bp.b_extra1` (`self.CaltonHeights`) (stale `self.Box.OnComponentBeginOverlap` _astram_bp))
    (set `/Game/Vehicle/train/tram_bp.b_extra2` (`self.Chinatown`) (stale `self.Box.OnComponentBeginOverlap` _astram_bp))
    (set `/Game/Vehicle/train/tram_bp.b_extra3` (`self.Downtown`) (stale `self.Box.OnComponentBeginOverlap` _astram_bp))
    (set `/Game/Vehicle/train/tram_bp.b_extra4` (`self.Garcia`) (stale `self.Box.OnComponentBeginOverlap` _astram_bp))
    (`/Game/Vehicle/train/tram_bp.destination` (stale `self.Box.OnComponentBeginOverlap` _astram_bp))))

(fn `UserConstructionScript`)