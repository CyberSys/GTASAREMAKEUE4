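; Track Blueprint that builds a spline from the Tracks data table in its construction script.
; Row positions are scaled by 100 with Y negated and added as CurveClamped local points, then the spline's leftover default end points are removed.
; SpawnTrain places Train_bp actors at Spacing intervals along the spline using local-space transforms, but its only call is disconnected, so it never runs.
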(event `self.ReceiveTick`
  (params (DeltaSeconds :type "Float (single-precision)")))

(event `self.ReceiveBeginPlay`)

(fn `paths`
  (params (tracks_data :type "DataTable Object Reference"))
  (bind _returnvalue (`AddComponent|NODE_AddSplineComponent-0`))
  (bind _output_get (set `self.spline` _returnvalue))
  (bind _outrownames (`DataTableFunctionLibrary.GetDataTableRowNames` tracks_data))
  (for (_array_element _array_index) _outrownames
    (bind _returnvalue_2 (`|GetDataTableRow` tracks_data (`KismetStringLibrary.Conv_StringToName` (`KismetStringLibrary.Conv_IntToString` (+ (`KismetStringLibrary.Conv_StringToInt` (`KismetStringLibrary.Conv_NameToString` _array_element)) 1))))
      (:`then`
        (bind (_x _y _z) (break `/Game/data/tracks/struct_tracks` _returnvalue_2))
        (bind _returnvalue_3 (+ _array_index 1))
        (`SplineComponent.AddSplinePointAtIndex` _output_get (`KismetMathLibrary.MakeVector` (* _x 100.0) (* _y -100.0) (* _z 100.0)) _returnvalue_3 "Local" true)
        (`SplineComponent.SetSplinePointType` _output_get _returnvalue_3 "CurveClamped" true))))
  ;[1 0.6751 0.1521] delet start and end point after loop so there are no additional points
  (`SplineComponent.RemoveSplinePoint` _output_get (`KismetArrayLibrary.Array_Length` _outrownames) true)
  (`SplineComponent.RemoveSplinePoint` _output_get 0 true))

(fn `Spawn Train`
  (bind _spline (`self.spline`))
  (bind _spacing (`self.Spacing`))
  ;[1 1 1] Spawn Train
  (for _index (range (+ (`.ReturnValue` (`KismetMathLibrary.FMod` (`SplineComponent.GetSplineLength` _spline) _spacing)) 1))
    (bind _returnvalue (* _index _spacing))
    (`|SpawnActorFromClass` "/Game/Vehicle/train/train_bp.train_bp_C" (`KismetMathLibrary.MakeTransform` (`SplineComponent.GetLocationAtDistanceAlongSpline` _spline _returnvalue "Local") (`SplineComponent.GetRotationAtDistanceAlongSpline` _spline _returnvalue "Local")) "Undefined" "OverrideRootScale" null null)))

(fn `UserConstructionScript`
  (`self.paths` (`self.tracks`)))