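; Map zone actor that places and sizes its box collision from a row in a data table.
; The construction script looks up its Name in DatMap and reads two corner positions, Pos1 and Pos2.
; A per-axis helper, ZoneSizeAndCoordinates, converts each pair into a center and half-extent scaled by 100, with Y negated to flip that axis.
; The center becomes the actor location and the half-extents become the Box extent.
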(event `self.ReceiveTick`
  (params (DeltaSeconds :type "Float (single-precision)")))

(fn `UserConstructionScript`
  ;[1 1 1] Set box collision
  (bind _returnvalue (`|GetDataTableRow` (`self.dat_map`) (`self.name`))
    (:`then`
      (bind (_pos1 _pos2) (break `/Game/data/zones/struct_map` _returnvalue))
      (bind (_boxextent _coordinates) (`self.zoneSizeAndCoordinates` (.x _pos1) (.x _pos2)))
      (bind (_boxextent_2 _coordinates_2) (`self.zoneSizeAndCoordinates` (* (.y _pos1) -1.0) (* (.y _pos2) -1.0)))
      (bind (_boxextent_3 _coordinates_3) (`self.zoneSizeAndCoordinates` (.z _pos1) (.z _pos2)))
      (`self.K2_SetActorLocation` (`KismetMathLibrary.MakeVector` _coordinates _coordinates_2 _coordinates_3))
      (`BoxComponent.SetBoxExtent` (`self.Box`) (`KismetMathLibrary.MakeVector` _boxextent _boxextent_2 _boxextent_3) true))))