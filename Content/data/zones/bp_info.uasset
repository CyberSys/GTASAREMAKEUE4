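; Zone info volume that places itself and sizes its box from the DatInfo data table row at index Id.
; The construction script turns two corner positions into center and extent, scaled by 100 with Y negated.
; Getter functions expose the row's name and GameName.
; The overlap event is empty; logic to show zone or island names on the player HUD is present but disconnected.
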(event `self.ReceiveActorBeginOverlap`
  (params (OtherActor :type "Actor Object Reference"))
  ;[1 1 1] Hud Zonename
)

(fn `getZoneName`
  (returns (name :type Name))
  (bind _outrownames (`DataTableFunctionLibrary.GetDataTableRowNames` (`self.dat_info`)))
  (return (`|GetArrayItem` _outrownames (`self.id`))))

(fn `getZoneText`
  (returns (name :type Name))
  (bind _outrownames (`DataTableFunctionLibrary.GetDataTableRowNames` (`self.dat_info`)))
  (bind _returnvalue (`|GetDataTableRow` (`self.dat_info`) (`|GetArrayItem` _outrownames (`self.id`)))
    (:`then`
      (return (`.gamename_39_65F5F65849061438B1B29986D28E9218` (break `/Game/data/zones/struct_info` _returnvalue))))))

(fn `UserConstructionScript`
  (bind _dat_info (`self.dat_info`))
  ;[1 1 1] Set box collision
  (bind _outrownames (`DataTableFunctionLibrary.GetDataTableRowNames` _dat_info))
  (bind _returnvalue (`|GetDataTableRow` _dat_info (`|GetArrayItem` _outrownames (`self.id`)))
    (:`then`
      (bind (_type _pos1 _pos2) (break `/Game/data/zones/struct_info` _returnvalue))
      (bind (_boxextent _coordinates) (`self.zoneSizeAndCoordinates` (.x _pos1) (.x _pos2)))
      (bind (_boxextent_2 _coordinates_2) (`self.zoneSizeAndCoordinates` (* (.y _pos1) -1.0) (* (.y _pos2) -1.0)))
      (bind (_boxextent_3 _coordinates_3) (`self.zoneSizeAndCoordinates` (.z _pos1) (.z _pos2)))
      (`self.K2_SetActorLocation` (`KismetMathLibrary.MakeVector` _coordinates _coordinates_2 _coordinates_3))
      (`BoxComponent.SetBoxExtent` (`self.Box`) (`KismetMathLibrary.MakeVector` _boxextent _boxextent_2 _boxextent_3) true))))