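; Sky sphere actor that colors the sky from a timecycle data table and tracks Sun and Moon actor rotations.
; Construction creates a dynamic sky material, then calls UpdateSunDirection to set light directions and derive star blending from sun pitch.
; That function samples color curves in the table's first row at Time for sky, sun core and low clouds.
; Event graph is empty, and older refresh logic with a no-Sun fallback is disconnected.
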(event `self.ReceiveTick`
  (params (DeltaSeconds :type "Float (single-precision)")))

(event `self.ReceiveBeginPlay`)

(fn `UpdateSunDirection`
  (bind _sky_material (`self.Sky material`))
  (bind _dat_timecyc (`self.dat_timecyc`))
  (bind _time (`self.time`))
  (bind _sun_height (`self.Sun height`))
  (`MaterialInstanceDynamic.SetVectorParameterValue` (`self.Sky material`) "MoonDirection" (`KismetMathLibrary.Conv_VectorToLinearColor` (`KismetMathLibrary.Conv_RotatorToVector` (`self.K2_GetActorRotation` (`self.moon`)))))
  (`MaterialInstanceDynamic.SetVectorParameterValue` (`self.Sky material`) "Light direction" (`KismetMathLibrary.Conv_VectorToLinearColor` (`KismetMathLibrary.Conv_RotatorToVector` (`self.K2_GetActorRotation` (`self.sun`)))))
  (set `self.Sun height` (`KismetMathLibrary.MapRangeUnclamped` (.pitch (`self.K2_GetActorRotation` (`self.sun`))) 0.0 -18.0 0.0 1.0))
  ;[1 1 1] Sky olor
  (bind _outrownames (`DataTableFunctionLibrary.GetDataTableRowNames` _dat_timecyc))
  (bind _returnvalue (`|GetDataTableRow` _dat_timecyc (`|GetArrayItem` _outrownames))
    (:`then`
      (bind (_amb _amb_obj _dir _sky_top _sky_bot _suncore _lowclouds) (break `/Game/data/timecyc/struct_timecyc` _returnvalue))
      (`MaterialInstanceDynamic.SetVectorParameterValue` _sky_material "Sky_top" (`CurveLinearColor.GetLinearColorValue` _sky_top _time))
      (`MaterialInstanceDynamic.SetVectorParameterValue` _sky_material "Sky_bot" (`CurveLinearColor.GetLinearColorValue` _sky_bot _time))
      (`MaterialInstanceDynamic.SetVectorParameterValue` _sky_material "SunCore" (`CurveLinearColor.GetLinearColorValue` _suncore _time))
      (`MaterialInstanceDynamic.SetVectorParameterValue` _sky_material "LowClouds" (`CurveLinearColor.GetLinearColorValue` _lowclouds _time))
      (`MaterialInstanceDynamic.SetScalarParameterValue` (`self.Sky material`) "Sun height" (`KismetMathLibrary.SelectFloat` (`KismetMathLibrary.Abs` _sun_height) 0.0 (< _sun_height 0.0))))))

(fn `UserConstructionScript`
  (bind _returnvalue (`PrimitiveComponent.CreateDynamicMaterialInstance` (`self.Sky Sphere mesh`) 0 "/Game/data/timecyc/Sky_mat.Sky_mat" "None"))
  (set `self.Sky material` _returnvalue)
  (`self.UpdateSunDirection`))