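; Pedestrian spawner for a GTA-style population cycle; currently only BeginPlay is live, caching the player controller, while the spawn logic is disconnected.
; The unwired graph rolls a weighted group from a popcycle DataTable, creates a random ped, then traces ground to spawn Bp_ped and start it walking.
; Helpers randomly offset the player's position, read zone gang and ped counts, and search path nodes within range.
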(event `self.ReceiveBeginPlay`
  (bind _asplayer_pc (cast `/Game/Player/blueprint/player_pc` (`GameplayStatics.GetPlayerController` 0)))
  (set `self.PlayerPC` _asplayer_pc))

(event `SpawnPed`)

(event `SwitchTime`
  (params (Hours :type "/Game/data/popcycle/enum_hours Enum" :default "NewEnumerator0") (Weekday :type "/Game/data/popcycle/enum_weekday Enum" :default "NewEnumerator0")))

(fn `GetNearestNodeinOverlappingZone`
  (params (ZoneNodes :type "Array of Vector2D Structure") (PlayerLocation :type "Vector2D Structure"))
  (returns (SpawnNode :type "Vector2D Structure"))
  (locals (tempnearestNode :type "Vector2D Structure"))
  (set `self.distance` 6000.0)
  (for _array_element ZoneNodes
    (bind (_x _y) (`KismetMathLibrary.BreakVector2D` _array_element))
    (bind _returnvalue (`|GetDataTableRow` (`|GetArrayItem` (`self.dat_ped`) (`KismetMathLibrary.FTrunc` _x)) (`KismetStringLibrary.Conv_StringToName` (`KismetStringLibrary.Conv_IntToString` (`KismetMathLibrary.FTrunc` _y))))
      (:`then`
        (bind ((`PosX_2_D572BE0742A650EA3D0E4CAC1F3FE955` _posx) (`PosY_4_F72151884933EF7C93500689E24A987C` _posy)) (break `/Game/data/Paths/peds/struct_nodes_peds` _returnvalue))
        (if (< (`KismetMathLibrary.VSize2D` (- (`KismetMathLibrary.MakeVector2D` _posx _posy) PlayerLocation)) (`self.distance`))
          (set `local.tempnearestNode` _array_element)))))
  (return (`local.tempnearestNode`)))

(fn `GetPlayerLocation`
  (returns (PlayerLocation :type "Vector2D Structure"))
  (bind _returnvalue (* (`KismetMathLibrary.RandomFloatInRange` 50.0 75.0) 100.0))
  (bind _returnvalue_2 (select `int` (`KismetMathLibrary.RandomInteger` 2) :`0` 1.0 :`1` -1.0 :!type "Float (single-precision)"))
  (bind (_returnvalue_x _returnvalue_y) (`KismetMathLibrary.BreakVector` (`self.K2_GetActorLocation` (`Controller.K2_GetPawn` (`self.PlayerPC`)))))
  (return (/ (`KismetMathLibrary.MakeVector2D` (+ _returnvalue_x (* _returnvalue _returnvalue_2)) (+ (* _returnvalue_y -1.0) (* _returnvalue _returnvalue_2))) 100.0)))

(fn `GetZoneInfos`
  (returns (ZoneNodes :type "Array of Vector2D Structure") (type :type Name) (Gang :type Name) (GangDensity :type Integer) (CurrentAmountPeds :type Integer))
  (bind _dat_info (`self.dat_info`))
  (bind _asbp_info (cast `/Game/data/zones/bp_info` (`|GetArrayItem` (`self.GetOverlappingActors` "/Game/data/zones/bp_info.bp_info_C"))))
  (bind _outrownames (`DataTableFunctionLibrary.GetDataTableRowNames` _dat_info))
  (bind _output (`|GetArrayItem` _outrownames (`/Game/data/zones/bp_info.id` _asbp_info)))
  (bind _returnvalue (`|GetDataTableRow` _dat_info _output)
    (:`then`
      (bind _asgta (cast `/Game/gta` (`GameplayStatics.GetGameMode`)))
      (bind _value (`BlueprintMapLibrary.Map_Find` (`/Game/gta.gangzones` _asgta) _output))
      (return _ "None" (break `/Game/data/zones/struct_gangzone` _value) (`.density_5_F780BF414E84876059D759832779145E` (break `/Game/data/zones/struct_gangzone` _value)) (`KismetArrayLibrary.Array_Length` (`self.GetOverlappingActors` _asbp_info "/Game/Peds/blueprints/bp_ped.bp_ped_C"))))))

(fn `UserConstructionScript`)