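; Parked car generator that spawns bp_car vehicles, chosen by row name from the DatVehicle table, at a given location and yaw.
; A vertical Visibility trace finds the surface, and the car's class-default first Length value lifts it above the hit.
; The Spawn event uses a long trace and retries every second until it hits, possibly waiting for ground to load.
; SetParkedCar makes a single attempt with a shorter trace.
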(event `Spawn`
  (params (Location :type "Vector Structure") (Angle :type "Float (double-precision)") (vehicle :type Name))
  (bind _returnvalue (`|GetDataTableRow` (`self.dat_vehicle`) vehicle)
    (:`then`
      (bind (_id _vehicle) (break `/Game/data/vehicles/struct_vehicles` _returnvalue))
      (bind _asbp_car (castclass `/Game/Vehicle/generic/blueprint/bp_car` _vehicle))
      (bind (_outhit _returnvalue_2) (`KismetSystemLibrary.LineTraceSingle` (+ Location (0.0 0.0 1000.0)) (- Location (0.0 0.0 1000.0)) "TraceTypeQuery1" :!label _label))
      (if _returnvalue_2
        (`|SpawnActorFromClass` _vehicle (`KismetMathLibrary.MakeTransform` (`KismetMathLibrary.MakeVector` (.x (`.Location` (`GameplayStatics.BreakHitResult` _outhit))) (.y (`.Location` (`GameplayStatics.BreakHitResult` _outhit))) (+ (.z (`.Location` (`GameplayStatics.BreakHitResult` _outhit))) (`|GetArrayItem` (`.Length` (defaults `/Game/data/bp_parked_car_generator` _asbp_car))))) (`KismetMathLibrary.MakeRotator` 0.0 0.0 Angle)) "Undefined" "OverrideRootScale" null null)
        (else
          (`KismetSystemLibrary.Delay` 1.0)
          (goto _label))))))

(fn `set_parked_car`
  (params (vehicle :type Name) (Location :type "Vector Structure") (Angle :type "Float (double-precision)"))
  (bind _returnvalue (`|GetDataTableRow` (`self.dat_vehicle`) vehicle)
    (:`then`
      (bind (_id _vehicle) (break `/Game/data/vehicles/struct_vehicles` _returnvalue))
      (bind _asbp_car (castclass `/Game/Vehicle/generic/blueprint/bp_car` _vehicle))
      (bind (_outhit _returnvalue_2) (`KismetSystemLibrary.LineTraceSingle` (+ Location (0.0 0.0 100.0)) (- Location (0.0 0.0 100.0)) "TraceTypeQuery1"))
      (if _returnvalue_2
        (`|SpawnActorFromClass` _vehicle (`KismetMathLibrary.MakeTransform` (`KismetMathLibrary.MakeVector` (.x (`.Location` (`GameplayStatics.BreakHitResult` _outhit))) (.y (`.Location` (`GameplayStatics.BreakHitResult` _outhit))) (+ (.z (`.Location` (`GameplayStatics.BreakHitResult` _outhit))) (`|GetArrayItem` (`.Length` (defaults `/Game/data/bp_parked_car_generator` _asbp_car))))) (`KismetMathLibrary.MakeRotator` 0.0 0.0 Angle)) "Undefined" "OverrideRootScale" null null)))))

(fn `UserConstructionScript`)