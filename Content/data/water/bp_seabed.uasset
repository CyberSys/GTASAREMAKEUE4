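; Seabed Blueprint that builds flat planes from the Water data table, with all work done in the construction script.
; Each row adds a WaterPlanes instance at the midpoint of Point1 and Point4, scaled by their absolute X and Y extents.
; Locations are multiplied by 100 with Y flipped to convert table coordinates to world space.
; Z scale stays at 1 because zero breaks material shading.
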(event `self.ReceiveTick`
  (params (DeltaSeconds :type "Float (single-precision)")))

(fn `UserConstructionScript`
  (bind _water (`self.water`))
  (bind _outrownames (`DataTableFunctionLibrary.GetDataTableRowNames` _water))
  (for _array_element _outrownames
    (bind _returnvalue (`|GetDataTableRow` _water _array_element)
      (:`then`
        (bind (_point_1 _point_1_speed _point_1_wave _point_1_waveheight _point_2 _point_2_speed _point_2_wave _point_2_waveheight _point_3 _point_3_speed _point_3_wave _point_3_waveheight _point_4) (break `/Game/data/water/struct_water` _returnvalue))
        (bind _returnvalue_2 (- _point_1 _point_4))
        (`InstancedStaticMeshComponent.AddInstanceWorldSpace` (`self.water_planes`) (`KismetMathLibrary.MakeTransform` (* (+ (/ _returnvalue_2 2.0) _point_4) (100.0 -100.0 100.0)) (struct) (`KismetMathLibrary.MakeVector` (.x (`KismetMathLibrary.Vector_GetAbs` _returnvalue_2)) (.y (`KismetMathLibrary.Vector_GetAbs` _returnvalue_2)) 1.0))) ; z factor has to be 1 - factor 0 produces material artifacts (wrong shading)
      ))))