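; Water Blueprint that builds water instances from the Water data table and switches environment state through an overlap box.
; The construction script adds one instanced mesh per row, centered and scaled between two corner points, converting to centimeters with Y flipped.
; BeginPlay hides its sky light, directional light and height fog.
; Box overlaps toggle the Timecycle actor's Interior flag and switch lighting and post-process modes on entry and exit.
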(event `self.ReceiveBeginPlay`
  (`SceneComponent.SetHiddenInGame` (`self.SkyLight`) true false)
  (`SceneComponent.SetHiddenInGame` (`self.DirectionalLight`) true false)
  (`SceneComponent.SetHiddenInGame` (`self.ExponentialHeightFog`) true false))

(event `self.Box.OnComponentBeginOverlap`
  (params (OverlappedComponent :type "PrimitiveComponent Object Reference") (OtherActor :type "Actor Object Reference") (OtherComp :type "PrimitiveComponent Object Reference") (OtherBodyIndex :type Integer) (bFromSweep :type Boolean) (SweepResult :type "HitResult Structure (by ref)"))
  (bind _outactors (`GameplayStatics.GetAllActorsOfClass` "/Game/data/timecycle/timecycle.timecycle_C"))
  (bind _astimecycle (cast `/Game/data/timecycle/timecycle` (`|GetArrayItem` _outactors)))
  (set `/Game/data/timecycle/timecycle.interior` true _astimecycle)
  (`/Game/data/bpfl_world.SwitchLighting` "NewEnumerator2")
  (`/Game/data/bpfl_world.SwitchPostProcess` "NewEnumerator2"))

(event `self.Box.OnComponentEndOverlap`
  (params (OverlappedComponent :type "PrimitiveComponent Object Reference") (OtherActor :type "Actor Object Reference") (OtherComp :type "PrimitiveComponent Object Reference") (OtherBodyIndex :type Integer))
  (bind _outactors (`GameplayStatics.GetAllActorsOfClass` "/Game/data/timecycle/timecycle.timecycle_C"))
  (bind _astimecycle (cast `/Game/data/timecycle/timecycle` (`|GetArrayItem` _outactors)))
  (set `/Game/data/timecycle/timecycle.interior` false _astimecycle)
  (`/Game/data/bpfl_world.SwitchLighting` "NewEnumerator0")
  (`/Game/data/bpfl_world.SwitchPostProcess` "NewEnumerator0"))

(fn `UserConstructionScript`
  (bind _water (`self.water`))
  (bind _outrownames (`DataTableFunctionLibrary.GetDataTableRowNames` _water))
  (for _array_element _outrownames
    (bind _returnvalue (`|GetDataTableRow` _water _array_element)
      (:`then`
        (bind (_point_1 _point_1_speed _point_1_wave _point_1_waveheight _point_2 _point_2_speed _point_2_wave _point_2_waveheight _point_3 _point_3_speed _point_3_wave _point_3_waveheight _point_4) (break `/Game/data/water/struct_water` _returnvalue))
        (bind _returnvalue_2 (- _point_1 _point_4))
        (`InstancedStaticMeshComponent.AddInstance` (`self.HierarchicalInstancedStaticMesh`) (`KismetMathLibrary.MakeTransform` (* (+ (/ _returnvalue_2 2.0) _point_4) (100.0 -100.0 100.0)) (struct) (`KismetMathLibrary.Vector_GetAbs` _returnvalue_2)))))))