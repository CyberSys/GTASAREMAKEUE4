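; Train actor that rides along the spline of a referenced track, restarting from zero distance at the end.
; Each tick Acceleration ramps throttle toward Speed or zero based on Input, and that value advances the spline distance and drives the engine sound's Speed parameter.
; Rear and front clack sounds fire at distance intervals offset by each bogie's position.
; Carriage spawning logic is present but unconnected.
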(event `self.ReceiveTick`
  (params (DeltaSeconds :type "Float (single-precision)"))
  (bind _tracksplinedistance (`self.TrackSplineDistance`))
  (bind _clackaudiodistance (`self.clackAudioDistance`))
  (bind _tracks (`self.tracks`))
  (bind _returnvalue (/ (`self.TrackSplineDistance`) 100.0))
  (bind _relativelocation_x (`KismetMathLibrary.BreakVector` (`SceneComponent.RelativeLocation` (`self.bogie_front`))))
  (bind _relativelocation_x_2 (`KismetMathLibrary.BreakVector` (`SceneComponent.RelativeLocation` (`self.bogie_rear`))))
  (set `self.DeltaTime` DeltaSeconds)
  (`self.Acceleration`)
  (`AudioComponent.SetFloatParameter` (`self.Audio_Engine`) "Speed" (`self.ThrottleValue`))
  (bind _output_get (set `self.TrackSplineTotalLength` (`SplineComponent.GetSplineLength` (`/Game/data/tracks/bp_tracks.spline` _tracks)) :!label _label))
  (`/Engine/EditorBlueprintResources/StandardMacros.CompareFloat` (`self.TrackSplineDistance`) _output_get
    (:`>`
      ;[1 1 1] endless loop
      (set `self.TrackSplineDistance` 0.0 :!label _label_2))
    (:`==`
      (goto _label_2))
    (:`<`
      (`self.K2_SetActorLocationAndRotation` (+ (`SplineComponent.GetLocationAtDistanceAlongSpline` (`/Game/data/tracks/bp_tracks.spline` _tracks) _tracksplinedistance "World") (`KismetMathLibrary.MakeVector` 0.0 0.0 (`KismetMathLibrary.Conv_IntToDouble` (`self.Offset`)))) (`SplineComponent.GetRotationAtDistanceAlongSpline` (`/Game/data/tracks/bp_tracks.spline` _tracks) _tracksplinedistance "World"))
      (set `self.TrackSplineDistance` (+ (`self.TrackSplineDistance`) (`self.ThrottleValue`)))
      ;[1 1 1] Sound clack
      (if (== (`KismetMathLibrary.Round` (mod (`KismetMathLibrary.Abs` (+ _relativelocation_x_2 _returnvalue)) _clackaudiodistance)) 0)
        (`AudioComponent.Play` (`self.Audio_clack_r`) 0.0)
        (elif (== (`KismetMathLibrary.Round` (mod (`KismetMathLibrary.Abs` (+ _relativelocation_x _returnvalue)) _clackaudiodistance)) 0)
          (`AudioComponent.Play` (`self.Audio_clack_f`) 0.0))))))

(event `self.ReceiveBeginPlay`
  (set `self.TrackSplineDistance` (* (`self.StartLocationAlongSpline%`) (/ (`SplineComponent.GetSplineLength` (`/Game/data/tracks/bp_tracks.spline` (`self.tracks`))) 100.0)))
  (goto _label))

(fn `Acceleration`
  (bind _throttlevalue (`self.ThrottleValue`))
  (bind _deltatime (`self.DeltaTime`))
  (if (!= (`self.Input`) 0.0)
    (set `self.ThrottleValue` (`KismetMathLibrary.FMin` (+ _throttlevalue (* _deltatime 5.0)) (`self.Speed`)))
    (else
      (set `self.ThrottleValue` (`KismetMathLibrary.FMax` (- _throttlevalue (* _deltatime 5.0)))))))

(fn `UserConstructionScript`)