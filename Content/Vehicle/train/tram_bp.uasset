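; Tram vehicle Blueprint with four optional "Extra" components, apparently used for its destination display.
; The construction script hides all four extras in game, and the Destination function then sets each one's visibility from the BExtra booleans.
; The pairing is offset by one: BExtra1 to BExtra3 drive Extra2 to Extra4, and BExtra4 drives Extra1.
; The event graph has no active logic.
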(fn `destination`
  (for _index (range 4)
    (`SceneComponent.SetHiddenInGame` (select `int` _index :`0` (`self.extra2`) :`1` (`self.extra3`) :`2` (`self.extra4`) :`3` (`self.extra1`) :!type "SceneComponent Object Reference") (not (select `int` _index :`0` (`self.b_extra1`) :`1` (`self.b_extra2`) :`2` (`self.b_extra3`) :`3` (`self.b_extra4`))) false)))

(fn `UserConstructionScript`
  (`parent.UserConstructionScript`)
  (`SceneComponent.SetHiddenInGame` (`self.extra1`) true false)
  (`SceneComponent.SetHiddenInGame` (`self.extra2`) true false)
  (`SceneComponent.SetHiddenInGame` (`self.extra3`) true false)
  (`SceneComponent.SetHiddenInGame` (`self.extra4`) true false))