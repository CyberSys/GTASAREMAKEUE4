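; Player-driven car Blueprint with custom raycast suspension and tire physics on four wheels.
; Each tick it traces from every top link, computes spring-damper load, derives load-scaled drive and lateral forces, applies them to the chassis and animates the wheels.
; Input handles camera look, front-wheel steering and throttle, which feeds a torque-curve engine RPM simulation not yet linked to the tire forces.
; Debug traces, force lines and load prints remain active.
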(event `InputAxis|LookUp`
  (params (AxisValue :type "Float (single-precision)"))
  (`self.AddControllerPitchInput` (* AxisValue -1.0)))

(event `InputAxis|MoveRight`
  (params (AxisValue :type "Float (single-precision)"))
  (`self.Steering` AxisValue))

(event `InputAxis|LookRight`
  (params (AxisValue :type "Float (single-precision)"))
  (`self.AddControllerYawInput` AxisValue))

(event `InputAxis|Forward`
  (params (AxisValue :type "Float (single-precision)")))

(event `InputAxis|Throttle`
  (params (AxisValue :type "Float (single-precision)"))
  (`self.GetThrottleValue` AxisValue)
  (`self.GetEngineTorque`))

(event `self.ReceiveBeginPlay`
  (`PlayerController.SetViewTargetWithBlend` (`GameplayStatics.GetPlayerController` 0) (`ChildActorComponent.ChildActor` (`self.bp_camera`)) 0.0 "VTBlend_Linear" 0.0 false)
  (`self.StoreComponentsToArray`)
  (`self.RayCastINI`)
  (`self.SuspensionINI`)
  (`self.GetUnitConvertMult`))

(event `self.ReceiveTick`
  (params (DeltaSeconds :type "Float (single-precision)"))
  (set `self.DeltaTime` DeltaSeconds)
  (`self.RayCast`)
  (`self.UpdateSuspensionLength`)
  (`self.GetSuspensionForce`)
  (`self.ApplySuspensionForce`)
  (`self.UpdateWheelLocation`)
  (`self.GetWheelLinearVelocityLocal`)
  (`self.GetTireForce`)
  (`self.ApplyTireForce`)
  (`self.WheelRotation`)
  ;[1 1 1] DebugForces
  (for _index (range 4)
    (for _index_2 (range 3)
      (bind _returnvalue (`SceneComponent.K2_GetComponentLocation` (`|GetArrayItem` (`self.WheelComponent`) _index)))
      (bind _output (`|GetArrayItem` (`self.TopLinkComponent`) _index))
      (`KismetSystemLibrary.DrawDebugLine` _returnvalue (+ _returnvalue (* (select `int` _index_2 :`0` (`SceneComponent.GetForwardVector` _output) :`1` (`SceneComponent.GetRightVector` _output) :`2` (`SceneComponent.GetUpVector` _output)) (/ (select `int` _index_2 :`0` (`|GetArrayItem` (`self.Fx`) _index) :`1` (`|GetArrayItem` (`self.Fy`) _index) :`2` (`|GetArrayItem` (`self.Fz`) _index)) 8.75))) (select `int` _index_2 :`0` (struct :`R` 1.0 :`A` 1.0) :`1` (struct :`G` 1.0 :`A` 1.0) :`2` (struct :`B` 1.0 :`A` 1.0) :!type "LinearColor Structure") 0.0 8.0))))

(fn `ApplySuspensionForce`
  (for _index (range 4)
    (bind _output (`|GetArrayItem` (`self.TopLinkComponent`) _index))
    (`PrimitiveComponent.AddForceAtLocation` (`self.chassis`) (* (`SceneComponent.GetUpVector` _output) (* (`|GetArrayItem` (`self.Fz`) _index) 100.0)) (`SceneComponent.K2_GetComponentLocation` _output) "None")))

(fn `ApplyTireForce`
  (for _index (range 4)
    (if (`|GetArrayItem` (`self.WheelContact`) _index)
      (bind _output (`|GetArrayItem` (`self.TopLinkComponent`) _index))
      (bind (_output_bblockinghit _output_binitialoverlap _output_time _output_distance _output_location) (`GameplayStatics.BreakHitResult` (`|GetArrayItem` (`self.HitRes`) _index)))
      (`PrimitiveComponent.AddForceAtLocation` (`self.chassis`) (* (+ (* (`SceneComponent.GetForwardVector` _output) (`|GetArrayItem` (`self.Fx`) _index)) (* (`SceneComponent.GetRightVector` _output) (`|GetArrayItem` (`self.Fy`) _index))) 100.0) _output_location "None"))))

(fn `GetEngineTorque`
  (bind (_engine_torque_curve _engine_idle_rpm _engine_max_rpm _engine_inertia _engine_back_torque) (break `/Game/Vehicle/generic/blueprint/newcar/newEngineStruct` (`self.Engine`)))
  (bind _throttlevalue (`self.ThrottleValue`))
  (bind (_engine_torque_curve_2 _engine_idle_rpm_2 _engine_max_rpm_2) (break `/Game/Vehicle/generic/blueprint/newcar/newEngineStruct` (`self.Engine`)))
  (bind _rpm_to_radps (`self.RPM_to_RadPS`))
  ;[1 1 1] AngularAcceleration=Torque/Inertia
  (bind _output_get (set `self.EngineTorque` (`KismetMathLibrary.Lerp` _engine_back_torque (* (`CurveFloat.GetFloatValue` _engine_torque_curve (`self.EngineRPM`)) _throttlevalue) _throttlevalue)))
  (bind _output_get_2 (set `self.EngineAngularVelocity` (`KismetMathLibrary.FClamp` (+ (`self.EngineAngularVelocity`) (* (/ _output_get _engine_inertia) (`self.DeltaTime`))) (* _rpm_to_radps _engine_idle_rpm_2) (* _rpm_to_radps _engine_max_rpm_2))))
  (set `self.EngineRPM` (* _output_get_2 (`self.RadPS_to_RPM`))))

(fn `GetSuspensionForce`
  (for _index (range 4)
    (bind (_output_rest_length _output_travel _output_stiffness _output_damper _output_force_min _output_force_max) (break `/Game/Vehicle/generic/blueprint/newcar/newSuspensionStruct` (`|GetArrayItem` (`self.Suspension`) _index)))
    (bind _output (`|GetArrayItem` (`self.Length`) _index))
    (`KismetArrayLibrary.Array_Set` (`self.Fz`) _index (`KismetMathLibrary.FClamp` (+ (* (- _output_rest_length _output) _output_stiffness) (* _output_damper (/ (- (`|GetArrayItem` (`self.LastLength`) _index) _output) (`self.DeltaTime`)))) _output_force_min _output_force_max))
    (`KismetArrayLibrary.Array_Set` (`self.LastLength`) _index (`|GetArrayItem` (`self.Length`) _index))))

(fn `GetThrottleValue`
  (params (InputPin :type "Float (double-precision)"))
  (bind _throttlevalue (`self.ThrottleValue`))
  (bind _deltatime (`self.DeltaTime`))
  (if (`self.ThrottleFilter`)
    (if (!= InputPin 0.0)
      (set `self.ThrottleValue` (`KismetMathLibrary.FMin` (+ _throttlevalue (* _deltatime 1.0)) 1.0))
      (else
        (set `self.ThrottleValue` (`KismetMathLibrary.FMax` (- _throttlevalue (* _deltatime 2.0))))))
    (else
      (set `self.ThrottleValue` InputPin))))

(fn `GetTireForce`
  (for _index (range 4)
    (if (`|GetArrayItem` (`self.WheelContact`) _index)
      (bind _output (`|GetArrayItem` (`self.Fz`) _index))
      (`KismetArrayLibrary.Array_Set` (`self.Fx`) _index (* (`self.GetInputAxisValue`) _output 0.5))
      (bind (_output_x _output_y) (`KismetMathLibrary.BreakVector` (`|GetArrayItem` (`self.WheelLinearVelocityLocal`) _index)))
      (`KismetArrayLibrary.Array_Set` (`self.Fy`) _index (`KismetMathLibrary.FClamp` (* _output _output_y -1.0) (* _output -1.0) _output))
      (`KismetSystemLibrary.PrintString` (`KismetStringLibrary.Conv_DoubleToString` _output) true true (struct :`G` 0.66 :`B` 1.0 :`A` 1.0) 0.0)
      (else
        (`KismetArrayLibrary.Array_Set` (`self.Fx`) _index)
        (`KismetArrayLibrary.Array_Set` (`self.Fy`) _index)))))

(fn `GetUnitConvertMult`
  (bind _output_get (set `self.RPM_to_RadPS` (/ (* (`KismetMathLibrary.GetPI`) 2.0) 60.0)))
  (set `self.RadPS_to_RPM` (/ 1.0 _output_get)))

(fn `GetWheelLinearVelocityLocal`
  (for _index (range 4)
    (bind _output (`|GetArrayItem` (`self.TopLinkComponent`) _index))
    (bind _output_radius (break `/Game/Vehicle/generic/blueprint/newcar/newWheelStruct` (`|GetArrayItem` (`self.Wheel`) _index)))
    (bind _returnvalue (`PrimitiveComponent.GetPhysicsLinearVelocityAtPoint` (`self.chassis`) (- (`SceneComponent.K2_GetComponentLocation` (`|GetArrayItem` (`self.WheelComponent`) _index)) (* (`SceneComponent.GetUpVector` _output) _output_radius)) "None"))
    (`KismetArrayLibrary.Array_Set` (`self.WheelLinearVelocityLocal`) _index (`KismetMathLibrary.TransformDirection` (`KismetMathLibrary.InvertTransform` (`SceneComponent.K2_GetComponentToWorld` _output)) (/ _returnvalue 100.0)))))

(fn `RayCast`
  (for _index (range 4)
    (bind _output (`|GetArrayItem` (`self.TopLinkComponent`) _index))
    (bind _returnvalue (`SceneComponent.K2_GetComponentLocation` _output))
    (bind (_outhit _returnvalue_2) (`KismetSystemLibrary.LineTraceSingle` :`Start` _returnvalue :`End` (- _returnvalue (* (`SceneComponent.GetUpVector` _output) (`|GetArrayItem` (`self.RayLength`) _index))) :`TraceChannel` "TraceTypeQuery1" :`bTraceComplex` true :`DrawDebugType` "ForOneFrame"))
    (`KismetArrayLibrary.Array_Set` (`self.WheelContact`) _index _returnvalue_2)
    (if _returnvalue_2
      (`KismetArrayLibrary.Array_Set` (`self.HitRes`) _index _outhit))))

(fn `RayCastINI`
  (for _index (range 4)
    (bind (_output_rest_length _output_travel) (break `/Game/Vehicle/generic/blueprint/newcar/newSuspensionStruct` (`|GetArrayItem` (`self.Suspension`) _index)))
    (bind _output_radius (break `/Game/Vehicle/generic/blueprint/newcar/newWheelStruct` (`|GetArrayItem` (`self.Wheel`) _index)))
    (`KismetArrayLibrary.Array_Set` (`self.RayLength`) _index (+ (+ _output_rest_length _output_travel) _output_radius))))

(fn `Steering`
  (params (Axis :type "Float (double-precision)"))
  (bind _steeringanglemax (`self.SteeringAngleMax`))
  (bind _steeringangle (`self.SteeringAngle`))
  (if (!= Axis 0.0)
    (set `self.SteeringAngle` (`KismetMathLibrary.FClamp` (+ _steeringangle (* Axis (* (`self.DeltaTime`) 120.0))) (* _steeringanglemax -1.0) _steeringanglemax))
    (else
      (set `self.SteeringAngle` (* _steeringangle 0.7))))
  (`SceneComponent.K2_SetRelativeRotation` (`self.Toplink_FL`) (`KismetMathLibrary.MakeRotator` 0.0 0.0 (`self.SteeringAngle`)) false false)
  (`SceneComponent.K2_SetRelativeRotation` (`self.Toplink_FR`) (`KismetMathLibrary.MakeRotator` 0.0 0.0 (`self.SteeringAngle`)) false false))

(fn `StoreComponentsToArray`
  (for _index (range 4)
    (`KismetArrayLibrary.Array_Set` (`self.TopLinkComponent`) _index (select `int` _index :`0` (`self.Toplink_FL`) :`1` (`self.Toplink_FR`) :`2` (`self.Toplink_RL`) :`3` (`self.Toplink_RR`)))
    (`KismetArrayLibrary.Array_Set` (`self.WheelComponent`) _index (select `int` _index :`0` (`self.wheel_FL`) :`1` (`self.wheel_FR`) :`2` (`self.wheel_RL`) :`3` (`self.wheel_RR`) :!type "SceneComponent Object Reference"))))

(fn `SuspensionINI`
  (for _index (range 4)
    (bind _output_rest_length (break `/Game/Vehicle/generic/blueprint/newcar/newSuspensionStruct` (`|GetArrayItem` (`self.Suspension`) _index)))
    (`KismetArrayLibrary.Array_Set` (`self.Length`) _index _output_rest_length)
    (`KismetArrayLibrary.Array_Set` (`self.LastLength`) _index _output_rest_length)))

(fn `UpdateSuspensionLength`
  (for _index (range 4)
    (if (`|GetArrayItem` (`self.WheelContact`) _index)
      (bind _output (`|GetArrayItem` (`self.TopLinkComponent`) _index))
      (bind (_output_bblockinghit _output_binitialoverlap _output_time _output_distance _output_location) (`GameplayStatics.BreakHitResult` (`|GetArrayItem` (`self.HitRes`) _index)))
      (bind _output_radius (break `/Game/Vehicle/generic/blueprint/newcar/newWheelStruct` (`|GetArrayItem` (`self.Wheel`) _index)))
      (bind (_output_rest_length _output_travel) (break `/Game/Vehicle/generic/blueprint/newcar/newSuspensionStruct` (`|GetArrayItem` (`self.Suspension`) _index)))
      (`KismetArrayLibrary.Array_Set` (`self.Length`) _index (`KismetMathLibrary.FClamp` (`KismetMathLibrary.VSize` (- (`SceneComponent.K2_GetComponentLocation` _output) (+ _output_location (* (`SceneComponent.GetUpVector` _output) _output_radius)))) (- _output_rest_length _output_travel) (+ _output_rest_length _output_travel)))
      (else
        (bind (_output_rest_length_2 _output_travel_2) (break `/Game/Vehicle/generic/blueprint/newcar/newSuspensionStruct` (`|GetArrayItem` (`self.Suspension`) _index)))
        (`KismetArrayLibrary.Array_Set` (`self.Length`) _index (+ _output_rest_length_2 _output_travel_2))))))

(fn `UpdateWheelLocation`
  (for _index (range 4)
    (`SceneComponent.K2_SetRelativeLocation` (select `int` _index :`0` (`self.wheel_FL`) :`1` (`self.wheel_FR`) :`2` (`self.wheel_RL`) :`3` (`self.wheel_RR`)) (`KismetMathLibrary.MakeVector` 0.0 0.0 (* (`|GetArrayItem` (`self.Length`) _index) -1.0)) false false)))

(fn `UserConstructionScript`)

(fn `WheelRotation`
  (for _index (range 4)
    (bind _output_x (`KismetMathLibrary.BreakVector` (`|GetArrayItem` (`self.WheelLinearVelocityLocal`) _index)))
    (bind _output_radius (break `/Game/Vehicle/generic/blueprint/newcar/newWheelStruct` (`|GetArrayItem` (`self.Wheel`) _index)))
    (`SceneComponent.K2_AddLocalRotation` (select `int` _index :`0` (`self.wheel_FL`) :`1` (`self.wheel_FR`) :`2` (`self.wheel_RL`) :`3` (`self.wheel_RR`)) (`KismetMathLibrary.MakeRotator` 0.0 (* (`KismetMathLibrary.RadiansToDegrees` (* (/ _output_x (/ _output_radius 100.0)) (`self.DeltaTime`))) (select `int` _index :`0` 1.0 :`1` -1.0 :`2` 1.0 :`3` -1.0 :!type "Float (single-precision)"))) false false)))