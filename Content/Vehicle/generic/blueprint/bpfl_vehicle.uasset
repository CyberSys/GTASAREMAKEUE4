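; Blueprint function library for modular vehicle meshes, handling part lookup, car-mod replacement and damage states.
; Parts are static mesh components found by attach socket (wheels by parent tag), with the mesh name stored in the first component tag.
; Mod name prefixes or socket names expand to socket groups, covering paired parts and four wheels.
; Other helpers read model and handling flags from data tables and give wheel rotation per side.
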(fn `getCarmodSocket`
  (params (meshname :type Name))
  (returns (sockets :type "Array of Name"))
  (locals (tempname :type "Array of Name"))
  (bind _tempname (`local.tempname`))
  (bind _tempname_2 (`local.tempname`))
  (bind _tempname_3 (`local.tempname`))
  (`KismetArrayLibrary.Array_Clear` (`local.tempname`))
  (switch `string` (`KismetStringLibrary.GetSubstring` (`KismetStringLibrary.Conv_NameToString` meshname) 0 3)
    (:`bbb`
      (`KismetArrayLibrary.Array_Add` _tempname_3 "ug_backbullbar"))
    (:`fbb`
      (`KismetArrayLibrary.Array_Add` _tempname_3 "ug_frontbullbar"))
    (:`bnt`
      (`KismetArrayLibrary.Array_Add` _tempname_3 "ug_bonnet_left")
      (`KismetArrayLibrary.Array_Add` (`local.tempname`) "ug_bonnet_right"))
    (:`fbm`
      (`KismetArrayLibrary.Array_Add` _tempname_3 "bump_front_dummy"))
    (:`lgt`
      (`KismetArrayLibrary.Array_Add` _tempname_3 "ug_lights"))
    (:`mis`
      (`KismetArrayLibrary.Array_Add` _tempname_3 "misc_c"))
    (:`nto`
      (`KismetArrayLibrary.Array_Add` _tempname "ug_nitro"))
    (:`rbm`
      (`KismetArrayLibrary.Array_Add` _tempname "bump_rear_dummy"))
    (:`rf_`
      (`KismetArrayLibrary.Array_Add` _tempname "ug_roof"))
    (:`spl`
      (`KismetArrayLibrary.Array_Add` _tempname "ug_spoiler"))
    (:`wg_`
      (`KismetArrayLibrary.Array_Add` _tempname "ug_wing_left")
      (`KismetArrayLibrary.Array_Add` (`local.tempname`) "ug_wing_right"))
    (:`whe`
      (`KismetArrayLibrary.Array_Add` _tempname "wheel_lb_dummy")
      (`KismetArrayLibrary.Array_Add` _tempname_2 "wheel_lf_dummy")
      (`KismetArrayLibrary.Array_Add` _tempname_2 "wheel_rb_dummy")
      (`KismetArrayLibrary.Array_Add` _tempname_2 "wheel_rf_dummy")))
  (return (`local.tempname`)))

(fn `getCarmodSockets`
  (params (Socket :type Name))
  (returns (sockets :type "Array of Name"))
  (locals (tempname :type "Array of Name"))
  (bind _returnvalue (`KismetStringLibrary.Conv_NameToString` Socket))
  (bind _tempname (`local.tempname`))
  (bind _tempname_2 (`local.tempname`))
  (bind _tempname_3 (`local.tempname`))
  (if (`KismetStringLibrary.Contains` _returnvalue "ug_bonnet")
    (`KismetArrayLibrary.Array_Add` _tempname_3 "ug_bonnet_left")
    (`KismetArrayLibrary.Array_Add` _tempname_3 "ug_bonnet_right")
    (elif (`KismetStringLibrary.Contains` _returnvalue "ug_wing")
      (`KismetArrayLibrary.Array_Add` _tempname "ug_wing_left")
      (`KismetArrayLibrary.Array_Add` _tempname "ug_wing_right")
      (elif (`KismetStringLibrary.Contains` _returnvalue "wheel")
        (`KismetArrayLibrary.Array_Add` _tempname_2 "wheel_lb_dummy")
        (`KismetArrayLibrary.Array_Add` _tempname_2 "wheel_lf_dummy")
        (`KismetArrayLibrary.Array_Add` _tempname_2 "wheel_rb_dummy")
        (`KismetArrayLibrary.Array_Add` _tempname_2 "wheel_rf_dummy")
        (else
          (`KismetArrayLibrary.Array_Add` _tempname_2 Socket)))))
  (return (`local.tempname`)))

(fn `getComponentAtSocket`
  (params (vehicle :type "/Game/Vehicle/generic/blueprint/bp_car Object Reference") (Socket :type Name))
  (returns (StaticMeshComponent :type "StaticMeshComponent Object Reference") (meshname :type Name))
  (locals (Found :type Boolean))
  (set `local.Found` false)
  (if (not (`KismetStringLibrary.Contains` (`KismetStringLibrary.Conv_NameToString` Socket) "wheel"))
    (for _array_element (`Actor.K2_GetComponentsByClass` vehicle "/Script/Engine.StaticMeshComponent")
      (if (== (`SceneComponent.GetAttachSocketName` _array_element) Socket)
        (set `local.Found` true)
        (break)))
    (return _array_element (select `bool` (`local.Found`) :`true` (`|GetArrayItem` (`ActorComponent.ComponentTags` _array_element))))
    (else
      (for _array_element_2 (`Actor.K2_GetComponentsByClass` vehicle "/Script/Engine.StaticMeshComponent")
        (if (== (`|GetArrayItem` (`ActorComponent.ComponentTags` (`SceneComponent.GetAttachParent` _array_element_2))) Socket)
          (return _array_element_2 (`|GetArrayItem` (`ActorComponent.ComponentTags` _array_element_2))))))))

(fn `getFlags`
  (params (vehicle :type "/Game/Vehicle/generic/blueprint/bp_car Object Reference"))
  (returns (modelFlags :type Integer) (handlingFlags :type Integer))
  ;[1 0.1458 0.8514] Switch Animation based on Vehicletype
  (bind _returnvalue (`|GetDataTableRow` (`/Game/Vehicle/generic/blueprint/bp_car.dat_vehicle` vehicle) (`/Game/Vehicle/generic/blueprint/bp_car.vehiclename` vehicle))
    (:`then`
      (bind _returnvalue_2 (`|GetDataTableRow` (`/Game/Vehicle/generic/blueprint/bp_car.dat_handling` vehicle) (`.HandlingID_11_AA73F3424CC2519E52AD71AE9EDA242C` (break `/Game/data/vehicles/struct_vehicles` _returnvalue)))
        (:`then`
          (bind ((`PercentSubmerged_92_4D1F26FB4046BF2AE4B2EEA7A1B58B40` _percentsubmerged) (`DriveType_90_49D66ADF4AADD299CE7EE78AA8B6153A` _drivetype) (`EngineType_91_6558AADB42B634A51768DE8B3286F79B` _enginetype) (`modelFlags_79_3A5D271E4291799BA104FCAD52200BAB` _modelflags) (`handlingFlags_81_CF676ED549B77F5710A6A3AE8178829B` _handlingflags)) (break `/Game/data/vehicles/struct_handling` _returnvalue_2))
          (return _modelflags _handlingflags))))))

(fn `getParentSocketOfComponent`
  (params (StaticMeshComponent :type "StaticMeshComponent Object Reference"))
  (returns (socket :type Name))
  (return (`SceneComponent.GetAttachSocketName` StaticMeshComponent)))

(fn `getWheelComponents`
  (params (name :type String))
  (returns (RotationZ :type "Float (double-precision)"))
  (locals (temprotationmultiplicator :type "Float (double-precision)"))
  (switch `string` name
    (:`wheel_lf_dummy`
      (set `local.temprotationmultiplicator` 180.0))
    (:`wheel_rf_dummy`
      (set `local.temprotationmultiplicator` 0.0))
    (:`wheel_lm_dummy`
      (set `local.temprotationmultiplicator` 180.0))
    (:`wheel_rm_dummy`
      (set `local.temprotationmultiplicator` 0.0))
    (:`wheel_lb_dummy`
      (set `local.temprotationmultiplicator` 180.0))
    (:`wheel_rb_dummy`
      (set `local.temprotationmultiplicator` 0.0)))
  (return (`local.temprotationmultiplicator`)))

(fn `setComponentAtSocket`
  (params (chassis :type "StaticMeshComponent Object Reference") (StaticMeshComponent :type "StaticMeshComponent Object Reference") (Socket :type Name) (name :type Name))
  (`SceneComponent.K2_AttachToComponent` StaticMeshComponent chassis Socket "SnapToTarget" "SnapToTarget" "KeepWorld" true)
  (set `ActorComponent.ComponentTags` (`|MakeArray` (select `bool` (== name "None") :`false` name)) StaticMeshComponent))

(fn `setDefaultComponent_damaged`
  (params (vehicle :type "/Game/Vehicle/generic/blueprint/bp_car Object Reference") (StaticMeshComponentToReplace :type "StaticMeshComponent Object Reference") (socket :type Name))
  (`StaticMeshComponent.SetStaticMesh` StaticMeshComponentToReplace (`.dam_7_70A604F04379F2422438EFB740EF3BC0` (break `/Game/Vehicle/generic/blueprint/default/struct_components` (`BlueprintMapLibrary.Map_Find` (`/Game/Vehicle/generic/blueprint/bp_car.mesh_components` vehicle) socket)))))

(fn `setDefaultComponent_ok`
  (params (vehicle :type "/Game/Vehicle/generic/blueprint/bp_car Object Reference") (StaticMeshComponentToReplace :type "StaticMeshComponent Object Reference") (socket :type Name))
  (bind _value (`BlueprintMapLibrary.Map_Find` (`/Game/Vehicle/generic/blueprint/bp_car.mesh_components` vehicle) socket))
  (`/Engine/EditorBlueprintResources/StandardMacros.IsValid` (break `/Game/Vehicle/generic/blueprint/default/struct_components` _value)
    (:`Is Valid`
      (`StaticMeshComponent.SetStaticMesh` StaticMeshComponentToReplace (break `/Game/Vehicle/generic/blueprint/default/struct_components` _value))
      (set `ActorComponent.ComponentTags` (`|MakeArray` "None" :!type "Name") StaticMeshComponentToReplace))
    (:`Is Not Valid`
      (`ActorComponent.K2_DestroyComponent` StaticMeshComponentToReplace))))

(fn `setReplaceComponent`
  (params (StaticMeshComponent :type "StaticMeshComponent Object Reference") (NewStaticMeshComponent :type "StaticMesh Object Reference") (meshname :type Name))
  (`StaticMeshComponent.SetStaticMesh` StaticMeshComponent NewStaticMeshComponent)
  (set `ActorComponent.ComponentTags` (`|MakeArray` meshname) StaticMeshComponent))