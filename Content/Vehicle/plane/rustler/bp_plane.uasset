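; Player-controlled plane pawn flown by applying forces and torques to a physics Chassis, viewed through a child-actor camera.
; A looping timer steps throttle from input, which drives engine Speed parameter and the forward velocity the chassis blends toward.
; Tick adds counter-torque damping and constant downward acceleration, spins the propeller and eases rudder and ailerons toward input.
; Yaw and pitch use torque, while roll also rotates the actor directly and eases back level.
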(event `InputAxis|LookRight`
  (params (AxisValue :type "Float (single-precision)"))
  (`self.AddControllerYawInput` AxisValue))

(event `InputAxis|LookUp`
  (params (AxisValue :type "Float (single-precision)"))
  (`self.AddControllerPitchInput` (* AxisValue -1.0)))

(event `InputAxis|Forward_Char`
  (params (AxisValue :type "Float (single-precision)"))
  (`/Engine/EditorBlueprintResources/StandardMacros.CompareFloat` AxisValue
    (:`>`
      (set `self.ThrottleUp` true)
      (set `self.ThrottleDown` false))
    (:`==`
      (set `self.ThrottleUp` false)
      (set `self.ThrottleDown` false))
    (:`<`
      (set `self.ThrottleUp` false)
      (set `self.ThrottleDown` true))))

(event `self.ReceiveTick`
  (params (DeltaSeconds :type "Float (single-precision)"))
  (bind _chassis (`self.chassis`))
  (`PrimitiveComponent.AddTorqueInDegrees` _chassis (/ (`KismetMathLibrary.NegateVector` (`PrimitiveComponent.GetPhysicsAngularVelocityInDegrees` _chassis "None")) 0.5) "None" true)
  (`PrimitiveComponent.AddForce` _chassis (0.0 0.0 -1500.0) "None" true)
  (`self.CalculateSpeed`)
  (`self.PropRudderElevator`)
  (`AudioComponent.SetFloatParameter` (`self.engine`) "Speed" (`KismetMathLibrary.Conv_IntToDouble` (`self.ThrottleAmount`))))

(event `self.ReceiveBeginPlay`
  (`KismetSystemLibrary.K2_SetTimer` null "ThrottleInput" 0.05 true)
  (`PlayerController.SetViewTargetWithBlend` (`GameplayStatics.GetPlayerController` 0) (`ChildActorComponent.ChildActor` (`self.bp_camera`)) 0.0 "VTBlend_Linear" 0.0 true))

(event `InputAxis|MoveRight`
  (params (AxisValue :type "Float (single-precision)"))
  (`PrimitiveComponent.AddTorqueInDegrees` (`self.chassis`) (`KismetMathLibrary.VLerp` (0.0 0.0 0.0) (* (`SceneComponent.GetUpVector` (`self.chassis`)) (* AxisValue (`self.Aircontrol`))) 0.1) "None" true))

(event `InputAxis|UpDown`
  (params (AxisValue :type "Float (single-precision)"))
  (`PrimitiveComponent.AddTorqueInDegrees` (`self.chassis`) (`KismetMathLibrary.VLerp` (0.0 0.0 0.0) (* (`SceneComponent.GetRightVector` (`self.chassis`)) (* AxisValue (`self.Aircontrol`))) 0.1) "None" true))

(event `InputAxis|Roll`
  (params (AxisValue :type "Float (single-precision)"))
  (bind (_returnvalue_roll _returnvalue_pitch _returnvalue_yaw) (`KismetMathLibrary.BreakRotator` (`self.K2_GetActorRotation`)))
  (bind (_returnvalue_roll_2 _returnvalue_pitch_2 _returnvalue_yaw_2) (`KismetMathLibrary.BreakRotator` (`self.K2_GetActorRotation`)))
  (bind (_returnvalue_x _returnvalue_y _returnvalue_z) (`KismetMathLibrary.BreakVector` (`SceneComponent.GetForwardVector` (`self.chassis`))))
  ;[1 1 1] Parachute Movement
  (`/Engine/EditorBlueprintResources/StandardMacros.CompareFloat` AxisValue
    (:`>`
      ;;[1 1 1] Rotate to the left
      (`self.K2_SetActorRotation` (`KismetMathLibrary.MakeRotator` (- _returnvalue_roll 0.5) _returnvalue_pitch _returnvalue_yaw))
      (`PrimitiveComponent.AddTorqueInDegrees` (`self.chassis`) (`KismetMathLibrary.VLerp` (0.0 0.0 0.0) (`KismetMathLibrary.MakeVector` 0.0 0.0 (* (`self.Aircontrol`) _returnvalue_z)) 0.1) "None" true :!label _label))
    (:`==`
      ;;[1 1 1] Reset Rotation when not pressing any buttons
      (`self.K2_SetActorRotation` (`KismetMathLibrary.MakeRotator` (`KismetMathLibrary.FInterpTo` _returnvalue_roll_2 0.0 (`GameplayStatics.GetWorldDeltaSeconds`) 0.5) _returnvalue_pitch_2 _returnvalue_yaw_2)))
    (:`<`
      ;;[1 1 1] Rotate to the right
      (`self.K2_SetActorRotation` (`KismetMathLibrary.MakeRotator` (+ _returnvalue_roll 0.5) _returnvalue_pitch _returnvalue_yaw))
      (goto _label))))

(fn `CalculateSpeed`
  (bind _chassis (`self.chassis`))
  (bind _returnvalue (`PrimitiveComponent.GetPhysicsLinearVelocity` _chassis "None"))
  (`PrimitiveComponent.SetPhysicsLinearVelocity` _chassis (`KismetMathLibrary.VLerp` _returnvalue (* (`SceneComponent.GetForwardVector` _chassis) (`KismetMathLibrary.FClamp` (* (`self.ThrottleAmount`) 250.0) 0.0 25000.0)) 0.01) false "None"))

(fn `PropRudderElevator`
  (bind _static_prop (`self.static_prop`))
  (bind _aileron_r (`self.aileron_r`))
  (bind _rudder (`self.rudder`))
  (bind _aileron_l (`self.aileron_l`))
  (bind _relativerotation_roll (`KismetMathLibrary.BreakRotator` (`SceneComponent.RelativeRotation` _static_prop)))
  (bind (_relativerotation_roll_2 _relativerotation_pitch) (`KismetMathLibrary.BreakRotator` (`SceneComponent.RelativeRotation` _aileron_r)))
  (bind (_relativerotation_roll_3 _relativerotation_pitch_2 _relativerotation_yaw) (`KismetMathLibrary.BreakRotator` (`SceneComponent.RelativeRotation` _rudder)))
  (bind (_relativerotation_roll_4 _relativerotation_pitch_3) (`KismetMathLibrary.BreakRotator` (`SceneComponent.RelativeRotation` _aileron_l)))
  (`SceneComponent.K2_SetRelativeRotation` _static_prop (`KismetMathLibrary.MakeRotator` (+ _relativerotation_roll 20.0)) false false)
  (`SceneComponent.K2_SetRelativeRotation` _rudder (`KismetMathLibrary.MakeRotator` 0.0 0.0 (`KismetMathLibrary.FInterpTo` _relativerotation_yaw (* (`self.GetInputAxisValue`) -35.0) (`GameplayStatics.GetWorldDeltaSeconds`) 10.0)) false false)
  (`SceneComponent.K2_SetRelativeRotation` _aileron_l (`KismetMathLibrary.MakeRotator` 0.0 (`KismetMathLibrary.FInterpTo` _relativerotation_pitch_3 (`KismetMathLibrary.FClamp` (+ (* (`self.GetInputAxisValue`) -30.0) (* (`self.GetInputAxisValue`) 30.0)) -30.0 30.0) (`GameplayStatics.GetWorldDeltaSeconds`) 10.0)) false false)
  (`SceneComponent.K2_SetRelativeRotation` _aileron_r (`KismetMathLibrary.MakeRotator` 0.0 (`KismetMathLibrary.FInterpTo` _relativerotation_pitch (`KismetMathLibrary.FClamp` (+ (* (`self.GetInputAxisValue`) 30.0) (* (`self.GetInputAxisValue`) 30.0)) -30.0 30.0) (`GameplayStatics.GetWorldDeltaSeconds`) 10.0)) false false))

(fn `ThrottleInput`
  (bind _throttleamount (`self.ThrottleAmount`))
  (if (`self.ThrottleUp`)
    (bind _result (`/Engine/EditorBlueprintResources/StandardMacros.IncrementInt` _throttleamount)
      (:`  `
        (bind _output_get (set `self.ThrottleAmount` (`KismetMathLibrary.Clamp` _result 0 30)))
        (`KismetSystemLibrary.PrintString` (`KismetStringLibrary.Conv_IntToString` _output_get))))
    (elif (`self.ThrottleDown`)
      (bind _result_2 (`/Engine/EditorBlueprintResources/StandardMacros.DecrementInt` _throttleamount)
        (:`  `
          (bind _output_get_2 (set `self.ThrottleAmount` (`KismetMathLibrary.Clamp` _result_2 0 30)))
          (`KismetSystemLibrary.PrintString` (`KismetStringLibrary.Conv_IntToString` _output_get_2)))))))

(fn `UserConstructionScript`)