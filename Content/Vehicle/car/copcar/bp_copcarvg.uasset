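; Police car Blueprint with flashing red and blue lights and a siren, toggled together with the T key.
; BeginPlay hides the six lights and creates a dynamic material on the chassis "siren" slot.
; A sped-up timeline, restarted whenever it finishes, drives the light intensities while the siren plays.
; The material's "active" parameter follows the toggle, and "phase" follows whether any blue light is lit.
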(event `self.ReceiveBeginPlay`
  (bind _chassis (`self.chassis`))
  (`parent.ReceiveBeginPlay`)
  (`SceneComponent.SetHiddenInGame` (`self.light_blue`) true false)
  (`SceneComponent.SetHiddenInGame` (`self.light_blue2`) true false)
  (`SceneComponent.SetHiddenInGame` (`self.light_blue3`) true false)
  (`SceneComponent.SetHiddenInGame` (`self.light red3`) true false)
  (`SceneComponent.SetHiddenInGame` (`self.light red2`) true false)
  (`SceneComponent.SetHiddenInGame` (`self.light red`) true false)
  (`TimelineComponent.SetPlayRate` (`self.policesiren`) 7.5)
  (for (_array_element _array_index) (`MeshComponent.GetMaterialSlotNames` _chassis)
    (if (== _array_element "siren")
      (bind _returnvalue (`PrimitiveComponent.CreateDynamicMaterialInstance` _chassis _array_index "/Game/Vehicle/car/copcar/material/copcarvg92_siren.copcarvg92_siren" "None"))
      (set `self.siren_mat` _returnvalue))))

(event `Key|T`
  (params (Key :type "Key Structure"))
  (bind _light (`self.light`))
  (bind _siren (`self.siren`))
  (bind _siren_mat (`self.siren_mat`))
  (bind _intensity (`self.intensity`))
  (bind _intensity_2 (`self.intensity`))
  (:`Pressed`
    (if (`self.light`)
      (set `self.light` false)
      (`|ExecutionSequence`
        (:`then_0`
          (`SceneComponent.SetHiddenInGame` (`self.light red`) (not _light) false :!label _label)
          (`SceneComponent.SetHiddenInGame` (`self.light red2`) (not _light) false)
          (`SceneComponent.SetHiddenInGame` (`self.light red3`) (not _light) false)
          (`SceneComponent.SetHiddenInGame` (`self.light_blue3`) (not _light) false)
          (`SceneComponent.SetHiddenInGame` (`self.light_blue2`) (not _light) false)
          (`SceneComponent.SetHiddenInGame` (`self.light_blue`) (not _light) false)
          (`MaterialInstanceDynamic.SetScalarParameterValue` (`self.siren_mat`) "active" (`KismetMathLibrary.Conv_BoolToDouble` _light)))
        (:`then_1`
          (bind (_direction _light_blue _light_red) (`Timeline|policesiren` :!via `Stop` :!label _label_2)
            (:`Update`
              (bind _returnvalue (* (.x _light_blue) _intensity_2))
              (`LightComponent.SetIntensity` (`self.light_blue`) _returnvalue)
              (bind _returnvalue_2 (* (.y _light_blue) _intensity_2))
              (`LightComponent.SetIntensity` (`self.light_blue2`) _returnvalue_2)
              (bind _returnvalue_3 (* (.z _light_blue) _intensity_2))
              (`LightComponent.SetIntensity` (`self.light_blue3`) _returnvalue_3)
              (`LightComponent.SetIntensity` (`self.light red3`) (* (.x _light_red) _intensity))
              (`LightComponent.SetIntensity` (`self.light red2`) (* (.y _light_red) _intensity))
              (`LightComponent.SetIntensity` (`self.light red`) (* (.z _light_red) _intensity))
              (if (or (> _returnvalue 0.0) (> _returnvalue_2 0.0) (> _returnvalue_3 0.0))
                (`MaterialInstanceDynamic.SetScalarParameterValue` _siren_mat "phase" 0.0)
                (else
                  (`MaterialInstanceDynamic.SetScalarParameterValue` _siren_mat "phase" 1.0))))
            (:`Finished`
              (goto _label_2 :!via `PlayFromStart`))))
        (:`then_2`
          (`AudioComponent.Stop` _siren)))
      (else
        (set `self.light` true)
        (`|ExecutionSequence`
          (:`then_0`
            (goto _label))
          (:`then_1`
            (goto _label_2 :!via `PlayFromStart`))
          (:`then_2`
            (`AudioComponent.Play` _siren 0.0)))))))

(fn `UserConstructionScript`
  (`parent.UserConstructionScript`))