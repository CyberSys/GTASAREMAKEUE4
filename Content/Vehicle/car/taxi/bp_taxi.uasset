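; Taxi vehicle Blueprint, a child class that adds a switchable illuminated roof sign.
; The construction script finds Chassis material slots named with "taxisign" and replaces them with a dynamic material instance, stored as Taxisign.
; Pressing T calls Taxiservice, which toggles Haspassenger and sets the sign's emissive multiplier, lighting it when a passenger is aboard and darkening it otherwise.
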(event `self.ReceiveBeginPlay`
  (`parent.ReceiveBeginPlay`))

(event `Key|T`
  (params (Key :type "Key Structure"))
  (:`Pressed`
    (`self.taxiservice`)))

(fn `taxiservice`
  (bind _taxisign (`self.taxisign`))
  (if (`self.haspassenger`)
    (set `self.haspassenger` false)
    (`MaterialInstanceDynamic.SetScalarParameterValue` _taxisign "EmissivMulitplier" 0.0)
    (else
      (set `self.haspassenger` true)
      (`MaterialInstanceDynamic.SetScalarParameterValue` _taxisign "EmissivMulitplier" 4.0))))

(fn `UserConstructionScript`
  (`parent.UserConstructionScript`)
  (for (_array_element _array_index) (`MeshComponent.GetMaterialSlotNames` (`self.chassis`))
    (if (`KismetStringLibrary.Contains` (`KismetStringLibrary.Conv_NameToString` _array_element) "taxisign" true)
      (bind _returnvalue (`PrimitiveComponent.CreateDynamicMaterialInstance` (`self.chassis`) _array_index "/Game/Vehicle/car/taxi/material/taxi92sign64.taxi92sign64" "None"))
      (set `self.taxisign` _returnvalue)
      (`PrimitiveComponent.SetMaterial` (`self.chassis`) _array_index (`self.taxisign`)))))