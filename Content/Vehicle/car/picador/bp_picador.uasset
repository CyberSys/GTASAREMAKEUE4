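; Picador car Blueprint that randomizes its optional extra parts each time an instance begins play.
; After the parent BeginPlay, it gives Extra1 and Extra2 an independent random boolean roll each and destroys the component on true, so either, both or neither can remain.
; The construction script only calls the parent, and the Tick and overlap events are disabled.
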(event `self.ReceiveBeginPlay`
  (`parent.ReceiveBeginPlay`)
  (for _array_element (`|MakeArray` (`self.extra1`) (`self.extra2`))
    (if (`KismetMathLibrary.RandomBool`)
      (`ActorComponent.K2_DestroyComponent` _array_element))))

(fn `UserConstructionScript`
  (`parent.UserConstructionScript`))