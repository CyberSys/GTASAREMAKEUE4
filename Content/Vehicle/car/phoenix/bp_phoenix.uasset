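; Phoenix car Blueprint, a child vehicle class that relies on its parent for construction and general per-frame behavior.
; On Tick, after the parent update, it sets the relative rotation of the MiscA component from engine RPM.
; The ratio of current RPM to the engine struct's maximum drives a rotation of up to a quarter turn, like a tachometer needle.
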(event `self.ReceiveTick`
  (params (DeltaSeconds :type "Float (single-precision)"))
  (`parent.ReceiveTick` DeltaSeconds)
  (`SceneComponent.K2_SetRelativeRotation` (`self.misc_a`) (`KismetMathLibrary.MakeRotator` 0.0 (* (/ (`self.EngineRPM`) (`KismetMathLibrary.Conv_IntToDouble` (`.max_rpm_13_990B2F094F6C9EDBFA7E59A56B2B5B59` (break `/Game/Vehicle/generic/blueprint/EngineStructure` (`self.Engine_struct`))))) 90.0)) false false))

(fn `UserConstructionScript`
  (`parent.UserConstructionScript`))