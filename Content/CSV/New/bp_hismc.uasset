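; Actor Blueprint that builds hierarchical instanced static meshes from a Locations DataTable at construction time.
; It first moves its pivot to the average of three sampled rows to avoid oversized auto-generated World Composition level bounds.
; Each row name gets one tagged HISM component, offset against the pivot, with mesh and collision profile from the Meshes table.
; Instance transforms convert units to centimeters and flip Y and yaw.
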(fn `UserConstructionScript`
  (locals (temp_midpoints :type "Array of Vector Structure") (pivot :type "Vector Structure"))
  (bind _locations (`self.Locations`))
  (bind _locations_2 (`self.Locations`))
  (bind _temp_midpoints (`local.temp_midpoints`))
  ;[1 0.411 0.291] set pivot of blueprint to a value inside the component bounds (bounds of the hism-components) to avoid extremely large level bounds (world composition) whose are auto generated
  (bind _outrownames (`DataTableFunctionLibrary.GetDataTableRowNames` _locations_2))
  (bind _returnvalue (/ (`KismetArrayLibrary.Array_Length` _outrownames) 3))
  (for _array_element (`|MakeArray` (`|GetArrayItem` _outrownames) (`|GetArrayItem` _outrownames _returnvalue) (`|GetArrayItem` _outrownames (* _returnvalue 2)))
    (bind _returnvalue_2 (`|GetDataTableRow` _locations_2 _array_element)
      (:`then`
        (bind (_name _posx _posy _posz) (break `/Game/CSV/New/struct_hism` _returnvalue_2))
        (`KismetArrayLibrary.Array_Add` (`local.temp_midpoints`) (`KismetMathLibrary.MakeVector` (* _posx 100.0) (* _posy -100.0) (* _posz 100.0))))))
  (for _array_element_2 _temp_midpoints
    (set `local.pivot` (+ _array_element_2 (`local.pivot`))))
  (bind _output_get (set `local.pivot` (/ (`local.pivot`) (`KismetArrayLibrary.Array_Length` _temp_midpoints))))
  (`self.K2_SetActorLocation` _output_get)
  ;[1 1 1 0.2476] create hism-component(s) and add instance(s)
  (bind _outrownames_2 (`DataTableFunctionLibrary.GetDataTableRowNames` _locations))
  (for _array_element_3 _outrownames_2
    (bind _returnvalue_3 (`|GetDataTableRow` _locations _array_element_3)
      (:`then`
        (bind (_name_2 _posx_2 _posy_2 _posz_2 _rotx _roty _rotz) (break `/Game/CSV/New/struct_hism` _returnvalue_3))
        (bind _returnvalue_4 (`self.GetComponentsByTag` "/Script/Engine.HierarchicalInstancedStaticMeshComponent" _name_2))
        (if (not (`KismetArrayLibrary.Array_IsValidIndex` _returnvalue_4))
          (bind _returnvalue_5 (`AddComponent|NODE_AddHierarchicalInstancedStaticMeshComponent-0` :`RelativeTransform` (`KismetMathLibrary.MakeTransform` (* (`local.pivot`) -1))))
          (set `ActorComponent.ComponentTags` (`|MakeArray` _name_2) _returnvalue_5)
          (bind _returnvalue_6 (`|GetDataTableRow` (`self.Meshes`) _name_2)
            (:`then`
              (bind _output (`|GetArrayItem` _returnvalue_4))
              (bind (_mesh _collision) (break `/Game/CSV/New/struct_hism_meshes` _returnvalue_6))
              (`StaticMeshComponent.SetStaticMesh` _output _mesh)
              (if _collision
                (`PrimitiveComponent.SetCollisionProfileName` _output "BlockAllDynamic")
                (else
                  (`PrimitiveComponent.SetCollisionProfileName` _output "NoCollision"))))))
        (`InstancedStaticMeshComponent.AddInstance` _output (`KismetMathLibrary.MakeTransform` (`KismetMathLibrary.MakeVector` (* _posx_2 100.0) (* _posy_2 -100.0) (* _posz_2 100.0)) (`KismetMathLibrary.MakeRotator` _rotx _roty (* _rotz -1.0))))))))