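; Pedestrian pawn that takes its mesh and walk cycle from a data table and can carry shop items.
; PedWalk loops AIMoveTo across area-indexed node tables, picking random linked neighbours; BeginPlay never starts it.
; A separate distance check, also not started here, destroys peds far from the player.
; Item functions spawn food or weapon child actors by shop type, attach or detach them at the right-hand socket, and jump montage lift sections.
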(event `self.PawnSensing.OnSeePawn`
  (params (Pawn :type "Pawn Object Reference")))

(event `self.ReceiveBeginPlay`
  (`self.SpawnDefaultController`)
  (set `self.isWalking` true)
  (set `self.enum_walk` "NewEnumerator1")
  (bind _outactors (`GameplayStatics.GetAllActorsOfClass` "/Game/data/Paths/trafficlight.trafficlight_C"))
  (bind _astrafficlight (cast `/Game/data/Paths/trafficlight` (`|GetArrayItem` _outactors)))
  (set `self.TrafficLight` _astrafficlight))

(event `CheckDistanceToPlayer`
  ;[1 1 1] DrawDistance
  (if (>= (`KismetMathLibrary.VSize` (- (`self.K2_GetActorLocation` (`Controller.K2_GetPawn` (`GameplayStatics.GetPlayerController` 0))) (`self.K2_GetActorLocation`))) 7500.0) :!label _label
    (`self.K2_DestroyActor`)
    (else
      (`KismetSystemLibrary.Delay` 1.0)
      (goto _label))))

(event `ped walk`
  (params (CurrentNode :type "Vector2D Structure"))
  (bind (_nextnode_x _nextnode_y) (`KismetMathLibrary.BreakVector2D` (`self.nextNode`)))
  ;[1 1 1] Ped Walk
  (set `self.currentnodeNode` CurrentNode)
  (set `self.nextNode` (`self.getNextNode`))
  (bind _returnvalue (`|GetDataTableRow` (`|GetArrayItem` (`self.pednodes`) (`KismetMathLibrary.FTrunc` _nextnode_x)) (`KismetStringLibrary.Conv_StringToName` (`KismetStringLibrary.Conv_IntToString` (`KismetMathLibrary.FTrunc` _nextnode_y))) :!label _label_2)
    (:`then`
      (bind ((`PosX_2_D572BE0742A650EA3D0E4CAC1F3FE955` _posx) (`PosY_4_F72151884933EF7C93500689E24A987C` _posy) (`PosZ_6_AB82B9BF4E69EEAF60A276A5AE182BDD` _posz)) (break `/Game/data/Paths/peds/struct_nodes_peds` _returnvalue))
      (`|AIMoveTo` self (`self.meter2centimeter` _posx _posy _posz) null 180.0
        (:`OnSuccess`
          (set `self.currentnodeNode` (`self.nextNode`))
          (`KismetSystemLibrary.PrintString` "node success" true true (struct :`R` 0.069925 :`G` 1.0 :`A` 1.0) 1.0)
          (set `self.nextNode` (`self.getNextNode`))
          (goto _label_2))))))

(fn `AttachItem`
  (bind _currentitem (`self.CurrentItem`))
  (`/Engine/EditorBlueprintResources/StandardMacros.IsValid` _currentitem
    (:`Is Valid`
      (if (== (`SceneComponent.GetAttachParent` _currentitem) (`self.Mesh`))
        (`self.SwapItem` (`self.ItemID`) :!label _label)
        (else
          (`SceneComponent.K2_AttachToComponent` (`self.CurrentItem`) (`self.Mesh`) "R-HandSocket" "SnapToTarget" "SnapToTarget" "KeepRelative" true))))
    (:`Is Not Valid`
      (goto _label))))

(fn `DestroyItem`
  (bind _currentitem (`self.CurrentItem`))
  (`/Engine/EditorBlueprintResources/StandardMacros.IsValid` _currentitem
    (:`Is Valid`
      (`ActorComponent.K2_DestroyComponent` _currentitem))))

(fn `DetachItem`
  (bind _currentitem (`self.CurrentItem`))
  (`/Engine/EditorBlueprintResources/StandardMacros.IsValid` _currentitem
    (:`Is Valid`
      (`SceneComponent.K2_DetachFromComponent` _currentitem "KeepWorld" "KeepWorld" "KeepWorld" false))))

(fn `getNextNode`
  (returns (NextNode :type "Vector2D Structure"))
  (locals (Nodes :type "Array of Vector2D Structure"))
  (bind (_currentnodenode_x _currentnodenode_y) (`KismetMathLibrary.BreakVector2D` (`self.currentnodeNode`)))
  (bind _nodes (`local.Nodes`))
  (bind _returnvalue (`KismetMathLibrary.FTrunc` _currentnodenode_x))
  (`KismetArrayLibrary.Array_Clear` (`local.Nodes`))
  (bind _returnvalue_2 (`|GetDataTableRow` (`|GetArrayItem` (`self.pednodes`) _returnvalue) (`KismetStringLibrary.Conv_StringToName` (`KismetStringLibrary.Conv_IntToString` (`KismetMathLibrary.FTrunc` _currentnodenode_y))))
    (:`then`
      (bind ((`LinkID_9_FCAB593D477E8F3CA8A748A8FF3EFD9B` _linkid) (`LinkCount_15_EE6EDBD54FC0F09CDC79D09A4544CA29` _linkcount)) (break `/Game/data/Paths/peds/struct_nodes_peds` _returnvalue_2))
      (for _index (range _linkid (+ (+ _linkid (- _linkcount 1)) 1))
        (bind _returnvalue_3 (`|GetDataTableRow` (`|GetArrayItem` (`self.link`) _returnvalue) (`KismetStringLibrary.Conv_StringToName` (`KismetStringLibrary.Conv_IntToString` _index)))
          (:`then`
            (bind ((`AreaID_7_D1A09C704CD9D90588A9EFA183B08CFA` _areaid) (`NodeID_4_996961CC47F754A33A54EEA8F84FD168` _nodeid)) (break `/Game/data/Paths/links/struct_link` _returnvalue_3))
            (bind _returnvalue_4 (`KismetMathLibrary.Conv_ByteToDouble` _areaid))
            (bind _returnvalue_5 (`KismetMathLibrary.Conv_IntToDouble` _nodeid))
            (if (!= (`KismetMathLibrary.MakeVector2D` _returnvalue_4 _returnvalue_5) (`self.currentnodeNode`))
              (`KismetArrayLibrary.Array_Add` (`local.Nodes`) (`KismetMathLibrary.MakeVector2D` _returnvalue_4 _returnvalue_5))))))
      (return (`|GetArrayItem` _nodes (`KismetMathLibrary.RandomInteger` (`KismetArrayLibrary.Array_Length` _nodes)))))))

(fn `JumpAnim`
  (params (AnimSection :type Name) (Index :type Integer))
  (bind _1h_lift (`self.1H_Lift`))
  (bind _2h_lift (`self.2H_Lift`))
  (bind _returnvalue (`SkeletalMeshComponent.GetAnimInstance` (`self.Mesh`)))
  (set `self.AnimSection` AnimSection)
  (`AnimInstance.Montage_JumpToSection` _returnvalue (select `int` Index :`0` _1h_lift :`1` _1h_lift :`2` _1h_lift :`3` _1h_lift :`4` _2h_lift :`5` _2h_lift :`6` _2h_lift :`7` _1h_lift :`8` _1h_lift :`9` _1h_lift :`10` _2h_lift :`11` _2h_lift :`12` _2h_lift :`13` _2h_lift :`14` "None" :`15` "None" :`16` "None" :`17` _1h_lift :`18` "None" :`19` (`self.AR_Lift`)) (`AnimInstance.GetCurrentActiveMontage` _returnvalue)))

(fn `SwapItem`
  (params (ItemID :type Integer))
  (bind _returnvalue (`KismetStringLibrary.Conv_StringToName` (`KismetStringLibrary.Conv_IntToString` ItemID)))
  (switch `/Game/data/shoppingOLD/enum_shops` (`self.enum_shop`)
    (:`NewEnumerator7`
      ;[0 0.224 1] Food
      (bind _returnvalue_2 (`|GetDataTableRow` (`self.dat_Food`) _returnvalue :!label _label)
        (:`then`
          (bind _returnvalue_3 (`AddComponent|NODE_AddChildActorComponent-1`))
          (bind _output_get (set `self.CurrentItem` _returnvalue_3))
          (bind _astray (cast `/Game/Models/interior/props/Tray` (`ChildActorComponent.ChildActor` _output_get)))
          (`StaticMeshComponent.SetStaticMesh` (`/Game/Models/interior/props/Tray.StaticMesh` _astray) (`.mesh_57_34DCCAA8422BA7113E12FFAAD88337CD` (break `/Game/data/shoppingOLD/struct_foodOLD` _returnvalue_2)))
          (`SceneComponent.K2_AttachToComponent` _output_get (`self.Mesh`) "R-HandSocket" "KeepRelative" "KeepRelative" "KeepRelative" true))))
    (:`NewEnumerator8`
      (goto _label))
    (:`NewEnumerator9`
      (goto _label))
    (:`NewEnumerator18`
      ;[0.4338 0.5156 0.1755] Weapons
      (bind _returnvalue_4 (`|GetDataTableRow` (`self.dat_Weapons`) _returnvalue :!label _label_2)
        (:`then`
          (bind _returnvalue_5 (`AddComponent|NODE_AddChildActorComponent-2`))
          (bind _output_get_2 (set `self.CurrentItem` _returnvalue_5))
          (bind _asbp_weapon_static (cast `/Game/Weapons/bp_weapon_static` (`ChildActorComponent.ChildActor` _output_get_2)))
          (`StaticMeshComponent.SetStaticMesh` (`/Game/Weapons/bp_weapon_static.staticmesh` _asbp_weapon_static) (`.mesh_57_34DCCAA8422BA7113E12FFAAD88337CD` (break `/Game/data/shoppingOLD/struct_weaponsOLD` _returnvalue_4)))
          (`SceneComponent.K2_AttachToComponent` _output_get_2 (`self.Mesh`) "R-HandSocket" "KeepRelative" "KeepRelative" "KeepRelative" true))))
    (:`NewEnumerator20`
      (goto _label_2))
    (:`NewEnumerator21`
      (goto _label_2))
    (:`NewEnumerator22`
      (goto _label_2))
    (:`NewEnumerator23`
      (goto _label_2))))

(fn `UserConstructionScript`
  ;[1 1 1] IntitializePed
  (bind _returnvalue (`|GetDataTableRow` (`self.dat_Peds`) (`self.Ped`))
    (:`then`
      (bind ((`model_80_020E2F0948DB0F69A21E469CB08F47BD` _model) (`walkcycle_77_1BE0A35D429C83F90B421B910EA1E1E4` _walkcycle)) (break `/Game/data/ped/struct_peds` _returnvalue))
      (`SkinnedMeshComponent.SetSkinnedAssetAndUpdate` (`self.Mesh`) _model true)
      (set `self.Walkcycle` _walkcycle))))