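; AN_BuyMenu is an animation notify that opens a shop buy menu during an animation.
; On notify it casts player character 0 to the player class, then calls OpenBuyMenu on the food shopping HUD reference if valid, otherwise on the weapons shopping HUD.
; The food HUD takes priority, and each branch prints a debug string.
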(fn `Received_Notify`
  (params (MeshComp :type "SkeletalMeshComponent Object Reference") (Animation :type "AnimSequenceBase Object Reference"))
  (returns (ReturnValue :type Boolean))
  (bind _asplayer (cast `/Game/Player/blueprint/player` (`GameplayStatics.GetPlayerCharacter` 0)))
  (bind _ref_hud_shopping_food (`/Game/Player/blueprint/player.REF_Hud_shopping_food` _asplayer))
  (`/Engine/EditorBlueprintResources/StandardMacros.IsValid` _ref_hud_shopping_food
    (:`Is Valid`
      (`/Game/UserInterface/menus/food/hud_shopping_food.OpenBuyMenu` _ref_hud_shopping_food)
      (`KismetSystemLibrary.PrintString` "food"))
    (:`Is Not Valid`
      (bind _ref_hud_shopping_weapons (`/Game/Player/blueprint/player.REF_Hud_shopping_weapons` _asplayer))
      (`/Engine/EditorBlueprintResources/StandardMacros.IsValid` _ref_hud_shopping_weapons
        (:`Is Valid`
          (`/Game/UserInterface/menus/weapon/hud_shopping_weapons.OpenBuyMenu` _ref_hud_shopping_weapons)
          (`KismetSystemLibrary.PrintString` "ammo")))))
  (return false))